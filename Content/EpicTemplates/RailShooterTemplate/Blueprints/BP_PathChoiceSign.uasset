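; Shootable fork sign for the rail shooter that lets players pick a left or right spline path.
; HealthComponent damage within range is converted to local space, where hit side and height decide the direction.
; Each player chooses once, subject to the path choice manager, and billboards show feedback in player color.
; Requests go to the manager for all players or just the shooter, optionally delayed through a next-tick countdown queue.
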(event `self.ReceiveBeginPlay`
  ;[1 1 1] BeginPlay
  (if (`self.bStartWithChoiceEnabled`)
    (`self.EnableChoice`)))

(event `EnableChoice`
  ;[1 1 1] Enable Choice
  (set `self.bChoiceEnabled` true)
  (`SceneComponent.SetVisibility` (`self.GoRightBillboard`) true false)
  (`SceneComponent.SetVisibility` (`self.GoLeftBillboard`) true false))

(event `self.HealthComponent.OnTookDamage`
  (params (Caller :type "/Game/EpicTemplates/TemplateAgnostic/Blueprints/Components/BP_HealthComponent Object Reference") (OldHealth :type "Float (double-precision)") (NewHealth :type "Float (double-precision)") (SpecialDamageName :type Name) (DamageStruct :type "/Game/EpicTemplates/TemplateAgnostic/Blueprints/Structs/DamageStruct Structure (by ref)"))
  (bind ((`DamageSource_5_8780F30649675B7DF1FC5694BCAD2A7E` _damagesource) (`DamageSourceOwner_16_93F98FB747ED83B90B1FAFB49CE3E4D5` _damagesourceowner) (`DamageLocation_8_F5A6C21543470034EA0BD6945175CC5B` _damagelocation)) (break `/Game/EpicTemplates/TemplateAgnostic/Blueprints/Structs/DamageStruct` DamageStruct))
  ;[1 1 1] Took damage
  (if (and (`self.bChoiceEnabled`) (or (not (`self.bChoiceMade`)) (not (`self.bOnlyOneChoiceAllowed`))))
    (bind (_choicevalid _choiceisright) (`self.Check for Path Decision` (`self.K2_GetActorLocation` _damagesource) _damagelocation))
    (if _choicevalid
      (bind _asplayer_controller (cast `PlayerController` _damagesourceowner))
      (`self.Player Try Choose Direction` _asplayer_controller _choiceisright))))

(event `ChoiceMadeFeedback`
  (params (ChoseRight :type Boolean) (ChoosingPlayer :type "PlayerController Object Reference"))
  (`|ExecutionSequence`
    (:`then_0`
      (if (`self.bOnlyOneChoiceAllowed`)
        (`SceneComponent.SetVisibility` (select `bool` ChoseRight :`false` (`self.GoRightBillboard`) :`true` (`self.GoLeftBillboard`) :!type "SceneComponent Object Reference") false false)))
    (:`then_1`
      (bind _returnvalue (`KismetMaterialLibrary.CreateDynamicMaterialInstance` "/Game/EpicTemplates/RailShooterTemplate/Materials/M_ChoiceSignBoard.M_ChoiceSignBoard"))
      (`MaterialInstanceDynamic.SetVectorParameterValue` _returnvalue "Color" (select `int` (`GameplayStatics.GetPlayerControllerID` ChoosingPlayer) :`0` (`/Game/EpicTemplates/TemplateAgnostic/Blueprints/EpicTemplatesFunctionLibrary.GetPlayer1Color`) :`1` (`/Game/EpicTemplates/TemplateAgnostic/Blueprints/EpicTemplatesFunctionLibrary.GetPlayer2Color`)))
      (`MaterialBillboardComponent.SetElements` (`self.GoRightBillboard`) (`|MakeArray` (make `MaterialSpriteElement` _returnvalue)))
      (`MaterialBillboardComponent.SetElements` (select `bool` ChoseRight :`false` (`self.GoLeftBillboard`) :`true` (`self.GoRightBillboard`)) (`|MakeArray` (make `MaterialSpriteElement` _returnvalue))))))

(fn `Check for Path Decision`
  (params (SourceLocation :type "Vector Structure (by ref)") (HitLocation :type "Vector Structure (by ref)"))
  (returns (ChoiceValid :type Boolean) (ChoiceIsRight :type Boolean))
  (locals (HitLocLocal :type "Vector Structure" :default (0.0 0.0 0.0)) (SourceLocLocal :type "Vector Structure"))
  (bind (_returnvalue_x _returnvalue_y) (`KismetMathLibrary.BreakVector` (`KismetMathLibrary.InverseTransformLocation` (`SceneComponent.K2_GetComponentToWorld` (`self.SceneRoot`)) SourceLocation)))
  (set `local.SourceLocLocal` (`KismetMathLibrary.MakeVector` _returnvalue_x _returnvalue_y))
  (if (or (<= (`self.MaxHorizontalDistForChoice`) 0.0) (< (`KismetMathLibrary.VSizeSquared` (`local.SourceLocLocal`)) (`KismetMathLibrary.Square` (`self.MaxHorizontalDistForChoice`))))
    (bind _output_get (set `local.HitLocLocal` (`KismetMathLibrary.InverseTransformLocation` (`SceneComponent.K2_GetComponentToWorld` (`self.SceneRoot`)) (`local.HitLocation`))))
    (bind _y (.y _output_get))
    (if (and (> (`KismetMathLibrary.Abs` _y) (`self.ValidDecisionMinimumHitHorizontalOffset`)) (> (.z _output_get) (`self.ValidDecisionMinimumHitHeight`)))
      (return true (< _y 0.0))
      (else
        (return false false)))
    (else
      (return false false))))

(fn `Player Try Choose Direction`
  (params (ChoosingPlayer :type "PlayerController Object Reference") (ChoseRight :type Boolean))
  (locals (ChoosingPlayerID :type Integer :default 0))
  (bind _output_get (set `local.ChoosingPlayerID` (`GameplayStatics.GetPlayerControllerID` ChoosingPlayer)))
  (if (not (`KismetArrayLibrary.Array_Contains` (`self.PlayersUsed`) _output_get))
    (`KismetArrayLibrary.Array_Add` (`self.PlayersUsed`) (`local.ChoosingPlayerID`))
    (`|ExecutionSequence`
      (:`then_0`
        (bind _pathchoicemanager (`/Game/EpicTemplates/RailShooterTemplate/Blueprints/RailShooterFunctionLibrary.GetPathChoiceManager`))
        (`/Engine/EditorBlueprintResources/StandardMacros.IsValid` _pathchoicemanager
          (:`Is Valid`
            (bind _canmakechoice (`/Game/EpicTemplates/RailShooterTemplate/Blueprints/BP_PathChoiceManager.CanPlayerMakePathChoice` _pathchoicemanager (`local.ChoosingPlayer`)))
            (if (not _canmakechoice)
              (return)))))
      (:`then_1`
        (set `self.bChoiceMade` true)
        (`self.ChoiceMadeFeedback` (`local.ChoseRight`) (`local.ChoosingPlayer`))
        (`self.OnChoseDirection` (`local.ChoseRight`) (`|ConvertAsset` (select `bool` false :`false` (`self.ChooseLeftPathActor`) :`true` (`self.ChooseRightPathActor`))) (`self.ChoiceMadeRequestDelay`))
        (if (> (`self.ChoiceMadeRequestDelay`) 0.0)
          (`KismetArrayLibrary.Array_Add` (`self.PendingChoices`) (make `/Game/EpicTemplates/RailShooterTemplate/Blueprints/Structs/PendingSplineChoice` (`local.ChoosingPlayer`) (`local.ChoseRight`) (`self.ChoiceMadeRequestDelay`)))
          (if (not (`KismetSystemLibrary.K2_IsTimerActiveHandle` (`self.TickPendingChoicesHandle`)))
            (bind _returnvalue (`KismetSystemLibrary.K2_SetTimerForNextTickDelegate` (`|CreateDelegate` :!event `TickPendingChoices`)))
            (set `self.TickPendingChoicesHandle` _returnvalue))
          (else
            (`self.RequestPathChoice` (`local.ChoosingPlayer`) (`local.ChoseRight`))))))))

(fn `RequestPathChoice`
  (params (Player :type "PlayerController Object Reference") (ChoseRight :type Boolean))
  (locals (ChosenPath :type "Actor Object Reference") (PathChoiceManager :type "/Game/EpicTemplates/RailShooterTemplate/Blueprints/BP_PathChoiceManager Object Reference"))
  (bind _pathchoicemanager (`/Game/EpicTemplates/RailShooterTemplate/Blueprints/RailShooterFunctionLibrary.GetPathChoiceManager`))
  (set `local.PathChoiceManager` _pathchoicemanager)
  (set `local.ChosenPath` (`|ConvertAsset` (select `bool` (`local.ChoseRight`) :`false` (`self.ChooseLeftPathActor`) :`true` (`self.ChooseRightPathActor`))))
  (switch `/Game/EpicTemplates/RailShooterTemplate/Blueprints/Enums/EPathSplitType` (`self.PathSplitType`)
    (:`NewEnumerator0`
      (`/Game/EpicTemplates/RailShooterTemplate/Blueprints/BP_PathChoiceManager.RequestNewSplineForAllPlayers` (`local.PathChoiceManager`) self (`local.ChosenPath`) "NewEnumerator0" "NewEnumerator0" (`/Game/EpicTemplates/RailShooterTemplate/Blueprints/RailShooterFunctionLibrary.SplineTargetEnd`)))
    (:`NewEnumerator1`
      (`/Game/EpicTemplates/RailShooterTemplate/Blueprints/BP_PathChoiceManager.RequestNewSplineForIndividualPlayer` (`local.PathChoiceManager`) self (`local.ChosenPath`) (`local.Player`) "NewEnumerator0" "NewEnumerator0" (`/Game/EpicTemplates/RailShooterTemplate/Blueprints/RailShooterFunctionLibrary.SplineTargetEnd`)))))

(fn `TickPendingChoices`
  (locals (TempChoiceDelay :type "Float (double-precision)") (TempIdx :type Integer))
  (bind ((`Requestee_8_1E58BCCB4A8B024BFB00F2B5C3701AAA` _requestee) (`ChoseRight_1_DFE240C147D5404AD73D35920CB84964` _choseright)) (break `/Game/EpicTemplates/RailShooterTemplate/Blueprints/Structs/PendingSplineChoice` (`|GetArrayItem` (`self.PendingChoices`) (`local.TempIdx`))))
  (`|ExecutionSequence`
    (:`then_0`
      (bind (_arrayindex _arrayelement) (`/Engine/EditorBlueprintResources/StandardMacros.ReverseForEachLoop` (`self.PendingChoices`))
        (:`LoopBody`
          (set `local.TempIdx` _arrayindex)
          (bind _output_get (set `local.TempChoiceDelay` (`.PendingChoiceDelay_20_A56C5B4C4934D0C73AE3C68C13C1C7E2` (break `/Game/EpicTemplates/RailShooterTemplate/Blueprints/Structs/PendingSplineChoice` _arrayelement))))
          (bind _outfloatcopy (`/Game/EpicTemplates/TemplateAgnostic/Blueprints/EpicTemplatesFunctionLibrary.MinusEqualsFloat` _output_get (`GameplayStatics.GetWorldDeltaSeconds`)))
          (if (< _outfloatcopy 0.0)
            (`self.RequestPathChoice` _requestee _choseright)
            (`KismetArrayLibrary.Array_Remove` (`self.PendingChoices`) (`local.TempIdx`))
            (else
              (setmembers `/Game/EpicTemplates/RailShooterTemplate/Blueprints/Structs/PendingSplineChoice` :`StructRef` (`|GetArrayItem` (`self.PendingChoices`) (`local.TempIdx`)) :`PendingChoiceDelay` (`local.TempChoiceDelay`)))))))
    (:`then_1`
      (if (`KismetArrayLibrary.Array_IsNotEmpty` (`self.PendingChoices`))
        (bind _returnvalue (`KismetSystemLibrary.K2_SetTimerForNextTickDelegate` (`|CreateDelegate` :!event `TickPendingChoices`)))
        (set `self.TickPendingChoicesHandle` _returnvalue)))))

(fn `UserConstructionScript`)