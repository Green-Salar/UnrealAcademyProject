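; Rail shooter weapon Blueprint that has a single clip of ammo and is discarded once it runs dry.
; It overrides FireWeaponIfHaveAmmo to spend AmmoPerShot from the ammo clip component before firing, playing an empty sound if the spend fails.
; After a shot, if too little ammo remains for another, it asks the wielder through WeaponWielderInterface to remove and destroy the weapon.
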(fn `FireWeaponIfHaveAmmo`
  (bind (_ammospent _spendrequestsuccessful) (`/Game/EpicTemplates/RailShooterTemplate/Blueprints/Interfaces/BPI_AmmoClip.TrySpendAmmo` (`self.AmmoClipComponent`) (`self.AmmoPerShot`) "NewEnumerator0"))
  (if _spendrequestsuccessful
    (`self.FireWeapon`)
    (bind _currentammo (`/Game/EpicTemplates/RailShooterTemplate/Blueprints/Interfaces/BPI_AmmoClip.GetCurrentAmmo` (`self.AmmoClipComponent`)))
    (if (< _currentammo (`self.AmmoPerShot`))
      (`/Game/EpicTemplates/TemplateAgnostic/Blueprints/Interfaces/BPI_WeaponWielder.RemoveWeapon` (`self.WeaponWielderInterface`) self true))
    (else
      (`self.PlayEmptySound`))))

(fn `UserConstructionScript`
  (`parent.UserConstructionScript`))