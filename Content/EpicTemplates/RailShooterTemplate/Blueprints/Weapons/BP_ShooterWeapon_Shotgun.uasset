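; BP_ShooterWeapon_Shotgun is the rail shooter template's shotgun, which traces multiple damaging pellets per shot.
; The construction script configures its ammo clip component from clip size and start-full settings.
; FireWeapon plays effects, requests a cursor muzzle flash, and line-traces pellets randomly within a cone around the wielder's aim.
; It reports one hit per shot to the hit registry, favoring the first valid hit.
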(fn `FireWeapon`
  (locals (HitActor :type "Actor Object Reference") (AnyHitsValid :type Boolean) (HitLocation :type "Vector Structure" :default (0.0 0.0 0.0)))
  (bind _wieldingplayercontroller (`self.WieldingPlayerController`))
  (`self.PlayFireSound`)
  (`self.SpawnFireParticle`)
  (`/Engine/EditorBlueprintResources/StandardMacros.IsValid` (`self.WieldingActor`)
    (:`Is Valid`
      (`|ExecutionSequence`
        (:`then_0`
          (`/Engine/EditorBlueprintResources/StandardMacros.IsValid` _wieldingplayercontroller
            (:`Is Valid`
              (bind (_cursorwidget _shootercursorinterface) (`/Game/EpicTemplates/RailShooterTemplate/Blueprints/RailShooterFunctionLibrary.GetPlayerShooterCursor` (`GameplayStatics.GetPlayerControllerID` _wieldingplayercontroller)))
              (`/Game/EpicTemplates/RailShooterTemplate/Blueprints/Interfaces/BPI_ShooterCursor.RequestMuzzleFlash` _shootercursorinterface "/Game/EpicTemplates/RailShooterTemplate/UI/W_CursorMuzzleFlash_Shotgun.W_CursorMuzzleFlash_Shotgun_C" 0.2))))
        (:`then_1`
          (bind (_aimstartloc _aimdir) (`/Game/EpicTemplates/TemplateAgnostic/Blueprints/Interfaces/BPI_WeaponWielder.GetAimDir` (`self.WeaponWielderInterface`)))
          (`|ExecutionSequence`
            (:`then_0`
              (for _ (range 1 (+ (`self.PelletsPerShot`) 1))
                (bind (_hitvalid _hitresult) (`self.LineTraceDamageInDirection` _aimstartloc (`KismetMathLibrary.RandomUnitVectorInConeInDegrees` _aimdir (`self.ShotSpreadHalfConeAngle`))))
                (if (not (`local.AnyHitsValid`))
                  (if _hitvalid
                    (set `local.AnyHitsValid` true)
                    (bind (_bblockinghit _binitialoverlap _time _distance _location _impactpoint _normal _impactnormal _physmat _hitactor) (`GameplayStatics.BreakHitResult` _hitresult))
                    (set `local.HitActor` _hitactor)
                    (set `local.HitLocation` _impactpoint)
                    (else
                      (`/Game/EpicTemplates/TemplateAgnostic/Blueprints/EpicTemplatesObjectMacroLibrary.!!!IsNOTValid!!!` (`local.HitActor`)
                        (:`Is NOT Valid`
                          (set `local.HitActor` _hitactor)
                          (set `local.HitLocation` _impactpoint))))))))
            (:`then_1`
              (if (`KismetSystemLibrary.IsValidInterface` (`self.HitRegistryInterface`))
                (`/Engine/EditorBlueprintResources/StandardMacros.IsValid` (`local.HitActor`)
                  (:`Is Valid`
                    (`/Game/EpicTemplates/RailShooterTemplate/Blueprints/Interfaces/BPI_HitRegistry.HitRegistered` (`self.HitRegistryInterface`) (`local.HitActor`) (`self.WieldingPlayerController`) (`local.HitLocation`) (`local.AnyHitsValid`))))))))))))

(fn `GetFirePointTransform`
  (returns (FirePointWorldTrans :type "Transform Structure"))
  (return (`SceneComponent.K2_GetComponentToWorld` (`self.FirePoint`))))

(fn `GetIsInDebug`
  (returns (bIsInDebug :type Boolean))
  (return false))

(fn `UserConstructionScript`
  (bind _ammoclipcomponent (`self.AmmoClipComponent`))
  (`/Game/EpicTemplates/RailShooterTemplate/Blueprints/Interfaces/BPI_AmmoClip.UpdateMaxAmmo` (`self.AmmoClipComponent`) (`self.ClipSize`))
  (if (`self.bStartWithFullClip`)
    (set `/Game/EpicTemplates/TemplateAgnostic/Blueprints/Components/BP_AmmoClipComponent.StartAmmo` (`self.ClipSize`) _ammoclipcomponent)
    (else
      (set `/Game/EpicTemplates/TemplateAgnostic/Blueprints/Components/BP_AmmoClipComponent.StartAmmo` 0.0 _ammoclipcomponent))))