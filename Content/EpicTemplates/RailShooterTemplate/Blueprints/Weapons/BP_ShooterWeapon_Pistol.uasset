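; Pistol weapon for the rail shooter template, firing hitscan shots along the wielder's aim direction.
; Construction sizes the ammo clip component from ClipSize and starts it full or empty.
; FireWeapon plays sound and particles, then, for a valid wielder, flashes the player's cursor muzzle widget if player-controlled and runs a damage line trace.
; Actors hit by the trace are reported, with a validity flag, through the hit registry interface.
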(fn `FireWeapon`
  (locals (AimStartLoc :type "Vector Structure") (AimDir :type "Vector Structure") (HitIsValid :type Boolean))
  (bind _wieldingplayercontroller (`self.WieldingPlayerController`))
  (`self.PlayFireSound`)
  (`self.SpawnFireParticle`)
  (`/Engine/EditorBlueprintResources/StandardMacros.IsValid` (`self.WieldingActor`)
    (:`Is Valid`
      (`|ExecutionSequence`
        (:`then_0`
          (`/Engine/EditorBlueprintResources/StandardMacros.IsValid` _wieldingplayercontroller
            (:`Is Valid`
              (bind (_cursorwidget _shootercursorinterface) (`/Game/EpicTemplates/RailShooterTemplate/Blueprints/RailShooterFunctionLibrary.GetPlayerShooterCursor` (`GameplayStatics.GetPlayerControllerID` _wieldingplayercontroller)))
              (`/Game/EpicTemplates/RailShooterTemplate/Blueprints/Interfaces/BPI_ShooterCursor.RequestMuzzleFlash` _shootercursorinterface "/Game/EpicTemplates/RailShooterTemplate/UI/W_CursorMuzzleFlash_Pistol.W_CursorMuzzleFlash_Pistol_C" 0.2))))
        (:`then_1`
          (bind (_aimstartloc _aimdir) (`/Game/EpicTemplates/TemplateAgnostic/Blueprints/Interfaces/BPI_WeaponWielder.GetAimDir` (`self.WeaponWielderInterface`)))
          (bind (_hitvalid _hitresult) (`self.LineTraceDamageInDirection` _aimstartloc _aimdir))
          (set `local.HitIsValid` _hitvalid)
          (if (`KismetSystemLibrary.IsValidInterface` (`self.HitRegistryInterface`))
            (bind (_bblockinghit _binitialoverlap _time _distance _location _impactpoint _normal _impactnormal _physmat _hitactor) (`GameplayStatics.BreakHitResult` _hitresult))
            (`/Engine/EditorBlueprintResources/StandardMacros.IsValid` _hitactor
              (:`Is Valid`
                (`/Game/EpicTemplates/RailShooterTemplate/Blueprints/Interfaces/BPI_HitRegistry.HitRegistered` (`self.HitRegistryInterface`) _hitactor (`self.WieldingPlayerController`) _impactpoint (`local.HitIsValid`))))))))))

(fn `GetFirePointTransform`
  (returns (FirePointWorldTrans :type "Transform Structure"))
  (return (`SceneComponent.K2_GetComponentToWorld` (`self.FirePoint`))))

(fn `GetIsInDebug`
  (returns (bIsInDebug :type Boolean))
  (return false))

(fn `UserConstructionScript`
  (bind _ammoclipcomponent (`self.AmmoClipComponent`))
  (`/Game/EpicTemplates/RailShooterTemplate/Blueprints/Interfaces/BPI_AmmoClip.UpdateMaxAmmo` (`self.AmmoClipComponent`) (`self.ClipSize`))
  (if (`self.bStartWithFullClip`)
    (set `/Game/EpicTemplates/TemplateAgnostic/Blueprints/Components/BP_AmmoClipComponent.StartAmmo` (`self.ClipSize`) _ammoclipcomponent)
    (else
      (set `/Game/EpicTemplates/TemplateAgnostic/Blueprints/Components/BP_AmmoClipComponent.StartAmmo` 0.0 _ammoclipcomponent))))