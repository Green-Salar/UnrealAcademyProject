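; Base rail shooter weapon that spends clip ammo on primary fire, leaving FireWeapon empty as a hook.
; Caches its wielder's controller, hit-registry and wielder interfaces, and turns the weapon pivot toward the wielder's aim each tick.
; Provides a line-trace damage helper that ignores tracked player pawns and prefers a damageable component over its actor.
; Fire, impact and empty-clip feedback use asynchronously played soft Niagara and sound assets.
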(event `self.UpdateWielder`
  (params (NewWielder :type "Actor Object Reference"))
  ;[1 1 1] BPI_Weapon
  (set `self.WieldingActor` NewWielder)
  (`|ExecutionSequence`
    (:`then_0`
      (bind _aspawn (cast `Pawn` (`self.WieldingActor`))
        (:`then`
          (bind _asplayer_controller (cast `PlayerController` (`Pawn.GetController` _aspawn)))
          (bind _output_get (set `self.WieldingPlayerController` _asplayer_controller))
          (bind (_interfaceimplementingobject _foundimplementingobject) (`/Game/EpicTemplates/TemplateAgnostic/Blueprints/EpicTemplatesFunctionLibrary.SearchActorForInterface` _output_get "/Game/EpicTemplates/RailShooterTemplate/Blueprints/Interfaces/BPI_HitRegistry.BPI_HitRegistry_C"))
          (if _foundimplementingobject
            (bind _asbpi_hit_registry (cast `/Game/EpicTemplates/RailShooterTemplate/Blueprints/Interfaces/BPI_HitRegistry` _interfaceimplementingobject))
            (set `self.HitRegistryInterface` _asbpi_hit_registry)
            (else
              (set `self.HitRegistryInterface` null))))
        (:`CastFailed`
          (set `self.WieldingPlayerController` null)
          (set `self.HitRegistryInterface` null))))
    (:`then_1`
      (bind _interfaceimplementingobject_2 (`/Game/EpicTemplates/TemplateAgnostic/Blueprints/EpicTemplatesFunctionLibrary.SearchActorForInterface` (`self.WieldingActor`) "/Game/EpicTemplates/TemplateAgnostic/Blueprints/Interfaces/BPI_WeaponWielder.BPI_WeaponWielder_C"))
      (bind _asbpi_weapon_wielder (cast `/Game/EpicTemplates/TemplateAgnostic/Blueprints/Interfaces/BPI_WeaponWielder` _interfaceimplementingobject_2)
        (:`then`
          (set `self.WeaponWielderInterface` _asbpi_weapon_wielder))
        (:`CastFailed`
          (set `self.WeaponWielderInterface` null))))))

(event `self.ReceiveBeginPlay`
  ;[1 1 1] BeginPlay
  (`self.PopulatePlayerPawns`))

(event `PlayerPossessedPawnChange`
  (params (OldPawn :type "Pawn Object Reference") (NewPawn :type "Pawn Object Reference"))
  (bind _playerpawns (`self.PlayerPawns`))
  ;[1 1 1] Possessed Pawn Changed
  (`KismetArrayLibrary.Array_RemoveItem` _playerpawns OldPawn)
  (`KismetArrayLibrary.Array_Add` _playerpawns NewPawn))

(event `self.ReceiveTick`
  (params (DeltaSeconds :type "Float (single-precision)"))
  ;[1 1 1] Tick
  (bind (_aimstartloc _aimdir) (`/Game/EpicTemplates/TemplateAgnostic/Blueprints/Interfaces/BPI_WeaponWielder.GetAimDir` (`self.WeaponWielderInterface`)))
  (`SceneComponent.K2_SetWorldRotation` (`self.WeaponPivot`) (`KismetMathLibrary.FindLookAtRotation` (`SceneComponent.K2_GetComponentLocation` (`self.WeaponPivot`)) (+ _aimstartloc (* _aimdir (`self.FireDistance`)))) false false))

(event `PlayerPawnedDestroyed`
  (params (DestroyedActor :type "Actor Object Reference"))
  ;[1 1 1] PossessedPawn Destroyed
  (`KismetArrayLibrary.Array_RemoveItem` (`self.PlayerPawns`) DestroyedActor))

(event `self.UpdateIsCurrentlyWielded`
  (params (bIsWielded :type Boolean))
  ;[1 1 1] BPI_Weapon
  (`self.SetActorTickEnabled` bIsWielded)
  (`self.SetActorHiddenInGame` (not bIsWielded)))

(event `self.PrimaryFirePressed`
  ;[1 1 1] BPI_Weapon
  (`self.FireWeaponIfHaveAmmo`))

(event `self.ReceiveEndPlay`
  (params (EndPlayReason :type "EEndPlayReason Enum" :default "Destroyed"))
  ;[1 1 1] EndPlay
  (for _index (range (`GameplayStatics.GetNumPlayerControllers`))
    (remove `Controller.OnPossessedPawnChanged` (`GameplayStatics.GetPlayerController` _index) (`|CreateDelegate` :!event `PlayerPossessedPawnChange`))))

(event `self.SecondaryFirePressed`
  ;[1 1 1] BPI_Weapon
)

(event `SpawnFireParticle`
  ;[1 1 1] Feedback
  (`/Game/EpicTemplates/TemplateAgnostic/Blueprints/EpicTemplatesActorMacroLibrary.PlaySoftNiagaraParticleAsyncAtLocation` (`self.FireParticle`) (.location (`self.GetFirePointTransform`)) (.rotation (`self.GetFirePointTransform`))))

(event `PlayFireSound`
  ;[1 1 1] Feedback
  (`/Game/EpicTemplates/TemplateAgnostic/Blueprints/EpicTemplatesActorMacroLibrary.PlaySoftSoundAsyncAtLocation` (`self.FireSound`) (.location (`self.GetFirePointTransform`))))

(event `PlayEmptySound`
  ;[1 1 1] Feedback
  (`/Game/EpicTemplates/TemplateAgnostic/Blueprints/EpicTemplatesActorMacroLibrary.PlaySoftSoundAsyncAtLocation` (`self.EmptyClipSound`) (`SceneComponent.K2_GetComponentLocation` (`self.WeaponPivot`))))

(event `SpawnHitParticle`
  (params (HitLocation :type "Vector Structure") (HitNormal :type "Vector Structure"))
  ;[1 1 1] Feedback
  (`/Game/EpicTemplates/TemplateAgnostic/Blueprints/EpicTemplatesActorMacroLibrary.PlaySoftNiagaraParticleAsyncAtLocation` (`self.HitParticle`) HitLocation (`KismetMathLibrary.MakeRotFromX` HitNormal)))

(event `self.UpdateIsInDebug`
  (params (bInIsDebug :type Boolean))
  (set `self.In Is Debug` bInIsDebug))

(fn `FireWeapon`
  (locals (AimStartLoc :type "Vector Structure" :default (0.0 0.0 0.0)) (AimDir :type "Vector Structure" :default (0.0 0.0 0.0)) (HitActor :type "Actor Object Reference") (DamageableInterfaceObject :type "Object Object Reference") (HitComponent :type "PrimitiveComponent Object Reference") (ImpactPoint :type "Vector Structure" :default (0.0 0.0 0.0)) (ImpactNormal :type "Vector Structure" :default (0.0 0.0 0.0)) (HitBoneName :type Name :default "None") (HitIsValid :type Boolean :default false)))

(fn `FireWeaponIfHaveAmmo`
  (bind (_ammospent _spendrequestsuccessful) (`/Game/EpicTemplates/RailShooterTemplate/Blueprints/Interfaces/BPI_AmmoClip.TrySpendAmmo` (`self.AmmoClipComponent`) (`self.AmmoPerShot`) "NewEnumerator0"))
  (if _spendrequestsuccessful
    (`self.FireWeapon`)
    (else
      (`self.PlayEmptySound`))))

(fn `GetAmmoType`
  (returns (AmmoType :type "/Game/EpicTemplates/RailShooterTemplate/Blueprints/Enums/EAmmoType Enum"))
  (return (`self.AmmoType`)))

(fn `GetDamageSourceOwner`
  (returns (DamageSourceOwner :type "Actor Object Reference"))
  (`/Engine/EditorBlueprintResources/StandardMacros.IsValid` (`self.WieldingPlayerController`)
    (:`Is Valid`
      (return (`self.WieldingPlayerController`)))
    (:`Is Not Valid`
      (`/Engine/EditorBlueprintResources/StandardMacros.IsValid` (`self.WieldingActor`)
        (:`Is Valid`
          (return (`self.WieldingActor`)))
        (:`Is Not Valid`
          (return self))))))

(fn `GetFirePointTransform`
  (returns (FirePointWorldTrans :type "Transform Structure"))
  (return))

(fn `GetIsInDebug`
  (returns (bIsInDebug :type Boolean))
  (return false))

(fn `GetWielder`
  (returns (Wielder :type "Actor Object Reference"))
  (return (`self.WieldingActor`)))

(fn `LineTraceDamageInDirection`
  (params (TraceStart :type "Vector Structure (by ref)") (TraceDir :type "Vector Structure (by ref)"))
  (returns (HitValid :type Boolean) (HitResult :type "HitResult Structure"))
  (locals (HitComponent :type "PrimitiveComponent Object Reference") (HitActor :type "Actor Object Reference") (DamageableInterfaceObject :type "Object Object Reference") (ImpactPoint :type "Vector Structure") (ImpactNormal :type "Vector Structure") (HitIsValid :type Boolean) (HitBoneName :type Name))
  (bind _damageableinterfaceobject (`local.DamageableInterfaceObject`))
  (bind _outhit (`KismetSystemLibrary.LineTraceSingle` TraceStart (+ TraceStart (* TraceDir (`self.FireDistance`))) "TraceTypeQuery3" false (`self.PlayerPawns`) "None" true (struct :`R` 1.0 :`A` 1.0) (struct :`G` 1.0 :`A` 1.0) 4.0))
  (bind (_bblockinghit _binitialoverlap _time _distance _location _impactpoint _normal _impactnormal _physmat _hitactor _hitcomponent _hitbonename) (`GameplayStatics.BreakHitResult` _outhit))
  (set `local.ImpactPoint` _impactpoint)
  (set `local.ImpactNormal` _impactnormal)
  (set `local.HitActor` _hitactor)
  (set `local.HitComponent` _hitcomponent)
  (set `local.HitBoneName` _hitbonename)
  (set `local.HitIsValid` false)
  (`|ExecutionSequence`
    (:`then_0`
      (`/Engine/EditorBlueprintResources/StandardMacros.IsValid` (`local.HitActor`)
        (:`Is Valid`
          (`self.SpawnHitParticle` (`local.ImpactPoint`) (`local.ImpactNormal`))
          (`|ExecutionSequence`
            (:`then_0`
              (if (`KismetSystemLibrary.DoesImplementInterface` (`local.HitComponent`) "/Game/EpicTemplates/TemplateAgnostic/Blueprints/Interfaces/BPI_Damageable.BPI_Damageable_C")
                (set `local.DamageableInterfaceObject` (`local.HitComponent`))
                (else
                  (bind _interfaceimplementingobject (`/Game/EpicTemplates/TemplateAgnostic/Blueprints/EpicTemplatesFunctionLibrary.SearchActorForInterface` (`local.HitActor`) "/Game/EpicTemplates/TemplateAgnostic/Blueprints/Interfaces/BPI_Damageable.BPI_Damageable_C"))
                  (`/Engine/EditorBlueprintResources/StandardMacros.IsValid` _interfaceimplementingobject
                    (:`Is Valid`
                      (set `local.DamageableInterfaceObject` _interfaceimplementingobject))))))
            (:`then_1`
              (`/Engine/EditorBlueprintResources/StandardMacros.IsValid` _damageableinterfaceobject
                (:`Is Valid`
                  (bind (_damagedealt _damageapplied) (message `/Game/EpicTemplates/TemplateAgnostic/Blueprints/Interfaces/BPI_Damageable.ApplyDamage` _damageableinterfaceobject (make `/Game/EpicTemplates/TemplateAgnostic/Blueprints/Structs/DamageStruct` (`self.WeaponDamage`) self (`self.GetDamageSourceOwner`) (`local.ImpactPoint`) (`local.TraceDir`) (`local.HitBoneName`))))
                  (set `local.HitIsValid` _damageapplied)
                  (if (`self.In Is Debug`)
                    (`KismetSystemLibrary.PrintString` (`KismetStringLibrary.Concat_StrStr` "Applying Damage to:" (`KismetSystemLibrary.GetDisplayName` (`local.HitActor`))) true true (struct :`G` 0.66 :`B` 1.0 :`A` 1.0) 10.0)))
                (:`Is Not Valid`
                  (if (`self.In Is Debug`)
                    (`/Engine/EditorBlueprintResources/StandardMacros.IsValid` (`local.HitActor`)
                      (:`Is Valid`
                        (`KismetSystemLibrary.PrintString` (`KismetStringLibrary.Concat_StrStr` "Hit actor that doesn't take damage: " (`KismetSystemLibrary.GetDisplayName` (`local.HitActor`))) true true (struct :`G` 0.66 :`B` 1.0 :`A` 1.0) 10.0))
                      (:`Is Not Valid`
                        (`KismetSystemLibrary.PrintString` "Hit Nothing" true true (struct :`G` 0.66 :`B` 1.0 :`A` 1.0) 10.0)))))))))))
    (:`then_1`
      (return (`local.HitIsValid`) _outhit))))

(fn `PopulatePlayerPawns`
  (locals (TempPawn :type "Pawn Object Reference") (TempPlayerCont :type "PlayerController Object Reference"))
  (bind _temppawn (`local.TempPawn`))
  (for _index (range (`GameplayStatics.GetNumPlayerControllers`))
    (bind _returnvalue (`GameplayStatics.GetPlayerController` _index))
    (set `local.TempPlayerCont` _returnvalue)
    (add `Controller.OnPossessedPawnChanged` _returnvalue (`|CreateDelegate` :!event `PlayerPossessedPawnChange`))
    (bind _output_get (set `local.TempPawn` (`Controller.K2_GetPawn` (`local.TempPlayerCont`))))
    (`/Engine/EditorBlueprintResources/StandardMacros.IsValid` _output_get
      (:`Is Valid`
        (`KismetArrayLibrary.Array_Add` (`self.PlayerPawns`) _temppawn)
        (add `self.OnDestroyed` _temppawn (`|CreateDelegate` :!event `PlayerPawnedDestroyed`))))))

(fn `UserConstructionScript`
  (bind _ammoclipcomponent (`self.AmmoClipComponent`))
  (`/Game/EpicTemplates/RailShooterTemplate/Blueprints/Interfaces/BPI_AmmoClip.UpdateMaxAmmo` (`self.AmmoClipComponent`) (`self.ClipSize`))
  (if (`self.bStartWithFullClip`)
    (set `/Game/EpicTemplates/TemplateAgnostic/Blueprints/Components/BP_AmmoClipComponent.StartAmmo` (`self.ClipSize`) _ammoclipcomponent)
    (else
      (set `/Game/EpicTemplates/TemplateAgnostic/Blueprints/Components/BP_AmmoClipComponent.StartAmmo` 0.0 _ammoclipcomponent))))