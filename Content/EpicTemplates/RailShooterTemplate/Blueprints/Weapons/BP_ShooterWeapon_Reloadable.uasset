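; Reloadable weapon for the rail shooter template, firing from an ammo clip component and refilling it on secondary fire.
; When the wielder changes, it caches that actor's BPI_AmmoSource, which reloads draw on to top up the clip.
; A successful spend refills the clip immediately, then a sound and duration-scaled timeline pitch the reload pivot.
; Primary fire and further reloads stay blocked until the timeline finishes.
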(event `/Game/EpicTemplates/TemplateAgnostic/Blueprints/Interfaces/BPI_Weapon.UpdateWielder`
  (params (NewWielder :type "Actor Object Reference"))
  ;[1 1 1] BPI_Weapon
  (`parent.UpdateWielder` NewWielder)
  (bind _interfaceimplementingobject (`/Game/EpicTemplates/TemplateAgnostic/Blueprints/EpicTemplatesFunctionLibrary.SearchActorForInterface` (`self.WieldingActor`) "/Game/EpicTemplates/RailShooterTemplate/Blueprints/Interfaces/BPI_AmmoSource.BPI_AmmoSource_C"))
  (bind _asbpi_ammo_source (cast `/Game/EpicTemplates/RailShooterTemplate/Blueprints/Interfaces/BPI_AmmoSource` _interfaceimplementingobject)
    (:`then`
      (set `self.AmmoSourceInterface` _asbpi_ammo_source))
    (:`CastFailed`
      (set `self.AmmoSourceInterface` null))))

(event `self.ReceiveBeginPlay`
  ;[1 1 1] BeginPlay
  (`parent.ReceiveBeginPlay`)
  (`TimelineComponent.SetPlayRate` (`self.TL_Reload`) (/ 1.0 (`self.ReloadDuration`))))

(event `self.PrimaryFirePressed`
  ;[1 1 1] BPI_Weapon
  (if (not (`self.bReloading`))
    (`self.FireWeaponIfHaveAmmo`)))

(event `self.SecondaryFirePressed`
  ;[1 1 1] BPI_Weapon
  (if (`KismetSystemLibrary.IsValidInterface` (`self.AmmoSourceInterface`))
    (`self.TryReload`)))

(event `ReloadFeedback`
  (`self.PlayReloadSound`)
  (bind (_direction _reloadpivotalpha) (`Timeline|TL_Reload` :!via `PlayFromStart`)
    (:`Update`
      (`SceneComponent.K2_SetRelativeRotation` (`self.ReloadPivot`) (`KismetMathLibrary.MakeRotator` 0.0 (* _reloadpivotalpha (`self.ReloadPitchDip`))) false false))
    (:`Finished`
      (set `self.bReloading` false))))

(event `PlayReloadSound`
  ;[1 1 1] Feedback
  (`/Game/EpicTemplates/TemplateAgnostic/Blueprints/EpicTemplatesActorMacroLibrary.PlaySoftSoundAsyncAtLocation` (`self.ReloadSound`) (.location (`self.GetFirePointTransform`))))

(fn `GetIsInDebug`
  (returns (bIsInDebug :type Boolean))
  (return false))

(fn `TryReload`
  (locals (DesiredAmmo :type "Float (double-precision)") (CurrentAmmo :type "Float (double-precision)" :default 0.0))
  (if (not (`self.bReloading`))
    (bind _currentammo (`/Game/EpicTemplates/RailShooterTemplate/Blueprints/Interfaces/BPI_AmmoClip.GetCurrentAmmo` (`self.AmmoClipComponent`)))
    (bind _output_get (set `local.CurrentAmmo` _currentammo))
    (bind _output_get_2 (set `local.DesiredAmmo` (- (`self.ClipSize`) _output_get)))
    (if (> _output_get_2 0.0)
      (bind (_ammospent _spendrequestsuccessful) (`/Game/EpicTemplates/RailShooterTemplate/Blueprints/Interfaces/BPI_AmmoSource.TrySpendAmmoOfType` (`self.AmmoSourceInterface`) (`self.AmmoType`) (`local.DesiredAmmo`) "NewEnumerator1"))
      (if _spendrequestsuccessful
        (set `self.bReloading` true)
        (`self.ReloadFeedback`)
        (`/Game/EpicTemplates/RailShooterTemplate/Blueprints/Interfaces/BPI_AmmoClip.UpdateAmmo` (`self.AmmoClipComponent`) (+ _ammospent (`local.CurrentAmmo`)))))))

(fn `UserConstructionScript`
  (bind _ammoclipcomponent (`self.AmmoClipComponent`))
  (`/Game/EpicTemplates/RailShooterTemplate/Blueprints/Interfaces/BPI_AmmoClip.UpdateMaxAmmo` (`self.AmmoClipComponent`) (`self.ClipSize`))
  (if (`self.bStartWithFullClip`)
    (set `/Game/EpicTemplates/TemplateAgnostic/Blueprints/Components/BP_AmmoClipComponent.StartAmmo` (`self.ClipSize`) _ammoclipcomponent)
    (else
      (set `/Game/EpicTemplates/TemplateAgnostic/Blueprints/Components/BP_AmmoClipComponent.StartAmmo` 0.0 _ammoclipcomponent))))