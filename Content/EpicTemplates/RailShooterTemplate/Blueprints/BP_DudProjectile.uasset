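; BP_DudProjectile is a rail shooter template projectile that flies along a launch direction and disappears on impact without applying damage.
; It can self-launch on BeginPlay, with ProjectileMovement providing the velocity.
; Overlaps ignore owner and instigator, and optionally teammates via BPI_TeamParticipant.
; Hits, valid overlaps or death disable and hide it for pooling through ReusableActorComponent, whose reset request restores collision, visibility, movement and health.
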(event `self.ReceiveBeginPlay`
  (if (`self.LaunchSelfOnBeginPlay`)
    (`/Game/EpicTemplates/TemplateAgnostic/Blueprints/Interfaces/BPI_Projectile.LaunchInDirection` (`self.GetOwner`) (`self.GetActorForwardVector`) (`self.DefaultLaunchSpeed`))))

(event `self.ReusableActorComponent.OnResetRequested`
  (params (Caller :type "/Game/EpicTemplates/TemplateAgnostic/Blueprints/Components/BP_ReusableActorComponent Object Reference") (ResetActor :type "Actor Object Reference"))
  (`PrimitiveComponent.SetCollisionEnabled` (`self.CollisionSphere`) "QueryOnly")
  (`self.SetActorHiddenInGame` false)
  (`ActorComponent.Activate` (`self.ProjectileMovement`) true)
  (`/Game/EpicTemplates/TemplateAgnostic/Blueprints/Interfaces/BPI_HealthSource.UpdateHealth` (`self.HealthComponent`) 1.0))

(event `self.HealthComponent.OnDied`
  (params (Caller :type "/Game/EpicTemplates/TemplateAgnostic/Blueprints/Components/BP_HealthComponent Object Reference") (KillingDamageSourceOwner :type "Actor Object Reference") (KillingDamageSource :type "Actor Object Reference") (KillingDamageLocation :type "Vector Structure") (KillingDamageDirection :type "Vector Structure") (HitBone :type Name) (SpecialDamageName :type Name))
  (`self.DisableProjectile`))

(event `self.CollisionSphere.OnComponentBeginOverlap`
  (params (OverlappedComponent :type "PrimitiveComponent Object Reference") (OtherActor :type "Actor Object Reference") (OtherComp :type "PrimitiveComponent Object Reference") (OtherBodyIndex :type Integer) (bFromSweep :type Boolean) (SweepResult :type "HitResult Structure (by ref)"))
  (`self.OverlapActor` OtherActor))

(event `self.CollisionSphere.OnComponentHit`
  (params (HitComponent :type "PrimitiveComponent Object Reference") (OtherActor :type "Actor Object Reference") (OtherComp :type "PrimitiveComponent Object Reference") (NormalImpulse :type "Vector Structure") (Hit :type "HitResult Structure (by ref)"))
  (`self.DisableProjectile`))

(event `self.ReusableActorComponent.OnRequestDestroySelf`
  (`self.K2_DestroyActor`))

(event `/Game/EpicTemplates/TemplateAgnostic/Blueprints/Interfaces/BPI_Projectile.LaunchInDirection`
  (params (ProjectileOwner :type "Actor Object Reference") (Direction :type "Vector Structure") (Speed :type "Float (double-precision)"))
  (`self.K2_SetActorRotation` (`KismetMathLibrary.Conv_VectorToRotator` Direction))
  (bind _output_get (set `self.CurrentProjectileSpeed` (select `bool` (<= Speed 0.0) :`false` Speed :`true` (`self.DefaultLaunchSpeed`))))
  (`ProjectileMovementComponent.SetVelocityInLocalSpace` (`self.ProjectileMovement`) (`KismetMathLibrary.MakeVector` _output_get)))

(fn `DisableProjectile`
  (`PrimitiveComponent.SetCollisionEnabled` (`self.CollisionSphere`) "NoCollision")
  (`self.SetActorHiddenInGame` true)
  (`ActorComponent.Deactivate` (`self.ProjectileMovement`))
  (`/Game/EpicTemplates/TemplateAgnostic/Blueprints/Components/BP_ReusableActorComponent.MarkReadyForReuse` (`self.ReusableActorComponent`)))

(fn `OverlapActor`
  (params (OtherActor :type "Actor Object Reference"))
  (if (and (!= (`local.OtherActor`) (`self.GetOwner`)) (!= (`local.OtherActor`) (`self.GetInstigator`)))
    (`|ExecutionSequence`
      (:`then_0`
        (if (`self.bOnlyHitObjectsOfOtherTeams`)
          (bind (_interfaceimplementingobject _foundimplementingobject) (`/Game/EpicTemplates/TemplateAgnostic/Blueprints/EpicTemplatesFunctionLibrary.SearchActorForInterface` (`local.OtherActor`) "/Game/EpicTemplates/TemplateAgnostic/Blueprints/Interfaces/BPI_TeamParticipant.BPI_TeamParticipant_C"))
          (if _foundimplementingobject
            (bind _team (message `/Game/EpicTemplates/TemplateAgnostic/Blueprints/Interfaces/BPI_TeamParticipant.GetTeam` _interfaceimplementingobject))
            (bind _team_2 (message `/Game/EpicTemplates/TemplateAgnostic/Blueprints/Interfaces/BPI_TeamParticipant.GetTeam` (`self.TeamComponent`)))
            (if (`|EnumEquality` _team_2 _team)
              (return)))))
      (:`then_1`
        (`self.DisableProjectile`)))))

(fn `UserConstructionScript`)