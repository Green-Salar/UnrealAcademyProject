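; Player pawn for the rail shooter template, carried along splines by SplineFollowComponent and given a cursor and game HUD on possession.
; Tick eases control rotation toward a switchable view target: actor, location, relative rotation, or player 1's or all players' averaged cursor position.
; Co-op setup offsets each player on the spline; with splitscreen disabled, secondary pawns stop following, attach to player 1's pawn and mount their mirrored weapon on its camera.
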(event `PrimaryPlayerControllerPossesedNewPawn`
  (params (OldPawn :type "Pawn Object Reference") (NewPawn :type "Pawn Object Reference"))
  (bind _asbp_player_pawn_rail_shooter (cast `/Game/EpicTemplates/RailShooterTemplate/Blueprints/Core/BP_PlayerPawn_RailShooter` NewPawn))
  (`SceneComponent.K2_AttachToComponent` (`self.WeaponPivot`) (`/Game/EpicTemplates/RailShooterTemplate/Blueprints/Core/BP_PlayerPawn_RailShooter.ViewCamera` _asbp_player_pawn_rail_shooter) "None" "KeepRelative" "KeepRelative" "KeepRelative" true))

(event `self.ReceivePossessed`
  (params (NewController :type "Controller Object Reference"))
  ;[1 1 1] Possessed
  (if (!= NewController (`self.OwningPlayerController`))
    (`self.SetupPlayerController` NewController)))

(event `EnhancedInput|/Game/EpicTemplates/RailShooterTemplate/Input/Actions/IA_GamepadMoveCursor`
  (params (ActionValue :type "Vector2D Structure") (ElapsedSeconds :type "Float (double-precision)") (TriggeredSeconds :type "Float (double-precision)") (InputAction :type "InputAction Object Reference" :default "/Game/EpicTemplates/RailShooterTemplate/Input/Actions/IA_GamepadMoveCursor.IA_GamepadMoveCursor"))
  (bind _owningplayercontroller (`self.OwningPlayerController`))
  ;[1 1 1] Input
  (:`Triggered`
    (`/Engine/EditorBlueprintResources/StandardMacros.IsValid` _owningplayercontroller
      (:`Is Valid`
        (message `/Game/EpicTemplates/TemplateAgnostic/Blueprints/Interfaces/BPI_CursorImplementor.AdjustCursorScreenPosition` _owningplayercontroller (* ActionValue (`self.GamepadCursorMoveSpeed`) (`GameplayStatics.GetWorldDeltaSeconds`)))))))

(event `SetupPlayerUI`
  (bind _gamecursor (`self.GameCursor`))
  (bind _gameui (`self.GameUI`))
  (`|ExecutionSequence`
    (:`then_0`
      (`|ExecutionSequence`
        (:`then_0`
          (`/Engine/EditorBlueprintResources/StandardMacros.IsValid` _gamecursor
            (:`Is Valid`
              (`Widget.RemoveFromParent` _gamecursor)
              (`Widget.RemoveFromParent` (`self.GameCursor`)))
            (:`Is Not Valid`
              (bind _returnvalue (`|CreateWidget` "/Game/EpicTemplates/RailShooterTemplate/UI/W_PlayerGameCursor_Shooter.W_PlayerGameCursor_Shooter_C" (`self.OwningPlayerController`)))
              (set `self.GameCursor` _returnvalue))))
        (:`then_1`
          (`UserWidget.AddToViewport` (`self.GameCursor`) 0))))
    (:`then_1`
      (`|ExecutionSequence`
        (:`then_0`
          (`/Engine/EditorBlueprintResources/StandardMacros.IsValid` _gameui
            (:`Is Valid`
              (`Widget.RemoveFromParent` _gameui)
              (`Widget.RemoveFromParent` (`self.GameUI`)))
            (:`Is Not Valid`
              (bind _returnvalue_2 (`|CreateWidget` "/Game/EpicTemplates/RailShooterTemplate/UI/W_GameUI_RailShooter.W_GameUI_RailShooter_C" (`self.OwningPlayerController`)))
              (set `self.GameUI` _returnvalue_2))))
        (:`then_1`
          (`UserWidget.AddToViewport` (`self.GameUI`) 0))))))

(event `AttachToNewSpline`
  (params (SplineActor :type "Actor Object Reference") (AttachToSplineType :type "/Game/EpicTemplates/RailShooterTemplate/Blueprints/Enums/EAttachToSplineType Enum" :default "NewEnumerator0") (SplineTarget :type "/Game/EpicTemplates/RailShooterTemplate/Blueprints/Structs/SplineTargetStruct Structure (by ref)"))
  (bind _splinefollowcomponent (`self.SplineFollowComponent`))
  ;[1 1 1] Attach to spline
  (bind _spline (`self.GetMostSuitableSplineFromActor` SplineActor))
  (`/Game/EpicTemplates/RailShooterTemplate/Blueprints/Components/BP_SplineFollowerComponent.AttachToActorSpline` _splinefollowcomponent _spline AttachToSplineType)
  (`/Game/EpicTemplates/RailShooterTemplate/Blueprints/Components/BP_SplineFollowerComponent.SetMoveTarget` _splinefollowcomponent SplineTarget))

(event `self.HealthComponent.OnDied`
  (params (Caller :type "/Game/EpicTemplates/TemplateAgnostic/Blueprints/Components/BP_HealthComponent Object Reference") (KillingDamageSourceOwner :type "Actor Object Reference") (KillingDamageSource :type "Actor Object Reference") (KillingDamageLocation :type "Vector Structure") (KillingDamageDirection :type "Vector Structure") (HitBone :type Name) (SpecialDamageName :type Name))
  ;[1 1 1] On died
  (`Widget.RemoveFromParent` (`self.GameCursor`))
  (`Widget.RemoveFromParent` (`self.GameUI`)))

(event `self.ReceiveBeginPlay`
  ;[1 1 1] Begin Play
  (set `self.PrimaryPlayerController` (`GameplayStatics.GetPlayerController` 0)))

(event `self.ReceiveTick`
  (params (DeltaSeconds :type "Float (single-precision)"))
  ;[1 1 1] Tick
  (`Controller.SetControlRotation` (`self.GetController`) (`KismetMathLibrary.RInterpTo` (`self.GetControlRotation`) (`self.GetViewTargetRotation`) DeltaSeconds (`self.ViewTargetInterpSpeed`))))

(event `/Game/EpicTemplates/TemplateAgnostic/Blueprints/Interfaces/BPI_Debuggable.UpdateIsInDebug`
  (params (bInIsDebug :type Boolean))
  ;[1 1 1] Update Debug
  (bind _output_get (set `self.InDebugMode` bInIsDebug))
  (`SceneComponent.SetHiddenInGame` (`self.CapsuleRoot`) (not _output_get) false)
  (`/Game/EpicTemplates/RailShooterTemplate/Blueprints/Components/BP_SplineFollowerComponent.UpdateIsInDebug` (`self.SplineFollowComponent`) (`self.InDebugMode`)))

(fn `ClearViewTarget`
  (params (bSnapToRotation :type Boolean))
  (set `self.CurrentViewTargetType` "NewEnumerator0")
  (set `self.CurrentViewTargetActor` null)
  (set `self.CurrentViewTargetPosition` (0.0 0.0 0.0))
  (set `self.CurrentViewTargetRelativeRotation` (struct)))

(fn `GetIsInDebug`
  (returns (bIsInDebug :type Boolean))
  (return (`self.InDebugMode`)))

(fn `GetMostSuitableSplineFromActor`
  (params (SplineActor :type "Actor Object Reference"))
  (returns (Spline :type "SplineComponent Object Reference"))
  (bind _splines (`/Game/EpicTemplates/TemplateAgnostic/Blueprints/EpicTemplatesFunctionLibrary.Get Splines From Actor` SplineActor))
  (return (`|GetArrayItem` _splines (`KismetMathLibrary.Max` (`GameplayStatics.GetPlayerControllerID` (`self.OwningPlayerController`)) (`KismetArrayLibrary.Array_Length` _splines)))))

(fn `GetViewTargetRotation`
  (returns (ViewTargetRotation :type "Rotator Structure"))
  (locals (ScreenCursorPos :type "Vector2D Structure"))
  (bind (_x _y) (`KismetMathLibrary.BreakVector2D` (`WidgetLayoutLibrary.GetViewportSize`)))
  (bind (_x_2 _y_2) (`KismetMathLibrary.BreakVector2D` (`WidgetLayoutLibrary.GetViewportSize`)))
  (switch `/Game/EpicTemplates/RailShooterTemplate/Blueprints/Enums/EViewTargetType` (`self.CurrentViewTargetType`)
    (:`NewEnumerator0`
      (return (`self.K2_GetActorRotation`)))
    (:`NewEnumerator1`
      (`/Engine/EditorBlueprintResources/StandardMacros.IsValid` (`self.CurrentViewTargetActor`)
        (:`Is Valid`
          (return (`KismetMathLibrary.FindLookAtRotation` (`SceneComponent.K2_GetComponentLocation` (`self.ViewCamera`)) (`self.K2_GetActorLocation` (`self.CurrentViewTargetActor`)))))
        (:`Is Not Valid`
          (return (`self.K2_GetActorRotation`)))))
    (:`NewEnumerator2`
      (return (`KismetMathLibrary.FindLookAtRotation` (`SceneComponent.K2_GetComponentLocation` (`self.ViewCamera`)) (`self.CurrentViewTargetPosition`))))
    (:`NewEnumerator3`
      (return (`KismetMathLibrary.TransformRotation` (`self.GetTransform`) (`self.CurrentViewTargetRelativeRotation`))))
    (:`NewEnumerator4`
      (bind _screenpos (message `/Game/EpicTemplates/TemplateAgnostic/Blueprints/Interfaces/BPI_CursorImplementor.GetCursorScreenPosition` (`GameplayStatics.GetPlayerController` 0)))
      (bind (_x_3 _y_3) (`KismetMathLibrary.BreakVector2D` _screenpos))
      (return (`KismetMathLibrary.TransformRotation` (`self.GetTransform`) (`KismetMathLibrary.MakeRotator` 0.0 (`KismetMathLibrary.MapRangeClamped` _y_3 0.0 _y_2 (* (`self.ViewTargetCursorMaxPitch`) -1.0) (`self.ViewTargetCursorMaxPitch`)) (`KismetMathLibrary.MapRangeClamped` _x_3 0.0 _x_2 (* (`self.ViewTargetCursorMaxYaw`) -1.0) (`self.ViewTargetCursorMaxYaw`))))))
    (:`NewEnumerator5`
      (for _index (range (`GameplayStatics.GetNumPlayerControllers`))
        (bind _screenpos_2 (message `/Game/EpicTemplates/TemplateAgnostic/Blueprints/Interfaces/BPI_CursorImplementor.GetCursorScreenPosition` (`GameplayStatics.GetPlayerController` _index)))
        (set `local.ScreenCursorPos` (+ _screenpos_2 (`local.ScreenCursorPos`))))
      (bind _output_get (set `local.ScreenCursorPos` (/ (`local.ScreenCursorPos`) (`KismetMathLibrary.Conv_IntToDouble` (`GameplayStatics.GetNumPlayerControllers`)))))
      (bind (_x_4 _y_4) (`KismetMathLibrary.BreakVector2D` _output_get))
      (return (`KismetMathLibrary.TransformRotation` (`self.GetTransform`) (`KismetMathLibrary.MakeRotator` 0.0 (`KismetMathLibrary.MapRangeClamped` _y_4 0.0 _y (* (`self.ViewTargetCursorMaxPitch`) -1.0)) (`KismetMathLibrary.MapRangeClamped` _x_4 0.0 _x (* (`self.ViewTargetCursorMaxYaw`) -1.0) (`self.ViewTargetCursorMaxYaw`))))))))

(fn `SetupPlayerController`
  (params (Controller :type "Object Object Reference"))
  (locals (PlayerIndex :type Integer :default 0))
  (bind _returnvalue (`GameplayStatics.GetPlayerController` 0))
  (bind _asplayer_controller (cast `PlayerController` Controller)
    (:`then`
      (bind _output_get (set `self.OwningPlayerController` _asplayer_controller))
      (set `local.PlayerIndex` (`GameplayStatics.GetPlayerControllerID` _output_get))
      (bind _issingleplayer (`/Game/EpicTemplates/TemplateAgnostic/Blueprints/EpicTemplatesFunctionLibrary.IsInSinglePlayerMode`))
      (`/Game/EpicTemplates/RailShooterTemplate/Blueprints/Components/BP_SplineFollowerComponent.UpdateSplineFollowOffset` (`self.SplineFollowComponent`) (select `bool` (or _issingleplayer (`GameplayStatics.IsSplitscreenForceDisabled`)) :`false` (select `int` (`local.PlayerIndex`) :`0` (`KismetMathLibrary.MakeVector` 0.0 (* (`self.SplineYOffset2Player`) -1.0)) :`1` (`KismetMathLibrary.MakeVector` 0.0 (`self.SplineYOffset2Player`)))) true)
      (`|ExecutionSequence`
        (:`then_0`
          (if (!= (`local.PlayerIndex`) 0)
            (`SceneComponent.K2_SetRelativeLocation` (`self.WeaponPivot`) (`KismetMathLibrary.MakeVector` (.x (`SceneComponent.RelativeLocation` (`self.WeaponPivot`))) (* (.y (`SceneComponent.RelativeLocation` (`self.WeaponPivot`))) -1.0) (.z (`SceneComponent.RelativeLocation` (`self.WeaponPivot`)))) false false)
            (if (`GameplayStatics.IsSplitscreenForceDisabled`)
              (`/Game/EpicTemplates/RailShooterTemplate/Blueprints/Components/BP_SplineFollowerComponent.LockSplineFollowLogic` (`self.SplineFollowComponent`))
              (add `Controller.OnPossessedPawnChanged` _returnvalue (`|CreateDelegate` :!event `PrimaryPlayerControllerPossesedNewPawn`))
              (bind _asbp_player_pawn_rail_shooter (cast `/Game/EpicTemplates/RailShooterTemplate/Blueprints/Core/BP_PlayerPawn_RailShooter` (`Controller.K2_GetPawn` _returnvalue)))
              (`SceneComponent.K2_AttachToComponent` (`self.WeaponPivot`) (`/Game/EpicTemplates/RailShooterTemplate/Blueprints/Core/BP_PlayerPawn_RailShooter.ViewCamera` _asbp_player_pawn_rail_shooter) "None" "KeepRelative" "KeepRelative" "KeepRelative" true)
              (`self.K2_AttachToActor` _asbp_player_pawn_rail_shooter "None" "SnapToTarget" "SnapToTarget" "SnapToTarget"))))
        (:`then_1`
          (`self.SetupPlayerUI`))))
    (:`CastFailed`
      (return))))

(fn `SetViewTargetAsActor`
  (params (TargetActor :type "Actor Object Reference") (bSnapToRotation :type Boolean))
  (set `self.CurrentViewTargetActor` TargetActor)
  (set `self.CurrentViewTargetType` "NewEnumerator1")
  (if bSnapToRotation
    (`SceneComponent.K2_SetWorldRotation` (`self.ViewCamera`) (`KismetMathLibrary.FindLookAtRotation` (`SceneComponent.K2_GetComponentLocation` (`self.ViewCamera`)) (`self.K2_GetActorLocation` (`self.CurrentViewTargetActor`))) false false)))

(fn `SetViewTargetAsLocation`
  (params (TargetWorldLocation :type "Vector Structure") (bSnapToRotation :type Boolean))
  (set `self.CurrentViewTargetPosition` TargetWorldLocation)
  (set `self.CurrentViewTargetType` "NewEnumerator2")
  (if bSnapToRotation
    (`SceneComponent.K2_SetWorldRotation` (`self.ViewCamera`) (`KismetMathLibrary.FindLookAtRotation` (`SceneComponent.K2_GetComponentLocation` (`self.ViewCamera`)) (`self.CurrentViewTargetPosition`)) false false)))

(fn `SetViewTargetAsRelativeRotation`
  (params (TargetRelativeRot :type "Rotator Structure") (bSnapToRotation :type Boolean))
  (set `self.CurrentViewTargetRelativeRotation` TargetRelativeRot)
  (set `self.CurrentViewTargetType` "NewEnumerator3")
  (if bSnapToRotation
    (`SceneComponent.K2_SetRelativeRotation` (`self.ViewCamera`) (`self.CurrentViewTargetRelativeRotation`) false false)))

(fn `SetViewTargetAveragePlayerCursors`
  (params (MaxYaw :type "Float (double-precision)") (MaxPitch :type "Float (double-precision)"))
  (set `self.ViewTargetCursorMaxYaw` MaxYaw)
  (set `self.ViewTargetCursorMaxPitch` MaxPitch)
  (set `self.CurrentViewTargetType` "NewEnumerator5"))

(fn `SetViewTargetPlayer1Cursor`
  (params (MaxYaw :type "Float (double-precision)") (MaxPitch :type "Float (double-precision)"))
  (set `self.ViewTargetCursorMaxYaw` MaxYaw)
  (set `self.ViewTargetCursorMaxPitch` MaxPitch)
  (set `self.CurrentViewTargetType` "NewEnumerator4"))

(fn `UserConstructionScript`
  (`BlueprintMapLibrary.Map_Add` (`/Game/EpicTemplates/RailShooterTemplate/Blueprints/Components/BP_AmmoComponent.StartAmmo` (`self.AmmoComponent`)) "NewEnumerator0" (`self.BasicStartAmmo`))
  (`BlueprintMapLibrary.Map_Add` (`/Game/EpicTemplates/RailShooterTemplate/Blueprints/Components/BP_AmmoComponent.StartMaxAmmo` (`self.AmmoComponent`)) "NewEnumerator0" (`self.BasicStartAmmo`))
  (`/Game/EpicTemplates/TemplateAgnostic/Blueprints/Components/BP_WeaponWielderComponent.AssignAttachComponent` (`self.WeaponComponent`) (`self.WeaponPivot`) "None"))