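; Game mode for the rail shooter template that places players on rails and holds shared per-player state.
; FindPlayerStart caches all player starts and picks one whose enum-derived tag is generic or matches the controller ID, else defers to the parent.
; InitStartSpot has rail shooter starts attach the player to their spline.
; It also lazily spawns the path choice manager and stores cursor widgets and interfaces by player index.
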(event `self.InitStartSpot`
  (params (StartSpot :type "Actor Object Reference") (NewPlayer :type "Controller Object Reference"))
  (bind _asbp_player_start_rail_shooter (cast `/Game/EpicTemplates/RailShooterTemplate/Blueprints/Core/BP_PlayerStart_RailShooter` StartSpot)
    (:`then`
      (`/Game/EpicTemplates/RailShooterTemplate/Blueprints/Core/BP_PlayerStart_RailShooter.AttachPlayerToSpline` _asbp_player_start_rail_shooter NewPlayer))
    (:`CastFailed`
      (`KismetSystemLibrary.PrintString` "BP_GameMode_RailShooter::InitStartSpot - Start spot for player is not a BP_PlayerStart_RailShooter, Rail will not be automatically applied"))))

(fn `AssignShooterCursor`
  (params (PlayerIndex :type Integer) (CursorWidget :type "Widget Object Reference") (ShooterCursorInterface :type "/Game/EpicTemplates/RailShooterTemplate/Blueprints/Interfaces/BPI_ShooterCursor Interface"))
  (`KismetArrayLibrary.Array_Set` (`self.PlayerCursorWidgets`) PlayerIndex CursorWidget true)
  (`KismetArrayLibrary.Array_Set` (`self.PlayerShooterCursorInterfaces`) PlayerIndex ShooterCursorInterface true))

(fn `FindPlayerStart`
  (params (Player :type "Controller Object Reference") (IncomingName :type String))
  (returns (ReturnValue :type "Actor Object Reference"))
  (locals (PlayerCont :type "PlayerController Object Reference"))
  (`|ExecutionSequence`
    (:`then_0`
      (if (`KismetArrayLibrary.Array_IsEmpty` (`self.PlayerStarts`))
        (bind _outactors (`GameplayStatics.GetAllActorsOfClass` "/Script/Engine.PlayerStart"))
        (set `self.PlayerStarts` _outactors)))
    (:`then_1`
      (bind _asplayer_controller (cast `PlayerController` (`local.Player`)))
      (set `local.PlayerCont` _asplayer_controller)
      (for _array_element (`self.PlayerStarts`)
        (if (`self.IsPlayerStartSuitableForPlayerController` _array_element (`local.PlayerCont`))
          (return _array_element))))
    (:`then_2`
      (bind _returnvalue (`parent.FindPlayerStart` Player IncomingName))
      (return _returnvalue))))

(fn `GetPathChoiceManager`
  (returns (PathChoiceManager :type "/Game/EpicTemplates/RailShooterTemplate/Blueprints/BP_PathChoiceManager Object Reference"))
  (`/Engine/EditorBlueprintResources/StandardMacros.IsValid` (`self.PathChoiceManager`)
    (:`Is Valid`
      _)
    (:`Is Not Valid`
      (bind _returnvalue (`|SpawnActorFromClass` "/Game/EpicTemplates/RailShooterTemplate/Blueprints/BP_PathChoiceManager.BP_PathChoiceManager_C" (`KismetMathLibrary.MakeTransform` (0.0 0.0 0.0)) "AlwaysSpawn" "MultiplyWithRoot" null null))
      (set `self.PathChoiceManager` _returnvalue)))
  (return (`self.PathChoiceManager`)))

(fn `GetShooterCursor`
  (params (PlayerIndex :type Integer))
  (returns (CursorWidget :type "Widget Object Reference") (ShooterCursorInterface :type "/Game/EpicTemplates/RailShooterTemplate/Blueprints/Interfaces/BPI_ShooterCursor Interface"))
  (return (`|GetArrayItem` (`self.PlayerCursorWidgets`) PlayerIndex) (`|GetArrayItem` (`self.PlayerShooterCursorInterfaces`) PlayerIndex)))

(fn `IsPlayerStartSuitableForPlayerController`
  (params (PlayerStart :type "PlayerStart Object Reference") (PlayerController :type "PlayerController Object Reference"))
  (returns (ReturnValue :type Boolean))
  (bind _playerstarttag (`PlayerStart.PlayerStartTag` PlayerStart))
  (return (or (== _playerstarttag (`KismetStringLibrary.Conv_StringToName` (`|GetEnumeratorNameAsString` (enumliteral `/Game/EpicTemplates/RailShooterTemplate/Blueprints/Enums/EPlayerStartType_Railshooter` "NewEnumerator0")))) (== _playerstarttag (`KismetStringLibrary.Conv_StringToName` (`|GetEnumeratorNameAsString` (enumliteral `/Game/EpicTemplates/RailShooterTemplate/Blueprints/Enums/EPlayerStartType_Railshooter` (select `int` (`GameplayStatics.GetPlayerControllerID` (`local.PlayerController`)) :`0` "NewEnumerator1" :`1` "NewEnumerator5" :!type "/Game/EpicTemplates/RailShooterTemplate/Blueprints/Enums/EPlayerStartType_Railshooter Enum"))))))))

(fn `UserConstructionScript`)