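; Player controller for the Rail Shooter template that sets up input and links its pawn to the path choice system.
; On BeginPlay it adds the default Enhanced Input mapping context one tick late, so gamepads register properly.
; On possess it registers the pawn's BP_SplineFollowerComponent, if present, with the path choice manager.
; It unregisters that component when the pawn is unpossessed or destroyed.
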(event `self.ReceiveBeginPlay`
  (`parent.ReceiveBeginPlay`)
  (`KismetSystemLibrary.DelayUntilNextTick`) ; Need to delay mapping context by a frame or gamepads don't register properly
  (message `EnhancedInputSubsystemInterface.AddMappingContext` (subsystem `EnhancedInputLocalPlayerSubsystem`) (`self.DefaultIMC`) 0 (make `ModifyContextOptions` true)))

(event `self.ReceivePossess`
  (params (PossessedPawn :type "Pawn Object Reference"))
  (`parent.ReceivePossess` PossessedPawn)
  (`self.RegisterSplineFollowerComponent` PossessedPawn))

(event `self.ReceiveUnPossess`
  (params (UnpossessedPawn :type "Pawn Object Reference"))
  (`parent.ReceiveUnPossess` UnpossessedPawn)
  (`self.UnregisterSplineFollowerComponent` UnpossessedPawn))

(event `self.PossessedPawnDestroyed`
  (params (DestroyedActor :type "Actor Object Reference"))
  (`self.UnregisterSplineFollowerComponent` DestroyedActor))

(fn `RegisterSplineFollowerComponent`
  (params (PossessedPawn :type "Actor Object Reference"))
  (locals (SplineFollowerComp :type "/Game/EpicTemplates/RailShooterTemplate/Blueprints/Components/BP_SplineFollowerComponent Object Reference"))
  (bind _output_get (set `local.SplineFollowerComp` (`self.GetComponentByClass` PossessedPawn "/Game/EpicTemplates/RailShooterTemplate/Blueprints/Components/BP_SplineFollowerComponent.BP_SplineFollowerComponent_C")))
  (`/Engine/EditorBlueprintResources/StandardMacros.IsValid` _output_get
    (:`Is Valid`
      (bind _pathchoicemanager (`/Game/EpicTemplates/RailShooterTemplate/Blueprints/RailShooterFunctionLibrary.GetPathChoiceManager`))
      (`/Game/EpicTemplates/RailShooterTemplate/Blueprints/BP_PathChoiceManager.RegisterPlayerSplineFollowingComponent` _pathchoicemanager self (`local.SplineFollowerComp`)))))

(fn `UnregisterSplineFollowerComponent`
  (params (PossessedPawn :type "Actor Object Reference"))
  (locals (SplineFollowerComp :type "/Game/EpicTemplates/RailShooterTemplate/Blueprints/Components/BP_SplineFollowerComponent Object Reference"))
  (bind _output_get (set `local.SplineFollowerComp` (`self.GetComponentByClass` PossessedPawn "/Game/EpicTemplates/RailShooterTemplate/Blueprints/Components/BP_SplineFollowerComponent.BP_SplineFollowerComponent_C")))
  (`/Engine/EditorBlueprintResources/StandardMacros.IsValid` _output_get
    (:`Is Valid`
      (bind _pathchoicemanager (`/Game/EpicTemplates/RailShooterTemplate/Blueprints/RailShooterFunctionLibrary.GetPathChoiceManager`))
      (`/Game/EpicTemplates/RailShooterTemplate/Blueprints/BP_PathChoiceManager.UnregisterPlayerSplineFollowingComponent` _pathchoicemanager self (`local.SplineFollowerComp`)))))

(fn `UserConstructionScript`)