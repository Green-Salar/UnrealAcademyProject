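; Player start for the rail shooter template that puts a player's pawn onto an initial spline rail.
; The construction script validates the chosen spline actor, clearing it with a warning if it has no splines, and derives PlayerStartTag from the PlayerValidity enum.
; AttachPlayerToSpline finds the pawn's spline follower component, attaches it to the spline indexed by player controller ID, and sets its move target.
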(fn `AttachPlayerToSpline`
  (params (Player :type "Controller Object Reference"))
  (locals (ControllerPawn :type "Pawn Object Reference") (SplineFollowerComp :type "/Game/EpicTemplates/RailShooterTemplate/Blueprints/Components/BP_SplineFollowerComponent Object Reference") (PlayerControllerID :type Integer) (ActorSplines :type "Array of SplineComponent Object Reference"))
  (bind _output_get (set `local.ControllerPawn` (`Controller.K2_GetPawn` Player)))
  (`/Engine/EditorBlueprintResources/StandardMacros.IsValid` _output_get
    (:`Is Valid`
      (bind _output_get_2 (set `local.SplineFollowerComp` (`self.GetComponentByClass` _output_get "/Game/EpicTemplates/RailShooterTemplate/Blueprints/Components/BP_SplineFollowerComponent.BP_SplineFollowerComponent_C")))
      (`/Engine/EditorBlueprintResources/StandardMacros.IsValid` _output_get_2
        (:`Is Valid`
          (`|ExecutionSequence`
            (:`then_0`
              (bind _asplayer_controller (cast `PlayerController` (`local.Player`))
                (:`then`
                  (set `local.PlayerControllerID` (`GameplayStatics.GetPlayerControllerID` _asplayer_controller)))
                (:`CastFailed`
                  (set `local.PlayerControllerID` 0))))
            (:`then_1`
              (bind _splines (`/Game/EpicTemplates/TemplateAgnostic/Blueprints/EpicTemplatesFunctionLibrary.Get Splines From Actor` (`|ConvertAsset` (`self.InitialSplineActor`))))
              (bind _output_get_3 (set `local.ActorSplines` _splines))
              (if (> (`KismetArrayLibrary.Array_Length` _output_get_3) 0)
                (`/Game/EpicTemplates/RailShooterTemplate/Blueprints/Components/BP_SplineFollowerComponent.AttachToActorSpline` (`local.SplineFollowerComp`) (`|GetArrayItem` (`local.ActorSplines`) (`local.PlayerControllerID`)) (`self.IntialSplineAttachLogic`))
                (`/Game/EpicTemplates/RailShooterTemplate/Blueprints/Components/BP_SplineFollowerComponent.SetMoveTarget` (`local.SplineFollowerComp`) (`self.Spline Target`))
                (else
                  (`KismetSystemLibrary.PrintString` (`KismetStringLibrary.Concat_StrStr` "BP_PlayerStart_RailShooter::AttachPlayerToSpline - Couldn't attach to spline as actor '" (`KismetSystemLibrary.GetDisplayName` (`|ConvertAsset` (`self.InitialSplineActor`))) "' does not return any spline components")))))))))))

(fn `UserConstructionScript`
  (bind _output (`|ConvertAsset` (`self.InitialSplineActor`)))
  (`|ExecutionSequence`
    (:`then_0`
      (`/Engine/EditorBlueprintResources/StandardMacros.IsValid` _output
        (:`Is Valid`
          (bind (_splines _bfoundsplines) (`/Game/EpicTemplates/TemplateAgnostic/Blueprints/EpicTemplatesFunctionLibrary.Get Splines From Actor` _output))
          (if (not _bfoundsplines)
            (`KismetSystemLibrary.PrintString` (`KismetStringLibrary.Concat_StrStr` "SplineActor '" (`KismetSystemLibrary.GetDisplayName` _output) "' doesn't implement spline interface or have any spline components") true true (struct :`R` 1.0 :`G` 0.275073 :`A` 1.0) 10.0)
            (set `self.InitialSplineActor` null)))))
    (:`then_1`
      (set `self.PlayerStartTag` (`KismetStringLibrary.Conv_StringToName` (`|GetEnumeratorNameAsString` (`self.PlayerValidity`)))))))