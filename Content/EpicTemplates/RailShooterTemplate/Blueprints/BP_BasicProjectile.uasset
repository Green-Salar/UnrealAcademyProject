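; Basic pooled projectile for the rail shooter that flies straight, damages what it overlaps, then disables itself.
; LaunchinDirection sets heading and speed, and AssignActorTarget restricts hits to one actor, with an async-loaded material when that target is player two.
; Overlaps skip owner and instigator, optionally check teams, and send damage through BPI_Damageable.
; Impact or death hides it and marks ReusableActorComponent ready for reuse, whose reset restores collision, visibility, movement and health.
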(event `self.ReceiveBeginPlay`
  ;[1 1 1] Begin Play
  (`ProjectileMovementComponent.SetVelocityInLocalSpace` (`self.ProjectileMovement`) (`KismetMathLibrary.MakeVector` (`self.ProjectileSpeed`))))

(event `self.HealthComponent.OnDied`
  (params (Caller :type "/Game/EpicTemplates/TemplateAgnostic/Blueprints/Components/BP_HealthComponent Object Reference") (KillingDamageSourceOwner :type "Actor Object Reference") (KillingDamageSource :type "Actor Object Reference") (KillingDamageLocation :type "Vector Structure") (KillingDamageDirection :type "Vector Structure") (HitBone :type Name) (SpecialDamageName :type Name))
  ;[1 1 1] Health Component
  (`self.DisableProjectile`))

(event `self.CollisionSphere.OnComponentBeginOverlap`
  (params (OverlappedComponent :type "PrimitiveComponent Object Reference") (OtherActor :type "Actor Object Reference") (OtherComp :type "PrimitiveComponent Object Reference") (OtherBodyIndex :type Integer) (bFromSweep :type Boolean) (SweepResult :type "HitResult Structure (by ref)"))
  ;[1 1 1] Overlap collision
  (`self.OverlapActor` OtherActor))

(event `self.ReusableActorComponent.OnRequestDestroySelf`
  ;[1 1 1] Reusable Actor Component
  (`self.K2_DestroyActor`))

(event `self.ReusableActorComponent.OnResetRequested`
  (params (Caller :type "/Game/EpicTemplates/TemplateAgnostic/Blueprints/Components/BP_ReusableActorComponent Object Reference") (ResetActor :type "Actor Object Reference"))
  ;[1 1 1] Reusable Actor Component
  (`PrimitiveComponent.SetCollisionEnabled` (`self.CollisionSphere`) "QueryOnly")
  (`self.SetActorHiddenInGame` false)
  (`ActorComponent.Activate` (`self.ProjectileMovement`) true)
  (`/Game/EpicTemplates/TemplateAgnostic/Blueprints/Interfaces/BPI_HealthSource.UpdateHealth` (`self.HealthComponent`) 1.0))

(event `/Game/EpicTemplates/TemplateAgnostic/Blueprints/Interfaces/BPI_Projectile.LaunchInDirection`
  (params (ProjectileOwner :type "Actor Object Reference") (Direction :type "Vector Structure") (Speed :type "Float (double-precision)"))
  ;[1 1 1] Projectile Interface
  (`self.K2_SetActorRotation` (`KismetMathLibrary.Conv_VectorToRotator` Direction))
  (bind _output_get (set `self.CurrentProjectileSpeed` (select `bool` (<= Speed 0.0) :`false` Speed :`true` (`self.DefaultLaunchSpeed`))))
  (`ProjectileMovementComponent.SetVelocityInLocalSpace` (`self.ProjectileMovement`) (`KismetMathLibrary.MakeVector` _output_get)))

(event `/Game/EpicTemplates/TemplateAgnostic/Blueprints/Interfaces/BPI_Projectile.AssignActorTarget`
  (params (Actor :type "Actor Object Reference"))
  ;[1 1 1] Projectile Interface
  (bind _output_get (set `self.SpecificTarget` Actor))
  (bind _aspawn (cast `Pawn` _output_get))
  (bind _returnvalue (`Pawn.GetController` _aspawn))
  (`/Engine/EditorBlueprintResources/StandardMacros.IsValid` _returnvalue
    (:`Is Valid`
      (if (== _returnvalue (`GameplayStatics.GetPlayerController` 1))
        (bind _object (`|LoadAsset` (`self.Player2TargetMaterial`))
          (:`Completed`
            (bind _asmaterial_interface (cast `MaterialInterface` _object))
            (`PrimitiveComponent.SetMaterial` (`self.Mesh`) 0 _asmaterial_interface)))
        (else
          (`PrimitiveComponent.SetMaterial` (`self.Mesh`) 0 (`self.DefaultMaterial`)))))))

(fn `DisableProjectile`
  (`PrimitiveComponent.SetCollisionEnabled` (`self.CollisionSphere`) "NoCollision")
  (`self.SetActorHiddenInGame` true)
  (`ActorComponent.Deactivate` (`self.ProjectileMovement`))
  (`/Game/EpicTemplates/TemplateAgnostic/Blueprints/Components/BP_ReusableActorComponent.MarkReadyForReuse` (`self.ReusableActorComponent`)))

(fn `OverlapActor`
  (params (OtherActor :type "Actor Object Reference"))
  (if (and (!= (`local.OtherActor`) (`self.GetOwner`)) (!= (`local.OtherActor`) (`self.GetInstigator`)) (or (not (`KismetSystemLibrary.IsValid` (`self.SpecificTarget`))) (== (`local.OtherActor`) (`self.SpecificTarget`))))
    (`|ExecutionSequence`
      (:`then_0`
        (if (`self.bOnlyHitObjectsOfOtherTeams`)
          (bind (_interfaceimplementingobject _foundimplementingobject) (`/Game/EpicTemplates/TemplateAgnostic/Blueprints/EpicTemplatesFunctionLibrary.SearchActorForInterface` (`local.OtherActor`) "/Game/EpicTemplates/TemplateAgnostic/Blueprints/Interfaces/BPI_TeamParticipant.BPI_TeamParticipant_C"))
          (if _foundimplementingobject
            (bind _team (message `/Game/EpicTemplates/TemplateAgnostic/Blueprints/Interfaces/BPI_TeamParticipant.GetTeam` _interfaceimplementingobject))
            (bind _team_2 (message `/Game/EpicTemplates/TemplateAgnostic/Blueprints/Interfaces/BPI_TeamParticipant.GetTeam` (`self.TeamComponent`)))
            (if (`|EnumEquality` _team_2 _team)
              (return)))))
      (:`then_1`
        (`|ExecutionSequence`
          (:`then_0`
            (bind (_interfaceimplementingobject_2 _foundimplementingobject_2) (`/Game/EpicTemplates/TemplateAgnostic/Blueprints/EpicTemplatesFunctionLibrary.SearchActorForInterface` (`local.OtherActor`) "/Game/EpicTemplates/TemplateAgnostic/Blueprints/Interfaces/BPI_Damageable.BPI_Damageable_C"))
            (if _foundimplementingobject_2
              (message `/Game/EpicTemplates/TemplateAgnostic/Blueprints/Interfaces/BPI_Damageable.ApplyDamage` _interfaceimplementingobject_2 (make `/Game/EpicTemplates/TemplateAgnostic/Blueprints/Structs/DamageStruct` (`self.Damage`) self (`self.GetInstigator`) (`self.K2_GetActorLocation`) (`self.GetActorForwardVector`)))))
          (:`then_1`
            (`self.DisableProjectile`)))))))

(fn `UserConstructionScript`
  (set `self.DefaultMaterial` (`PrimitiveComponent.GetMaterial` (`self.Mesh`) 0)))