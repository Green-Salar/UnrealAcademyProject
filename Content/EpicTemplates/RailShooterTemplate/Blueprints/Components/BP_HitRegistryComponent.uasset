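; Actor component for the rail shooter template that records shot hits and tallies valid and invalid ones.
; The HitRegistered event feeds RegisterHit, which counts each hit and logs valid ones with the hit actor's class, hitting player and location.
; Locations are stored relative to the hit actor, falling back to world space without one.
; Getters expose the registry, total hits and valid-hit ratio.
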(event `/Game/EpicTemplates/RailShooterTemplate/Blueprints/Interfaces/BPI_HitRegistry.HitRegistered`
  (params (HitActor :type "Actor Object Reference") (HittingPlayer :type "PlayerController Object Reference") (HitWorldLocation :type "Vector Structure (by ref)") (bValidHit :type Boolean))
  (`self.RegisterHit` HitActor HittingPlayer HitWorldLocation bValidHit))

(fn `GetFullValidRegistry`
  (returns (RegisteredHits :type "Array of /Game/EpicTemplates/RailShooterTemplate/Blueprints/Structs/HitRegistryStruct Structure"))
  (return (`self.RegisteredHits`)))

(fn `GetTotalHits`
  (returns (TotalHits :type Integer))
  (return (+ (`self.ValidHits`) (`self.InvalidHits`))))

(fn `GetValidHitPercentage`
  (returns (ValidHitPercent :type "Float (double-precision)"))
  (if (<= (+ (`self.ValidHits`) (`self.InvalidHits`)) 0)
    (return 0.0)
    (else
      (return (/ (`KismetMathLibrary.Conv_IntToDouble` (`self.ValidHits`)) (`KismetMathLibrary.Conv_IntToDouble` (+ (`self.InvalidHits`) (`self.ValidHits`))))))))

(fn `RegisterHit`
  (params (HitActor :type "Actor Object Reference") (HittingPlayer :type "PlayerController Object Reference") (HitWorldLocation :type "Vector Structure") (ValidHit :type Boolean))
  (locals (HitActorClass :type "Actor Class Reference"))
  (bind _hitactor (`local.HitActor`))
  (bind _hitactor_2 (`local.HitActor`))
  (if ValidHit
    (`/Engine/EditorBlueprintResources/StandardMacros.IncrementInt` (`self.ValidHits`)
      (:`  `
        (`|ExecutionSequence`
          (:`then_0`
            (`/Engine/EditorBlueprintResources/StandardMacros.IsValid` _hitactor
              (:`Is Valid`
                (set `local.HitActorClass` (`GameplayStatics.GetObjectClass` _hitactor)))
              (:`Is Not Valid`
                (set `local.HitActorClass` null))))
          (:`then_1`
            (`KismetArrayLibrary.Array_Add` (`self.RegisteredHits`) (make `/Game/EpicTemplates/RailShooterTemplate/Blueprints/Structs/HitRegistryStruct` (`local.HitActorClass`) (select `bool` (`KismetSystemLibrary.IsValid` _hitactor_2) :`false` HitWorldLocation :`true` (`KismetMathLibrary.InverseTransformLocation` (`Actor.GetTransform` _hitactor_2) HitWorldLocation)) (`local.HittingPlayer`)))))))
    (else
      (`/Engine/EditorBlueprintResources/StandardMacros.IncrementInt` (`self.InvalidHits`)))))