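; BP_Hatch is a breakable hatch for the rail shooter template that can also damage what it touches.
; When its health component reports damage, it spawns a BP_DestructableHatch in its place, passing on velocity and hit location, then fires OnHatchDestroyed and destroys itself.
; While ApplyDamage is set, overlaps on DamageCollision send damage through BPI_Damageable.
; The construction script caches the mesh's default material.
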(event `self.BP_HealthComponent.OnTookDamage`
  (params (Caller :type "/Game/EpicTemplates/TemplateAgnostic/Blueprints/Components/BP_HealthComponent Object Reference") (OldHealth :type "Float (double-precision)") (NewHealth :type "Float (double-precision)") (SpecialDamageName :type Name) (DamageStruct :type "/Game/EpicTemplates/TemplateAgnostic/Blueprints/Structs/DamageStruct Structure (by ref)"))
  (`PrimitiveComponent.SetCollisionEnabled` (`self.Mesh`) "NoCollision")
  (bind _returnvalue (`|SpawnActorFromClass` "/Game/EpicTemplates/RailShooterTemplate/DestructableMeshes/BP_DestructableHatch.BP_DestructableHatch_C" (`self.GetTransform`) "Undefined" "MultiplyWithRoot" null null))
  (`/Game/EpicTemplates/RailShooterTemplate/DestructableMeshes/BP_DestructableHatch.AddImpulse` _returnvalue (`self.GetVelocity`))
  (`/Game/EpicTemplates/RailShooterTemplate/DestructableMeshes/BP_DestructableHatch.ApplyHit` _returnvalue (`.DamageLocation_8_F5A6C21543470034EA0BD6945175CC5B` (break `/Game/EpicTemplates/TemplateAgnostic/Blueprints/Structs/DamageStruct` DamageStruct)))
  (`self.OnHatchDestroyed`)
  (`self.K2_DestroyActor`))

(event `self.DamageCollision.OnComponentBeginOverlap`
  (params (OverlappedComponent :type "PrimitiveComponent Object Reference") (OtherActor :type "Actor Object Reference") (OtherComp :type "PrimitiveComponent Object Reference") (OtherBodyIndex :type Integer) (bFromSweep :type Boolean) (SweepResult :type "HitResult Structure (by ref)"))
  (if (`self.bApplyDamage`)
    (bind (_interfaceimplementingobject _foundimplementingobject) (`/Game/EpicTemplates/TemplateAgnostic/Blueprints/EpicTemplatesFunctionLibrary.SearchActorForInterface` OtherActor "/Game/EpicTemplates/TemplateAgnostic/Blueprints/Interfaces/BPI_Damageable.BPI_Damageable_C"))
    (if _foundimplementingobject
      (message `/Game/EpicTemplates/TemplateAgnostic/Blueprints/Interfaces/BPI_Damageable.ApplyDamage` _interfaceimplementingobject (make `/Game/EpicTemplates/TemplateAgnostic/Blueprints/Structs/DamageStruct` 1.0 self null (`self.K2_GetActorLocation`) (`self.GetActorForwardVector`))))))

(fn `UserConstructionScript`
  (set `self.DefaultMeshMaterial` (`PrimitiveComponent.GetMaterial` (`self.Mesh`) 0)))