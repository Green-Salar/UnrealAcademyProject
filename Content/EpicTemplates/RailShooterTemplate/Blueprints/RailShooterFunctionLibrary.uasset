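; Blueprint function library with shared helpers for the Rail Shooter template.
; The path choice manager and per-player shooter cursor getters cast the game mode to BP_GameMode_RailShooter and forward its results.
; If that cast fails, they print an error saying the game mode should use that class.
; SplineTargetStart and SplineTargetEnd build preset spline target structs for the start and end targets.
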(fn `GetPathChoiceManager`
  (returns (PathChoiceManager :type "/Game/EpicTemplates/RailShooterTemplate/Blueprints/BP_PathChoiceManager Object Reference"))
  (`|ExecutionSequence`
    (:`then_0`
      (bind _asbp_game_mode_rail_shooter (cast `/Game/EpicTemplates/RailShooterTemplate/Blueprints/Core/BP_GameMode_RailShooter` (`GameplayStatics.GetGameMode` null))
        (:`then`
          (return (`/Game/EpicTemplates/RailShooterTemplate/Blueprints/Core/BP_GameMode_RailShooter.GetPathChoiceManager` _asbp_game_mode_rail_shooter)))
        (:`CastFailed`
          (`KismetSystemLibrary.PrintString` null "RailShooterFunctionLibrary::GetPathChoiceManager - Game mode couldn't be cast to BP_GameMode_RailShooter. The game mode should be set to use this class." true true (struct :`R` 1.0 :`G` 0.042531 :`A` 1.0) 10.0))))
    (:`then_1`
      (return null))))

(fn `GetPlayerShooterCursor`
  (params (PlayerIndex :type Integer))
  (returns (CursorWidget :type "Widget Object Reference") (ShooterCursorInterface :type "/Game/EpicTemplates/RailShooterTemplate/Blueprints/Interfaces/BPI_ShooterCursor Interface"))
  (bind _asbp_game_mode_rail_shooter (cast `/Game/EpicTemplates/RailShooterTemplate/Blueprints/Core/BP_GameMode_RailShooter` (`GameplayStatics.GetGameMode` null))
    (:`then`
      (bind (_cursorwidget _shootercursorinterface) (`/Game/EpicTemplates/RailShooterTemplate/Blueprints/Core/BP_GameMode_RailShooter.GetShooterCursor` _asbp_game_mode_rail_shooter PlayerIndex))
      (return _cursorwidget _shootercursorinterface))
    (:`CastFailed`
      (`KismetSystemLibrary.PrintString` null "RailShooterFunctionLibrary::GetPlayerShooterCursor - Game mode couldn't be cast to BP_GameMode_RailShooter. The game mode should be set to use this class." true true (struct :`R` 1.0 :`G` 0.042531 :`A` 1.0) 10.0))))

(fn `SplineTargetEnd`
  (returns (NewParam :type "/Game/EpicTemplates/RailShooterTemplate/Blueprints/Structs/SplineTargetStruct Structure"))
  (return (make `/Game/EpicTemplates/RailShooterTemplate/Blueprints/Structs/SplineTargetStruct` "NewEnumerator2" -1.0)))

(fn `SplineTargetStart`
  (returns (NewParam :type "/Game/EpicTemplates/RailShooterTemplate/Blueprints/Structs/SplineTargetStruct Structure"))
  (return (make `/Game/EpicTemplates/RailShooterTemplate/Blueprints/Structs/SplineTargetStruct` "NewEnumerator4" -1.0)))