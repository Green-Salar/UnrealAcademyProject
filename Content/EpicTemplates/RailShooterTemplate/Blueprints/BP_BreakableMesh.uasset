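; BP_BreakableMesh is a rail shooter prop that swaps its mesh for a destructible actor when damaged.
; BP_HealthComponent's OnTookDamage hides the Cube, disables its collision and async-loads the DestructableActor class.
; Once loaded, it spawns that actor at the Cube's location and rotation with unit scale.
; A Field System falloff force then blasts it apart, and the original actor destroys itself.
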(event `self.BP_HealthComponent.OnTookDamage`
  (params (Caller :type "/Game/EpicTemplates/TemplateAgnostic/Blueprints/Components/BP_HealthComponent Object Reference") (OldHealth :type "Float (double-precision)") (NewHealth :type "Float (double-precision)") (SpecialDamageName :type Name) (DamageStruct :type "/Game/EpicTemplates/TemplateAgnostic/Blueprints/Structs/DamageStruct Structure (by ref)"))
  (bind _cube (`self.Cube`))
  (bind (_returnvalue_location _returnvalue_rotation) (`KismetMathLibrary.BreakTransform` (`SceneComponent.K2_GetComponentToWorld` (`self.Cube`))))
  (`PrimitiveComponent.SetCollisionEnabled` _cube "NoCollision")
  (`SceneComponent.SetVisibility` _cube false false)
  (bind _class (`|LoadAssetClass` (`self.DestructableActor`))
    (:`Completed`
      (`|ExecutionSequence`
        (:`then_0`
          (bind _asactor (castclass `Actor` _class))
          (`|SpawnActorFromClass` _asactor (`KismetMathLibrary.MakeTransform` _returnvalue_location _returnvalue_rotation) "AlwaysSpawn" "MultiplyWithRoot" null null)
          (`FieldSystemComponent.ApplyUniformVectorFalloffForce` (`self.FieldSystem`) true (0.0 0.0 0.0) (0.0 0.0 0.0) 100.0 999999.0))
        (:`then_1`
          (`self.K2_DestroyActor`))))))

(fn `UserConstructionScript`)