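; Rail shooter manager that decides which spline paths players follow, for one player or all.
; It maps players to registered spline follow components and filters requests by acceptance rule and type.
; Accepted requests either attach followers immediately, picking splines by controller ID, or queue while players move.
; Movement-finished events run queued requests; individual requests are rejected when splitscreen is force-disabled.
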(event `SplineMovementComponentFinished`
  (params (Caller :type "/Game/EpicTemplates/RailShooterTemplate/Blueprints/Components/BP_SplineFollowerComponent Object Reference") (FollowingActor :type "Actor Object Reference") (FollowedSpline :type "SplineComponent Object Reference") (ReachedDistance :type "Float (double-precision)") (ReachedKey :type "Float (double-precision)"))
  (remove `/Game/EpicTemplates/RailShooterTemplate/Blueprints/Components/BP_SplineFollowerComponent.OnSplineMovementCompletelyFinished` Caller (delegate `SplineMovementComponentFinished`))
  (`self.CheckPendingRequestsForExecute` Caller)
  (`self.Remove Follow Component From Pending Requests` Caller))

(fn `AreAnyPlayersMoving`
  (returns (ReturnValue :type Boolean))
  (bind _values (`BlueprintMapLibrary.Map_Values` (`self.PlayerToSplineFollowComps`)))
  (for _array_element _values
    (if (`/Game/EpicTemplates/RailShooterTemplate/Blueprints/Components/BP_SplineFollowerComponent.IsMovingAlongSpline` _array_element)
      (return true)))
  (return false))

(fn `CanPlayerMakePathChoice`
  (params (Player :type "PlayerController Object Reference"))
  (returns (CanMakeChoice :type Boolean))
  (if (`|EnumEquality` (`self.CurrentPathChooserRule`) "NewEnumerator1")
    (return (== (`GameplayStatics.GetPlayerControllerID` Player) 0))
    (else
      (return true))))

(fn `CheckActorSuitableForPath`
  (params (PathActor :type "Actor Object Reference"))
  (returns (SuitableForPaths :type Boolean))
  (bind _returnvalue (`KismetSystemLibrary.DoesImplementInterface` PathActor "/Game/EpicTemplates/RailShooterTemplate/Blueprints/Interfaces/BPI_SplinePathImplementor.BPI_SplinePathImplementor_C"))
  (if _returnvalue
    (return _returnvalue)
    (elif (`KismetSystemLibrary.IsValid` (`self.GetComponentByClass` PathActor "/Script/Engine.SplineComponent"))
      (return true)
      (else
        (`KismetSystemLibrary.PrintString` (`KismetStringLibrary.Concat_StrStr` "BP_PathChoiceManager::TryRequestNewPath - PathActor '" (`KismetSystemLibrary.GetDisplayName` (`local.PathActor`)) "' Neither implements the BPi_PathImplementer interface, nor has spline components") true true (struct :`R` 1.0 :`G` 0.222252 :`A` 1.0) 10.0)
        (return false)))))

(fn `CheckPendingRequestsForExecute`
  (params (SplineFollowerToCheck :type "/Game/EpicTemplates/RailShooterTemplate/Blueprints/Components/BP_SplineFollowerComponent Object Reference (by ref)"))
  (locals (TempRequest :type "/Game/EpicTemplates/RailShooterTemplate/Blueprints/Structs/PendingSplineRequest Structure") (TempRequestIdx :type Integer))
  (for (_array_element _array_index) (`self.PendingSpineRequests`)
    (set `local.TempRequest` _array_element)
    (set `local.TempRequestIdx` _array_index)
    (if (> (`KismetArrayLibrary.Array_Find` (`.SplineComponentsToFollow_7_A78AE980471BCC67243A0EB62119F640` (break `/Game/EpicTemplates/RailShooterTemplate/Blueprints/Structs/PendingSplineRequest` (`local.TempRequest`))) SplineFollowerToCheck) -1)
      (for _array_element_2 (`.SplineComponentsToFollow_7_A78AE980471BCC67243A0EB62119F640` (break `/Game/EpicTemplates/RailShooterTemplate/Blueprints/Structs/PendingSplineRequest` (`local.TempRequest`)))
        (if (`/Game/EpicTemplates/RailShooterTemplate/Blueprints/Components/BP_SplineFollowerComponent.IsMovingAlongSpline` _array_element_2)
          (return)))
      (`KismetArrayLibrary.Array_Remove` (`self.PendingSpineRequests`) (`local.TempRequestIdx`))
      (`self.ExecutePendingSplineRequest` (`local.TempRequest`))
      (return)))
  (return))

(fn `CreateNewPendingRequest`
  (params (Requestee :type "PlayerController Object Reference") (RequestedPathActor :type "Actor Object Reference") (PathSplitType :type "/Game/EpicTemplates/RailShooterTemplate/Blueprints/Enums/EPathSplitType Enum" :default "NewEnumerator0") (AttachToSplineType :type "/Game/EpicTemplates/RailShooterTemplate/Blueprints/Enums/EAttachToSplineType Enum" :default "NewEnumerator0") (SplineTarget :type "/Game/EpicTemplates/RailShooterTemplate/Blueprints/Structs/SplineTargetStruct Structure (by ref)"))
  (locals (TempSplineFollowComp :type "/Game/EpicTemplates/RailShooterTemplate/Blueprints/Components/BP_SplineFollowerComponent Object Reference") (NewRequest :type "/Game/EpicTemplates/RailShooterTemplate/Blueprints/Structs/PendingSplineRequest Structure"))
  (if (`|EnumEquality` PathSplitType "NewEnumerator1")
    (set `local.TempSplineFollowComp` (`BlueprintMapLibrary.Map_Find` (`self.PlayerToSplineFollowComps`) (`local.Requestee`)))
    (bind _output_get (set `local.NewRequest` (make `/Game/EpicTemplates/RailShooterTemplate/Blueprints/Structs/PendingSplineRequest` (`local.RequestedPathActor`) (`|MakeArray` (`local.TempSplineFollowComp`)) (`local.AttachToSplineType`) (`local.SplineTarget`))))
    (`KismetArrayLibrary.Array_Add` (`self.PendingSpineRequests`) _output_get)
    (add `/Game/EpicTemplates/RailShooterTemplate/Blueprints/Components/BP_SplineFollowerComponent.OnSplineMovementCompletelyFinished` (`local.TempSplineFollowComp`) (`|CreateDelegate` :!event `SplineMovementComponentFinished`))
    (else
      (set `local.NewRequest` (make `/Game/EpicTemplates/RailShooterTemplate/Blueprints/Structs/PendingSplineRequest` :`PathActor` (`local.RequestedPathActor`) :`AttachToSplineType` (`local.AttachToSplineType`) :`SplineTarget` (`local.SplineTarget`)))
      (bind _values (`BlueprintMapLibrary.Map_Values` (`self.PlayerToSplineFollowComps`)))
      (for _array_element _values
        (`KismetArrayLibrary.Array_Add` (`.SplineComponentsToFollow_7_A78AE980471BCC67243A0EB62119F640` (break `/Game/EpicTemplates/RailShooterTemplate/Blueprints/Structs/PendingSplineRequest` (`local.NewRequest`))) _array_element)
        (add `/Game/EpicTemplates/RailShooterTemplate/Blueprints/Components/BP_SplineFollowerComponent.OnSplineMovementCompletelyFinished` _array_element (`|CreateDelegate` :!event `SplineMovementComponentFinished`)))
      (`KismetArrayLibrary.Array_Add` (`self.PendingSpineRequests`) (`local.NewRequest`)))))

(fn `ExecutePendingSplineRequest`
  (params (PendingRequest :type "/Game/EpicTemplates/RailShooterTemplate/Blueprints/Structs/PendingSplineRequest Structure"))
  (locals (Splines :type "Array of SplineComponent Object Reference") (TempSplineFollowComp :type "/Game/EpicTemplates/RailShooterTemplate/Blueprints/Components/BP_SplineFollowerComponent Object Reference"))
  (bind _splines (`local.Splines`))
  (bind ((`AttachToSplineType_11_A0DA925545476E4723BD8D975BEBE337` _attachtosplinetype) (`SplineTarget_20_FF580E234D000F709494DDA0D5C44728` _splinetarget)) (break `/Game/EpicTemplates/RailShooterTemplate/Blueprints/Structs/PendingSplineRequest` (`local.PendingRequest`)))
  (bind (_pathspline1 _pathspline2) (message `/Game/EpicTemplates/RailShooterTemplate/Blueprints/Interfaces/BPI_SplinePathImplementor.GetSplines` (`.PathActor_3_E75443854F639FFB0D9FA1B69A19A659` (break `/Game/EpicTemplates/RailShooterTemplate/Blueprints/Structs/PendingSplineRequest` PendingRequest))))
  (`KismetArrayLibrary.Array_Add` _splines _pathspline1)
  (`KismetArrayLibrary.Array_Add` _splines _pathspline2)
  (for (_array_element _array_index) (`.SplineComponentsToFollow_7_A78AE980471BCC67243A0EB62119F640` (break `/Game/EpicTemplates/RailShooterTemplate/Blueprints/Structs/PendingSplineRequest` (`local.PendingRequest`)))
    (set `local.TempSplineFollowComp` _array_element)
    (`/Game/EpicTemplates/RailShooterTemplate/Blueprints/Components/BP_SplineFollowerComponent.AttachToActorSpline` (`local.TempSplineFollowComp`) (`|GetArrayItem` (`local.Splines`) (select `bool` (`KismetArrayLibrary.Array_IsValidIndex` (`local.Splines`) _array_index) :`true` _array_index)) _attachtosplinetype)
    (`/Game/EpicTemplates/RailShooterTemplate/Blueprints/Components/BP_SplineFollowerComponent.SetMoveTarget` (`local.TempSplineFollowComp`) _splinetarget)))

(fn `NewSplineRequest`
  (params (RequestSource :type "Actor Object Reference") (RequestedPathActor :type "Actor Object Reference") (PlayerForSpline :type "PlayerController Object Reference") (RequestType :type "/Game/EpicTemplates/RailShooterTemplate/Blueprints/Enums/EPathRequestType Enum" :default "NewEnumerator0") (PathSplitType :type "/Game/EpicTemplates/RailShooterTemplate/Blueprints/Enums/EPathSplitType Enum" :default "NewEnumerator0") (AttachToSplineType :type "/Game/EpicTemplates/RailShooterTemplate/Blueprints/Enums/EAttachToSplineType Enum" :default "NewEnumerator0") (SplineTarget :type "/Game/EpicTemplates/RailShooterTemplate/Blueprints/Structs/SplineTargetStruct Structure"))
  (returns (RequestAccepted :type Boolean))
  (locals (RequesteePlayerID :type Integer :default 0) (Splines :type "Array of SplineComponent Object Reference") (TempSplineFollowComp :type "/Game/EpicTemplates/RailShooterTemplate/Blueprints/Components/BP_SplineFollowerComponent Object Reference") (RequesteeFollowComp :type "/Game/EpicTemplates/RailShooterTemplate/Blueprints/Components/BP_SplineFollowerComponent Object Reference"))
  (`|ExecutionSequence`
    (:`then_0`
      (if (or (and (`|EnumEquality` (`self.CurrentRequestAcceptanceRule`) "NewEnumerator1") (`|EnumEquality` (`local.RequestType`) "NewEnumerator1")) (`|EnumEquality` (`self.CurrentRequestAcceptanceRule`) "NewEnumerator2"))
        (return false)))
    (:`then_1`
      (bind (_splines _bfoundsplines) (`/Game/EpicTemplates/TemplateAgnostic/Blueprints/EpicTemplatesFunctionLibrary.Get Splines From Actor` (`local.RequestedPathActor`)))
      (set `local.Splines` _splines)
      (if (not _bfoundsplines)
        (`KismetSystemLibrary.PrintString` (`KismetStringLibrary.Concat_StrStr` "BP_PathChoiceManager::PlayerRequestNewSpline - Spline request ignored, actor '" (`KismetSystemLibrary.GetDisplayName` (`local.RequestedPathActor`)) "' doesn't have splines or implement spline interface") true true (struct :`R` 1.0 :`G` 0.159982 :`A` 1.0) 10.0)
        (return false)))
    (:`then_2`
      (if (or (`|EnumEquality` (`local.RequestType`) "NewEnumerator0") (`|EnumEquality` (`self.CurrentRequestAcceptanceRule`) "NewEnumerator1"))
        (if (or (and (`|EnumEquality` (`local.PathSplitType`) "NewEnumerator1") (`/Game/EpicTemplates/RailShooterTemplate/Blueprints/Components/BP_SplineFollowerComponent.IsMovingAlongSpline` (`BlueprintMapLibrary.Map_Find` (`self.PlayerToSplineFollowComps`) (`local.PlayerForSpline`)))) (and (`|EnumEquality` (`local.PathSplitType`) "NewEnumerator0") (`self.AreAnyPlayersMoving`)))
          (`|ExecutionSequence`
            (:`then_0`
              (`self.CreateNewPendingRequest` (`local.PlayerForSpline`) (`local.RequestedPathActor`) (`local.PathSplitType`) (`local.AttachToSplineType`) (`local.SplineTarget`)))
            (:`then_1`
              (return true))))))
    (:`then_3`
      (bind _output_get (set `local.RequesteeFollowComp` (`BlueprintMapLibrary.Map_Find` (`self.PlayerToSplineFollowComps`) (`local.PlayerForSpline`))))
      (`self.Remove Follow Component From Pending Requests` _output_get)
      (remove `/Game/EpicTemplates/RailShooterTemplate/Blueprints/Components/BP_SplineFollowerComponent.OnSplineMovementCompletelyFinished` (`local.RequesteeFollowComp`) (`|CreateDelegate` :!event `SplineMovementComponentFinished`))
      (`|ExecutionSequence`
        (:`then_0`
          (switch `/Game/EpicTemplates/RailShooterTemplate/Blueprints/Enums/EPathSplitType` (`local.PathSplitType`)
            (:`NewEnumerator0`
              (bind _keys (`BlueprintMapLibrary.Map_Keys` (`self.PlayerToSplineFollowComps`)))
              (for _array_element _keys
                (bind _output_get_2 (set `local.TempSplineFollowComp` (`BlueprintMapLibrary.Map_Find` (`self.PlayerToSplineFollowComps`) _array_element)))
                (`/Game/EpicTemplates/RailShooterTemplate/Blueprints/Components/BP_SplineFollowerComponent.AttachToActorSpline` _output_get_2 (`|GetArrayItem` (`local.Splines`) (`KismetMathLibrary.Min` (`GameplayStatics.GetPlayerControllerID` _array_element) (`KismetArrayLibrary.Array_LastIndex` (`local.Splines`)))) (`local.AttachToSplineType`))
                (`/Game/EpicTemplates/RailShooterTemplate/Blueprints/Components/BP_SplineFollowerComponent.SetMoveTarget` (`local.TempSplineFollowComp`) (`local.SplineTarget`))))
            (:`NewEnumerator1`
              (`/Game/EpicTemplates/RailShooterTemplate/Blueprints/Components/BP_SplineFollowerComponent.AttachToActorSpline` (`local.RequesteeFollowComp`) (`|GetArrayItem` (`local.Splines`) (`KismetMathLibrary.Min` (`GameplayStatics.GetPlayerControllerID` (`local.PlayerForSpline`)) (`KismetArrayLibrary.Array_LastIndex` (`local.Splines`)))) (`local.AttachToSplineType`))
              (`/Game/EpicTemplates/RailShooterTemplate/Blueprints/Components/BP_SplineFollowerComponent.SetMoveTarget` (`local.RequesteeFollowComp`) (`local.SplineTarget`)))))
        (:`then_1`
          (return true))))))

(fn `RegisterPlayerSplineFollowingComponent`
  (params (Player :type "PlayerController Object Reference") (SplineFollowingComp :type "/Game/EpicTemplates/RailShooterTemplate/Blueprints/Components/BP_SplineFollowerComponent Object Reference"))
  (`BlueprintMapLibrary.Map_Add` (`self.PlayerToSplineFollowComps`) Player SplineFollowingComp))

(fn `Remove Follow Component From Pending Requests`
  (params (FollowComp :type "/Game/EpicTemplates/RailShooterTemplate/Blueprints/Components/BP_SplineFollowerComponent Object Reference"))
  (locals (TempRequest :type "/Game/EpicTemplates/RailShooterTemplate/Blueprints/Structs/PendingSplineRequest Structure") (TempRequestIdx :type Integer) (FoundIndex :type Integer :default 0) (PlayerFollowComp :type "/Game/EpicTemplates/RailShooterTemplate/Blueprints/Components/BP_SplineFollowerComponent Object Reference") (PlayerRemoved :type Boolean))
  (bind ((`SplineComponentsToFollow_7_A78AE980471BCC67243A0EB62119F640` _splinecomponentstofollow)) (break `/Game/EpicTemplates/RailShooterTemplate/Blueprints/Structs/PendingSplineRequest` (`local.TempRequest`)))
  (bind (_arrayindex _arrayelement) (`/Engine/EditorBlueprintResources/StandardMacros.ReverseForEachLoop` (`self.PendingSpineRequests`))
    (:`LoopBody`
      (set `local.TempRequest` _arrayelement)
      (set `local.TempRequestIdx` _arrayindex)
      (bind _output_get (set `local.FoundIndex` (`KismetArrayLibrary.Array_Find` (`.SplineComponentsToFollow_7_A78AE980471BCC67243A0EB62119F640` (break `/Game/EpicTemplates/RailShooterTemplate/Blueprints/Structs/PendingSplineRequest` (`local.TempRequest`))) (`local.FollowComp`))))
      (if (> _output_get -1)
        (`KismetArrayLibrary.Array_Remove` _splinecomponentstofollow (`local.FoundIndex`))
        (if (== (`KismetArrayLibrary.Array_Length` _splinecomponentstofollow) 0)
          (`KismetArrayLibrary.Array_Remove` (`self.PendingSpineRequests`) (`local.TempRequestIdx`))
          (else
            (for _array_element (`.SplineComponentsToFollow_7_A78AE980471BCC67243A0EB62119F640` (break `/Game/EpicTemplates/RailShooterTemplate/Blueprints/Structs/PendingSplineRequest` (`local.TempRequest`)))
              (if (`/Game/EpicTemplates/RailShooterTemplate/Blueprints/Components/BP_SplineFollowerComponent.IsMovingAlongSpline` _array_element)
                (break)))
            (`KismetArrayLibrary.Array_Remove` (`self.PendingSpineRequests`) (`local.TempRequestIdx`))
            (`self.ExecutePendingSplineRequest` (`local.TempRequest`))))))))

(fn `RequestNewSplineForAllPlayers`
  (params (RequestSource :type "Actor Object Reference") (RequestedPathActor :type "Actor Object Reference") (RequestType :type "/Game/EpicTemplates/RailShooterTemplate/Blueprints/Enums/EPathRequestType Enum" :default "NewEnumerator0") (AttachToSplineType :type "/Game/EpicTemplates/RailShooterTemplate/Blueprints/Enums/EAttachToSplineType Enum" :default "NewEnumerator0") (SplineTarget :type "/Game/EpicTemplates/RailShooterTemplate/Blueprints/Structs/SplineTargetStruct Structure (by ref)"))
  (returns (RequestAccepted :type Boolean))
  (locals (RequesteePlayerID :type Integer :default 0) (Splines :type "Array of SplineComponent Object Reference") (TempSplineFollowComp :type "/Game/EpicTemplates/RailShooterTemplate/Blueprints/Components/BP_SplineFollowerComponent Object Reference") (RequesteeFollowComp :type "/Game/EpicTemplates/RailShooterTemplate/Blueprints/Components/BP_SplineFollowerComponent Object Reference"))
  (`|ExecutionSequence`
    (:`then_0`
      (if (or (and (`|EnumEquality` (`self.CurrentRequestAcceptanceRule`) "NewEnumerator1") (`|EnumEquality` (`local.RequestType`) "NewEnumerator1")) (`|EnumEquality` (`self.CurrentRequestAcceptanceRule`) "NewEnumerator2"))
        (return false)))
    (:`then_1`
      (bind (_splines _bfoundsplines) (`/Game/EpicTemplates/TemplateAgnostic/Blueprints/EpicTemplatesFunctionLibrary.Get Splines From Actor` (`local.RequestedPathActor`)))
      (set `local.Splines` _splines)
      (if (not _bfoundsplines)
        (`KismetSystemLibrary.PrintString` (`KismetStringLibrary.Concat_StrStr` "BP_PathChoiceManager::RequestNewSplineForAllPlayers - Spline request ignored, actor '" (`KismetSystemLibrary.GetDisplayName` (`local.RequestedPathActor`)) "' doesn't have splines or implement spline interface") true true (struct :`R` 1.0 :`G` 0.159982 :`A` 1.0) 10.0)
        (return false)))
    (:`then_2`
      (if (or (`|EnumEquality` (`local.RequestType`) "NewEnumerator0") (`|EnumEquality` (`self.CurrentRequestAcceptanceRule`) "NewEnumerator1"))
        (if (`self.AreAnyPlayersMoving`)
          (`|ExecutionSequence`
            (:`then_0`
              (`self.CreateNewPendingRequest` null (`local.RequestedPathActor`) "NewEnumerator0" (`local.AttachToSplineType`) (`local.SplineTarget`)))
            (:`then_1`
              (return true))))))
    (:`then_3`
      (`|ExecutionSequence`
        (:`then_0`
          (bind _keys (`BlueprintMapLibrary.Map_Keys` (`self.PlayerToSplineFollowComps`)))
          (for _array_element _keys
            (bind _output_get (set `local.TempSplineFollowComp` (`BlueprintMapLibrary.Map_Find` (`self.PlayerToSplineFollowComps`) _array_element)))
            (`/Game/EpicTemplates/RailShooterTemplate/Blueprints/Components/BP_SplineFollowerComponent.AttachToActorSpline` _output_get (`|GetArrayItem` (`local.Splines`) (`KismetMathLibrary.Min` (`GameplayStatics.GetPlayerControllerID` _array_element) (`KismetArrayLibrary.Array_LastIndex` (`local.Splines`)))) (`local.AttachToSplineType`))
            (`/Game/EpicTemplates/RailShooterTemplate/Blueprints/Components/BP_SplineFollowerComponent.SetMoveTarget` (`local.TempSplineFollowComp`) (`local.SplineTarget`))))
        (:`then_1`
          (return true))))))

(fn `RequestNewSplineForIndividualPlayer`
  (params (RequestSource :type "Actor Object Reference") (RequestedPathActor :type "Actor Object Reference") (Player :type "PlayerController Object Reference") (RequestType :type "/Game/EpicTemplates/RailShooterTemplate/Blueprints/Enums/EPathRequestType Enum" :default "NewEnumerator0") (AttachToSplineType :type "/Game/EpicTemplates/RailShooterTemplate/Blueprints/Enums/EAttachToSplineType Enum" :default "NewEnumerator0") (SplineTarget :type "/Game/EpicTemplates/RailShooterTemplate/Blueprints/Structs/SplineTargetStruct Structure"))
  (returns (RequestAccepted :type Boolean))
  (locals (RequesteePlayerID :type Integer :default 0) (Splines :type "Array of SplineComponent Object Reference") (TempSplineFollowComp :type "/Game/EpicTemplates/RailShooterTemplate/Blueprints/Components/BP_SplineFollowerComponent Object Reference") (RequesteeFollowComp :type "/Game/EpicTemplates/RailShooterTemplate/Blueprints/Components/BP_SplineFollowerComponent Object Reference"))
  (`|ExecutionSequence`
    (:`then_0`
      (if (`GameplayStatics.IsSplitscreenForceDisabled`)
        (`KismetSystemLibrary.PrintString` "BP_PathChoiceManager::RequestNewSplineForIndividualPlayer - Requesting spline path for individual player when split screen is disabled, this shouldn't be done." true true (struct :`R` 1.0 :`G` 0.171533 :`A` 1.0) 10.0)
        (return false)))
    (:`then_1`
      (bind _requestaccepted (`self.NewSplineRequest` RequestSource RequestedPathActor Player RequestType "NewEnumerator1" AttachToSplineType SplineTarget))
      (return _requestaccepted))))

(fn `UnregisterPlayerSplineFollowingComponent`
  (params (Player :type "PlayerController Object Reference") (SplineFollowingComp :type "/Game/EpicTemplates/RailShooterTemplate/Blueprints/Components/BP_SplineFollowerComponent Object Reference"))
  (if (== (`BlueprintMapLibrary.Map_Find` (`self.PlayerToSplineFollowComps`) Player) (`local.SplineFollowingComp`))
    (`BlueprintMapLibrary.Map_Remove` (`self.PlayerToSplineFollowComps`) (`local.Player`))))

(fn `UserConstructionScript`)