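; Rail shooter wave node that spawns enemy waves and tracks when they are all killed.
; On activation it updates pre-placed actors' target logic via interface and spawns configured classes at spawn points, all at once or on randomized timers.
; Registered actors report health-component death, or destruction without one, toward a kill count that fires the all-killed event.
; Single-player mode trims flagged entries, and failed spawns lower the required count.
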(event `Debug_DrawPreSpawnedActors`
  (for _array_element (`self.PreSpawnedActors`)
    (bind _output (`|ConvertAsset` (`.Actor_16_A437BEF648E6F5A746905A8823640695` (break `/Game/EpicTemplates/RailShooterTemplate/Blueprints/Structs/WaveNodePreSpawnedStruct` _array_element))))
    (`/Engine/EditorBlueprintResources/StandardMacros.IsValid` _output
      (:`Is Valid`
        (`KismetSystemLibrary.DrawDebugLine` (`self.K2_GetActorLocation`) (`self.K2_GetActorLocation` _output) (struct :`G` 0.762422 :`B` 1.0 :`A` 1.0) 5.0)))))

(event `self.ReceiveBeginPlay`
  (`self.TrimSpawnsIfSinglePlayer`)
  (`/Game/EpicTemplates/TemplateAgnostic/Blueprints/EpicTemplatesFunctionLibrary.PlusEqualsInt` (`self.RequiredKillCount`) (`KismetArrayLibrary.Array_Length` (`self.PreSpawnedActors`)))
  (`self.RegisterPreSpawnedActors`)
  (if (`self.bActivateOnBeginPlay`)
    (`self.ActivateNode`)))

(event `SpawnNextEntity`
  (if (< (`self.CurrentSpawnedIndex`) (`KismetArrayLibrary.Array_Length` (`self.Spawns`)))
    (bind _bsuccessfullyspawned (`self.SpawnEntityFromSpawnStruct` (`|GetArrayItem` (`self.Spawns`) (`self.CurrentSpawnedIndex`))))
    (`|ExecutionSequence`
      (:`then_0`
        (if (not _bsuccessfullyspawned)
          (`/Engine/EditorBlueprintResources/StandardMacros.DecrementInt` (`self.RequiredKillCount`))))
      (:`then_1`
        (bind _result (`/Engine/EditorBlueprintResources/StandardMacros.IncrementInt` (`self.CurrentSpawnedIndex`))
          (:`  `
            (if (< _result (`KismetArrayLibrary.Array_Length` (`self.Spawns`)))
              (bind _returnvalue (`KismetSystemLibrary.K2_SetTimerDelegate` (`|CreateDelegate` :!event `SpawnNextEntity`) (`KismetMathLibrary.FMax` (+ (`self.BetweenSpawnDelay`) (`KismetMathLibrary.RandomFloatInRange` (* (`self.BetweenSpawnDelayVariance`) -1.0) (`self.BetweenSpawnDelayVariance`))) 0.01)))
              (set `self.NextSpawnHandle` _returnvalue)
              (else
                (set `self.bReactivateLocked` false)
                (`self.OnFinishedSpawning` self)))))))))

(event `ActivateNode`
  (if (and (or (not (`self.bOnlyActivateOnce`)) (not (`self.bNodeActivated`))) (not (`self.bReactivateLocked`)))
    (set `self.bNodeActivated` true)
    (set `self.bReactivateLocked` true)
    (`|ExecutionSequence`
      (:`then_0`
        (for _array_element (`self.PreSpawnedActors`)
          (bind ((`Actor_16_A437BEF648E6F5A746905A8823640695` _actor) (`TargetLogicToApply_18_844522C14395980CCC3ECE90BDC9C6DE` _targetlogictoapply)) (break `/Game/EpicTemplates/RailShooterTemplate/Blueprints/Structs/WaveNodePreSpawnedStruct` _array_element))
          (`self.UpdateSpawnedActorTargetLogic` (`|ConvertAsset` _actor) _targetlogictoapply)))
      (:`then_1`
        (set `self.CurrentSpawnedIndex` 0)
        (`/Game/EpicTemplates/TemplateAgnostic/Blueprints/EpicTemplatesFunctionLibrary.PlusEqualsInt` (`self.RequiredKillCount`) (`KismetArrayLibrary.Array_Length` (`self.Spawns`)))
        (if (> (`self.BetweenSpawnDelay`) 0.0)
          (`self.SpawnNextEntity`)
          (else
            (for (_array_element_2 _array_index) (`self.Spawns`)
              (set `self.CurrentSpawnedIndex` _array_index)
              (bind _bsuccessfullyspawned (`self.SpawnEntityFromSpawnStruct` _array_element_2))
              (if (not _bsuccessfullyspawned)
                (`/Engine/EditorBlueprintResources/StandardMacros.DecrementInt` (`self.RequiredKillCount`))))
            (set `self.bReactivateLocked` false)
            (`self.OnFinishedSpawning` self)))))))

(event `SpawnedActorDestroyed`
  (params (DestroyedActor :type "Actor Object Reference"))
  (`self.TryRemoveActorFromSpawnedList` DestroyedActor))

(event `SpawnedActorDied`
  (params (Caller :type "/Game/EpicTemplates/TemplateAgnostic/Blueprints/Components/BP_HealthComponent Object Reference") (KillingDamageSourceOwner :type "Actor Object Reference") (KillingDamageSource :type "Actor Object Reference") (KillingDamageLocation :type "Vector Structure") (KillingDamageDirection :type "Vector Structure") (HitBone :type Name) (SpecialDamageName :type Name))
  (`self.TryRemoveActorFromSpawnedList` (`ActorComponent.GetOwner` Caller)))

(fn `HandlePreSpawnStruct`
  (params (PreSpawnStruct :type "/Game/EpicTemplates/RailShooterTemplate/Blueprints/Structs/WaveNodePreSpawnedStruct Structure (by ref)"))
  (locals (Actor :type "Actor Object Reference")))

(fn `RegisterActorToNode`
  (params (ActorToRegister :type "Actor Object Reference"))
  (locals (HealthComp :type "/Game/EpicTemplates/TemplateAgnostic/Blueprints/Components/BP_HealthComponent Object Reference"))
  (`KismetArrayLibrary.Array_Add` (`self.RegisteredActors`) ActorToRegister)
  (bind _output_get (set `local.HealthComp` (`self.GetComponentByClass` (`local.ActorToRegister`) "/Game/EpicTemplates/TemplateAgnostic/Blueprints/Components/BP_HealthComponent.BP_HealthComponent_C")))
  (`/Engine/EditorBlueprintResources/StandardMacros.IsValid` _output_get
    (:`Is Valid`
      (add `/Game/EpicTemplates/TemplateAgnostic/Blueprints/Components/BP_HealthComponent.OnDied` (`local.HealthComp`) (`|CreateDelegate` :!event `SpawnedActorDied`)))
    (:`Is Not Valid`
      (add `self.OnDestroyed` (`local.ActorToRegister`) (`|CreateDelegate` :!event `SpawnedActorDestroyed`)))))

(fn `RegisterPreSpawnedActors`
  (locals (bIsSinglePlayer :type Boolean :default false) (TempIndex :type Integer) (TempActor :type "Actor Object Reference"))
  (for _array_element (`self.PreSpawnedActors`)
    (bind _output_get (set `local.TempActor` (`|ConvertAsset` (`.Actor_16_A437BEF648E6F5A746905A8823640695` (break `/Game/EpicTemplates/RailShooterTemplate/Blueprints/Structs/WaveNodePreSpawnedStruct` _array_element)))))
    (`/Engine/EditorBlueprintResources/StandardMacros.IsValid` _output_get
      (:`Is Valid`
        (`self.RegisterActorToNode` (`local.TempActor`)))
      (:`Is Not Valid`
        (`/Engine/EditorBlueprintResources/StandardMacros.DecrementInt` (`self.RequiredKillCount`))))))

(fn `Spawn Actor At Spawn Point with Target Logic`
  (params (ActorClass :type "Actor Class Reference") (SpawnPoint :type "Actor Object Reference") (Offset :type "Vector Structure") (SpawnSpace :type "/Game/EpicTemplates/RailShooterTemplate/Blueprints/Enums/ESpawnSpace Enum" :default "NewEnumerator0") (TargetLogic :type "/Game/EpicTemplates/RailShooterTemplate/Blueprints/Enums/EEnemyTargetLogic Enum" :default "NewEnumerator4"))
  (returns (SpawnedActor :type "Actor Object Reference"))
  (locals (SpawnTrans :type "Transform Structure") (TempSpawnedActor :type "Actor Object Reference") (HealthComp :type "/Game/EpicTemplates/TemplateAgnostic/Blueprints/Components/BP_HealthComponent Object Reference"))
  (`|ExecutionSequence`
    (:`then_0`
      (`/Engine/EditorBlueprintResources/StandardMacros.IsValid` (`local.SpawnPoint`)
        (:`Is Valid`
          (if (`KismetSystemLibrary.DoesImplementInterface` (`local.SpawnPoint`) "/Game/EpicTemplates/RailShooterTemplate/Blueprints/Interfaces/BPI_SpawnPoint.BPI_SpawnPoint_C")
            (bind _spawntransform (message `/Game/EpicTemplates/RailShooterTemplate/Blueprints/Interfaces/BPI_SpawnPoint.GetSpawnTransform` (`local.SpawnPoint`)))
            (set `local.SpawnTrans` _spawntransform)
            (else
              (set `local.SpawnTrans` (`self.GetTransform` (`local.SpawnPoint`))))))
        (:`Is Not Valid`
          (set `local.SpawnTrans` (`self.GetTransform`)))))
    (:`then_1`
      (bind _returnvalue (`|SpawnActorFromClass` (`local.ActorClass`) (select `/Game/EpicTemplates/RailShooterTemplate/Blueprints/Enums/ESpawnSpace` (`local.SpawnSpace`) :`NewEnumerator0` (`KismetMathLibrary.ComposeTransforms` (`KismetMathLibrary.MakeTransform` (`local.Offset`)) (`local.SpawnTrans`)) :`NewEnumerator1` (`KismetMathLibrary.ComposeTransforms` (`local.SpawnTrans`) (`KismetMathLibrary.MakeTransform` (`local.Offset`)))) "Undefined" "MultiplyWithRoot" null null))
      (bind _output_get (set `local.TempSpawnedActor` _returnvalue))
      (`/Engine/EditorBlueprintResources/StandardMacros.IsValid` _output_get
        (:`Is Valid`
          (`self.RegisterActorToNode` (`local.TempSpawnedActor`))
          (`|ExecutionSequence`
            (:`then_0`
              (if (`|EnumInequality` (`local.TargetLogic`) "NewEnumerator4")
                (`self.UpdateSpawnedActorTargetLogic` (`local.TempSpawnedActor`) (`local.TargetLogic`))))
            (:`then_1`
              (return (`local.TempSpawnedActor`)))))
        (:`Is Not Valid`
          (return null))))))

(fn `SpawnEntityFromSpawnStruct`
  (params (SpawnStruct :type "/Game/EpicTemplates/RailShooterTemplate/Blueprints/Structs/WaveNodeSpawnStruct Structure (by ref)"))
  (returns (bSuccessfullySpawned :type Boolean) (SpawnedActor :type "Actor Object Reference"))
  (bind ((`SpawnPoint_7_A437BEF648E6F5A746905A8823640695` _spawnpoint) (`SpawnOffset_10_844522C14395980CCC3ECE90BDC9C6DE` _spawnoffset) (`SpawnOffsetSpace_15_1F610936461810BA9AF79CBE1DB6EDE1` _spawnoffsetspace) (`TargetLogicToApply_18_9573F1724A1A3EDC95D771A8DA212718` _targetlogictoapply)) (break `/Game/EpicTemplates/RailShooterTemplate/Blueprints/Structs/WaveNodeSpawnStruct` (`local.SpawnStruct`)))
  (bind _returnvalue (`KismetSystemLibrary.LoadClassAsset_Blocking` (`.ActorToSpawn_4_25C291054856CC00D67C08A5F5259689` (break `/Game/EpicTemplates/RailShooterTemplate/Blueprints/Structs/WaveNodeSpawnStruct` (`local.SpawnStruct`)))))
  (bind _asactor (castclass `Actor` _returnvalue)
    (:`then`
      (bind _spawnedactor (`self.Spawn Actor At Spawn Point with Target Logic` _asactor (`|ConvertAsset` _spawnpoint) _spawnoffset _spawnoffsetspace _targetlogictoapply))
      (return (`KismetSystemLibrary.IsValid` _spawnedactor) _spawnedactor))
    (:`CastFailed`
      (return false null))))

(fn `TrimSpawnsIfSinglePlayer`
  (locals (TempIndex :type Integer) (TempActor :type "Actor Object Reference"))
  (bind _issingleplayer (`/Game/EpicTemplates/TemplateAgnostic/Blueprints/EpicTemplatesFunctionLibrary.IsInSinglePlayerMode`))
  (if _issingleplayer
    (`|ExecutionSequence`
      (:`then_0`
        (bind (_arrayindex _arrayelement) (`/Engine/EditorBlueprintResources/StandardMacros.ReverseForEachLoop` (`self.PreSpawnedActors`))
          (:`LoopBody`
            (set `local.TempIndex` _arrayindex)
            (bind ((`Actor_16_A437BEF648E6F5A746905A8823640695` _actor) (`bDestroyIfSinglePlayer_22_CDF7C594412B9679E67917A7736DDC0F` _bdestroyifsingleplayer)) (break `/Game/EpicTemplates/RailShooterTemplate/Blueprints/Structs/WaveNodePreSpawnedStruct` _arrayelement))
            (if _bdestroyifsingleplayer
              (set `local.TempActor` (`|ConvertAsset` _actor))
              (`|ExecutionSequence`
                (:`then_0`
                  (`/Engine/EditorBlueprintResources/StandardMacros.IsValid` (`local.TempActor`)
                    (:`Is Valid`
                      (`self.K2_DestroyActor` (`local.TempActor`)))))
                (:`then_1`
                  (`KismetArrayLibrary.Array_Remove` (`self.PreSpawnedActors`) (`local.TempIndex`))))))))
      (:`then_1`
        (bind (_arrayindex_2 _arrayelement_2) (`/Engine/EditorBlueprintResources/StandardMacros.ReverseForEachLoop` (`self.Spawns`))
          (:`LoopBody`
            (set `local.TempIndex` _arrayindex_2)
            (if (`.bSkipSpawnInSinglePlayer_23_144356DC425AFF7DC7F399834CAC57C6` (break `/Game/EpicTemplates/RailShooterTemplate/Blueprints/Structs/WaveNodeSpawnStruct` _arrayelement_2))
              (`KismetArrayLibrary.Array_Remove` (`self.Spawns`) (`local.TempIndex`)))))))))

(fn `TryRemoveActorFromSpawnedList`
  (params (Actor :type "Actor Object Reference (by ref)"))
  (if (> (`KismetArrayLibrary.Array_Length` (`self.RegisteredActors`)) 0)
    (bind _returnvalue (`KismetArrayLibrary.Array_RemoveItem` (`self.RegisteredActors`) Actor))
    (if _returnvalue
      (bind _result (`/Engine/EditorBlueprintResources/StandardMacros.IncrementInt` (`self.KillCount`))
        (:`  `
          (if (== _result (`self.RequiredKillCount`))
            (`self.OnAllSpawnedEntitiesKilled` self)))))))

(fn `UpdateSpawnedActorTargetLogic`
  (params (Actor :type "Actor Object Reference") (TargetLogic :type "/Game/EpicTemplates/RailShooterTemplate/Blueprints/Enums/EEnemyTargetLogic Enum" :default "NewEnumerator4"))
  (bind (_interfaceimplementingobject _foundimplementingobject) (`/Game/EpicTemplates/TemplateAgnostic/Blueprints/EpicTemplatesFunctionLibrary.SearchActorForInterface` Actor "/Game/EpicTemplates/RailShooterTemplate/Blueprints/Interfaces/BPI_TargetLogicImplementor.BPI_TargetLogicImplementor_C"))
  (if _foundimplementingobject
    (message `/Game/EpicTemplates/RailShooterTemplate/Blueprints/Interfaces/BPI_TargetLogicImplementor.UpdateTargetLogic` _interfaceimplementingobject (`local.TargetLogic`))))

(fn `UserConstructionScript`)