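; Rail shooter boss enemy that fires projectiles at randomly picked players, plus stray dud projectiles.
; A valid target starts the fire timer after an initial delay; each shot re-picks a player and schedules the next with random variance.
; A target-logic change can start looping dud fire, launched in a cone around the aim direction; dying clears both timers.
; Projectiles spawn as reusable actors from soft-loaded, cached classes and launch through messages.
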(event `FireProjectile`
  (`self.UpdateTargetAsRandomPlayer`)
  (`self.FireNewProjectile`)
  (`self.SetNextProjectileTimer`))

(event `SpawnAndLaunchProjectile`
  (bind _loadedclass (`/Game/EpicTemplates/TemplateAgnostic/Blueprints/EpicTemplatesActorMacroLibrary.GetActorClassOrLoadSoft` (`self.ProjectileClass_Hard`) (`self.ProjectileClass_Soft`))
    (:`ClassAlreadyValid`
      _)
    (:`ClassNeededLoad`
      (set `self.ProjectileClass_Hard` _loadedclass)))
  (bind _actorinstance (`/Game/EpicTemplates/TemplateAgnostic/Blueprints/EpicTemplatesFunctionLibrary.SpawnReusableActorFromClass` (`self.ProjectileClass_Hard`) (`self.GetNewProjectileTransform`) self self))
  (`self.LaunchProjectile` _actorinstance))

(event `self.TargetUpdated`
  (params (NewTarget :type "Actor Object Reference"))
  (`/Engine/EditorBlueprintResources/StandardMacros.IsValid` NewTarget
    (:`Is Valid`
      (bind _returnvalue (`KismetSystemLibrary.K2_SetTimerDelegate` (`|CreateDelegate` :!event `FireProjectile`) (`self.InitialProjectileDelay`)))
      (set `self.FireProjectileHandle` _returnvalue))
    (:`Is Not Valid`
      (`KismetSystemLibrary.K2_ClearAndInvalidateTimerHandle` (`self.FireProjectileHandle`)))))

(event `SpawnAndLaunchDud`
  (bind _loadedclass (`/Game/EpicTemplates/TemplateAgnostic/Blueprints/EpicTemplatesActorMacroLibrary.GetActorClassOrLoadSoft` (`self.DudProjectileClass_Hard`) (`self.DudProjectileClass_Soft`))
    (:`ClassAlreadyValid`
      _)
    (:`ClassNeededLoad`
      (set `self.DudProjectileClass_Hard` _loadedclass)))
  (bind _actorinstance (`/Game/EpicTemplates/TemplateAgnostic/Blueprints/EpicTemplatesFunctionLibrary.SpawnReusableActorFromClass` (`self.DudProjectileClass_Hard`) (`self.GetNewProjectileTransform`) self self))
  (`self.LaunchDudProjectile` _actorinstance))

(event `/Game/EpicTemplates/RailShooterTemplate/Blueprints/Interfaces/BPI_TargetLogicImplementor.UpdateTargetLogic`
  (params (NewTargetLogic :type "/Game/EpicTemplates/RailShooterTemplate/Blueprints/Enums/EEnemyTargetLogic Enum" :default "NewEnumerator4"))
  (`parent.UpdateTargetLogic` NewTargetLogic)
  (if (`|EnumInequality` NewTargetLogic "NewEnumerator4")
    (bind _returnvalue (`KismetSystemLibrary.K2_SetTimerDelegate` (`|CreateDelegate` :!event `Fire New Dud Projectile`) (`self.DudProjectileFrequency`) true))
    (set `self.DudProjectileHandle` _returnvalue)))

(event `self.DyingStarted`
  (`KismetSystemLibrary.K2_ClearAndInvalidateTimerHandle` (`self.FireProjectileHandle`))
  (`KismetSystemLibrary.K2_ClearAndInvalidateTimerHandle` (`self.DudProjectileHandle`)))

(fn `Fire New Dud Projectile`
  (locals (ReusableActorComponent :type "/Game/EpicTemplates/TemplateAgnostic/Blueprints/Components/BP_ReusableActorComponent Object Reference") (TempProjectile :type "Actor Object Reference"))
  (`self.SpawnAndLaunchDud`))

(fn `FireNewProjectile`
  (locals (ReusableActorComponent :type "/Game/EpicTemplates/TemplateAgnostic/Blueprints/Components/BP_ReusableActorComponent Object Reference") (TempProjectile :type "Actor Object Reference"))
  (`self.SpawnAndLaunchProjectile`))

(fn `GetNewProjectileTransform`
  (returns (ReturnValue :type "Transform Structure"))
  (`/Engine/EditorBlueprintResources/StandardMacros.IsValid` (`self.CurrentTarget`)
    (:`Is Valid`
      (return (`KismetMathLibrary.MakeTransform` (`SceneComponent.K2_GetComponentLocation` (`self.FirePoint`)) (`KismetMathLibrary.FindLookAtRotation` (`SceneComponent.K2_GetComponentLocation` (`self.FirePoint`)) (`self.GetActorEyesViewPoint` (`self.CurrentTarget`))))))
    (:`Is Not Valid`
      (return (`KismetMathLibrary.MakeTransform` (`SceneComponent.K2_GetComponentLocation` (`self.FirePoint`)) (`SceneComponent.K2_GetComponentRotation` (`self.FirePoint`)))))))

(fn `LaunchDudProjectile`
  (params (ProjectileActor :type "Object Object Reference"))
  (message `/Game/EpicTemplates/TemplateAgnostic/Blueprints/Interfaces/BPI_Projectile.LaunchInDirection` ProjectileActor self (`KismetMathLibrary.RandomUnitVectorInConeInDegrees` (`KismetMathLibrary.TransformDirection` (`self.GetNewProjectileTransform`) (1.0 0.0 0.0)) 30.0) (`self.OverrideProjectileSpeed`)))

(fn `LaunchProjectile`
  (params (ProjectileActor :type "Actor Object Reference"))
  (message `/Game/EpicTemplates/TemplateAgnostic/Blueprints/Interfaces/BPI_Projectile.AssignActorTarget` ProjectileActor (`self.CurrentTarget`))
  (message `/Game/EpicTemplates/TemplateAgnostic/Blueprints/Interfaces/BPI_Projectile.LaunchInDirection` (`local.ProjectileActor`) self (`KismetMathLibrary.TransformDirection` (`self.GetNewProjectileTransform`) (1.0 0.0 0.0)) (`self.OverrideProjectileSpeed`)))

(fn `SetNextProjectileTimer`
  (bind _returnvalue (`KismetSystemLibrary.K2_SetTimerDelegate` (`|CreateDelegate` :!event `FireProjectile`) (+ (`self.ProjectileFrequency`) (`KismetMathLibrary.RandomFloatInRange` (* (`self.ProjectileFrequencyVariance`) -1.0) (`self.ProjectileFrequencyVariance`)))))
  (set `self.FireProjectileHandle` _returnvalue))

(fn `UserConstructionScript`
  (`parent.UserConstructionScript`))