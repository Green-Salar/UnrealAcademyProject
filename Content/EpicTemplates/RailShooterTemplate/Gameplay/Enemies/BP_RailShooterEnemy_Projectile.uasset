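; Rail shooter enemy Blueprint that fires projectiles from its FirePoint at the current target.
; A valid target starts an initial delay timer and async-loads the soft projectile class, while target loss or dying clears the timer.
; Each shot spawns a reusable actor aimed at the target's eye viewpoint, passes it the target and launches it through message calls.
; The next shot is then scheduled at the base frequency with random variance.
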(event `FireNextProjectile`
  (`self.SpawnAndLaunchNewProjectile`)
  (`self.SetNextProjectileTimer`))

(event `self.TargetUpdated`
  (params (NewTarget :type "Actor Object Reference"))
  (`parent.TargetUpdated` NewTarget)
  (`/Engine/EditorBlueprintResources/StandardMacros.IsValid` NewTarget
    (:`Is Valid`
      (bind _returnvalue (`KismetSystemLibrary.K2_SetTimerDelegate` (`|CreateDelegate` :!event `FireNextProjectile`) (`self.InitialProjectileDelay`)))
      (set `self.FireProjectileHandle` _returnvalue)
      (bind _class (`|LoadAssetClass` (`self.ProjectileClass_Soft`))
        (:`Completed`
          (bind _asactor (castclass `Actor` _class))
          (set `self.ProjectileClass_Hard` _asactor))))
    (:`Is Not Valid`
      (`KismetSystemLibrary.K2_ClearAndInvalidateTimerHandle` (`self.FireProjectileHandle`)))))

(event `self.DyingStarted`
  (`KismetSystemLibrary.K2_ClearAndInvalidateTimerHandle` (`self.FireProjectileHandle`)))

(event `SpawnAndLaunchNewProjectile`
  (bind _loadedclass (`/Game/EpicTemplates/TemplateAgnostic/Blueprints/EpicTemplatesActorMacroLibrary.GetActorClassOrLoadSoft` (`self.ProjectileClass_Hard`) (`self.ProjectileClass_Soft`))
    (:`ClassAlreadyValid`
      _)
    (:`ClassNeededLoad`
      (set `self.ProjectileClass_Hard` _loadedclass)))
  (bind _actorinstance (`/Game/EpicTemplates/TemplateAgnostic/Blueprints/EpicTemplatesFunctionLibrary.SpawnReusableActorFromClass` (`self.ProjectileClass_Hard`) (`self.GetNewProjectileTransform`) self self))
  (`self.LaunchProjectile` _actorinstance))

(fn `GetNewProjectileTransform`
  (returns (ReturnValue :type "Transform Structure"))
  (`/Engine/EditorBlueprintResources/StandardMacros.IsValid` (`self.CurrentTarget`)
    (:`Is Valid`
      (return (`KismetMathLibrary.MakeTransform` (`SceneComponent.K2_GetComponentLocation` (`self.FirePoint`)) (`KismetMathLibrary.FindLookAtRotation` (`SceneComponent.K2_GetComponentLocation` (`self.FirePoint`)) (`self.GetActorEyesViewPoint` (`self.CurrentTarget`))))))
    (:`Is Not Valid`
      (return (`KismetMathLibrary.MakeTransform` (`SceneComponent.K2_GetComponentLocation` (`self.FirePoint`)) (`SceneComponent.K2_GetComponentRotation` (`self.FirePoint`)))))))

(fn `LaunchProjectile`
  (params (ProjectileActor :type "Actor Object Reference"))
  (message `/Game/EpicTemplates/TemplateAgnostic/Blueprints/Interfaces/BPI_Projectile.AssignActorTarget` ProjectileActor (`self.CurrentTarget`))
  (message `/Game/EpicTemplates/TemplateAgnostic/Blueprints/Interfaces/BPI_Projectile.LaunchInDirection` (`local.ProjectileActor`) self (`KismetMathLibrary.TransformDirection` (`self.GetNewProjectileTransform`) (1.0 0.0 0.0)) (`self.OverrideProjectileSpeed`)))

(fn `SetNextProjectileTimer`
  (bind _returnvalue (`KismetSystemLibrary.K2_SetTimerDelegate` (`|CreateDelegate` :!event `FireNextProjectile`) (+ (`self.ProjectileFrequency`) (`KismetMathLibrary.RandomFloatInRange` (* (`self.ProjectileFrequencyVariance`) -1.0) (`self.ProjectileFrequencyVariance`)))))
  (set `self.FireProjectileHandle` _returnvalue))

(fn `UserConstructionScript`
  (`parent.UserConstructionScript`))