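; Rail shooter enemy template with health, player targeting, hit reactions and headshot damage.
; A selectable targeting logic picks a player pawn by index, proximity, randomness, aggro overlap or damage, optionally yawing toward it; UpdateTarget changes flash an animated alert.
; Headshots are detected by distance from the capsule's top and multiply damage.
; Death enables capsule physics with a distance-scaled impulse, notifies listeners and optionally destroys the actor after a delay.
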(event `self.HealthComponent.OnTookDamage`
  (params (Caller :type "/Game/EpicTemplates/TemplateAgnostic/Blueprints/Components/BP_HealthComponent Object Reference") (OldHealth :type "Float (double-precision)") (NewHealth :type "Float (double-precision)") (SpecialDamageName :type Name) (DamageStruct :type "/Game/EpicTemplates/TemplateAgnostic/Blueprints/Structs/DamageStruct Structure (by ref)"))
  (bind ((`DamageSourceOwner_16_93F98FB747ED83B90B1FAFB49CE3E4D5` _damagesourceowner)) (break `/Game/EpicTemplates/TemplateAgnostic/Blueprints/Structs/DamageStruct` DamageStruct))
  ;[1 1 1] Damage and dying
  (if (or (`|EnumEquality` (`self.TargetingLogic`) "NewEnumerator6") (not (`KismetSystemLibrary.IsValid` (`self.CurrentTarget`))))
    (`/Game/EpicTemplates/TemplateAgnostic/Blueprints/EpicTemplatesObjectMacroLibrary.!!!IsNOTValid!!!` (`self.CurrentTarget`)
      (:`Is NOT Valid`
        (bind _asplayer_controller (cast `PlayerController` _damagesourceowner)
          (:`then`
            (`self.UpdateTarget` (`Controller.K2_GetPawn` _asplayer_controller)))
          (:`CastFailed`
            (set `self.CurrentTarget` _damagesourceowner)))))))

(event `self.ReceiveBeginPlay`
  ;[1 1 1] Begin Play
  (`self.CheckForTarget`))

(event `self.HealthComponent.OnDied`
  (params (Caller :type "/Game/EpicTemplates/TemplateAgnostic/Blueprints/Components/BP_HealthComponent Object Reference") (KillingDamageSourceOwner :type "Actor Object Reference") (KillingDamageSource :type "Actor Object Reference") (KillingDamageLocation :type "Vector Structure") (KillingDamageDirection :type "Vector Structure") (HitBone :type Name) (SpecialDamageName :type Name))
  ;[1 1 1] Damage and dying
  (set `self.bIsAlive` false)
  (`self.DyingStarted`)
  (`PrimitiveComponent.SetSimulatePhysics` (`self.CapsuleRoot`) true)
  (`PrimitiveComponent.AddImpulseAtLocation` (`self.CapsuleRoot`) (* KillingDamageDirection (`self.DeathImpulsePower`) (`KismetMathLibrary.MapRangeClamped` (`KismetMathLibrary.Vector_Distance` KillingDamageLocation (`self.K2_GetActorLocation` KillingDamageSource)) 0.0 3000.0 1.0 0.2) (select `bool` (== SpecialDamageName "Headshot") :`false` 1.0 :`true` 2.0 :!type "Float (single-precision)")) KillingDamageLocation "None")
  (`self.SetActorTickEnabled` false)
  (`TimelineComponent.Stop` (`self.TL_NewTarget`))
  (`SceneComponent.SetHiddenInGame` (`self.AlertedVisual`) true false)
  (`self.OnKilled` self)
  (if (`self.bDestroyOnDie`)
    (`KismetSystemLibrary.Delay` (`self.DestroyDelay`))
    (`self.K2_DestroyActor`)))

(event `self.ReceiveTick`
  (params (DeltaSeconds :type "Float (single-precision)"))
  ;[1 1 1] Tick
  (if (`self.bFaceTarget`)
    (`/Engine/EditorBlueprintResources/StandardMacros.IsValid` (`self.CurrentTarget`)
      (:`Is Valid`
        (`self.K2_SetActorRotation` (`KismetMathLibrary.MakeRotator` (.roll (`self.K2_GetActorRotation`)) (.pitch (`self.K2_GetActorRotation`)) (.yaw (`KismetMathLibrary.FindLookAtRotation` (`self.K2_GetActorLocation`) (`self.K2_GetActorLocation` (`self.CurrentTarget`))))))))))

(event `DyingStarted`
  ;[1 1 1] Damage and dying
)

(event `/Game/EpicTemplates/RailShooterTemplate/Blueprints/Interfaces/BPI_TargetLogicImplementor.UpdateTargetLogic`
  (params (NewTargetLogic :type "/Game/EpicTemplates/RailShooterTemplate/Blueprints/Enums/EEnemyTargetLogic Enum" :default "NewEnumerator4"))
  ;[1 1 1] Target code
  (if (`self.bIsAlive`)
    (set `self.TargetingLogic` NewTargetLogic)
    (`self.CheckForTarget`)))

(event `self.AggroSphere.OnComponentBeginOverlap`
  (params (OverlappedComponent :type "PrimitiveComponent Object Reference") (OtherActor :type "Actor Object Reference") (OtherComp :type "PrimitiveComponent Object Reference") (OtherBodyIndex :type Integer) (bFromSweep :type Boolean) (SweepResult :type "HitResult Structure (by ref)"))
  ;[1 1 1] Target code
  (if (`|EnumEquality` (`self.TargetingLogic`) "NewEnumerator5")
    (`/Game/EpicTemplates/TemplateAgnostic/Blueprints/EpicTemplatesObjectMacroLibrary.!!!IsNOTValid!!!` (`self.CurrentTarget`)
      (:`Is NOT Valid`
        (bind _aspawn (cast `Pawn` OtherActor))
        (cast `PlayerController` (`self.GetController` _aspawn))
        (set `self.CurrentTarget` _aspawn)))))

(event `TargetUpdated`
  (params (NewTarget :type "Actor Object Reference"))
  ;[1 1 1] Target code
  (`/Engine/EditorBlueprintResources/StandardMacros.IsValid` NewTarget
    (:`Is Valid`
      (if (`self.bIsAlive`)
        (`SceneComponent.SetHiddenInGame` (`self.AlertedVisual`) false false)
        (bind (_direction _alertedmovealpha _alertedcolor) (`Timeline|TL_NewTarget` :!via `PlayFromStart`)
          (:`Update`
            (`SceneComponent.K2_SetRelativeLocation` (`self.AlertedVisual`) (`KismetMathLibrary.MakeVector` 0.0 0.0 (* _alertedmovealpha (`self.AlertVerticalMovement`))) false false)
            (`TextRenderComponent.SetTextRenderColor` (`self.AlertedVisual`) (`KismetMathLibrary.Conv_LinearColorToColor` _alertedcolor)))
          (:`Finished`
            (`SceneComponent.SetHiddenInGame` (`self.AlertedVisual`) true false)))))))

(fn `CheckForDamageModifiers`
  (params (Damage :type "/Game/EpicTemplates/TemplateAgnostic/Blueprints/Structs/DamageStruct Structure (by ref)"))
  (returns (Multiplier :type "Float (double-precision)") (DamageModifierName :type Name))
  (bind _capsuleroot (`self.CapsuleRoot`))
  (if (<= (`KismetMathLibrary.Vector_DistanceSquared` (`.DamageLocation_8_F5A6C21543470034EA0BD6945175CC5B` (break `/Game/EpicTemplates/TemplateAgnostic/Blueprints/Structs/DamageStruct` Damage)) (`KismetMathLibrary.TransformLocation` (`SceneComponent.K2_GetComponentToWorld` (`self.CapsuleRoot`)) (`KismetMathLibrary.MakeVector` 0.0 0.0 (- (`CapsuleComponent.GetUnscaledCapsuleHalfHeight` _capsuleroot) (`CapsuleComponent.GetUnscaledCapsuleRadius` _capsuleroot))))) (`KismetMathLibrary.Square` (+ (`CapsuleComponent.GetScaledCapsuleRadius` (`self.CapsuleRoot`)) (`self.HeadshotAreaOverCapsuleRadius`))))
    (return 3.0 "Headshot")
    (else
      (return 1.0 "None"))))

(fn `CheckForTarget`
  (switch `/Game/EpicTemplates/RailShooterTemplate/Blueprints/Enums/EEnemyTargetLogic` (`self.TargetingLogic`)
    (:`NewEnumerator4`
      (`self.UpdateTarget` null))
    (:`NewEnumerator0`
      (`self.UpdateTargetAsRandomPlayer`))
    (:`NewEnumerator1`
      (`self.UpdateTarget` (`GameplayStatics.GetPlayerPawn` 0)))
    (:`NewEnumerator2`
      (`self.UpdateTarget` (`GameplayStatics.GetPlayerPawn` (`KismetMathLibrary.Max` (- (`GameplayStatics.GetNumPlayerControllers`) 1)))))
    (:`NewEnumerator3`
      (bind _closestplayerpawn (`self.GetClosestPlayerPawn` 0.0))
      (`self.UpdateTarget` _closestplayerpawn))
    (:`NewEnumerator5`
      (bind _closestplayerpawn_2 (`self.GetClosestPlayerPawn` (`self.AggroRange`)))
      (`self.UpdateTarget` _closestplayerpawn_2))
    (:`NewEnumerator6`
      (`self.UpdateTarget` null))))

(fn `GetClosestPlayerPawn`
  (params (MaxRange :type "Float (double-precision)"))
  (returns (ClosestPlayerPawn :type "Pawn Object Reference"))
  (locals (ClosestPawn :type "Pawn Object Reference") (TempPawn :type "Pawn Object Reference") (PawnSqDist :type "Float (double-precision)" :default 0.0))
  (bind _maxrange (`local.MaxRange`))
  (for _index (range (`GameplayStatics.GetNumPlayerControllers`))
    (set `local.TempPawn` (`GameplayStatics.GetPlayerPawn` _index))
    (set `local.PawnSqDist` (`KismetMathLibrary.VSizeSquared` (- (`self.K2_GetActorLocation`) (`self.K2_GetActorLocation` (`local.TempPawn`)))))
    (if (or (<= _maxrange 0.0) (< (`local.PawnSqDist`) (`KismetMathLibrary.Square` _maxrange)))
      (if (not (`KismetSystemLibrary.IsValid` (`local.ClosestPawn`)))
        (set `local.ClosestPawn` (`local.TempPawn`) :!label _label)
        (elif (< (`local.PawnSqDist`) (`KismetMathLibrary.VSizeSquared` (- (`self.K2_GetActorLocation`) (`self.K2_GetActorLocation` (`local.ClosestPawn`)))))
          (goto _label)))))
  (return (`local.ClosestPawn`)))

(fn `UpdateTarget`
  (params (NewTarget :type "Actor Object Reference"))
  (if (!= NewTarget (`self.CurrentTarget`))
    (bind _output_get (set `self.CurrentTarget` (`local.NewTarget`)))
    (`self.TargetUpdated` _output_get)))

(fn `UpdateTargetAsRandomPlayer`
  (`self.UpdateTarget` (`GameplayStatics.GetPlayerPawn` (`KismetMathLibrary.RandomIntegerInRange` 0 (- (`GameplayStatics.GetNumPlayerControllers`) 1)))))

(fn `UserConstructionScript`
  (bind _healthcomponent (`self.HealthComponent`))
  (bind _starthealth (`self.StartHealth`))
  (`SceneComponent.K2_SetRelativeLocation` (`self.MeshPivot`) (`KismetMathLibrary.MakeVector` 0.0 0.0 (* (`CapsuleComponent.CapsuleHalfHeight` (`self.CapsuleRoot`)) -1.0)) false false)
  (set `/Game/EpicTemplates/TemplateAgnostic/Blueprints/Components/BP_HealthComponent.StartHealth` _starthealth _healthcomponent)
  (set `/Game/EpicTemplates/TemplateAgnostic/Blueprints/Components/BP_HealthComponent.StartMaxHealth` _starthealth _healthcomponent)
  (`SphereComponent.SetSphereRadius` (`self.AggroSphere`) (`self.AggroRange`) true)
  (`/Game/EpicTemplates/TemplateAgnostic/Blueprints/Components/BP_HitReactComponent.RegisterReactMesh` :`self` (`self.HitReactComponent`) :`MeshComponent` (`self.Mesh`) :`bAddAllMaterialSlots` true))