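; Template player controller that handles global input mapping, menus, pausing, button prompts and cursors, including split-screen clamping.
; The first open menu becomes the base menu and owns input mode until closed; the pause menu class loads asynchronously.
; Key presses detect gamepad versus mouse/keyboard, updating cursor and focus and notifying listeners.
; Possessed pawns' health component deaths trigger the game-over check, while debug keys drive slomo cheats and debuggable interfaces.
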(event Custom|PossessedPawnRevived
  (params (Caller :type BP%20Health%20Component%20Object%20Reference) (ReviveSource :type Actor%20Object%20Reference))
  ;[1 1 1] Died/Revived
)

(event Custom|PauseMenuClosed
  (params (Caller :type W%20Menu%20Widget%20Object%20Reference))
  ;[1 1 1] Pause
  (Game|SetGamePaused false))

(event Custom|BaseMenuRemoved
  (params (Caller :type W%20Menu%20Widget%20Object%20Reference))
  ;[1 1 1] Menu Handler Interface
  (EventDispatchers|UnbindEventfromOnMenuClosed Caller (delegate Custom|BaseMenuRemoved))
  (if (== Caller (Variables|Default|GetBaseMenu))
    (Variables|Default|SetBaseMenu 0)
    (Input|SetInputModeGameOnly self false)
    (Variables|Default|SetbShowMouseCursor false)))

(event Custom|PossessedPawnDied
  (params (Caller :type BP%20Health%20Component%20Object%20Reference) (KillingDamageSourceOwner :type Actor%20Object%20Reference) (KillingDamageSource :type Actor%20Object%20Reference) (KillingDamageLocation :type Vector) (KillingDamageDirection :type Vector) (HitBone :type Name) (SpecialDamageName :type Name))
  ;[1 1 1] Died/Revived
  (bind _asbp_game_mode_template_base (Utilities|Casting|CastToBP_GameMode_TemplateBase (Game|GetGameMode)))
  (Default|CheckforGameOver _asbp_game_mode_template_base))

(event Custom|MenuWidgetDetectedKey
  (params (Key :type Key%20Structure%20%28by%20ref%29 :default "None"))
  ;[1 1 1] Input method changed binding
  (CallFunction|HandleKeyPressDetected Key))

(event Input|EnhancedActionEvents|EnhancedInputActionIA_Pause
  (params (ActionValue :type Boolean) (ElapsedSeconds :type Float%20%28double-precision%29) (TriggeredSeconds :type Float%20%28double-precision%29) (InputAction :type Input%20Action%20Object%20Reference :default "/Game/EpicTemplates/TemplateAgnostic/Input/IA_Pause.IA_Pause"))
  ;[1 1 1] Pause
  (Game|SetGamePaused true)
  (Utilities|!!!IsNOTValid!!! (Variables|Default|GetPauseMenu)
    (:Is%20NOT%20Valid
      (bind _class (Utilities|AsyncLoadClassAsset (Variables|Default|GetPauseMenuClass))
        (:Completed
          (bind _asw_menu_widget (Utilities|Casting|CastToW_MenuWidgetClass _class))
          (bind _returnvalue (UserInterface|CreateWidget _asw_menu_widget))
          (bind _output_get (Variables|Default|SetPauseMenu _returnvalue))
          (EventDispatchers|BindEventtoOnMenuClosed _output_get (delegate Custom|PauseMenuClosed))
          (CallFunction|DisplayGamewideMenu (Variables|Default|GetPauseMenu)))))))

(event EventPossess
  (params (PossessedPawn :type Pawn%20Object%20Reference))
  ;[1 1 1] Possess
  (CallFunction|BindPawnHealthEvents PossessedPawn))

(event EventAdjustCursorScreenPosition
  (params (Delta :type Vector%202D%20Structure))
  ;[1 1 1] Cusor Implementer Interface
  (Variables|Default|SetCurrentCursorPos (+ (Variables|Default|GetCurrentCursorPos) Delta))
  (if (== (Class|GameplayStatics|GetPlayerControllerID self) 0)
    (Class|PlayerController|SetMouseLocation (Math|Float|Truncate (.X (Math|Vector2D|BreakVector2D (Variables|Default|GetCurrentCursorPos)))) (Math|Float|Truncate (.Y (Math|Vector2D|BreakVector2D (Variables|Default|GetCurrentCursorPos)))))))

(event EventBeginPlay
  ;[1 1 1] Begin Play
  (Utilities|FlowControl|DelayUntilNextTick)
  (Utilities|FlowControl|Sequence
    (:then_0
      (Input|AddMappingContext (PlayerController|LocalPlayerSubsystems|GetEnhancedInputLocalPlayerSubsystem) "/Game/EpicTemplates/TemplateAgnostic/Input/IMC_Global.IMC_Global" 0 "(bIgnoreAllPressedKeysUntilRelease=True,bForceImmediately=False,bNotifyUserSettings=False)"))
    (:then_1
      (if (not (Utilities|IsValid (Variables|Default|GetBaseMenu)))
        (Input|SetInputModeGameOnly self false)
        (CallFunction|SetCursorScreenPosition (* (Viewport|GetViewportSize) 0.5))))
    (:then_2
      (if (Variables|Default|GetbUtilisePromptScreen)
        (bind _returnvalue (UserInterface|CreateWidget "/Game/EpicTemplates/TemplateAgnostic/UI/W_PromptScreen.W_PromptScreen_C"))
        (bind _output_get (Variables|Default|SetPromptScreen _returnvalue))
        (UserInterface|Viewport|AddtoPlayerScreen _output_get)))
    (:then_3
      (bind _issingleplayer (CallFunction|IsinSinglePlayerMode))
      (bind _output_get_2 (Variables|Default|SetbIsSinglePlayerMode _issingleplayer))
      (if (not _output_get_2)
        _))))

(event EventMenuBeingDisplayed
  (params (Caller :type W%20Menu%20Widget%20Object%20Reference))
  ;[1 1 1] Menu Handler Interface
  (if (not (Utilities|IsValid (Variables|Default|GetBaseMenu)))
    (bind _output_get (Variables|Default|SetBaseMenu Caller))
    (Input|SetInputModeUIOnly self _output_get "LockAlways" false)
    (Variables|Default|SetbShowMouseCursor (not (Variables|Default|GetbIsGamepad)))
    (EventDispatchers|BindEventtoOnMenuClosed (Variables|Default|GetBaseMenu) (delegate Custom|BaseMenuRemoved))
    (Default|DisplayMenu (Variables|Default|GetBaseMenu) (Variables|Default|GetbIsGamepad))))

(event EventSetCursorScreenPosition
  (params (ScreenPos :type Vector%202D%20Structure))
  ;[1 1 1] Cusor Implementer Interface
  (bind _output_get (Variables|Default|SetCurrentCursorPos ScreenPos))
  (if (== (Class|GameplayStatics|GetPlayerControllerID self) 0)
    (Class|PlayerController|SetMouseLocation (Math|Float|Truncate (.X (Math|Vector2D|BreakVector2D _output_get))) (Math|Float|Truncate (.Y (Math|Vector2D|BreakVector2D _output_get))))))

(event Input|KeyboardEvents|AnyKey
  (params (Key :type Key%20Structure :default "None"))
  ;[1 1 1] Input method changed binding
  (:Pressed
    (CallFunction|HandleKeyPressDetected Key)))

(event Input|KeyboardEvents|DebugKey#
  (params (Key :type Key%20Structure) (ActionValue :type Input%20Action%20Value%20Structure))
  (:Pressed
    (bind _isa (Utilities|FlowControl|FlipFlop)
      (:A
        _)
      (:B
        _))
    (bind _outactors (Actor|GetAllActorswithInterface "/Game/EpicTemplates/TemplateAgnostic/Blueprints/Interfaces/BPI_Debuggable.BPI_Debuggable_C"))
    (for _array_element _outactors
      (Class|BPIDebuggable|UpdateIsinDebug(Message) _array_element _isa)
      (for _array_element_2 (Class|Actor|GetComponentsbyInterface _array_element "/Game/EpicTemplates/TemplateAgnostic/Blueprints/Interfaces/BPI_Debuggable.BPI_Debuggable_C")
        (Class|BPIDebuggable|UpdateIsinDebug(Message) _array_element_2 _isa)))))

(event Input|KeyboardEvents|DebugKeyHyphen
  (params (Key :type Key%20Structure) (ActionValue :type Input%20Action%20Value%20Structure))
  (:Pressed
    (bind _asbp_template_cheat_manager (Utilities|Casting|CastToBP_TemplateCheatManager (Variables|Default|GetCheatManager)))
    (Default|SlomoDown _asbp_template_cheat_manager)))

(event Input|KeyboardEvents|DebugKeyEquals
  (params (Key :type Key%20Structure) (ActionValue :type Input%20Action%20Value%20Structure))
  (:Pressed
    (bind _asbp_template_cheat_manager (Utilities|Casting|CastToBP_TemplateCheatManager (Variables|Default|GetCheatManager)))
    (Default|SlomoUp _asbp_template_cheat_manager)))

(fn ConstructionScript)

(fn BindEventtoInputMethodChanged
  (params (Event :type Delegate%20%28by%20ref%29) (callOnBind :type Boolean))
  (EventDispatchers|BindEventtoOnInputMethodChanged Event)
  (if callOnBind
    (EventDispatchers|UnbindallEventsfromOnInputMethodChangedCallatBind)
    (EventDispatchers|BindEventtoOnInputMethodChangedCallatBind Event)
    (Default|CallOnInputMethodChangedCallatBind self (Variables|Default|GetbIsGamepad))
    (EventDispatchers|UnbindEventfromOnInputMethodChangedCallatBind Event)))

(fn UnbindEventfromInputMethodChanged
  (params (Event :type Delegate%20%28by%20ref%29))
  (EventDispatchers|UnbindEventfromOnInputMethodChanged Event))

(fn DisplayButtonPrompt
  (params (PromptID :type Name%20%28by%20ref%29) (NewInputAction :type Input%20Action%20Object%20Reference) (PromptText :type Text) (PromptLocation :type EPromptLocation%20Enum :default "NewEnumerator0"))
  (bind _promptscreen (Variables|Default|GetPromptScreen))
  (Utilities|IsValid _promptscreen
    (:Is%20Valid
      (Default|DisplayButtonPrompt _promptscreen PromptID NewInputAction PromptText PromptLocation))))

(fn HideButtonPrompt
  (params (PromptID :type Name%20%28by%20ref%29))
  (bind _promptscreen (Variables|Default|GetPromptScreen))
  (Utilities|IsValid _promptscreen
    (:Is%20Valid
      (Default|HideButtonPrompt _promptscreen PromptID))))

(fn BindPawnHealthEvents
  (params (PawnActor :type Actor%20Object%20Reference))
  (bind _output_get (LocalVariables|SetHealthComponent (Actor|GetComponentbyClass PawnActor "/Game/EpicTemplates/TemplateAgnostic/Blueprints/Components/BP_HealthComponent.BP_HealthComponent_C")))
  (Utilities|IsValid _output_get
    (:Is%20Valid
      (EventDispatchers|BindEventtoOnDied (LocalVariables|GetHealthComponent) (EventDispatchers|CreateEvent :!event Custom|PossessedPawnDied))
      (EventDispatchers|BindEventtoOnRevived (LocalVariables|GetHealthComponent) (EventDispatchers|CreateEvent :!event Custom|PossessedPawnRevived)))))

(fn UnbindPawnHealthEvents
  (params (PawnActor :type Actor%20Object%20Reference))
  (bind _output_get (LocalVariables|SetHealthComponent (Actor|GetComponentbyClass PawnActor "/Game/EpicTemplates/TemplateAgnostic/Blueprints/Components/BP_HealthComponent.BP_HealthComponent_C")))
  (Utilities|IsValid _output_get
    (:Is%20Valid
      (EventDispatchers|UnbindEventfromOnDied (LocalVariables|GetHealthComponent) (EventDispatchers|CreateEvent :!event Custom|PossessedPawnDied))
      (EventDispatchers|UnbindEventfromOnRevived (LocalVariables|GetHealthComponent) (EventDispatchers|CreateEvent :!event Custom|PossessedPawnRevived)))))

(fn ShouldCursorsbeClampedtoHalfScreen
  (Utilities|FlowControl|Sequence
    (:then_0
      (if (not (Variables|Default|GetbIsSinglePlayerMode))
        (if (not (Class|GameplayStatics|IsSplitscreenForceDisabled))
          (Utilities|!!!IsNOTValid!!! (Variables|Default|GetBaseMenu)
            (:Is%20NOT%20Valid
              (return true))))))
    (:then_1
      (return false))))

(fn HandleKeyPressDetected
  (params (Key :type Key%20Structure%20%28by%20ref%29 :default "None"))
  (bind (_locationx _locationy) (Game|Player|GetMousePosition))
  (bind _returnvalue (Class|KismetInputLibrary|KeyIsGamepadKey Key))
  (if (!= _returnvalue (Variables|Default|GetbIsGamepad))
    (Variables|Default|SetbIsGamepad _returnvalue)
    (Utilities|FlowControl|Sequence
      (:then_0
        (Utilities|IsValid (Variables|Default|GetBaseMenu)
          (:Is%20Valid
            (Variables|Default|SetbShowMouseCursor (not (Variables|Default|GetbIsGamepad)))
            (Class|PlayerController|SetMouseLocation (Math|Float|Truncate _locationx) (Math|Float|Truncate _locationy)) ; Moving the mouse, even a tiny amount, after updating set show cursor seems \nto refresh the cursor, and make it more likely it hides when it should
            (if (Variables|Default|GetbIsGamepad)
              (Widget|SetFocus (Variables|Default|GetBaseMenu))))))
      (:then_1
        (Default|CallOnInputMethodChanged self (Variables|Default|GetbIsGamepad))))))

(fn GetCursorScreenPosition
  (Utilities|FlowControl|Sequence
    (:then_0
      (if (== (Class|GameplayStatics|GetPlayerControllerID self) 0)
        (bind _returnvalue (Class|WidgetLayoutLibrary|GetMousePositiononViewport))
        (Variables|Default|SetCurrentCursorPos (* _returnvalue (Class|WidgetLayoutLibrary|GetViewportScale)))))
    (:then_1
      (if (CallFunction|ShouldCursorsbeClampedtoHalfScreen)
        (if (== (Class|GameplayStatics|GetPlayerControllerID self) 0)
          (LocalVariables|SetOldX (.X (Math|Vector2D|BreakVector2D (Variables|Default|GetCurrentCursorPos))))
          (Variables|Default|SetCurrentCursorPos (Math|Vector2D|MakeVector2D (Math|Float|Min(Float) (LocalVariables|GetOldX) (* (.SizeX (HUD|GetViewportSize)) 0.5)) (.Y (Math|Vector2D|BreakVector2D (Variables|Default|GetCurrentCursorPos)))))
          (if (!= (LocalVariables|GetOldX) (.X (Math|Vector2D|BreakVector2D (Variables|Default|GetCurrentCursorPos))))
            (Class|PlayerController|SetMouseLocation (Math|Float|Truncate (.X (Math|Vector2D|BreakVector2D (Variables|Default|GetCurrentCursorPos)))) (Math|Float|Truncate (.Y (Math|Vector2D|BreakVector2D (Variables|Default|GetCurrentCursorPos))))))
          (else
            (Variables|Default|SetCurrentCursorPos (Math|Vector2D|MakeVector2D (Math|Float|Max(Float) (.X (Math|Vector2D|BreakVector2D (Variables|Default|GetCurrentCursorPos))) (* (.SizeX (HUD|GetViewportSize)) 0.5)) (.Y (Math|Vector2D|BreakVector2D (Variables|Default|GetCurrentCursorPos)))))))))
    (:then_2
      (return (Variables|Default|GetCurrentCursorPos)))))

(fn IsPlayerAlive
  (bind _returnvalue (Pawn|GetControlledPawn))
  (Utilities|IsValid _returnvalue
    (:Is%20Valid
      (bind _interfaceimplementingobject (CallFunction|SearchActorforInterface _returnvalue "/Game/EpicTemplates/TemplateAgnostic/Blueprints/Interfaces/BPI_HealthSource.BPI_HealthSource_C" false))
      (Utilities|IsValid _interfaceimplementingobject
        (:Is%20Valid
          (bind _bisdead (Class|BPIHealthSource|IsDead(Message) _interfaceimplementingobject))
          (return (not _bisdead)))
        (:Is%20Not%20Valid
          (return true))))
    (:Is%20Not%20Valid
      (return false))))