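; Camera target logic for a side-view character, producing a desired camera location on the Y/Z plane from the owner's position and movement component.
; On the ground it sits ahead along the expected Y direction, tolerating small backtracks and easing the side-swap offset by speed after a reversal.
; In the air it keeps its jump-start Y offset and shifts Z only past up/down thresholds, with velocity prediction.
; Targets are interpolated each update, with debug shapes exposed.
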(fn `Cleanup`
  (params (OwnerActor :type "Actor Object Reference") (OwningComponent :type "ActorComponent Object Reference"))
  (`|ExecutionSequence`
    (:`then_0`
      (`/Engine/EditorBlueprintResources/StandardMacros.IsValid` (`self.CharacterMovementComponent`)
        (:`Is Valid`
          (`ActorComponent.RemoveTickPrerequisiteComponent` OwningComponent (`self.CharacterMovementComponent`)))))
    (:`then_1`
      (set `self.OwnerActor` null))))

(fn `DebugValues`
  (params (DebugLines :type "Array of /Game/EpicTemplates/PlatformerTemplate/Blueprints/Structs/DebugLineStruct Structure (by ref)") (DebugArrows :type "Array of /Game/EpicTemplates/PlatformerTemplate/Blueprints/Structs/DebugLineStruct Structure (by ref)") (DebugSpheres :type "Array of /Game/EpicTemplates/PlatformerTemplate/Blueprints/Structs/DebugSphereStruct Structure (by ref)") (DebugStrings :type "Array of /Game/EpicTemplates/PlatformerTemplate/Blueprints/Structs/DebugStringStruct Structure (by ref)"))
  (locals (TempX :type "Float (double-precision)") (TempY :type "Float (double-precision)") (TempZ :type "Float (double-precision)"))
  (bind _tempz (`local.TempZ`))
  (bind _tempy (`local.TempY`))
  (bind _lastsafez (`self.LastSafeZ`))
  (bind _lastsafey (`self.LastSafeY`))
  (bind _returnvalue_x (`KismetMathLibrary.BreakVector` (`Actor.K2_GetActorLocation` (`self.OwnerActor`))))
  (bind _returnvalue (`KismetMathLibrary.MakeVector` (`local.TempX`) (`self.TargetDesiredY`) (`self.TargetDesiredZ`)))
  (bind _returnvalue_2 (`KismetMathLibrary.MakeVector` (`local.TempX`) (+ _tempy 1000.0) _lastsafez))
  (bind _returnvalue_3 (`KismetMathLibrary.MakeVector` (`local.TempX`) (- _tempy 1000.0) _lastsafez))
  (bind _returnvalue_4 (`KismetMathLibrary.MakeVector` _returnvalue_x (`self.CurrentDesiredY`) (`self.CurrentDesiredZ`)))
  (bind _returnvalue_5 (`KismetMathLibrary.MakeVector` (`local.TempX`) _lastsafey (+ _tempz 1000.0)))
  (bind _returnvalue_6 (`KismetMathLibrary.MakeVector` (`local.TempX`) _lastsafey (- _tempz 1000.0)))
  (bind _returnvalue_7 (* (+ _returnvalue_5 _returnvalue_6) 0.5))
  (set `local.TempX` (.x (`Actor.K2_GetActorLocation` (`self.OwnerActor`))))
  (set `local.TempY` (.y (`Actor.K2_GetActorLocation` (`self.OwnerActor`))))
  (set `local.TempZ` (.z (`Actor.K2_GetActorLocation` (`self.OwnerActor`))))
  (`KismetArrayLibrary.Array_Resize` (`local.DebugLines`) 2)
  (`KismetArrayLibrary.Array_Resize` (`local.DebugArrows`) 1)
  (`KismetArrayLibrary.Array_Resize` (`local.DebugSpheres`) 2)
  (`KismetArrayLibrary.Array_Resize` (`local.DebugStrings`) 4)
  (`KismetArrayLibrary.Array_Set` (`local.DebugSpheres`) 0 (make `/Game/EpicTemplates/PlatformerTemplate/Blueprints/Structs/DebugSphereStruct` _returnvalue_4 20.0 (struct :`G` 1.0 :`A` 1.0)))
  (`KismetArrayLibrary.Array_Set` (`local.DebugStrings`) 0 (make `/Game/EpicTemplates/PlatformerTemplate/Blueprints/Structs/DebugStringStruct` _returnvalue_4 "Current Desired location" (struct :`R` 1.0 :`G` 1.0 :`B` 1.0 :`A` 1.0)))
  (`KismetArrayLibrary.Array_Set` (`local.DebugSpheres`) 1 (make `/Game/EpicTemplates/PlatformerTemplate/Blueprints/Structs/DebugSphereStruct` _returnvalue 25.0 (struct :`R` 1.0 :`G` 0.5 :`A` 1.0)))
  (`KismetArrayLibrary.Array_Set` (`local.DebugStrings`) 1 (make `/Game/EpicTemplates/PlatformerTemplate/Blueprints/Structs/DebugStringStruct` _returnvalue "Target Desired location" (struct :`R` 1.0 :`G` 1.0 :`B` 1.0 :`A` 1.0)))
  (`KismetArrayLibrary.Array_Set` (`local.DebugLines`) 0 (make `/Game/EpicTemplates/PlatformerTemplate/Blueprints/Structs/DebugLineStruct` _returnvalue_5 _returnvalue_6 (struct :`G` 1.0 :`A` 1.0)))
  (`KismetArrayLibrary.Array_Set` (`local.DebugStrings`) 2 (make `/Game/EpicTemplates/PlatformerTemplate/Blueprints/Structs/DebugStringStruct` _returnvalue_7 "Last Safe Y" (struct :`R` 1.0 :`G` 1.0 :`B` 1.0 :`A` 1.0)))
  (`KismetArrayLibrary.Array_Set` (`local.DebugArrows`) 0 (make `/Game/EpicTemplates/PlatformerTemplate/Blueprints/Structs/DebugLineStruct` _returnvalue_7 (+ _returnvalue_7 (`KismetMathLibrary.MakeVector` 0.0 (* (`self.ExpectedMoveDirection`) 200.0))) (struct :`G` 1.0 :`A` 1.0)))
  (`KismetArrayLibrary.Array_Set` (`local.DebugLines`) 1 (make `/Game/EpicTemplates/PlatformerTemplate/Blueprints/Structs/DebugLineStruct` _returnvalue_3 _returnvalue_2 (struct :`G` 1.0 :`B` 1.0 :`A` 1.0)))
  (`KismetArrayLibrary.Array_Set` (`local.DebugStrings`) 3 (make `/Game/EpicTemplates/PlatformerTemplate/Blueprints/Structs/DebugStringStruct` (* (+ _returnvalue_3 _returnvalue_2) 0.5) "Last Safe Z" (struct :`R` 1.0 :`G` 1.0 :`B` 1.0 :`A` 1.0)))
  (return))

(fn `Setup`
  (params (InOwnerActor :type "Actor Object Reference") (InOwningComponent :type "ActorComponent Object Reference"))
  (`|ExecutionSequence`
    (:`then_0`
      (set `self.OwnerActor` InOwnerActor)
      (bind _output_get (set `self.CharacterMovementComponent` (`Actor.GetComponentByClass` (`self.OwnerActor`) "/Script/Engine.CharacterMovementComponent")))
      (`/Engine/EditorBlueprintResources/StandardMacros.IsValid` _output_get
        (:`Is Valid`
          (`ActorComponent.AddTickPrerequisiteComponent` InOwningComponent (`self.CharacterMovementComponent`)))))
    (:`then_1`
      (bind _output_get_2 (set `self.LastSafeY` (.y (`Actor.K2_GetActorLocation` (`local.InOwnerActor`)))))
      (bind _output_get_3 (set `self.TargetDesiredY` _output_get_2))
      (set `self.CurrentDesiredY` _output_get_3)
      (bind _output_get_4 (set `self.LastSafeZ` (.z (`Actor.K2_GetActorLocation` (`local.InOwnerActor`)))))
      (bind _output_get_5 (set `self.TargetDesiredZ` _output_get_4))
      (set `self.CurrentDesiredZ` _output_get_5))))

(fn `Update Data and Targets`
  (params (DeltaSeconds :type "Float (double-precision)"))
  (locals (TempYVel :type "Float (double-precision)") (TempZVel :type "Float (double-precision)") (TempZ :type "Float (double-precision)") (TempY :type "Float (double-precision)"))
  (bind _tempyvel (`local.TempYVel`))
  (set `local.TempY` (.y (`Actor.K2_GetActorLocation` (`self.OwnerActor`))))
  (set `local.TempZ` (.z (`Actor.K2_GetActorLocation` (`self.OwnerActor`))))
  (`/Engine/EditorBlueprintResources/StandardMacros.IsValid` (`self.CharacterMovementComponent`)
    (:`Is Valid`
      (set `local.TempYVel` (.y (`CharacterMovementComponent.GetLastUpdateVelocity` (`self.CharacterMovementComponent`))))
      (set `local.TempZVel` (.z (`CharacterMovementComponent.GetLastUpdateVelocity` (`self.CharacterMovementComponent`))))
      (`|ExecutionSequence`
        (:`then_0`
          (if (`NavMovementComponent.IsFalling` (`self.CharacterMovementComponent`))
            ;[1 1 1] In-air
            (`|ExecutionSequence`
              (:`then_0`
                (if (not (`self.bWasFalling`))
                  (set `self.CameraYOffsetAtJumpStart` (- (`self.CurrentDesiredY`) (`local.TempY`)))))
              (:`then_1`
                (`|ExecutionSequence`
                  (:`then_0`
                    (if (> (- (`local.TempZ`) (`self.LastSafeZ`)) (`self.FollowZUpThreshold`))
                      (set `self.TargetDesiredZ` (+ (- (`local.TempZ`) (`self.FollowZUpThreshold`)) (* (`self.ZVelocityPredictionMultiplier`) (`local.TempZVel`))))
                      (elif (< (- (`local.TempZ`) (`self.LastSafeZ`)) (* (`self.FollowZDownThreshold`) -1.0))
                        (set `self.TargetDesiredZ` (+ (`local.TempZ`) (`self.FollowZDownThreshold`) (* (`self.ZVelocityPredictionMultiplier`) (`local.TempZVel`)))))))
                  (:`then_1`
                    (set `self.TargetDesiredY` (+ (`local.TempY`) (`self.CameraYOffsetAtJumpStart`) (* (`self.YVelocityPredictionMultiplier`) (`local.TempYVel`))))
                    (set `self.LastSafeY` (- (`local.TempY`) (`self.LastOffsetFromSafeY`)))))))
            (else
              ;[1 1 1] On ground
              (`|ExecutionSequence`
                (:`then_0`
                  (bind _output_get (set `self.LastSafeZ` (`local.TempZ`)))
                  (set `self.TargetDesiredZ` _output_get))
                (:`then_1`
                  (`|ExecutionSequence`
                    (:`then_0`
                      (bind _output_get_2 (set `self.LastOffsetFromSafeY` (- (`local.TempY`) (`self.LastSafeY`))))
                      (if (== (* (`KismetMathLibrary.SignOfFloat` _output_get_2) (`self.ExpectedMoveDirection`)) -1.0)
                        (if (> (`KismetMathLibrary.Abs` (`self.LastOffsetFromSafeY`)) (`self.YBacktrackThreshold`))
                          (set `self.ExpectedMoveDirection` (`KismetMathLibrary.SignOfFloat` (`self.LastOffsetFromSafeY`)))
                          (set `self.SwapSideOffset` (- (`self.CurrentDesiredY`) (+ (`local.TempY`) (* (`self.ExpectedMoveDirection`) (`self.SitAheadOfPlayerYDistance`)))))
                          (set `self.bBackTracking` false)
                          (else
                            (set `self.bBackTracking` true)))
                        (else
                          (set `self.bBackTracking` false))))
                    (:`then_1`
                      (if (`self.bBackTracking`)
                        (set `self.TargetDesiredY` (+ (`self.LastSafeY`) (* (`self.ExpectedMoveDirection`) (`self.SitAheadOfPlayerYDistance`)) (`self.SwapSideOffset`)))
                        (else
                          (set `self.SwapSideOffset` (`KismetMathLibrary.FInterpTo_Constant` (`self.SwapSideOffset`) 0.0 (`local.DeltaSeconds`) (`KismetMathLibrary.SelectFloat` (* (`KismetMathLibrary.Abs` _tempyvel) (`self.SafeYSwitchSideVelocityMultiplier`)) 0.0 (== (`KismetMathLibrary.SignOfFloat` _tempyvel) (* (`KismetMathLibrary.SignOfFloat` (`self.SwapSideOffset`)) -1.0)))))
                          (set `self.LastSafeY` (`local.TempY`))
                          (set `self.TargetDesiredY` (+ (`self.LastSafeY`) (* (`self.ExpectedMoveDirection`) (`self.SitAheadOfPlayerYDistance`)) (* (`local.TempYVel`) (`self.YVelocityPredictionMultiplier`)) (`self.SwapSideOffset`))))))))))))
        (:`then_1`
          (set `self.bWasFalling` (`NavMovementComponent.IsFalling` (`self.CharacterMovementComponent`))))))
    (:`Is Not Valid`
      ;[1 1 1] No Move Component
      (set `self.LastSafeZ` (`local.TempZ`))
      (set `self.LastSafeY` (`local.TempY`))
      (set `self.TargetDesiredZ` (`local.TempZ`))
      (set `self.TargetDesiredY` (`local.TempY`)))))

(fn `Update Logic`
  (params (DeltaSeconds :type "Float (double-precision)"))
  (returns (DesiredLocation :type "Vector Structure") (DesiredViewPlaneWidth :type "Float (double-precision)"))
  (`self.Update Data and Targets` DeltaSeconds)
  (set `self.CurrentDesiredZ` (`KismetMathLibrary.FInterpTo` (`self.CurrentDesiredZ`) (`self.TargetDesiredZ`) DeltaSeconds (`self.DesiredZInterpSpeed`)))
  (set `self.CurrentDesiredY` (`KismetMathLibrary.FInterpTo` (`self.CurrentDesiredY`) (`self.TargetDesiredY`) DeltaSeconds (`self.DesiredYInterpSpeed`)))
  (`parent.Update Logic` (`local.DeltaSeconds`))
  (return (`KismetMathLibrary.MakeVector` (.x (`Actor.K2_GetActorLocation` (`self.OwnerActor`))) (`self.CurrentDesiredY`) (`self.CurrentDesiredZ`)) (`self.CurrentDesiredPlaneWidth`)))