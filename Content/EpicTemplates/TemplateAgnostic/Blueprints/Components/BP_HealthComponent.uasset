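; Health component that tracks an actor's health and max health, applies damage, and handles death, revival, invincibility and instant kills.
; Damage is scaled by a multiplier from the owner's damage modifier interface, then took-damage is broadcast before died so reactions run first.
; On death, the owner's score source can add to or subtract from the killer's score storage, with a double modifier for headshots.
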(event `EnableInvincibility`
  (set `self.bIgnoreDamage` true))

(event `self.ReceiveBeginPlay`
  ;[1 1 1] Begin Play
  (`self.UpdateMaxHealth_Internal` (`self.StartMaxHealth`))
  (`self.UpdateHealth_Internal` (`self.StartHealth`)))

(event `DisableInvincibility`
  (set `self.bIgnoreDamage` false))

(event `/Game/EpicTemplates/TemplateAgnostic/Blueprints/Interfaces/BPI_HealthSource.UpdateHealth`
  (params (NewHealth :type "Float (double-precision)"))
  ;[0 0.9651 1] BPi_Health
  (`self.UpdateHealth_Internal` NewHealth))

(event `/Game/EpicTemplates/TemplateAgnostic/Blueprints/Interfaces/BPI_HealthSource.UpdateMaxHealth`
  (params (NewMaxHealth :type "Float (double-precision)"))
  ;[0 0.9651 1] BPi_Health
  (`self.UpdateMaxHealth_Internal` NewMaxHealth))

(event `/Game/EpicTemplates/TemplateAgnostic/Blueprints/Interfaces/BPI_HealthSource.Revive`
  (params (ReviveSource :type "Actor Object Reference") (ReviveHealthBehaviour :type "/Game/EpicTemplates/TemplateAgnostic/Blueprints/Enums/EReviveHealthBehaviour Enum" :default "NewEnumerator0"))
  ;[0 0.9651 1] BPi_Health
  (bind _bisdead (`self.IsDead`))
  (if _bisdead
    (`|ExecutionSequence`
      (:`then_0`
        (switch `/Game/EpicTemplates/TemplateAgnostic/Blueprints/Enums/EReviveHealthBehaviour` ReviveHealthBehaviour
          (:`NewEnumerator0`
            (`self.UpdateHealth_Internal` (`self.MaxHealth`)))
          (:`NewEnumerator1`
            (`self.UpdateHealth_Internal` 1.0))))
      (:`then_1`
        (`self.OnRevived` self ReviveSource)))))

(fn `ApplyDamage`
  (params (InDamage :type "/Game/EpicTemplates/TemplateAgnostic/Blueprints/Structs/DamageStruct Structure (by ref)"))
  (returns (DamageDealt :type "Float (double-precision)") (DamageApplied :type Boolean))
  (locals (DamageMultiplier :type "Float (double-precision)") (OldHealth :type "Float (double-precision)") (OldIsDead :type Boolean) (DamageModifierName :type Name) (bHasDied :type Boolean) (ScoreSourceObject :type "Object Object Reference") (ScoreStorageObject :type "Object Object Reference") (OldHealth :type "Float (double-precision)") (OldIsDead :type Boolean) (DamageMultiplier :type "Float (double-precision)") (SpecialDamageName :type Name) (InDamage :type "/Game/EpicTemplates/TemplateAgnostic/Blueprints/Structs/DamageStruct Structure (by ref)") (bHasDied :type Boolean) (ScoreSourceObject :type "Object Object Reference") (ScoreStorageObject :type "Object Object Reference"))
  (bind ((`DamageSource_5_8780F30649675B7DF1FC5694BCAD2A7E` _damagesource) (`DamageSourceOwner_16_93F98FB747ED83B90B1FAFB49CE3E4D5` _damagesourceowner) (`DamageLocation_8_F5A6C21543470034EA0BD6945175CC5B` _damagelocation) (`DamageDirection_20_DE80E36A475894D4B74BC0909E89EF39` _damagedirection) (`HitBone_19_E692A9A64588FB8A77B34DA43E2451A2` _hitbone)) (break `/Game/EpicTemplates/TemplateAgnostic/Blueprints/Structs/DamageStruct` (`local.InDamage`)))
  (if (`self.bIgnoreDamage`)
    (return 0.0 false)
    (else
      (set `local.OldHealth` (`self.Health`))
      (bind _bisdead (`/Game/EpicTemplates/TemplateAgnostic/Blueprints/Interfaces/BPI_HealthSource.IsDead` self))
      (set `local.OldIsDead` _bisdead)
      (`|ExecutionSequence`
        (:`then_0`
          ;[1 1 1] Check for damage modifiers
          (if (`KismetSystemLibrary.DoesImplementInterface` (`self.GetOwner`) "/Game/EpicTemplates/RailShooterTemplate/Blueprints/Interfaces/BPI_DamageModifierImplementor.BPI_DamageModifierImplementor_C")
            (bind (_multiplier _damagemodifiername) (message `/Game/EpicTemplates/RailShooterTemplate/Blueprints/Interfaces/BPI_DamageModifierImplementor.CheckForDamageModifiers` (`self.GetOwner`) (`local.InDamage`)))
            (set `local.DamageMultiplier` _multiplier)
            (set `local.DamageModifierName` _damagemodifiername)
            (else
              (set `local.DamageMultiplier` 1.0)
              (set `local.DamageModifierName` "None"))))
        (:`then_1`
          ;[1 1 1] Change health based on damage
          (set `self.Health` (- (`self.Health`) (* (`local.DamageMultiplier`) (`.Damage_11_4BDBE22E4671030D7F6B5BBB0A6FB960` (break `/Game/EpicTemplates/TemplateAgnostic/Blueprints/Structs/DamageStruct` (`local.InDamage`)))))))
        (:`then_2`
          ;[1 1 1] Check for has died from this damage
          (bind _bisdead_2 (`/Game/EpicTemplates/TemplateAgnostic/Blueprints/Interfaces/BPI_HealthSource.IsDead` self))
          (if (and _bisdead_2 (not (`local.OldIsDead`)))
            (set `local.bHasDied` true)
            (`self.HandledHasDied` (`local.InDamage`) (`local.DamageModifierName`))))
        (:`then_3`
          ;[1 1 1] Always call took damage, even if we also died.
          ; For damage reaction behaviour, we call OnTookDamage before calling OnDied
          (`self.OnTookDamage` self (`local.OldHealth`) (`self.Health`) (`local.DamageModifierName`) (`local.InDamage`))
          (if (`local.bHasDied`)
            (`self.OnDied` self _damagesourceowner _damagesource _damagelocation _damagedirection _hitbone (`local.DamageModifierName`))))
        (:`then_4`
          (return (* (`local.DamageMultiplier`) (`.Damage_11_4BDBE22E4671030D7F6B5BBB0A6FB960` (break `/Game/EpicTemplates/TemplateAgnostic/Blueprints/Structs/DamageStruct` (`local.InDamage`)))) true))))))

(fn `GetCurrentHealth`
  (returns (CurrentHealth :type "Float (double-precision)"))
  (return (`self.Health`)))

(fn `GetMaxHealth`
  (returns (MaxHealth :type "Float (double-precision)"))
  (return (`self.MaxHealth`)))

(fn `HandledHasDied`
  (params (InDamage :type "/Game/EpicTemplates/TemplateAgnostic/Blueprints/Structs/DamageStruct Structure (by ref)") (DamageModifierName :type Name))
  (locals (ScoreStorageObject :type "Object Object Reference") (ScoreSourceObject :type "Object Object Reference"))
  (if (`|EnumInequality` (`self.DeathScoreBehaviour`) "NewEnumerator0")
    (bind (_interfaceimplementingobject _foundimplementingobject) (`/Game/EpicTemplates/TemplateAgnostic/Blueprints/EpicTemplatesFunctionLibrary.SearchActorForInterface` (`self.GetOwner`) "/Game/EpicTemplates/TemplateAgnostic/Blueprints/Interfaces/BPI_GameScoreSource.BPI_GameScoreSource_C"))
    (set `local.ScoreSourceObject` _interfaceimplementingobject)
    (if _foundimplementingobject
      (bind (_interfaceimplementingobject_2 _foundimplementingobject_2) (`/Game/EpicTemplates/TemplateAgnostic/Blueprints/EpicTemplatesFunctionLibrary.SearchActorForInterface` (`.DamageSourceOwner_16_93F98FB747ED83B90B1FAFB49CE3E4D5` (break `/Game/EpicTemplates/TemplateAgnostic/Blueprints/Structs/DamageStruct` (`local.InDamage`))) "/Game/EpicTemplates/TemplateAgnostic/Blueprints/Interfaces/BPI_GameScoreStorage.BPI_GameScoreStorage_C"))
      (set `local.ScoreStorageObject` _interfaceimplementingobject_2)
      (if _foundimplementingobject_2
        (`|ExecutionSequence`
          (:`then_0`
            (switch `name` (`local.DamageModifierName`)
              (:`Headshot`
                (message `/Game/EpicTemplates/TemplateAgnostic/Blueprints/Interfaces/BPI_GameScoreSource.AddModifier` (`local.ScoreSourceObject`) (make `/Game/EpicTemplates/TemplateAgnostic/Blueprints/Structs/ScoreModifierStruct` "Headshot" 2.0)))))
          (:`then_1`
            (bind _asbpi_game_score_source (cast `/Game/EpicTemplates/TemplateAgnostic/Blueprints/Interfaces/BPI_GameScoreSource` (`local.ScoreSourceObject`)))
            (switch `/Game/EpicTemplates/TemplateAgnostic/Blueprints/Enums/EDeathScoreBehaviour` (`self.DeathScoreBehaviour`)
              (:`NewEnumerator1`
                (message `/Game/EpicTemplates/TemplateAgnostic/Blueprints/Interfaces/BPI_GameScoreStorage.AddScore` (`local.ScoreStorageObject`) _asbpi_game_score_source))
              (:`NewEnumerator2`
                (message `/Game/EpicTemplates/TemplateAgnostic/Blueprints/Interfaces/BPI_GameScoreStorage.SubtractScore` (`local.ScoreStorageObject`) _asbpi_game_score_source)))))))))

(fn `InstantKill`
  (params (KillDamageInfo :type "/Game/EpicTemplates/TemplateAgnostic/Blueprints/Structs/DamageStruct Structure"))
  (returns (KillAccepted :type Boolean) (DamageDealt :type "Float (double-precision)"))
  (locals (WasIgnoringDamage :type Boolean :default false))
  (bind (_killdamageinfo_damage _killdamageinfo_damagesource _killdamageinfo_damagesourceowner _killdamageinfo_damagelocation _killdamageinfo_damagedirection _killdamageinfo_hitbone) (break `/Game/EpicTemplates/TemplateAgnostic/Blueprints/Structs/DamageStruct` (`local.KillDamageInfo`)))
  (if (`self.bCanInstantKill`)
    (set `local.WasIgnoringDamage` (`self.bIgnoreDamage`))
    (set `self.bIgnoreDamage` false)
    (bind _damagedealt (`/Game/EpicTemplates/TemplateAgnostic/Blueprints/Interfaces/BPI_Damageable.ApplyDamage` (make `/Game/EpicTemplates/TemplateAgnostic/Blueprints/Structs/DamageStruct` (`self.Health`) _killdamageinfo_damagesource _killdamageinfo_damagesourceowner _killdamageinfo_damagelocation _killdamageinfo_damagedirection _killdamageinfo_hitbone)))
    (set `self.bIgnoreDamage` (`local.WasIgnoringDamage`))
    (return true _damagedealt)
    (else
      (bind _damagedealt_2 (`/Game/EpicTemplates/TemplateAgnostic/Blueprints/Interfaces/BPI_Damageable.ApplyDamage` KillDamageInfo))
      (return false _damagedealt_2))))

(fn `IsDead`
  (returns (bIsDead :type Boolean))
  (return (<= (`self.Health`) 0.0)))

(fn `UpdateHealth_Internal`
  (params (NewHealth :type "Float (double-precision)"))
  (locals (OldHealth :type "Float (double-precision)"))
  (set `local.OldHealth` (`self.Health`))
  (bind _output_get (set `self.Health` (`KismetMathLibrary.FMin` NewHealth (`self.MaxHealth`))))
  (if (!= _output_get (`local.OldHealth`))
    (`self.OnHealthUpdated` self 0.0 _output_get)))

(fn `UpdateMaxHealth_Internal`
  (params (NewMaxHealth :type "Float (double-precision)"))
  (locals (OldMaxHealth :type "Float (double-precision)" :default 0.0))
  (set `local.OldMaxHealth` (`self.MaxHealth`))
  (bind _output_get (set `self.MaxHealth` NewMaxHealth))
  (if (!= _output_get (`local.OldMaxHealth`))
    (`self.OnMaxHealthUpdated` null (`local.OldMaxHealth`) (`self.MaxHealth`))))