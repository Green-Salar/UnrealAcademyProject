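; Actor component that spawns a requested quantity of a soft-referenced Actor class in random-sized batches, on a looping timer or all at once when frequency is zero.
; LoadClass async-loads and caches the class, while DirectSpawn falls back to a blocking load if needed.
; Spawn transforms come from the owner's BPI_SpawnPoint interface or its actor transform.
; Spawns optionally use actor recycling, and callbacks report loading, each spawn and completion.
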(event `self.ReceiveBeginPlay`
  (bind _asbpi_spawn_point (cast `/Game/EpicTemplates/RailShooterTemplate/Blueprints/Interfaces/BPI_SpawnPoint` (`self.GetOwner`)))
  (set `self.OwnerSpawnPointInterface` _asbpi_spawn_point))

(event `LoadClass`
  (params (ClassToLoad :type "Actor Soft Class Reference"))
  (if (!= ClassToLoad (`|ConvertAsset` (`self.LoadedActorClass`)))
    (set `self.LoadedActorClass` null)
    (bind _output_get (set `self.ActorClassToLoad` ClassToLoad))
    (bind _class (`|LoadAssetClass` _output_get)
      (:`Completed`
        (bind _asactor (castclass `Actor` _class))
        (bind _output_get_2 (set `self.LoadedActorClass` _asactor))
        (`self.OnFinishedLoadingClass` self _output_get_2)))
    (else
      (`self.OnFinishedLoadingClass` self (`self.LoadedActorClass`)))))

(event `StartSpawning`
  (params (QuantityToSpawn :type Integer) (MinSimulaneousSpawnCount :type Integer) (MaxSimultaneousSpawnCount :type Integer) (SpawnFrequency :type "Float (double-precision)"))
  (set `self.QuantityLeftToSpawn` QuantityToSpawn)
  (set `self.Min Simulaneous Spawn Count` MinSimulaneousSpawnCount)
  (set `self.Max Simultaneous Spawn Count` MaxSimultaneousSpawnCount)
  (set `self.SpawnFrequency` SpawnFrequency)
  (`self.ResumeSpawning`))

(event `StopSpawning`
  (params (bClearAmountLeftToSpawn :type Boolean) (bClearLoadedClass :type Boolean))
  (set `self.bIsSpawning` false)
  (`KismetSystemLibrary.K2_ClearAndInvalidateTimerHandle` (`self.SpawnTimerHandle`))
  (`|ExecutionSequence`
    (:`then_0`
      (if bClearAmountLeftToSpawn
        (set `self.QuantityLeftToSpawn` 0)))
    (:`then_1`
      (if bClearLoadedClass
        (`self.EmptyLoadedCache`)))))

(event `ResumeSpawning`
  (set `self.bIsSpawning` true)
  (if (and (> (`self.QuantityLeftToSpawn`) 0) (`KismetSystemLibrary.IsValidClass` (`self.LoadedActorClass`)))
    (if (`self.bFirstSpawnInstantaneous`)
      (`self.SpawnNextBatch`)
      (if (> (`self.QuantityLeftToSpawn`) 0)
        (if (> (`self.SpawnFrequency`) 0.0) :!label _label
          (bind _returnvalue (`KismetSystemLibrary.K2_SetTimerDelegate` (`|CreateDelegate` :!event `SpawnNextBatch`) (`self.SpawnFrequency`) true))
          (set `self.SpawnTimerHandle` _returnvalue)
          (else
            (`self.SpawnNextBatch`))))
      (else
        (goto _label)))))

(fn `DirectSpawn`
  (params (SpawnTransform :type "Transform Structure (by ref)") (InOwner :type "Actor Object Reference") (InInstigator :type "Pawn Object Reference"))
  (returns (ActorInstance :type "Actor Object Reference"))
  (`|ExecutionSequence`
    (:`then_0`
      (if (and (`KismetSystemLibrary.IsValidSoftClassReference` (`self.ActorClassToLoad`)) (not (`KismetSystemLibrary.IsValidClass` (`self.LoadedActorClass`))))
        (bind _returnvalue (`KismetSystemLibrary.LoadClassAsset_Blocking` (`self.ActorClassToLoad`)))
        (bind _asactor (castclass `Actor` _returnvalue))
        (set `self.LoadedActorClass` _asactor)))
    (:`then_1`
      (if (`self.bTryUseActorRecyclerForSpawns`)
        (bind _actorinstance (`/Game/EpicTemplates/TemplateAgnostic/Blueprints/EpicTemplatesFunctionLibrary.SpawnReusableActorFromClass` (`self.LoadedActorClass`) (`local.SpawnTransform`) (`local.InOwner`) (`local.InInstigator`)))
        (return _actorinstance)
        (else
          (bind _returnvalue_2 (`|SpawnActorFromClass` (`self.LoadedActorClass`) (`local.SpawnTransform`) "AlwaysSpawn" "MultiplyWithRoot" (`local.InOwner`) (`local.InInstigator`)))
          (return _returnvalue_2))))))

(fn `EmptyLoadedCache`
  (set `self.ActorClassToLoad` null)
  (if (not (`KismetSystemLibrary.K2_IsTimerActiveHandle` (`self.SpawnTimerHandle`)))
    (set `self.LoadedActorClass` null)))

(fn `GetLoadedClass`
  (returns (LoadedClass :type "Actor Class Reference") (bIsLoaded :type Boolean))
  (if (`KismetSystemLibrary.IsValidClass` (`self.LoadedActorClass`))
    (return (`self.LoadedActorClass`) true)
    (else
      (return null false))))

(fn `GetSpawnerIndex`
  (returns (LoaderIndex :type Integer))
  (return (`self.SpawnerIndex`)))

(fn `GetSpawnTrans`
  (returns (SpawnTrans :type "Transform Structure"))
  (if (`KismetSystemLibrary.IsValidInterface` (`self.OwnerSpawnPointInterface`))
    (bind _spawntransform (`/Game/EpicTemplates/RailShooterTemplate/Blueprints/Interfaces/BPI_SpawnPoint.GetSpawnTransform` (`self.OwnerSpawnPointInterface`)))
    (return _spawntransform)
    (else
      (return (`Actor.GetTransform` (`self.GetOwner`))))))

(fn `IsStillLoading`
  (returns (IsLoaded :type Boolean))
  (return (and (`KismetSystemLibrary.IsValidSoftClassReference` (`self.ActorClassToLoad`)) (not (`KismetSystemLibrary.IsValidClass` (`self.LoadedActorClass`))))))

(fn `IsStillSpawning`
  (returns (StillSpawning :type Boolean))
  (return (and (`KismetSystemLibrary.K2_IsTimerActiveHandle` (`self.SpawnTimerHandle`)) (> (`self.QuantityLeftToSpawn`) 0))))

(fn `SpawnNextBatch`
  (locals (AmountToSpawn :type Integer :default 0))
  (`|ExecutionSequence`
    (:`then_0`
      (set `local.AmountToSpawn` (`KismetMathLibrary.Min` (`KismetMathLibrary.RandomIntegerInRange` (`self.Min Simulaneous Spawn Count`) (`self.Max Simultaneous Spawn Count`)) (`self.QuantityLeftToSpawn`)))
      (for _ (range (`local.AmountToSpawn`))
        (bind _actorinstance (`self.DirectSpawn` (`self.GetSpawnTrans`) (`self.GetOwner`)))
        (`self.OnSpawnedActor` self _actorinstance)))
    (:`then_1`
      (bind _outintcopy (`/Game/EpicTemplates/TemplateAgnostic/Blueprints/EpicTemplatesFunctionLibrary.MinusEqualsInt` (`self.QuantityLeftToSpawn`) (`local.AmountToSpawn`)))
      (if (<= _outintcopy 0)
        (`KismetSystemLibrary.K2_ClearAndInvalidateTimerHandle` (`self.SpawnTimerHandle`))
        (`self.OnFinishedSpawning` self)
        (elif (<= (`self.SpawnFrequency`) 0.0)
          (`self.SpawnNextBatch`))))))