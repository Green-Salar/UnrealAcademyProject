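; Camera target component that supplies a desired camera location, view plane width and owner root bounds.
; It delegates to a swappable logic object built from a class, cleaning up the old one when the class changes.
; Each tick it caches that logic's output for its getters and, in debug, draws the logic's lines, arrows, spheres and strings.
; It also tracks which camera currently targets it.
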(event `self.ReceiveBeginPlay`
  (`self.UpdateTargetLogic` (`self.DefaultCameraTargetLogic`))
  (`/Game/EpicTemplates/TemplateAgnostic/Blueprints/CameraTargetLogics/BP_CameraTargetLogicBase.UpdateDesiredPlaneWidth` (`self.CurrentCameraTargetLogic`) (`self.StartDesiredPlaneWidth`) "NewEnumerator1")
  (set `self.CurrentDesiredPlaneWidth` (`self.StartDesiredPlaneWidth`)))

(event `self.ReceiveTick`
  (params (DeltaSeconds :type "Float (single-precision)"))
  (bind (_desiredlocation _desiredviewplanewidth) (`/Game/EpicTemplates/TemplateAgnostic/Blueprints/CameraTargetLogics/BP_CameraTargetLogicBase.Update Logic` (`self.CurrentCameraTargetLogic`) DeltaSeconds))
  (set `self.CurrentDesiredX` (.x _desiredlocation))
  (set `self.CurrentDesiredY` (.y _desiredlocation))
  (set `self.CurrentDesiredZ` (.z _desiredlocation))
  (set `self.CurrentDesiredPlaneWidth` _desiredviewplanewidth)
  (if (`self.IsInDebug`)
    (`/Game/EpicTemplates/TemplateAgnostic/Blueprints/CameraTargetLogics/BP_CameraTargetLogicBase.DebugValues` (`self.CurrentCameraTargetLogic`) (`self.DebugLines`) (`self.Debug Arrows`) (`self.Debug Spheres`) (`self.Debug Strings`))
    (`|ExecutionSequence`
      (:`then_0`
        (for _array_element (`self.DebugLines`)
          (bind (_start _end _color) (break `/Game/EpicTemplates/PlatformerTemplate/Blueprints/Structs/DebugLineStruct` _array_element))
          (`KismetSystemLibrary.DrawDebugLine` _start _end _color)))
      (:`then_1`
        (for _array_element_2 (`self.Debug Arrows`)
          (bind (_start_2 _end_2 _color_2) (break `/Game/EpicTemplates/PlatformerTemplate/Blueprints/Structs/DebugLineStruct` _array_element_2))
          (`KismetSystemLibrary.DrawDebugLine` _start_2 _end_2 _color_2)))
      (:`then_2`
        (for _array_element_3 (`self.Debug Spheres`)
          (bind (_loc _radius _color_3) (break `/Game/EpicTemplates/PlatformerTemplate/Blueprints/Structs/DebugSphereStruct` _array_element_3))
          (`KismetSystemLibrary.DrawDebugSphere` _loc _radius 12 _color_3)))
      (:`then_3`
        (for _array_element_4 (`self.Debug Strings`)
          (bind (_location _string _color_4) (break `/Game/EpicTemplates/PlatformerTemplate/Blueprints/Structs/DebugStringStruct` _array_element_4))
          (`KismetSystemLibrary.DrawDebugString` _location _string null _color_4))))))

(event `/Game/EpicTemplates/TemplateAgnostic/Blueprints/Interfaces/BPI_Debuggable.UpdateIsInDebug`
  (params (bInIsDebug :type Boolean))
  (set `self.IsInDebug` bInIsDebug))

(event `/Game/EpicTemplates/PlatformerTemplate/Blueprints/Interfaces/BPI_CameraTarget.UpdateDesiredPlaneWidth`
  (params (NewDesiredPlaneWidth :type "Float (double-precision)") (UpdateType :type "/Game/EpicTemplates/PlatformerTemplate/Blueprints/Enums/EUpdateDesiredPlaneWidthType Enum" :default "NewEnumerator0"))
  (`/Game/EpicTemplates/TemplateAgnostic/Blueprints/CameraTargetLogics/BP_CameraTargetLogicBase.UpdateDesiredPlaneWidth` (`self.CurrentCameraTargetLogic`) NewDesiredPlaneWidth UpdateType))

(event `/Game/EpicTemplates/PlatformerTemplate/Blueprints/Interfaces/BPI_CameraTarget.StartedBeingTargetedByCamera`
  (params (NewTargetingCamera :type "Actor Object Reference"))
  (set `self.CurrentTargetingCamera` NewTargetingCamera))

(event `/Game/EpicTemplates/PlatformerTemplate/Blueprints/Interfaces/BPI_CameraTarget.StoppedBeingTargetedByCamera`
  (params (NewTargetingCamera :type "Actor Object Reference"))
  (if (== NewTargetingCamera (`self.CurrentTargetingCamera`))
    (set `self.CurrentTargetingCamera` null)))

(fn `GetCurrentTargetingCamera`
  (returns (TargetingCameraActor :type "Actor Object Reference"))
  (return (`self.CurrentTargetingCamera`)))

(fn `GetDesiredCameraLoc`
  (returns (DesiredLocation :type "Vector Structure"))
  (return (`KismetMathLibrary.MakeVector` (`self.CurrentDesiredX`) (`self.CurrentDesiredY`) (`self.CurrentDesiredZ`))))

(fn `GetDesiredCameraViewPlaneWidth`
  (returns (DesiredViewPlaneWidth :type "Float (double-precision)"))
  (return (`self.CurrentDesiredPlaneWidth`)))

(fn `GetIsInDebug`
  (returns (bIsInDebug :type Boolean))
  (return (`self.IsInDebug`)))

(fn `GetMinimumViewBounds`
  (returns (BoundsCentre :type "Vector Structure") (BoundsExtents :type "Vector Structure"))
  (bind (_origin _boxextent) (`KismetSystemLibrary.GetComponentBounds` (`Actor.RootComponent` (`self.GetOwner`))))
  (return _origin _boxextent))

(fn `UpdateTargetLogic`
  (params (NewLogicClass :type "/Game/EpicTemplates/TemplateAgnostic/Blueprints/CameraTargetLogics/BP_CameraTargetLogicBase Class Reference"))
  (if (`KismetSystemLibrary.IsValidClass` NewLogicClass)
    (`|ExecutionSequence`
      (:`then_0`
        (`/Engine/EditorBlueprintResources/StandardMacros.IsValid` (`self.CurrentCameraTargetLogic`)
          (:`Is Valid`
            (if (== (`GameplayStatics.GetObjectClass` (`self.CurrentCameraTargetLogic`)) (`local.NewLogicClass`))
              (return)
              (else
                (`/Game/EpicTemplates/TemplateAgnostic/Blueprints/CameraTargetLogics/BP_CameraTargetLogicBase.Cleanup` (`self.CurrentCameraTargetLogic`) (`self.GetOwner`) self))))))
      (:`then_1`
        (bind _returnvalue (`|GenericCreateObject` NewLogicClass))
        (bind _output_get (set `self.CurrentCameraTargetLogic` _returnvalue))
        (`/Game/EpicTemplates/TemplateAgnostic/Blueprints/CameraTargetLogics/BP_CameraTargetLogicBase.Setup` _output_get (`self.GetOwner`) self)))))