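; Actor component that lets its owner wield weapons, spawning an async-loaded default weapon at BeginPlay and forwarding fire and cycle inputs.
; Weapons are driven through BPI_Weapon, attached to a configurable component socket, and optionally held in an unequipped list for cycling.
; Giving a weapon replaces same-class duplicates, while removing the current one falls back to the protected default.
; Owner death via BP_HealthComponent releases fire and can strip non-default weapons.
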(event `self.ReceiveBeginPlay`
  ;[1 1 1] Begin Play
  (`|ExecutionSequence`
    (:`then_0`
      (bind _aspawn (cast `Pawn` (`self.GetOwner`)))
      (set `self.OwningPawn` _aspawn))
    (:`then_1`
      (`/Game/EpicTemplates/TemplateAgnostic/Blueprints/EpicTemplatesObjectMacroLibrary.!!!IsNOTValid!!!` (`self.WeaponAttachComponent`)
        (:`Is NOT Valid`
          (set `self.WeaponAttachComponent` (`Actor.RootComponent` (`self.GetOwner`))))))
    (:`then_2`
      (bind _class (`|LoadAssetClass` (`self.StartWeapon`))
        (:`Completed`
          (bind _asactor (castclass `Actor` _class))
          (bind _returnvalue (`|SpawnActorFromClass` _asactor (`Actor.GetTransform` (`self.GetOwner`)) "AlwaysSpawn" "MultiplyWithRoot" null null))
          (bind _output_get (set `self.DefaultWeapon` _returnvalue))
          (`/Game/EpicTemplates/TemplateAgnostic/Blueprints/Interfaces/BPI_WeaponWielder.GiveWeapon` _output_get))))
    (:`then_3`
      (`self.BindToOwnerDied`))))

(event `OwnerDied`
  (params (Caller :type "/Game/EpicTemplates/TemplateAgnostic/Blueprints/Components/BP_HealthComponent Object Reference") (KillingDamageSourceOwner :type "Actor Object Reference") (KillingDamageSource :type "Actor Object Reference") (KillingDamageLocation :type "Vector Structure") (KillingDamageDirection :type "Vector Structure") (HitBone :type Name) (SpecialDamageName :type Name))
  ;[1 1 1] Owner died
  (`|ExecutionSequence`
    (:`then_0`
      (`self.PrimaryFireReleased`)
      (`self.SecondaryFireReleased`))
    (:`then_1`
      (if (`self.bRemoveNonDefaultWeaponsOnOwnerDied`)
        (`|ExecutionSequence`
          (:`then_0`
            (bind (_arrayindex _arrayelement) (`/Engine/EditorBlueprintResources/StandardMacros.ReverseForEachLoop` (`self.UnequippedWeapons`))
              (:`LoopBody`
                (if (!= _arrayelement (`self.DefaultWeapon`))
                  (`self.HandleRemoveWeapon` _arrayelement true)))))
          (:`then_1`
            (if (!= (`self.CurrentWeaponActor`) (`self.DefaultWeapon`))
              (`self.HandleRemoveWeapon` (`self.CurrentWeaponActor`) true))))))))

(event `/Game/EpicTemplates/TemplateAgnostic/Blueprints/Interfaces/BPI_WeaponWielder.GiveWeapon`
  (params (NewWeapon :type "Actor Object Reference"))
  ;[1 1 1] BPI_WeaponWielder
  (if (`KismetSystemLibrary.DoesImplementInterface` NewWeapon "/Game/EpicTemplates/TemplateAgnostic/Blueprints/Interfaces/BPI_Weapon.BPI_Weapon_C")
    (`self.HandleGiveWeapon` NewWeapon)))

(event `EnhancedInput|/Game/EpicTemplates/RailShooterTemplate/Input/Actions/IA_PrimaryFire`
  (params (ActionValue :type Boolean) (ElapsedSeconds :type "Float (double-precision)") (TriggeredSeconds :type "Float (double-precision)") (InputAction :type "InputAction Object Reference" :default "/Game/EpicTemplates/RailShooterTemplate/Input/Actions/IA_PrimaryFire.IA_PrimaryFire"))
  ;[1 1 1] Inputs
  (:`Triggered`
    (if (`self.IsInputAllowed`)
      (set `self.PrimaryFireHeld` ActionValue)
      (if ActionValue
        (`self.PrimaryFirePressed`)
        (else
          (`self.PrimaryFireReleased`))))))

(event `/Game/EpicTemplates/TemplateAgnostic/Blueprints/Interfaces/BPI_WeaponWielder.GiveWeaponOfClass`
  (params (WeaponClass :type "Actor Soft Class Reference"))
  ;[1 1 1] BPI_WeaponWielder
  (bind _class (`|LoadAssetClass` WeaponClass)
    (:`Completed`
      (bind _asactor (castclass `Actor` _class))
      (if (`KismetSystemLibrary.DoesClassImplementInterface` _asactor "/Game/EpicTemplates/TemplateAgnostic/Blueprints/Interfaces/BPI_Weapon.BPI_Weapon_C")
        (bind _returnvalue (`|SpawnActorFromClass` _asactor (`Actor.GetTransform` (`self.GetOwner`)) "AlwaysSpawn" "MultiplyWithRoot" null null))
        (`/Game/EpicTemplates/TemplateAgnostic/Blueprints/Interfaces/BPI_WeaponWielder.GiveWeapon` _returnvalue)))))

(event `/Game/EpicTemplates/TemplateAgnostic/Blueprints/Interfaces/BPI_WeaponWielder.RemoveWeapon`
  (params (RemovingWeapon :type "Actor Object Reference") (bShouldDestroy :type Boolean))
  ;[1 1 1] BPI_WeaponWielder
  (`self.HandleRemoveWeapon` RemovingWeapon bShouldDestroy))

(event `EnhancedInput|/Game/EpicTemplates/RailShooterTemplate/Input/Actions/IA_SecondaryFire`
  (params (ActionValue :type Boolean) (ElapsedSeconds :type "Float (double-precision)") (TriggeredSeconds :type "Float (double-precision)") (InputAction :type "InputAction Object Reference" :default "/Game/EpicTemplates/RailShooterTemplate/Input/Actions/IA_SecondaryFire.IA_SecondaryFire"))
  ;[1 1 1] Inputs
  (:`Triggered`
    (if (`self.IsInputAllowed`)
      (bind _output_get (set `self.SecondaryFireHeld` ActionValue))
      (if _output_get
        (`self.SecondaryFirePressed`)
        (else
          (`self.SecondaryFireReleased`))))))

(event `EnhancedInput|/Game/EpicTemplates/TopDownTemplate/Input/IA_CycleWeapons`
  (params (ActionValue :type Boolean) (ElapsedSeconds :type "Float (double-precision)") (TriggeredSeconds :type "Float (double-precision)") (InputAction :type "InputAction Object Reference" :default "/Game/EpicTemplates/TopDownTemplate/Input/IA_CycleWeapons.IA_CycleWeapons"))
  ;[1 1 1] Inputs
  (:`Triggered`
    (if (`self.IsInputAllowed`)
      (if (`self.bAllowMultipleWeapons`)
        (`self.HandleTryCycleWeapon` true)))))

(event `/Game/EpicTemplates/TemplateAgnostic/Blueprints/Interfaces/BPI_Debuggable.UpdateIsInDebug`
  (params (bInIsDebug :type Boolean))
  ;[1 1 1] BPI_Debuggable
  (set `self.Is in Debug` bInIsDebug)
  (`|ExecutionSequence`
    (:`then_0`
      (`/Engine/EditorBlueprintResources/StandardMacros.IsValid` (`self.CurrentWeaponActor`)
        (:`Is Valid`
          (message `/Game/EpicTemplates/TemplateAgnostic/Blueprints/Interfaces/BPI_Debuggable.UpdateIsInDebug` (`self.CurrentWeaponActor`) (`self.Is in Debug`)))))
    (:`then_1`
      (for _array_element (`self.UnequippedWeapons`)
        (message `/Game/EpicTemplates/TemplateAgnostic/Blueprints/Interfaces/BPI_Debuggable.UpdateIsInDebug` _array_element (`self.Is in Debug`))))))

(fn `AssignAttachComponent`
  (params (InWeaponAttachComponent :type "SceneComponent Object Reference") (WeaponAttachSocket :type Name))
  (set `self.WeaponAttachComponent` InWeaponAttachComponent)
  (set `self.WeaponAttachSocket` WeaponAttachSocket))

(fn `BindToOwnerDied`
  (locals (OwnerHealthComponent :type "/Game/EpicTemplates/TemplateAgnostic/Blueprints/Components/BP_HealthComponent Object Reference"))
  (bind _output_get (set `local.OwnerHealthComponent` (`Actor.GetComponentByClass` (`self.GetOwner`) "/Game/EpicTemplates/TemplateAgnostic/Blueprints/Components/BP_HealthComponent.BP_HealthComponent_C")))
  (`/Engine/EditorBlueprintResources/StandardMacros.IsValid` _output_get
    (:`Is Valid`
      (add `/Game/EpicTemplates/TemplateAgnostic/Blueprints/Components/BP_HealthComponent.OnDied` (`local.OwnerHealthComponent`) (`|CreateDelegate` :!event `OwnerDied`)))))

(fn `CurrentWeaponCleared`)

(fn `CurrentWeaponUpdated`
  (params (NewWeapon :type "Actor Object Reference")))

(fn `Equip Weapon`
  (params (NewWeapon :type "Actor Object Reference"))
  (locals (OldWeaponActor :type "Actor Object Reference"))
  (if (== NewWeapon (`self.CurrentWeaponActor`))
    (return)
    (else
      (`|ExecutionSequence`
        (:`then_0`
          (bind _output_get (set `local.OldWeaponActor` (`self.CurrentWeaponActor`)))
          (`/Engine/EditorBlueprintResources/StandardMacros.IsValid` _output_get
            (:`Is Valid`
              (`self.TryUnequipWeapon` (`local.OldWeaponActor`) (not (`self.bAllowMultipleWeapons`)))
              (if (`self.bAllowMultipleWeapons`)
                (`KismetArrayLibrary.Array_AddUnique` (`self.UnequippedWeapons`) (`local.OldWeaponActor`))
                (elif (!= (`local.OldWeaponActor`) (`self.DefaultWeapon`))
                  (`Actor.K2_DestroyActor` (`local.OldWeaponActor`)))))))
        (:`then_1`
          (`/Engine/EditorBlueprintResources/StandardMacros.IsValid` (`local.NewWeapon`)
            (:`Is Valid`
              (set `self.CurrentWeaponActor` (`local.NewWeapon`))
              (`|ExecutionSequence`
                (:`then_0`
                  (`/Engine/EditorBlueprintResources/StandardMacros.IsValid` (`self.WeaponAttachComponent`)
                    (:`Is Valid`
                      (`Actor.K2_AttachToComponent` (`self.CurrentWeaponActor`) (`self.WeaponAttachComponent`) (`self.WeaponAttachSocket`) "SnapToTarget" "SnapToTarget" "SnapToTarget" true))
                    (:`Is Not Valid`
                      (`Actor.K2_AttachToActor` (`self.CurrentWeaponActor`) (`self.GetOwner`) (`self.WeaponAttachSocket`) "SnapToTarget" "SnapToTarget" "SnapToTarget" true))))
                (:`then_1`
                  (bind _asbpi_weapon (cast `/Game/EpicTemplates/TemplateAgnostic/Blueprints/Interfaces/BPI_Weapon` (`local.NewWeapon`)))
                  (bind _output_get_2 (set `self.CurrentWeaponInterface` _asbpi_weapon))
                  (`/Game/EpicTemplates/TemplateAgnostic/Blueprints/Interfaces/BPI_Weapon.UpdateWielder` _output_get_2 (`self.GetOwner`))
                  (`/Game/EpicTemplates/TemplateAgnostic/Blueprints/Interfaces/BPI_Weapon.UpdateIsCurrentlyWielded` (`self.CurrentWeaponInterface`) true))
                (:`then_2`
                  (`self.CurrentWeaponUpdated` (`self.CurrentWeaponActor`)))))))))))

(fn `GetAimDir`
  (returns (AimStartLoc :type "Vector Structure") (AimDir :type "Vector Structure"))
  (return (0.0 0.0 0.0) (0.0 0.0 0.0)))

(fn `GetCurrentWeaponInterface`
  (returns (WeaponInterface :type "/Game/EpicTemplates/TemplateAgnostic/Blueprints/Interfaces/BPI_Weapon Interface"))
  (return (`self.CurrentWeaponInterface`)))

(fn `GetCurrentWieldedWeapon`
  (returns (WeaponActor :type "Actor Object Reference"))
  (return (`self.CurrentWeaponActor`)))

(fn `GetIsInDebug`
  (returns (bIsInDebug :type Boolean))
  (return (`self.Is in Debug`)))

(fn `HandleGiveWeapon`
  (params (GivenWeapon :type "Actor Object Reference"))
  (if (== GivenWeapon (`self.CurrentWeaponActor`))
    (return)
    (elif (`KismetArrayLibrary.Array_Contains` (`self.UnequippedWeapons`) (`local.GivenWeapon`))
      (`self.Equip Weapon` (`local.GivenWeapon`))
      (`KismetArrayLibrary.Array_RemoveItem` (`self.UnequippedWeapons`) (`local.GivenWeapon`))
      (else
        (`self.Equip Weapon` (`local.GivenWeapon`))
        (`self.Remove Duplicate Weapons` (`local.GivenWeapon`))))))

(fn `HandleRemoveWeapon`
  (params (RemovingWeaponActor :type "Actor Object Reference") (bCanDestroy :type Boolean))
  (locals (WeaponIndex :type Integer) (OldWeaponInterface :type "/Game/EpicTemplates/TemplateAgnostic/Blueprints/Interfaces/BPI_Weapon Interface"))
  (if (== (`self.DefaultWeapon`) RemovingWeaponActor)
    (return)
    (else
      (`|ExecutionSequence`
        (:`then_0`
          (bind _bwascurrentweapon (`self.TryUnequipWeapon` (`local.RemovingWeaponActor`) true))
          (if _bwascurrentweapon
            (`/Engine/EditorBlueprintResources/StandardMacros.IsValid` (`self.DefaultWeapon`)
              (:`Is Valid`
                (`self.Equip Weapon` (`self.DefaultWeapon`))))
            (else
              (for (_array_element _array_index) (`self.UnequippedWeapons`)
                (set `local.WeaponIndex` _array_index)
                (if (== _array_element (`local.RemovingWeaponActor`))
                  (`|ExecutionSequence`
                    (:`then_0`
                      (bind _asbpi_weapon (cast `/Game/EpicTemplates/TemplateAgnostic/Blueprints/Interfaces/BPI_Weapon` (`local.RemovingWeaponActor`)))
                      (`/Game/EpicTemplates/TemplateAgnostic/Blueprints/Interfaces/BPI_Weapon.UpdateWielder` _asbpi_weapon null))
                    (:`then_1`
                      (`KismetArrayLibrary.Array_Remove` (`self.UnequippedWeapons`) (`local.WeaponIndex`))
                      (break))))))))
        (:`then_1`
          (if (`local.bCanDestroy`)
            (`Actor.K2_DestroyActor` (`local.RemovingWeaponActor`))))))))

(fn `HandleTryCycleWeapon`
  (params (CycleForward :type Boolean))
  (locals (NewWeapon :type "Actor Object Reference"))
  (if (> (`KismetArrayLibrary.Array_Length` (`self.UnequippedWeapons`)) 0)
    (bind _output_get (set `local.NewWeapon` (`|GetArrayItem` (`self.UnequippedWeapons`) (`KismetMathLibrary.SelectInt` 0 (`KismetArrayLibrary.Array_LastIndex` (`self.UnequippedWeapons`)) CycleForward))))
    (`self.Equip Weapon` _output_get)
    (if (== (`self.CurrentWeaponActor`) (`local.NewWeapon`))
      (`KismetArrayLibrary.Array_RemoveItem` (`self.UnequippedWeapons`) (`local.NewWeapon`)))))

(fn `IsCurrentWeaponDefault`
  (returns (IsDefaultWeapon :type Boolean))
  (return (== (`self.CurrentWeaponActor`) (`self.DefaultWeapon`))))

(fn `IsCurrentWeaponValid`
  (returns (IsValid :type Boolean))
  (return (`KismetSystemLibrary.IsValidInterface` (`self.CurrentWeaponInterface`))))

(fn `IsInputAllowed`
  (returns (InputAllowed :type Boolean))
  (`/Engine/EditorBlueprintResources/StandardMacros.IsValid` (`self.OwningPawn`)
    (:`Is Valid`
      (return (not (`Pawn.IsMoveInputIgnored` (`self.OwningPawn`)))))
    (:`Is Not Valid`
      (return true))))

(fn `PrimaryFirePressed`
  (`/Game/EpicTemplates/TemplateAgnostic/Blueprints/Interfaces/BPI_Weapon.PrimaryFirePressed` (`self.CurrentWeaponInterface`)))

(fn `PrimaryFireReleased`
  (`/Game/EpicTemplates/TemplateAgnostic/Blueprints/Interfaces/BPI_Weapon.PrimaryFireReleased` (`self.CurrentWeaponInterface`)))

(fn `Remove Duplicate Weapons`
  (params (WeaponActor :type "Actor Object Reference"))
  (locals (TempWeaponActor :type "Actor Object Reference") (TempIndex :type Integer))
  (for (_array_element _array_index) (`self.UnequippedWeapons`)
    (set `local.TempWeaponActor` _array_element)
    (set `local.TempIndex` _array_index)
    (if (== (`GameplayStatics.GetObjectClass` (`local.TempWeaponActor`)) (`GameplayStatics.GetObjectClass` (`local.WeaponActor`)))
      (`KismetArrayLibrary.Array_Remove` (`self.UnequippedWeapons`) (`local.TempIndex`))
      (`|ExecutionSequence`
        (:`then_0`
          (bind _asbpi_weapon (cast `/Game/EpicTemplates/TemplateAgnostic/Blueprints/Interfaces/BPI_Weapon` (`local.TempWeaponActor`)))
          (`/Game/EpicTemplates/TemplateAgnostic/Blueprints/Interfaces/BPI_Weapon.UpdateWielder` _asbpi_weapon null))
        (:`then_1`
          (`Actor.K2_DestroyActor` (`local.TempWeaponActor`))
          (return))))))

(fn `RemoveCurrentWeapon`
  (params (ShouldDestroy :type Boolean))
  (bind _currentweaponactor (`self.CurrentWeaponActor`))
  (`/Engine/EditorBlueprintResources/StandardMacros.IsValid` _currentweaponactor
    (:`Is Valid`
      (`self.HandleRemoveWeapon` _currentweaponactor ShouldDestroy))))

(fn `SecondaryFirePressed`
  (`/Game/EpicTemplates/TemplateAgnostic/Blueprints/Interfaces/BPI_Weapon.SecondaryFirePressed` (`self.CurrentWeaponInterface`)))

(fn `SecondaryFireReleased`
  (`/Game/EpicTemplates/TemplateAgnostic/Blueprints/Interfaces/BPI_Weapon.SecondaryFireReleased` (`self.CurrentWeaponInterface`)))

(fn `TryCycleWeapon`
  (params (CycleForward :type Boolean :default true))
  (`self.HandleTryCycleWeapon` CycleForward))

(fn `TryUnequipWeapon`
  (params (WeaponToUnequip :type "Object Object Reference") (bRemoveWielder :type Boolean :default false))
  (returns (bWasCurrentWeapon :type Boolean))
  (locals (OldWeaponInterface :type "/Game/EpicTemplates/TemplateAgnostic/Blueprints/Interfaces/BPI_Weapon Interface"))
  (bind _oldweaponinterface (`local.OldWeaponInterface`))
  (if (== (`self.CurrentWeaponActor`) WeaponToUnequip)
    (`|ExecutionSequence`
      (:`then_0`
        (if (`KismetSystemLibrary.IsValidInterface` (`self.CurrentWeaponInterface`))
          (set `local.OldWeaponInterface` (`self.CurrentWeaponInterface`))
          (set `self.CurrentWeaponInterface` null)
          (`/Game/EpicTemplates/TemplateAgnostic/Blueprints/Interfaces/BPI_Weapon.UpdateIsCurrentlyWielded` _oldweaponinterface false)
          (if (and (`local.bRemoveWielder`) (!= (`self.DefaultWeapon`) (`local.WeaponToUnequip`)))
            (`/Game/EpicTemplates/TemplateAgnostic/Blueprints/Interfaces/BPI_Weapon.UpdateWielder` _oldweaponinterface null))))
      (:`then_1`
        (set `self.CurrentWeaponActor` null)
        (`self.CurrentWeaponCleared`))
      (:`then_2`
        (return true)))
    (else
      (return false))))