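; BP_Spring is a platformer spring pad that launches characters overlapping its trigger, optionally only player-controlled ones.
; Launch velocity overrides the character's own and is built from LaunchAngle and LauchPower in the world YZ plane, ignoring actor rotation.
; A timeline animates the pop by moving the spring head while shifting and stretching the spring plane beneath it.
; The construction script tilts the mesh pivot to LaunchAngle and caches rest heights for that animation.
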(event `self.Trigger.OnComponentBeginOverlap`
  (params (OverlappedComponent :type "PrimitiveComponent Object Reference") (OtherActor :type "Actor Object Reference") (OtherComp :type "PrimitiveComponent Object Reference") (OtherBodyIndex :type Integer) (bFromSweep :type Boolean) (SweepResult :type "HitResult Structure (by ref)"))
  (bind _launchangle (`self.LaunchAngle`))
  (bind _ascharacter (cast `Character` OtherActor))
  (if (or (`Pawn.IsPlayerControlled` _ascharacter) (not (`self.bOnlyLaunchPlayers`)))
    (`Character.LaunchCharacter` _ascharacter (* (`KismetMathLibrary.MakeVector` 0.0 (`KismetMathLibrary.DegSin` _launchangle) (`KismetMathLibrary.DegCos` _launchangle)) (`self.LauchPower`)) true true)
    (bind (_direction _springalpha) (`Timeline|TL_Spring` :!via `PlayFromStart`)
      (:`Update`
        (`SceneComponent.K2_SetRelativeLocation` (`self.SpringHeadMesh`) (`KismetMathLibrary.MakeVector` 0.0 0.0 (+ (`self.SpringHeadStartDist`) (* _springalpha (`self.SpringHeadSpringDist`)))) false false)
        (`SceneComponent.K2_SetRelativeLocation` (`self.SpringPlane`) (`KismetMathLibrary.MakeVector` 0.0 0.0 (+ (`self.SpringPlaneStartDist`) (* (* _springalpha (`self.SpringHeadSpringDist`)) 0.5))) false false)
        (`SceneComponent.SetRelativeScale3D` (`self.SpringPlane`) (`KismetMathLibrary.MakeVector` 1.0 (* (+ (`self.SpringHeadStartDist`) (* _springalpha (`self.SpringHeadSpringDist`))) 0.01) 1.0))))))

(fn `UserConstructionScript`
  (`SceneComponent.K2_SetRelativeRotation` (`self.MeshPivot`) (`KismetMathLibrary.MakeRotator` (`self.LaunchAngle`)) false false)
  (set `self.SpringHeadStartDist` (.z (`SceneComponent.RelativeLocation` (`self.SpringHeadMesh`))))
  (set `self.SpringPlaneStartDist` (.z (`SceneComponent.RelativeLocation` (`self.SpringPlane`)))))