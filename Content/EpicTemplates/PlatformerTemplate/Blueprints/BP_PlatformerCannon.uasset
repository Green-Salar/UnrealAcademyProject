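; BP_PlatformerCannon is a platformer cannon that fires projectiles at a regular interval while active.
; Activate and Deactivate events toggle Tick, whose timer carries over leftover time and catches up on missed shots.
; Fire spawns a reusable projectile from a soft class, blocking, then launches it by message along the spawn point's right vector.
; The construction script sets stand visibility and the initial active state.
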(event `ActivateCannon`
  (`self.SetActorTickEnabled` true))

(event `DeactivateCannon`
  (`self.SetActorTickEnabled` false))

(event `self.ReceiveTick`
  (params (DeltaSeconds :type "Float (single-precision)"))
  (bind _outfloatcopy (`/Game/EpicTemplates/TemplateAgnostic/Blueprints/EpicTemplatesFunctionLibrary.PlusEqualsFloat` (`self.CurrentFireTime`) DeltaSeconds))
  (if (> _outfloatcopy (`self.FireFrequency`))
    (while (> (`self.CurrentFireTime`) (`self.FireFrequency`))
      (`/Game/EpicTemplates/TemplateAgnostic/Blueprints/EpicTemplatesFunctionLibrary.MinusEqualsFloat` (`self.CurrentFireTime`) (`self.FireFrequency`))
      (`self.Fire`))))

(event `Fire`
  (bind _actorinstance (`/Game/EpicTemplates/TemplateAgnostic/Blueprints/EpicTemplatesFunctionLibrary.SpawnReusableActorFromSoftClassBlocking` (`self.ProjectileClass`) (`SceneComponent.K2_GetComponentToWorld` (`self.ProjectilSpawnPoint`)) self))
  (`/Engine/EditorBlueprintResources/StandardMacros.IsValid` _actorinstance
    (:`Is Valid`
      (message `/Game/EpicTemplates/TemplateAgnostic/Blueprints/Interfaces/BPI_Projectile.LaunchInDirection` _actorinstance null (`SceneComponent.GetRightVector` (`self.ProjectilSpawnPoint`)) (`self.ProjectileOverrideSpeed`)))))

(fn `UserConstructionScript`
  (`SceneComponent.SetVisibility` (`self.StandMesh`) (`self.bShowStand`) false)
  (`self.SetActorTickEnabled` (`self.bIsCannonActiveOnStart`)))