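; Actor component that moves its owner, such as a moving platform, through staged target actor locations as a function of externally sampled time.
; InitialSetup builds a time-to-stage map from start delay, waits and travel times (constant-speed or per-stage), optionally spawning a start-position marker.
; BPi_TimeSampleable's SampletoTime finds the current segment and lerps location, applying optional per-stage curves that can invert on reverse.
; GetTotalTimeRange exposes the timeline's length.
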(event `self.ReceiveBeginPlay`
  (if (not (`self.IsSetup`))
    (`self.InitialSetup`)))

(event `/Game/EpicTemplates/PlatformerTemplate/Blueprints/Interfaces/BPI_TimeSampleable.SampleToTime`
  (params (Time :type "Float (double-precision)") (SampleDirection :type "/Game/EpicTemplates/PlatformerTemplate/Blueprints/Enums/ESampleablePlayDirection Enum" :default "NewEnumerator0"))
  ;[1 1 1] BPi_TimeSampleable
  (if (!= Time (`self.CurrentTime`))
    (set `self.CurrentTime` Time)
    (`self.SampleToCurrentTime` SampleDirection)))

(fn `GetCurvedAlphaFromMovementIndex`
  (params (TargetIndex :type Integer) (RawAlpha :type "Float (double-precision)") (SampleDirection :type "/Game/EpicTemplates/PlatformerTemplate/Blueprints/Enums/ESampleablePlayDirection Enum" :default "NewEnumerator0"))
  (returns (CurvedAlpha :type "Float (double-precision)"))
  (locals (TempMovement :type "/Game/EpicTemplates/PlatformerTemplate/Blueprints/Structs/StagedMovementStruct Structure"))
  (bind _returnvalue (`KismetSystemLibrary.LoadAsset_Blocking` (`.MovementCurve_21_B3BD8FF04AA6E6DCD079BC93C7E1DA18` (break `/Game/EpicTemplates/PlatformerTemplate/Blueprints/Structs/StagedMovementStruct` (`|GetArrayItem` (`self.Movements`) TargetIndex)))))
  (`/Engine/EditorBlueprintResources/StandardMacros.IsValid` _returnvalue
    (:`Is Valid`
      (bind _ascurve_float (cast `CurveFloat` _returnvalue))
      (if (and (`.bInvertCurveOnReverse_24_696382EF4A7024164CD182A044FF72E6` (break `/Game/EpicTemplates/PlatformerTemplate/Blueprints/Structs/StagedMovementStruct` (`|GetArrayItem` (`self.Movements`) (`local.TargetIndex`)))) (`|EnumEquality` (`local.SampleDirection`) "NewEnumerator2"))
        (return (- 1.0 (`CurveFloat.GetFloatValue` _ascurve_float (- 1.0 (`local.RawAlpha`)))))
        (else
          (return (`CurveFloat.GetFloatValue` _ascurve_float (`local.RawAlpha`))))))
    (:`Is Not Valid`
      (return (`local.RawAlpha`)))))

(fn `GetTargetLocationByIndex`
  (params (Index :type Integer))
  (returns (TargetLoc :type "Vector Structure"))
  (return (`Actor.K2_GetActorLocation` (`|ConvertAsset` (`.TransformTarget_3_B470CB7A42A7FC0D2DE4FB9C0B9D67E2` (break `/Game/EpicTemplates/PlatformerTemplate/Blueprints/Structs/StagedMovementStruct` (`|GetArrayItem` (`self.Movements`) Index)))))))

(fn `GetTotalTimeRange`
  (returns (StartTime :type "Float (double-precision)") (EndTime :type "Float (double-precision)"))
  (`|ExecutionSequence`
    (:`then_0`
      (if (not (`self.IsSetup`))
        (`self.InitialSetup`)))
    (:`then_1`
      (return 0.0 (`self.TotalMovementTime`)))))

(fn `InitialSetup`
  (locals (StartTrans :type "Transform Structure") (TempMovementStageIndex :type Integer) (TempCurrentMovementStage :type "/Game/EpicTemplates/PlatformerTemplate/Blueprints/Structs/StagedMovementStruct Structure") (MovementTime :type "Float (double-precision)") (WaitTime :type "Float (double-precision)"))
  (if (`self.IsSetup`)
    (return)
    (else
      (`BlueprintMapLibrary.Map_Clear` (`self.TimeToStageIndexes`))
      (`BlueprintMapLibrary.Map_Add` (`self.TimeToStageIndexes`))
      (`|ExecutionSequence`
        (:`then_0`
          (if (> (`self.DelayAtStart`) 0.0)
            (bind _output_get (set `self.TotalMovementTime` (`self.DelayAtStart`)))
            (`BlueprintMapLibrary.Map_Add` (`self.TimeToStageIndexes`) _output_get)
            (else
              (set `self.TotalMovementTime` 0.0))))
        (:`then_1`
          (if (`self.bAutoGenerateFirstMovementStageFromStartLocation`)
            (bind _returnvalue (`|SpawnActorFromClass` "/Game/EpicTemplates/PlatformerTemplate/Blueprints/BP_MovingPlatformStartPosition.BP_MovingPlatformStartPosition_C" (`Actor.GetTransform` (`self.GetOwner`)) "AlwaysSpawn" "MultiplyWithRoot" null null))
            (`KismetArrayLibrary.Array_Insert` (`self.Movements`) (make `/Game/EpicTemplates/PlatformerTemplate/Blueprints/Structs/StagedMovementStruct` (`|ConvertAsset` _returnvalue) (`.TimeToTarget_17_C18ECFDD4C6C82A1F57BD6B141C4E487` (break `/Game/EpicTemplates/PlatformerTemplate/Blueprints/Structs/StagedMovementStruct` (`|GetArrayItem` (`self.Movements`)))) 0.0 null))))
        (:`then_2`
          (if (< (`KismetArrayLibrary.Array_Length` (`self.Movements`)) 2)
            (`KismetSystemLibrary.PrintString` (`KismetStringLibrary.Concat_StrStr` "BP_StagedMovementComponent::InitialSetup - The component on actor '" (`KismetSystemLibrary.GetDisplayName` (`self.GetOwner`)) "' has fewer than 2 points, meaning it cannot move. Either assign more movement stages, or ensure bAutoGenerateLastMovementStageFromStartLocation is true if you haven't assigned a starting point.") true true (struct :`R` 1.0 :`G` 0.265546 :`A` 1.0) 20.0)))
        (:`then_3`
          (for _index (range (+ (- (`KismetArrayLibrary.Array_Length` (`self.Movements`)) 2) 1))
            (set `local.TempCurrentMovementStage` (`|GetArrayItem` (`self.Movements`) _index))
            (set `local.TempMovementStageIndex` (+ _index 1))
            (`|ExecutionSequence`
              (:`then_0`
                (if (`|EnumEquality` (`self.MovementType`) "NewEnumerator0")
                  (set `local.MovementTime` (/ (`KismetMathLibrary.Vector_Distance` (`self.GetTargetLocationByIndex` (`local.TempMovementStageIndex`)) (`self.GetTargetLocationByIndex` (- (`local.TempMovementStageIndex`) 1))) (`self.ConstantMoveSpeed`)))
                  (else
                    (set `local.MovementTime` (`.TimeToTarget_17_C18ECFDD4C6C82A1F57BD6B141C4E487` (break `/Game/EpicTemplates/PlatformerTemplate/Blueprints/Structs/StagedMovementStruct` (`local.TempCurrentMovementStage`)))))))
              (:`then_1`
                (bind _outfloatcopy (`/Game/EpicTemplates/TemplateAgnostic/Blueprints/EpicTemplatesFunctionLibrary.PlusEqualsFloat` (`self.TotalMovementTime`) (`local.MovementTime`)))
                (`BlueprintMapLibrary.Map_Add` (`self.TimeToStageIndexes`) _outfloatcopy (`local.TempMovementStageIndex`)))
              (:`then_2`
                (bind _output_get_2 (set `local.WaitTime` (`.WaitAtTargetTime_7_258DADEF429DEC0B6B2B63B92DB5AEA3` (break `/Game/EpicTemplates/PlatformerTemplate/Blueprints/Structs/StagedMovementStruct` (`local.TempCurrentMovementStage`)))))
                (if (> _output_get_2 0.0)
                  (bind _outfloatcopy_2 (`/Game/EpicTemplates/TemplateAgnostic/Blueprints/EpicTemplatesFunctionLibrary.PlusEqualsFloat` (`self.TotalMovementTime`) (`local.WaitTime`)))
                  (`BlueprintMapLibrary.Map_Add` (`self.TimeToStageIndexes`) _outfloatcopy_2 (`local.TempMovementStageIndex`)))))))
        (:`then_4`
          (set `self.IsSetup` true))))))

(fn `SampleToCurrentTime`
  (params (SampleDirection :type "/Game/EpicTemplates/PlatformerTemplate/Blueprints/Enums/ESampleablePlayDirection Enum" :default "NewEnumerator0"))
  (locals (Times :type "Array of Float (double-precision)") (TempTimeIdx :type Integer) (StageIndexes :type "Array of Integer") (RawAlpha :type "Float (double-precision)" :default 0.0))
  (bind _times (`local.Times`))
  (bind _timetostageindexes (`self.TimeToStageIndexes`))
  (if (`self.IsSetup`)
    (bind _keys (`BlueprintMapLibrary.Map_Keys` _timetostageindexes))
    (set `local.Times` _keys)
    (bind _values (`BlueprintMapLibrary.Map_Values` _timetostageindexes))
    (set `local.StageIndexes` _values)
    (for _index (range 1 (`KismetArrayLibrary.Array_Length` (`local.Times`)))
      (bind _output_get (set `local.TempTimeIdx` _index))
      (if (<= (`self.CurrentTime`) (`|GetArrayItem` (`local.Times`) _output_get))
        (bind _output_get_2 (set `local.RawAlpha` (`KismetMathLibrary.MapRangeClamped` (`self.CurrentTime`) (`|GetArrayItem` _times (- (`local.TempTimeIdx`) 1)) (`|GetArrayItem` _times (`local.TempTimeIdx`)) 0.0 1.0)))
        (bind _curvedalpha (`self.GetCurvedAlphaFromMovementIndex` (`|GetArrayItem` (`local.StageIndexes`) (`local.TempTimeIdx`)) _output_get_2 (`local.SampleDirection`)))
        (`Actor.K2_SetActorLocation` (`self.GetOwner`) (`KismetMathLibrary.VLerp` (`self.GetTargetLocationByIndex` (`|GetArrayItem` (`local.StageIndexes`) (- (`local.TempTimeIdx`) 1))) (`self.GetTargetLocationByIndex` (`|GetArrayItem` (`local.StageIndexes`) (`local.TempTimeIdx`))) _curvedalpha) false false)
        (return)))))