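; Actor component that acts as a timeline player for sibling components implementing BPI_TimeSampleable.
; On BeginPlay it caches those components, takes their latest end time as the total duration, and optionally auto-plays.
; Tick advances a shared time forward or backward and samples every component to it, handling single, wrap or ping-pong playback at the ends.
; Stop disables tick and saves the mode, which Resume replays forward.
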(event `self.ReceiveBeginPlay`
  (`|ExecutionSequence`
    (:`then_0`
      (`self.PopulateSampleableInterfaces`))
    (:`then_1`
      (if (`|EnumInequality` (`self.PlayModeOnStart`) "NewEnumerator0")
        (`self.Play` (`self.PlayModeOnStart`))))))

(event `Play`
  (params (CurrentPlayMode :type "/Game/EpicTemplates/PlatformerTemplate/Blueprints/Enums/ESampleablePlayMode Enum" :default "NewEnumerator0") (PlayDirection :type "/Game/EpicTemplates/PlatformerTemplate/Blueprints/Enums/ESampleablePlayDirection Enum" :default "NewEnumerator0"))
  (if (`|EnumInequality` CurrentPlayMode "NewEnumerator0")
    (set `self.CurrentPlayMode` CurrentPlayMode)
    (set `self.CurrentPlayDirection` PlayDirection)
    (`self.SetComponentTickEnabled` true)
    (else
      (`self.Stop`))))

(event `Stop`
  (set `self.PlayModeOnStop` (`self.CurrentPlayMode`))
  (set `self.CurrentPlayMode` "NewEnumerator0")
  (`self.SetComponentTickEnabled` false))

(event `Resume`
  (`self.Play` (`self.PlayModeOnStop`))
  (`self.SetComponentTickEnabled` true))

(event `self.ReceiveTick`
  (params (DeltaSeconds :type "Float (single-precision)"))
  (if (`|EnumEquality` (`self.CurrentPlayMode`) "NewEnumerator0")
    (`self.Stop`)
    (else
      (`|ExecutionSequence`
        (:`then_0`
          (switch `/Game/EpicTemplates/PlatformerTemplate/Blueprints/Enums/ESampleablePlayDirection` (`self.CurrentPlayDirection`)
            (:`NewEnumerator0`
              (bind _outfloatcopy (`/Game/EpicTemplates/TemplateAgnostic/Blueprints/EpicTemplatesFunctionLibrary.PlusEqualsFloat` (`self.CurrentSampleTime`) DeltaSeconds))
              (if (>= _outfloatcopy (`self.TotalSampleTime`))
                (`self.HandleMovementReachedEnd`)))
            (:`NewEnumerator2`
              (bind _outfloatcopy_2 (`/Game/EpicTemplates/TemplateAgnostic/Blueprints/EpicTemplatesFunctionLibrary.MinusEqualsFloat` (`self.CurrentSampleTime`) DeltaSeconds))
              (if (<= _outfloatcopy_2 0.0)
                (`self.HandleMovementReachedEnd`)))))
        (:`then_1`
          (for _array_element (`self.SampleableInterfaces`)
            (`/Game/EpicTemplates/PlatformerTemplate/Blueprints/Interfaces/BPI_TimeSampleable.SampleToTime` _array_element (`self.CurrentSampleTime`) (`self.CurrentPlayDirection`))))))))

(event `HandleMovementReachedEnd`
  (switch `/Game/EpicTemplates/PlatformerTemplate/Blueprints/Enums/ESampleablePlayMode` (`self.CurrentPlayMode`)
    (:`NewEnumerator1`
      (set `self.CurrentSampleTime` (`KismetMathLibrary.FClamp` (`self.CurrentSampleTime`) 0.0 (`self.TotalSampleTime`)))
      (`self.Stop`))
    (:`NewEnumerator2`
      (set `self.CurrentSampleTime` (select `/Game/EpicTemplates/PlatformerTemplate/Blueprints/Enums/ESampleablePlayDirection` (`self.CurrentPlayDirection`) :`NewEnumerator0` (mod (`self.CurrentSampleTime`) (`self.TotalSampleTime`)) :`NewEnumerator2` (+ (`self.TotalSampleTime`) (`self.CurrentSampleTime`)))))
    (:`NewEnumerator3`
      (set `self.CurrentSampleTime` (select `/Game/EpicTemplates/PlatformerTemplate/Blueprints/Enums/ESampleablePlayDirection` (`self.CurrentPlayDirection`) :`NewEnumerator0` (- (`self.TotalSampleTime`) (- (`self.CurrentSampleTime`) (`self.TotalSampleTime`))) :`NewEnumerator2` (* (`self.CurrentSampleTime`) -1.0)))
      (set `self.CurrentPlayDirection` (select `/Game/EpicTemplates/PlatformerTemplate/Blueprints/Enums/ESampleablePlayDirection` (`self.CurrentPlayDirection`) :`NewEnumerator0` "NewEnumerator2" :`NewEnumerator2` "NewEnumerator0" :!type "/Game/EpicTemplates/PlatformerTemplate/Blueprints/Enums/ESampleablePlayDirection Enum")))))

(fn `PopulateSampleableInterfaces`
  (locals (SampleableComponents :type "Array of ActorComponent Object Reference"))
  (bind _output_get (set `local.SampleableComponents` (`Actor.GetComponentsByInterface` (`self.GetOwner`) "/Game/EpicTemplates/PlatformerTemplate/Blueprints/Interfaces/BPI_TimeSampleable.BPI_TimeSampleable_C")))
  (for _array_element _output_get
    (bind _asbpi_time_sampleable (cast `/Game/EpicTemplates/PlatformerTemplate/Blueprints/Interfaces/BPI_TimeSampleable` _array_element))
    (`KismetArrayLibrary.Array_Add` (`self.SampleableInterfaces`) _asbpi_time_sampleable)
    (bind (_starttime _endtime) (`/Game/EpicTemplates/PlatformerTemplate/Blueprints/Interfaces/BPI_TimeSampleable.GetTotalTimeRange` _asbpi_time_sampleable))
    (set `self.TotalSampleTime` (`KismetMathLibrary.FMax` _endtime (`self.TotalSampleTime`)))))