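; Platformer camera trigger volume that applies 2D camera bounds and blends the view toward a target actor while player pawns are inside.
; Overlap tracks player pawns, pushes bounds via the cached platformer camera interface and can clear them once empty.
; With a target set, Tick maps the closest pawn's distance from BlendCentre between outer and inner radii to override blend alpha.
; Axis options and Forward or Down perspective shape distances and debug drawing.
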(event `self.Box.OnComponentBeginOverlap`
  (params (OverlappedComponent :type "PrimitiveComponent Object Reference") (OtherActor :type "Actor Object Reference") (OtherComp :type "PrimitiveComponent Object Reference") (OtherBodyIndex :type Integer) (bFromSweep :type Boolean) (SweepResult :type "HitResult Structure (by ref)"))
  ;[1 1 1] Begin/End Overlap
  (bind _aspawn (cast `Pawn` OtherActor))
  (cast `PlayerController` (`Pawn.GetController` _aspawn))
  (`KismetArrayLibrary.Array_Add` (`self.CurrentPlayerPawns`) _aspawn)
  (`|ExecutionSequence`
    (:`then_0`
      (switch `/Game/EpicTemplates/PlatformerTemplate/Blueprints/Enums/ECameraTriggerBoundsLogic` (`self.BoundsLogic`)
        (:`NewEnumerator2`
          _)
        (:`NewEnumerator1`
          _))
      (`/Game/EpicTemplates/PlatformerTemplate/Blueprints/Interfaces/BPI_Camera2D.UpdateCameraBounds` (`self.GetCameraPlatformerInterface`) (`self.GetCameraBounds`)))
    (:`then_1`
      (if (`KismetSystemLibrary.IsValidSoftObjectReference` (`self.CameraTarget`))
        (`self.SetActorTickEnabled` true)
        (`self.AddTickPrerequisiteActor` _aspawn)))))

(event `self.Box.OnComponentEndOverlap`
  (params (OverlappedComponent :type "PrimitiveComponent Object Reference") (OtherActor :type "Actor Object Reference") (OtherComp :type "PrimitiveComponent Object Reference") (OtherBodyIndex :type Integer))
  ;[1 1 1] Begin/End Overlap
  (bind _aspawn (cast `Pawn` OtherActor))
  (bind _returnvalue (`KismetArrayLibrary.Array_RemoveItem` (`self.CurrentPlayerPawns`) _aspawn))
  (if _returnvalue
    (`self.RemoveTickPrerequisiteActor` _aspawn)
    (if (`KismetArrayLibrary.Array_IsEmpty` (`self.CurrentPlayerPawns`))
      (`self.SetActorTickEnabled` false)
      (`|ExecutionSequence`
        (:`then_0`
          (if (`|EnumEquality` (`self.BoundsLogic`) "NewEnumerator1")
            (`/Game/EpicTemplates/PlatformerTemplate/Blueprints/Interfaces/BPI_Camera2D.ClearBoundsByTag` (`self.GetCameraPlatformerInterface`) (`.BoundsTagKey_30_27B50CC9491AB42635280684667CF383` (break `/Game/EpicTemplates/PlatformerTemplate/Blueprints/Structs/CameraBounds2D` (`self.CameraBounds`))))))
        (:`then_1`
          (if (`self.bAlwaysRemoveOverrideOnEndOverlap`)
            (`/Game/EpicTemplates/PlatformerTemplate/Blueprints/Interfaces/BPI_Camera2D.ClearSpecificViewTargetOverride` (`self.GetCameraPlatformerInterface`) (`self.CameraTarget`))))))))

(event `self.ReceiveTick`
  (params (DeltaSeconds :type "Float (single-precision)"))
  ;[1 1 1] Tick
  (bind (_blendalpha _isinblendradius) (`self.GetClosestPawnBlendAlpha`))
  (if _isinblendradius
    (`/Game/EpicTemplates/PlatformerTemplate/Blueprints/Interfaces/BPI_Camera2D.AssignViewTargetOverride` (`self.GetCameraPlatformerInterface`) (make `/Game/EpicTemplates/PlatformerTemplate/Blueprints/Structs/CameraViewTargetOverride` (`self.CameraTarget`) _blendalpha))
    (else
      (`/Game/EpicTemplates/PlatformerTemplate/Blueprints/Interfaces/BPI_Camera2D.ClearSpecificViewTargetOverride` (`self.GetCameraPlatformerInterface`) (`self.CameraTarget`)))))

(fn `Debug Draw Bounds`
  (locals (Left :type "Float (double-precision)") (Right :type "Float (double-precision)") (CalculatedBounds :type "/Game/EpicTemplates/PlatformerTemplate/Blueprints/Structs/CameraBounds2D Structure") (ActorY :type "Float (double-precision)" :default 0.0) (ActorZ :type "Float (double-precision)" :default 0.0) (Top :type "Float (double-precision)") (Bottom :type "Float (double-precision)"))
  (bind _actorz (`local.ActorZ`))
  (bind _actory (`local.ActorY`))
  (bind (_rightbound _rightboundenforced _leftbound _leftboundenforced _topbound _topboundenforced _bottombound _bottomboundenforced) (break `/Game/EpicTemplates/PlatformerTemplate/Blueprints/Structs/CameraBounds2D` (`local.CalculatedBounds`)))
  (bind _output_get (set `local.CalculatedBounds` (`self.GetCameraBounds`)))
  (bind ((`RightBoundEnforced_5_3D3FFBC949F919D4D65818935D5F1501` _rightboundenforced_2) (`LeftBoundEnforced_13_84183321427389C686D88F988E67DFE7` _leftboundenforced_2) (`TopBoundEnforced_15_E73BC6294A163985CF6926A7D62F4436` _topboundenforced_2) (`BottomBoundEnforced_17_9C9E89D844DA269EA0699A94B3C3384E` _bottomboundenforced_2)) (break `/Game/EpicTemplates/PlatformerTemplate/Blueprints/Structs/CameraBounds2D` _output_get))
  (if (or _rightboundenforced_2 _leftboundenforced_2 _topboundenforced_2 _bottomboundenforced_2)
    (set `local.ActorY` (.y (`self.K2_GetActorLocation`)))
    (set `local.ActorZ` (.z (`self.K2_GetActorLocation`)))
    (set `local.Right` (`KismetMathLibrary.SelectFloat` _rightbound (+ _actory 99999.0) _rightboundenforced))
    (set `local.Left` (`KismetMathLibrary.SelectFloat` _leftbound (- _actory 99999.0) _leftboundenforced))
    (set `local.Top` (`KismetMathLibrary.SelectFloat` _topbound (+ _actorz 99999.0) _topboundenforced))
    (set `local.Bottom` (`KismetMathLibrary.SelectFloat` _bottombound (- _actorz 99999.0) _bottomboundenforced))
    (switch `/Game/EpicTemplates/TemplateAgnostic/Blueprints/Enums/E2DCameraViewDirection` (`self.GamePerspective`)
      (:`NewEnumerator0`
        (`KismetSystemLibrary.DrawDebugBox` (`KismetMathLibrary.MakeVector` (.x (`self.K2_GetActorLocation`)) (`KismetMathLibrary.Lerp` (`local.Left`) (`local.Right`) 0.5) (`KismetMathLibrary.Lerp` (`local.Bottom`) (`local.Top`) 0.5)) (`KismetMathLibrary.MakeVector` 1.0 (* (- (`local.Right`) (`local.Left`)) 0.5) (* (- (`local.Top`) (`local.Bottom`)) 0.5)) (`self.DebugOuterLineColor`) (struct) (`self.DebugLineTime`)))
      (:`NewEnumerator1`
        (`KismetSystemLibrary.DrawDebugBox` (`KismetMathLibrary.MakeVector` (`KismetMathLibrary.Lerp` (`local.Bottom`) (`local.Top`) 0.5) (`KismetMathLibrary.Lerp` (`local.Left`) (`local.Right`) 0.5) (.z (`self.K2_GetActorLocation`))) (`KismetMathLibrary.MakeVector` (* (- (`local.Top`) (`local.Bottom`)) 0.5) (* (- (`local.Right`) (`local.Left`)) 0.5) 1.0) (`self.DebugOuterLineColor`) (struct) (`self.DebugLineTime`))))))

(fn `Debug Draw Horizontal Blend Radius`
  (locals (Top :type "Float (double-precision)") (Bottom :type "Float (double-precision)") (Depth :type "Float (double-precision)") (InnerRight :type "Float (double-precision)") (InnerLeft :type "Float (double-precision)") (OuterRight :type "Float (double-precision)") (OuterLeft :type "Float (double-precision)"))
  (bind _innerblendradius (`self.InnerBlendRadius`))
  (bind _depth (`local.Depth`))
  (bind _innerleft (`local.InnerLeft`))
  (bind _depth_2 (`local.Depth`))
  (bind _outerleft (`local.OuterLeft`))
  (bind _depth_3 (`local.Depth`))
  (bind _innerright (`local.InnerRight`))
  (bind _outerblendradius (`self.OuterBlendRadius`))
  (bind _depth_4 (`local.Depth`))
  (bind _outerright (`local.OuterRight`))
  (bind (_origin _boxextent) (`KismetSystemLibrary.GetComponentBounds` (`self.Box`)))
  (bind (_origin_2 _boxextent_2) (`KismetSystemLibrary.GetComponentBounds` (`self.Box`)))
  (bind _y (.y (`SceneComponent.K2_GetComponentLocation` (`self.BlendCentre`))))
  (bind _x (.x _boxextent))
  (bind _z (.z _origin_2))
  (bind _z_2 (.z _boxextent_2))
  (bind _x_2 (.x _origin))
  (`|ExecutionSequence`
    (:`then_0`
      (switch `/Game/EpicTemplates/TemplateAgnostic/Blueprints/Enums/E2DCameraViewDirection` (`self.GamePerspective`)
        (:`NewEnumerator0`
          (set `local.Top` (+ _z _z_2))
          (set `local.Bottom` (- _z _z_2))
          (set `local.Depth` (.x (`SceneComponent.K2_GetComponentLocation` (`self.BlendCentre`)))))
        (:`NewEnumerator1`
          (set `local.Top` (+ _x_2 _x))
          (set `local.Bottom` (- _x_2 _x))
          (set `local.Depth` (.z (`SceneComponent.K2_GetComponentLocation` (`self.BlendCentre`)))))))
    (:`then_1`
      (set `local.InnerRight` (+ _y _innerblendradius))
      (set `local.InnerLeft` (- _y _innerblendradius))
      (set `local.OuterRight` (+ _y _outerblendradius))
      (set `local.OuterLeft` (- _y _outerblendradius))
      (`KismetSystemLibrary.DrawDebugLine` (`KismetMathLibrary.MakeVector` _depth_4 _outerright (`local.Top`)) (`KismetMathLibrary.MakeVector` _depth_4 _outerright (`local.Bottom`)) (`self.DebugOuterLineColor`) (`self.DebugLineTime`))
      (`KismetSystemLibrary.DrawDebugLine` (`KismetMathLibrary.MakeVector` _depth_2 _outerleft (`local.Top`)) (`KismetMathLibrary.MakeVector` _depth_2 _outerleft (`local.Bottom`)) (`self.DebugOuterLineColor`) (`self.DebugLineTime`))
      (`KismetSystemLibrary.DrawDebugLine` (`KismetMathLibrary.MakeVector` _depth_3 _innerright (`local.Top`)) (`KismetMathLibrary.MakeVector` _depth_3 _innerright (`local.Bottom`)) (`self.DebugInnerLineColor`) (`self.DebugLineTime`))
      (`KismetSystemLibrary.DrawDebugLine` (`KismetMathLibrary.MakeVector` _depth _innerleft (`local.Top`)) (`KismetMathLibrary.MakeVector` _depth _innerleft (`local.Bottom`)) (`self.DebugInnerLineColor`) (`self.DebugLineTime`)))))

(fn `Debug Draw Vertical Blend Radius`
  (locals (Right :type "Float (double-precision)") (Left :type "Float (double-precision)") (Depth :type "Float (double-precision)") (InnerTop :type "Float (double-precision)") (InnerBottom :type "Float (double-precision)") (OuterTop :type "Float (double-precision)") (OuterBottom :type "Float (double-precision)"))
  (bind _innerblendradius (`self.InnerBlendRadius`))
  (bind _depth (`local.Depth`))
  (bind _innerbottom (`local.InnerBottom`))
  (bind _depth_2 (`local.Depth`))
  (bind _outerbottom (`local.OuterBottom`))
  (bind _depth_3 (`local.Depth`))
  (bind _innertop (`local.InnerTop`))
  (bind _innerblendradius_2 (`self.InnerBlendRadius`))
  (bind _outerblendradius (`self.OuterBlendRadius`))
  (bind _outerblendradius_2 (`self.OuterBlendRadius`))
  (bind _depth_4 (`local.Depth`))
  (bind _outertop (`local.OuterTop`))
  (bind (_origin _boxextent) (`KismetSystemLibrary.GetComponentBounds` (`self.Box`)))
  (bind _z (.z (`SceneComponent.K2_GetComponentLocation` (`self.BlendCentre`))))
  (bind _y (.y _boxextent))
  (bind _x (.x (`SceneComponent.K2_GetComponentLocation` (`self.BlendCentre`))))
  (bind _y_2 (.y _origin))
  (`|ExecutionSequence`
    (:`then_0`
      (set `local.Right` (+ _y_2 _y))
      (set `local.Left` (- _y_2 _y))
      (switch `/Game/EpicTemplates/TemplateAgnostic/Blueprints/Enums/E2DCameraViewDirection` (`self.GamePerspective`)
        (:`NewEnumerator0`
          (set `local.Depth` (.x (`SceneComponent.K2_GetComponentLocation` (`self.BlendCentre`))))
          (set `local.InnerTop` (+ _z _innerblendradius_2))
          (set `local.InnerBottom` (- _z _innerblendradius_2))
          (set `local.OuterTop` (+ _z _outerblendradius))
          (set `local.OuterBottom` (- _z _outerblendradius)))
        (:`NewEnumerator1`
          (set `local.Depth` (.z (`SceneComponent.K2_GetComponentLocation` (`self.BlendCentre`))))
          (set `local.InnerTop` (+ _x _innerblendradius))
          (set `local.InnerBottom` (- _x _innerblendradius))
          (set `local.OuterTop` (+ _x _outerblendradius_2))
          (set `local.OuterBottom` (- _x _outerblendradius_2)))))
    (:`then_1`
      (`KismetSystemLibrary.DrawDebugLine` (`KismetMathLibrary.MakeVector` _depth_4 (`local.Left`) _outertop) (`KismetMathLibrary.MakeVector` _depth_4 (`local.Right`) _outertop) (`self.DebugOuterLineColor`) (`self.DebugLineTime`))
      (`KismetSystemLibrary.DrawDebugLine` (`KismetMathLibrary.MakeVector` _depth_2 (`local.Left`) _outerbottom) (`KismetMathLibrary.MakeVector` _depth_2 (`local.Right`) _outerbottom) (`self.DebugOuterLineColor`) (`self.DebugLineTime`))
      (`KismetSystemLibrary.DrawDebugLine` (`KismetMathLibrary.MakeVector` _depth_3 (`local.Left`) _innertop) (`KismetMathLibrary.MakeVector` _depth_3 (`local.Right`) _innertop) (`self.DebugInnerLineColor`) (`self.DebugLineTime`))
      (`KismetSystemLibrary.DrawDebugLine` (`KismetMathLibrary.MakeVector` _depth (`local.Left`) _innerbottom) (`KismetMathLibrary.MakeVector` _depth (`local.Right`) _innerbottom) (`self.DebugInnerLineColor`) (`self.DebugLineTime`)))))

(fn `DebugDrawBlendRadius`
  (bind _returnvalue (select `/Game/EpicTemplates/TemplateAgnostic/Blueprints/Enums/E2DCameraViewDirection` (`self.GamePerspective`) :`NewEnumerator0` (0.0 0.0 1.0) :`NewEnumerator1` (1.0 0.0 0.0) :!type "Vector Structure"))
  (switch `/Game/EpicTemplates/PlatformerTemplate/Blueprints/Enums/ECameraBlendAxis` (`self.BlendWorldAxis`)
    (:`NewEnumerator0`
      (`KismetSystemLibrary.DrawDebugCircle` (`SceneComponent.K2_GetComponentLocation` (`self.BlendCentre`)) (`self.OuterBlendRadius`) 20 (`self.DebugOuterLineColor`) (`self.DebugLineTime`) 0.0 (0.0 1.0 0.0) _returnvalue)
      (`KismetSystemLibrary.DrawDebugCircle` (`SceneComponent.K2_GetComponentLocation` (`self.BlendCentre`)) (`self.InnerBlendRadius`) 20 (`self.DebugInnerLineColor`) (`self.DebugLineTime`) 0.0 (0.0 1.0 0.0) _returnvalue))
    (:`NewEnumerator1`
      (`self.Debug Draw Horizontal Blend Radius`))
    (:`NewEnumerator2`
      (`self.Debug Draw Vertical Blend Radius`))))

(fn `GetCameraBounds`
  (returns (CameraBounds :type "/Game/EpicTemplates/PlatformerTemplate/Blueprints/Structs/CameraBounds2D Structure"))
  (locals (ActorLeftRight :type "Float (double-precision)" :default 0.0) (ActorUpDown :type "Float (double-precision)" :default 0.0))
  (bind _actorleftright (`local.ActorLeftRight`))
  (bind _actorupdown (`local.ActorUpDown`))
  (bind (_rightbound _rightboundenforced _leftbound _leftboundenforced _topbound _topboundenforced _bottombound _bottomboundenforced _clamptype _boundstagkey) (break `/Game/EpicTemplates/PlatformerTemplate/Blueprints/Structs/CameraBounds2D` (`self.CameraBounds`)))
  (bind _y (.y (`self.K2_GetActorLocation`)))
  (if (`self.bBoundsAreRelative`)
    (`|ExecutionSequence`
      (:`then_0`
        (switch `/Game/EpicTemplates/TemplateAgnostic/Blueprints/Enums/E2DCameraViewDirection` (`self.GamePerspective`)
          (:`NewEnumerator0`
            (set `local.ActorLeftRight` _y)
            (set `local.ActorUpDown` (.z (`self.K2_GetActorLocation`))))
          (:`NewEnumerator1`
            (set `local.ActorLeftRight` _y)
            (set `local.ActorUpDown` (.x (`self.K2_GetActorLocation`))))))
      (:`then_1`
        (return (make `/Game/EpicTemplates/PlatformerTemplate/Blueprints/Structs/CameraBounds2D` (+ _rightbound _actorleftright) _rightboundenforced (+ _leftbound _actorleftright) _leftboundenforced (+ _topbound _actorupdown) _topboundenforced (+ _bottombound _actorupdown) _bottomboundenforced _clamptype _boundstagkey))))
    (else
      (return (`self.CameraBounds`)))))

(fn `GetCameraPlatformerInterface`
  (returns (CameraInterface :type "/Game/EpicTemplates/PlatformerTemplate/Blueprints/Interfaces/BPI_Camera2D Interface"))
  (if (`KismetSystemLibrary.IsValidInterface` (`self.CachedPlatformerCameraInterface`))
    (return (`self.CachedPlatformerCameraInterface`))
    (else
      (bind (_cameraactor _camerainterface) (`/Game/EpicTemplates/PlatformerTemplate/Blueprints/PlatformerFunctionLibrary.GetPlatformerCamera`))
      (bind _output_get (set `self.CachedPlatformerCameraInterface` _camerainterface))
      (return _output_get))))

(fn `GetClosestPawnBlendAlpha`
  (returns (BlendAlpha :type "Float (double-precision)") (IsInBlendRadius :type Boolean))
  (locals (ClosestDistSq :type "Float (double-precision)" :default 0.0) (TempDistSq :type "Float (double-precision)" :default 0.0) (TempPawn :type "Pawn Object Reference"))
  (bind _x (.x (`self.K2_GetActorLocation` (`local.TempPawn`))))
  (bind _y (.y (`self.K2_GetActorLocation` (`local.TempPawn`))))
  (bind _y_2 (.y (`SceneComponent.K2_GetComponentLocation` (`self.BlendCentre`))))
  (bind _z (.z (`SceneComponent.K2_GetComponentLocation` (`self.BlendCentre`))))
  (bind _x_2 (.x (`SceneComponent.K2_GetComponentLocation` (`self.BlendCentre`))))
  (bind _y_3 (.y (`SceneComponent.K2_GetComponentLocation` (`self.BlendCentre`))))
  (bind _y_4 (.y (`self.K2_GetActorLocation` (`local.TempPawn`))))
  (bind _z_2 (.z (`self.K2_GetActorLocation` (`local.TempPawn`))))
  (set `local.ClosestDistSq` -1.0)
  (`|ExecutionSequence`
    (:`then_0`
      (for _array_element (`self.CurrentPlayerPawns`)
        (set `local.TempPawn` _array_element)
        (`|ExecutionSequence`
          (:`then_0`
            (switch `/Game/EpicTemplates/TemplateAgnostic/Blueprints/Enums/E2DCameraViewDirection` (`self.GamePerspective`)
              (:`NewEnumerator0`
                (set `local.TempDistSq` (select `/Game/EpicTemplates/PlatformerTemplate/Blueprints/Enums/ECameraBlendAxis` (`self.BlendWorldAxis`) :`NewEnumerator0` (`KismetMathLibrary.VSize2DSquared` (- (`KismetMathLibrary.MakeVector2D` _y_4 _z_2) (`KismetMathLibrary.MakeVector2D` _y_2 _z))) :`NewEnumerator1` (`KismetMathLibrary.Square` (- _y_4 _y_2)) :`NewEnumerator2` (`KismetMathLibrary.Square` (- _z_2 _z)))))
              (:`NewEnumerator1`
                (set `local.TempDistSq` (select `/Game/EpicTemplates/PlatformerTemplate/Blueprints/Enums/ECameraBlendAxis` (`self.BlendWorldAxis`) :`NewEnumerator0` (`KismetMathLibrary.VSize2DSquared` (- (`KismetMathLibrary.MakeVector2D` _y _x) (`KismetMathLibrary.MakeVector2D` _y_3 _x_2))) :`NewEnumerator1` (`KismetMathLibrary.Square` (- _y _y_3)) :`NewEnumerator2` (`KismetMathLibrary.Square` (- _x _x_2)))))))
          (:`then_1`
            (if (or (< (`local.TempDistSq`) (`local.ClosestDistSq`)) (< (`local.ClosestDistSq`) 0.0))
              (set `local.ClosestDistSq` (`local.TempDistSq`)))))))
    (:`then_1`
      (if (and (>= (`local.ClosestDistSq`) 0.0) (<= (`local.ClosestDistSq`) (`KismetMathLibrary.Square` (`self.OuterBlendRadius`))))
        (return (`KismetMathLibrary.MapRangeClamped` (`KismetMathLibrary.Sqrt` (`local.ClosestDistSq`)) (`self.OuterBlendRadius`) (`self.InnerBlendRadius`) 0.0 1.0) true)
        (else
          (return 0.0 false))))))

(fn `UserConstructionScript`
  (bind (_x _y) (`KismetMathLibrary.BreakVector2D` (`self.NormalisedBlendCentre`)))
  (bind _y_2 (.y (`BoxComponent.BoxExtent` (`self.Box`))))
  (bind _z (.z (`BoxComponent.BoxExtent` (`self.Box`))))
  (`BoxComponent.SetBoxExtent` (`self.Box`) (* (`self.TriggerSize`) 0.5) true)
  (`SceneComponent.K2_SetRelativeLocation` (`self.BlendCentre`) (`KismetMathLibrary.MakeVector` 0.0 (`KismetMathLibrary.MapRangeClamped` _x 0.0 1.0 (* _y_2 -1.0) _y_2) (`KismetMathLibrary.MapRangeClamped` _y 0.0 1.0 (* _z -1.0) _z)) false false))