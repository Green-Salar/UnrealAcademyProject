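; Controllable floating pawn that stands in for a dead actor until player-sourced damage revives it.
; Input accelerates it in the YZ plane with clamped speed and deceleration, using swept movement and bouncing off hits via reflected velocity.
; AddActortoRevive stores the target and activates the pawn.
; Its health interface reports dead, but ApplyDamage from a PlayerController hides the pawn and calls Revive on the target's BP_HealthComponent.
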(event `EnhancedInput|/Game/EpicTemplates/WalkingSimTemplate/Input/IA_MoveRight`
  (params (ActionValue :type "Float (double-precision)") (ElapsedSeconds :type "Float (double-precision)") (TriggeredSeconds :type "Float (double-precision)") (InputAction :type "InputAction Object Reference" :default "/Game/EpicTemplates/WalkingSimTemplate/Input/IA_MoveRight.IA_MoveRight"))
  ;[1 1 1] Input
  (:`Triggered`
    (set `self.InputVec` (`KismetMathLibrary.MakeVector2D` ActionValue (`.Y` (`KismetMathLibrary.BreakVector2D` (`self.InputVec`)))) :!label _label))
  (:`Completed`
    (goto _label)))

(event `self.ReceiveTick`
  (params (DeltaSeconds :type "Float (single-precision)"))
  (bind (_returnvalue_x _returnvalue_y) (`KismetMathLibrary.BreakVector2D` (* (`self.InputVec`) (`self.AccelerationSpeed`) DeltaSeconds)))
  ;[1 1 1] Tick
  (`|ExecutionSequence`
    (:`then_0`
      (if (> (`KismetMathLibrary.VSize2DSquared` (`self.InputVec`)) 1.0)
        (`KismetMathLibrary.Normalize2D` (`self.InputVec`))))
    (:`then_1`
      (if (> (`KismetMathLibrary.VSize2DSquared` (`self.InputVec`)) 0.0)
        (set `self.CurrentVelocity` (`KismetMathLibrary.ClampVectorSize` (+ (`self.CurrentVelocity`) (`KismetMathLibrary.MakeVector` 0.0 _returnvalue_x _returnvalue_y)) 0.0 (`self.MaxSpeed`)))
        (else
          (set `self.CurrentVelocity` (`KismetMathLibrary.VInterpTo_Constant` (`self.CurrentVelocity`) (0.0 0.0 0.0) DeltaSeconds (`self.DecelerationSpeed`))))))
    (:`then_2`
      (`self.K2_AddActorWorldOffset` (* (`self.CurrentVelocity`) DeltaSeconds) true))))

(event `EnhancedInput|/Game/EpicTemplates/WalkingSimTemplate/Input/IA_MoveForward`
  (params (ActionValue :type "Float (double-precision)") (ElapsedSeconds :type "Float (double-precision)") (TriggeredSeconds :type "Float (double-precision)") (InputAction :type "InputAction Object Reference" :default "/Game/EpicTemplates/WalkingSimTemplate/Input/IA_MoveForward.IA_MoveForward"))
  ;[1 1 1] Input
  (:`Triggered`
    (set `self.InputVec` (`KismetMathLibrary.MakeVector2D` (`KismetMathLibrary.BreakVector2D` (`self.InputVec`)) ActionValue) :!label _label_2))
  (:`Completed`
    (goto _label_2)))

(event `self.SphereRoot.OnComponentHit`
  (params (HitComponent :type "PrimitiveComponent Object Reference") (OtherActor :type "Actor Object Reference") (OtherComp :type "PrimitiveComponent Object Reference") (NormalImpulse :type "Vector Structure") (Hit :type "HitResult Structure (by ref)"))
  ;[1 1 1] Health Interface
  (set `self.CurrentVelocity` (`KismetMathLibrary.ClampVectorSize` (* (`KismetMathLibrary.GetReflectionVector` (`self.CurrentVelocity`) (`.ImpactNormal` (`GameplayStatics.BreakHitResult` Hit))) 1.1) (`self.MinBounceKickback`) (`self.MaxSpeed`))))

(event `/Game/EpicTemplates/PlatformerTemplate/Blueprints/Interfaces/BPI_RevivalSource.AddActorToRevive`
  (params (ActorToRevive :type "Actor Object Reference"))
  ;[1 1 1] Reviver Interface
  (set `self.ActorToRevive` ActorToRevive)
  (`self.SetActorHiddenInGame` false)
  (`PrimitiveComponent.SetCollisionEnabled` (`self.SphereRoot`) "QueryAndPhysics")
  (`self.SetActorTickEnabled` true))

(fn `ApplyDamage`
  (params (InDamage :type "/Game/EpicTemplates/TemplateAgnostic/Blueprints/Structs/DamageStruct Structure (by ref)"))
  (returns (DamageDealt :type "Float (double-precision)") (DamageApplied :type Boolean))
  (cast `PlayerController` (`.DamageSourceOwner_16_93F98FB747ED83B90B1FAFB49CE3E4D5` (break `/Game/EpicTemplates/TemplateAgnostic/Blueprints/Structs/DamageStruct` InDamage))
    (:`then`
      (`self.SetActorHiddenInGame` true)
      (`PrimitiveComponent.SetCollisionEnabled` (`self.SphereRoot`) "NoCollision")
      (`self.SetActorTickEnabled` false)
      (`/Game/EpicTemplates/TemplateAgnostic/Blueprints/Interfaces/BPI_HealthSource.Revive` (`self.GetComponentByClass` (`self.ActorToRevive`) "/Game/EpicTemplates/TemplateAgnostic/Blueprints/Components/BP_HealthComponent.BP_HealthComponent_C") self "NewEnumerator0")
      (return 0.0 true))
    (:`CastFailed`
      (return 0.0 false))))

(fn `GetCurrentHealth`
  (returns (CurrentHealth :type "Float (double-precision)"))
  (return 0.0))

(fn `GetMaxHealth`
  (returns (MaxHealth :type "Float (double-precision)"))
  (return 0.0))

(fn `InstantKill`
  (params (KillDamageInfo :type "/Game/EpicTemplates/TemplateAgnostic/Blueprints/Structs/DamageStruct Structure"))
  (returns (KillAccepted :type Boolean) (DamageDealt :type "Float (double-precision)"))
  (return false 0.0))

(fn `IsDead`
  (returns (bIsDead :type Boolean))
  (return true))

(fn `UserConstructionScript`)