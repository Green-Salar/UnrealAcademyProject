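; Blueprint function library for a platformer template, providing camera helpers.
; GetClampedLocationAgainstCameraBounds keeps a 2D camera location inside enforced world bounds, using the rotated view plane's axis-aligned half extents to inset each edge.
; When the view would break both opposing bounds on an axis, it centers between them instead.
; GetPlatformerCamera fetches the camera actor and its interface from the platformer game mode.
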(fn `Get Clamped Location Against Camera Bounds`
  (params (DesiredWorldLocation :type "Vector2D Structure (by ref)") (PlaneRotation :type "Float (double-precision)") (ViewPlaneWidth :type "Float (double-precision)") (ViewPlaneHeight :type "Float (double-precision)") (WorldCameraBounds2D :type "/Game/EpicTemplates/PlatformerTemplate/Blueprints/Structs/CameraBounds2D Structure (by ref)"))
  (returns (ClampedWorldLoc :type "Vector2D Structure"))
  (locals (WorldSpaceHalfPlaneWidth :type "Float (double-precision)") (WorldSpaceHalfPlaneHeight :type "Float (double-precision)") (AdjustedRightBound :type "Float (double-precision)") (AdjustedLeftBound :type "Float (double-precision)") (AdjustedTopBound :type "Float (double-precision)") (AdjustedBottomBound :type "Float (double-precision)") (OutputX :type "Float (double-precision)" :default 0.0) (OutputY :type "Float (double-precision)" :default 0.0) (bWantsToBreakRightBound :type Boolean) (bWantsToBreakTopBound :type Boolean))
  (bind (_x _y) (`KismetMathLibrary.BreakVector2D` DesiredWorldLocation))
  (bind _planerotation (`local.PlaneRotation`))
  (bind _planerotation_2 (`local.PlaneRotation`))
  (bind ((`BottomBound_20_4E0F3BC84135212F4EBA348704CC56D3` _bottombound) (`BottomBoundEnforced_17_9C9E89D844DA269EA0699A94B3C3384E` _bottomboundenforced)) (break `/Game/EpicTemplates/PlatformerTemplate/Blueprints/Structs/CameraBounds2D` (`local.WorldCameraBounds2D`)))
  (bind (_rightbound _rightboundenforced) (break `/Game/EpicTemplates/PlatformerTemplate/Blueprints/Structs/CameraBounds2D` (`local.WorldCameraBounds2D`)))
  (bind ((`LeftBound_18_804958EB4226E33CCC4E61A4E67CF02A` _leftbound) (`LeftBoundEnforced_13_84183321427389C686D88F988E67DFE7` _leftboundenforced)) (break `/Game/EpicTemplates/PlatformerTemplate/Blueprints/Structs/CameraBounds2D` (`local.WorldCameraBounds2D`)))
  (bind ((`TopBound_19_AFFFFCB14FD1EBF8C402B0ACE31DF3AC` _topbound) (`TopBoundEnforced_15_E73BC6294A163985CF6926A7D62F4436` _topboundenforced)) (break `/Game/EpicTemplates/PlatformerTemplate/Blueprints/Structs/CameraBounds2D` (`local.WorldCameraBounds2D`)))
  (set `local.OutputX` _x)
  (set `local.OutputY` _y)
  (set `local.WorldSpaceHalfPlaneWidth` (* (+ (`KismetMathLibrary.Abs` (* (`KismetMathLibrary.DegCos` _planerotation_2) (`local.ViewPlaneWidth`))) (`KismetMathLibrary.Abs` (* (`KismetMathLibrary.DegSin` _planerotation_2) (`local.ViewPlaneHeight`)))) 0.5))
  (set `local.WorldSpaceHalfPlaneHeight` (* (+ (`KismetMathLibrary.Abs` (* (`KismetMathLibrary.DegSin` _planerotation) (`local.ViewPlaneWidth`))) (`KismetMathLibrary.Abs` (* (`KismetMathLibrary.DegCos` _planerotation) (`local.ViewPlaneHeight`)))) 0.5))
  (`|ExecutionSequence`
    (:`then_0`
      (if _rightboundenforced
        (bind _output_get (set `local.AdjustedRightBound` (- _rightbound (`local.WorldSpaceHalfPlaneWidth`))))
        (if (> (`local.OutputX`) _output_get)
          (set `local.OutputX` (`local.AdjustedRightBound`))
          (set `local.bWantsToBreakRightBound` true))))
    (:`then_1`
      (if _leftboundenforced
        (bind _output_get_2 (set `local.AdjustedLeftBound` (+ _leftbound (`local.WorldSpaceHalfPlaneWidth`))))
        (if (< (`local.OutputX`) _output_get_2)
          (if (`local.bWantsToBreakRightBound`)
            (set `local.OutputX` (* (+ (`local.AdjustedLeftBound`) (`local.AdjustedRightBound`)) 0.5))
            (else
              (set `local.OutputX` (`local.AdjustedLeftBound`)))))))
    (:`then_2`
      (if _topboundenforced
        (set `local.AdjustedTopBound` (- _topbound (`local.WorldSpaceHalfPlaneHeight`)))
        (if (> (`local.OutputY`) (`local.AdjustedTopBound`))
          (set `local.OutputY` (`local.AdjustedTopBound`))
          (set `local.bWantsToBreakTopBound` true))))
    (:`then_3`
      (if _bottomboundenforced
        (set `local.AdjustedBottomBound` (+ _bottombound (`local.WorldSpaceHalfPlaneHeight`)))
        (if (< (`local.OutputY`) (`local.AdjustedBottomBound`))
          (if (`local.bWantsToBreakTopBound`)
            (set `local.OutputY` (* (+ (`local.AdjustedBottomBound`) (`local.AdjustedTopBound`)) 0.5))
            (else
              (set `local.OutputY` (`local.AdjustedBottomBound`)))))))
    (:`then_4`
      (return (`KismetMathLibrary.MakeVector2D` (`local.OutputX`) (`local.OutputY`))))))

(fn `GetPlatformerCamera`
  (returns (CameraActor :type "Actor Object Reference") (CameraInterface :type "/Game/EpicTemplates/PlatformerTemplate/Blueprints/Interfaces/BPI_Camera2D Interface"))
  (bind _asbp_game_mode_platformer (cast `/Game/EpicTemplates/PlatformerTemplate/Blueprints/Core/BP_GameMode_Platformer` (`GameplayStatics.GetGameMode` null))
    (:`then`
      (bind (_cameraactor _camerainterface) (`/Game/EpicTemplates/PlatformerTemplate/Blueprints/Core/BP_GameMode_Platformer.GetPlatformerCamera` _asbp_game_mode_platformer))
      (return _cameraactor _camerainterface))
    (:`CastFailed`
      (return null null))))