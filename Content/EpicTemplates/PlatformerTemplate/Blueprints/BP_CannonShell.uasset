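; Pooled cannon shell projectile that damages what it strikes and explodes.
; On launch it aligns local Y to the given direction and sets ProjectileMovement velocity, falling back to a default speed.
; A sphere hit or overlap applies damage through BPI_Damageable, spawns an async-loaded Niagara explosion, then hides and disables the shell.
; ReusableActorComponent marks it for reuse and drives reset or destruction, avoiding a respawn per shot.
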(event `self.ReusableActorComponent.OnResetRequested`
  (params (Caller :type "/Game/EpicTemplates/TemplateAgnostic/Blueprints/Components/BP_ReusableActorComponent Object Reference") (ResetActor :type "Actor Object Reference"))
  (`PrimitiveComponent.SetCollisionEnabled` (`self.SphereCollision`) "QueryOnly")
  (`self.SetActorHiddenInGame` false)
  (`ActorComponent.Activate` (`self.ProjectileMovement`) true))

(event `self.ReusableActorComponent.OnRequestDestroySelf`
  (`self.K2_DestroyActor`))

(event `self.SphereCollision.OnComponentHit`
  (params (HitComponent :type "PrimitiveComponent Object Reference") (OtherActor :type "Actor Object Reference") (OtherComp :type "PrimitiveComponent Object Reference") (NormalImpulse :type "Vector Structure") (Hit :type "HitResult Structure (by ref)"))
  (`self.HandleCollision` OtherActor))

(event `self.SphereCollision.OnComponentBeginOverlap`
  (params (OverlappedComponent :type "PrimitiveComponent Object Reference") (OtherActor :type "Actor Object Reference") (OtherComp :type "PrimitiveComponent Object Reference") (OtherBodyIndex :type Integer) (bFromSweep :type Boolean) (SweepResult :type "HitResult Structure (by ref)"))
  (`self.HandleCollision` OtherActor))

(event `/Game/EpicTemplates/TemplateAgnostic/Blueprints/Interfaces/BPI_Projectile.LaunchInDirection`
  (params (ProjectileOwner :type "Actor Object Reference") (Direction :type "Vector Structure") (Speed :type "Float (double-precision)"))
  ;[1 1 1] Projectile Interface
  (`self.K2_SetActorRotation` (`KismetMathLibrary.MakeRotFromY` Direction))
  (bind _output_get (set `self.CurrentProjectileSpeed` (select `bool` (<= Speed 0.0) :`false` Speed :`true` (`self.DefaultLaunchSpeed`))))
  (`ProjectileMovementComponent.SetVelocityInLocalSpace` (`self.ProjectileMovement`) (`KismetMathLibrary.MakeVector` 0.0 _output_get)))

(event `PlayExplosionParticle`
  (bind _object (`|LoadAsset` (`self.ExplosionParticle`))
    (:`Completed`
      (bind _asniagara_system (cast `NiagaraSystem` _object))
      (`NiagaraFunctionLibrary.SpawnSystemAtLocation` _asniagara_system (`self.K2_GetActorLocation`) (struct) (1.0 1.0 1.0) true true "AutoRelease"))))

(fn `DisableProjectile`
  (`PrimitiveComponent.SetCollisionEnabled` (`self.SphereCollision`) "NoCollision")
  (`self.SetActorHiddenInGame` true)
  (`ActorComponent.Deactivate` (`self.ProjectileMovement`))
  (`/Game/EpicTemplates/TemplateAgnostic/Blueprints/Components/BP_ReusableActorComponent.MarkReadyForReuse` (`self.ReusableActorComponent`)))

(fn `HandleCollision`
  (params (Actor :type "Actor Object Reference"))
  (`|ExecutionSequence`
    (:`then_0`
      (bind _interfaceimplementingobject (`/Game/EpicTemplates/TemplateAgnostic/Blueprints/EpicTemplatesFunctionLibrary.SearchActorForInterface` Actor "/Game/EpicTemplates/TemplateAgnostic/Blueprints/Interfaces/BPI_Damageable.BPI_Damageable_C"))
      (`/Engine/EditorBlueprintResources/StandardMacros.IsValid` _interfaceimplementingobject
        (:`Is Valid`
          (message `/Game/EpicTemplates/TemplateAgnostic/Blueprints/Interfaces/BPI_Damageable.ApplyDamage` _interfaceimplementingobject (make `/Game/EpicTemplates/TemplateAgnostic/Blueprints/Structs/DamageStruct` (`self.Damage`) self self (`self.K2_GetActorLocation`) (`MovementComponent.Velocity` (`self.ProjectileMovement`)))))))
    (:`then_1`
      (`self.PlayExplosionParticle`)
      (`self.DisableProjectile`))))

(fn `UserConstructionScript`)