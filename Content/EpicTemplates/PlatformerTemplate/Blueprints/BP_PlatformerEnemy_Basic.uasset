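; Basic side-scrolling platformer enemy that walks left or right along Y and damages what it bumps into through BPI_Damageable.
; Tick feeds movement input and capsule-traces ahead for ledges to stop or turn around as configured, switching itself off when walking stops.
; Capsule hits apply damage, and roughly sideways ones steer it away from the impact.
; On death it drops collision, launches upward and shifts its plane constraint origin.
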(event `self.CapsuleComponent.OnComponentHit`
  (params (HitComponent :type "PrimitiveComponent Object Reference") (OtherActor :type "Actor Object Reference") (OtherComp :type "PrimitiveComponent Object Reference") (NormalImpulse :type "Vector Structure") (Hit :type "HitResult Structure (by ref)"))
  ;[1 1 1] CapsuleHit
  (`self.HandleHit` OtherActor Hit))

(event `self.HealthComponent.OnDied`
  (params (Caller :type "/Game/EpicTemplates/TemplateAgnostic/Blueprints/Components/BP_HealthComponent Object Reference") (KillingDamageSourceOwner :type "Actor Object Reference") (KillingDamageSource :type "Actor Object Reference") (KillingDamageLocation :type "Vector Structure") (KillingDamageDirection :type "Vector Structure") (HitBone :type Name) (SpecialDamageName :type Name))
  (bind _charactermovement (`self.CharacterMovement`))
  ;[1 1 1] OnDied
  (`PrimitiveComponent.SetCollisionEnabled` (`self.CapsuleComponent`) "NoCollision")
  (`self.OnEnemyDied`)
  (`self.LaunchCharacter` (* (0.0 0.0 1.0) (`self.DeathLaunchVelocity`)))
  (set `CharacterMovementComponent.GravityScale` (`self.DeathGravity`) _charactermovement)
  (`MovementComponent.SetPlaneConstraintOrigin` _charactermovement (- (`MovementComponent.GetPlaneConstraintOrigin` _charactermovement) (1.0 0.0 0.0))))

(event `self.ReceiveBeginPlay`
  ;[1 1 1] BeginPlay
  (`self.UpdateWalkDirection` (`self.StartWalkDirection`)))

(event `self.ReceiveTick`
  (params (DeltaSeconds :type "Float (single-precision)"))
  ;[1 1 1] Tick
  (`self.CheckForLedge`)
  (`PawnMovementComponent.AddInputVector` (`self.CharacterMovement`) (select `/Game/EpicTemplates/PlatformerTemplate/Blueprints/Enums/EEnemyWalkDirection` (`self.CurrentWalkDirection`) :`NewEnumerator1` (0.0 1.0 0.0) :`NewEnumerator2` (0.0 -1.0 0.0) :!type "Vector Structure") false))

(event `UpdateWalkDirection`
  (params (NewWalkDirection :type "/Game/EpicTemplates/PlatformerTemplate/Blueprints/Enums/EEnemyWalkDirection Enum" :default "NewEnumerator0"))
  ;[1 1 1] UpdateWalkDirection
  (if (`|EnumInequality` NewWalkDirection (`self.CurrentWalkDirection`))
    (bind _output_get (set `self.CurrentWalkDirection` NewWalkDirection))
    (`self.SetActorTickEnabled` (`|EnumInequality` _output_get "NewEnumerator0"))))

(fn `CheckForLedge`
  (locals (CapsuleTraceStart :type "Vector Structure"))
  (bind _capsulecomponent (`self.CapsuleComponent`))
  (if (`|EnumInequality` (`self.LedgeBehaviour`) "NewEnumerator0")
    (set `local.CapsuleTraceStart` (+ (`self.K2_GetActorLocation`) (`KismetMathLibrary.MakeVector` 0.0 (* (* (`CapsuleComponent.GetScaledCapsuleRadius` (`self.CapsuleComponent`)) 2.0) (select `/Game/EpicTemplates/PlatformerTemplate/Blueprints/Enums/EEnemyWalkDirection` (`self.CurrentWalkDirection`) :`NewEnumerator1` 1.0 :`NewEnumerator2` -1.0)))))
    (bind (_outhit _returnvalue) (`KismetSystemLibrary.CapsuleTraceSingleByProfile` (`local.CapsuleTraceStart`) (- (`local.CapsuleTraceStart`) (`KismetMathLibrary.MakeVector` 0.0 0.0 (+ (`CharacterMovementComponent.MaxStepHeight` (`self.CharacterMovement`)) 1.0))) (`CapsuleComponent.GetScaledCapsuleRadius` _capsulecomponent) (`CapsuleComponent.GetScaledCapsuleHalfHeight` _capsulecomponent) (`PrimitiveComponent.GetCollisionProfileName` _capsulecomponent)))
    (if (not _returnvalue)
      (`self.UpdateWalkDirection` (select `/Game/EpicTemplates/PlatformerTemplate/Blueprints/Enums/EEnemyLedgeBehavior` (`self.LedgeBehaviour`) :`NewEnumerator0` "NewEnumerator0" :`NewEnumerator1` "NewEnumerator0" :`NewEnumerator2` (select `/Game/EpicTemplates/PlatformerTemplate/Blueprints/Enums/EEnemyWalkDirection` (`self.CurrentWalkDirection`) :`NewEnumerator0` "NewEnumerator0" :`NewEnumerator1` "NewEnumerator2" :`NewEnumerator2` "NewEnumerator1" :!type "/Game/EpicTemplates/PlatformerTemplate/Blueprints/Enums/EEnemyWalkDirection Enum"))))))

(fn `HandleHit`
  (params (HitActor :type "Actor Object Reference") (Hit :type "HitResult Structure (by ref)"))
  (bind (_bblockinghit _binitialoverlap _time _distance _location _impactpoint _normal _impactnormal _physmat _hitactor _hitcomponent _hitbonename) (`GameplayStatics.BreakHitResult` (`local.Hit`)))
  (`|ExecutionSequence`
    (:`then_0`
      (bind _interfaceimplementingobject (`/Game/EpicTemplates/TemplateAgnostic/Blueprints/EpicTemplatesFunctionLibrary.SearchActorForInterface` (`local.HitActor`) "/Game/EpicTemplates/TemplateAgnostic/Blueprints/Interfaces/BPI_Damageable.BPI_Damageable_C"))
      (`/Engine/EditorBlueprintResources/StandardMacros.IsValid` _interfaceimplementingobject
        (:`Is Valid`
          (message `/Game/EpicTemplates/TemplateAgnostic/Blueprints/Interfaces/BPI_Damageable.ApplyDamage` _interfaceimplementingobject (make `/Game/EpicTemplates/TemplateAgnostic/Blueprints/Structs/DamageStruct` (`self.HitPlayerDamage`) self self _impactpoint (select `/Game/EpicTemplates/PlatformerTemplate/Blueprints/Enums/EEnemyWalkDirection` (`self.CurrentWalkDirection`) :`NewEnumerator1` (0.0 1.0 0.0) :`NewEnumerator2` (0.0 -1.0 0.0) :!type "Vector Structure") _hitbonename)))))
    (:`then_1`
      (if (`|EnumInequality` (`self.CurrentWalkDirection`) "NewEnumerator0")
        (if (> (`KismetMathLibrary.Abs` (.y (`.Normal` (`GameplayStatics.BreakHitResult` (`local.Hit`))))) 0.707)
          (`self.UpdateWalkDirection` (select `bool` (<= (.y (`KismetMathLibrary.InverseTransformLocation` (`self.GetTransform`) (`.ImpactPoint` (`GameplayStatics.BreakHitResult` (`local.Hit`))))) 0.0) :`false` "NewEnumerator2" :`true` "NewEnumerator1" :!type "/Game/EpicTemplates/PlatformerTemplate/Blueprints/Enums/EEnemyWalkDirection Enum")))))))

(fn `UserConstructionScript`)