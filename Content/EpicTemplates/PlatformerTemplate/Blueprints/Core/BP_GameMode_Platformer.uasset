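; Platformer game mode Blueprint that provides and tracks the game's shared 2D platformer camera.
; GetPlatformerCamera returns the cached camera, otherwise takes the first actor implementing BPI_Camera2D, or blocking-loads and spawns the fallback camera class at a fixed location.
; Both the actor and its interface reference are cached, and UpdatePlatformerCamera replaces them when given a new camera actor.
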(fn `GetPlatformerCamera`
  (returns (CameraActor :type "Actor Object Reference") (CameraInterface :type "/Game/EpicTemplates/PlatformerTemplate/Blueprints/Interfaces/BPI_Camera2D Interface"))
  (`/Engine/EditorBlueprintResources/StandardMacros.IsValid` (`self.PlatformerCameraActor`)
    (:`Is Valid`
      (return (`self.PlatformerCameraActor`) (`self.PlatformerCameraInterface`)))
    (:`Is Not Valid`
      (bind _outactors (`GameplayStatics.GetAllActorsWithInterface` "/Game/EpicTemplates/PlatformerTemplate/Blueprints/Interfaces/BPI_Camera2D.BPI_Camera2D_C"))
      (if (> (`KismetArrayLibrary.Array_Length` _outactors) 0)
        (bind _output_get (set `self.PlatformerCameraActor` (`|GetArrayItem` _outactors)))
        (`|ExecutionSequence`
          (:`then_0`
            (bind _asbpi_camera_2d (cast `/Game/EpicTemplates/PlatformerTemplate/Blueprints/Interfaces/BPI_Camera2D` _output_get))
            (set `self.PlatformerCameraInterface` _asbpi_camera_2d))
          (:`then_1`
            (return (`self.PlatformerCameraActor`) (`self.PlatformerCameraInterface`))))
        (else
          (bind _returnvalue (`KismetSystemLibrary.LoadClassAsset_Blocking` (`self.FallbackCameraClass`)))
          (bind _asactor (castclass `Actor` _returnvalue))
          (bind _returnvalue_2 (`|SpawnActorFromClass` _asactor (`KismetMathLibrary.MakeTransform` (-1000.0 0.0 0.0)) "Undefined" "MultiplyWithRoot" null null))
          (bind _output_get_2 (set `self.PlatformerCameraActor` _returnvalue_2))
          (`|ExecutionSequence`
            (:`then_0`
              (bind _asbpi_camera_2d_2 (cast `/Game/EpicTemplates/PlatformerTemplate/Blueprints/Interfaces/BPI_Camera2D` _output_get_2))
              (set `self.PlatformerCameraInterface` _asbpi_camera_2d_2))
            (:`then_1`
              (return (`self.PlatformerCameraActor`) (`self.PlatformerCameraInterface`)))))))))

(fn `UpdatePlatformerCamera`
  (params (PlatformerCameraActor :type "Actor Object Reference"))
  (bind _output_get (set `self.PlatformerCameraActor` PlatformerCameraActor))
  (bind _asbpi_camera_2d (cast `/Game/EpicTemplates/PlatformerTemplate/Blueprints/Interfaces/BPI_Camera2D` _output_get))
  (set `self.PlatformerCameraInterface` _asbpi_camera_2d))

(fn `UserConstructionScript`
  (`parent.UserConstructionScript`))