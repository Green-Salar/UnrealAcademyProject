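; Player character for a side-scrolling platformer, with plane-locked movement, screen-edge blocking and enemy stomping.
; Jump apex, release and head-bump events switch gravity scale for hover and drop, while landing restores it and damages whatever is stomped.
; HealthComponent events drive knockback, flicker, input lockout, and death via possessing a separate dead-player pawn until revived.
; Looping timers record the last safe static floor and respawn the player below a Z threshold.
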(event `EnhancedInput|/Game/EpicTemplates/WalkingSimTemplate/Input/IA_MoveRight`
  (params (ActionValue :type "Float (double-precision)") (ElapsedSeconds :type "Float (double-precision)") (TriggeredSeconds :type "Float (double-precision)") (InputAction :type "InputAction Object Reference" :default "/Game/EpicTemplates/WalkingSimTemplate/Input/IA_MoveRight.IA_MoveRight"))
  ;[1 1 1] Input
  (:`Triggered`
    (bind _caninput (`self.CheckForScreenEdgeInputBlock` ActionValue))
    (if _caninput
      (`PawnMovementComponent.AddInputVector` (`self.CharacterMovement`) (`KismetMathLibrary.MakeVector` 0.0 ActionValue) false))))

(event `/Game/EpicTemplates/TemplateAgnostic/Blueprints/Interfaces/BPI_Debuggable.UpdateIsInDebug`
  (params (bInIsDebug :type Boolean))
  ;[1 1 1] Debuggable Interface
  (set `self.In Is Debug` bInIsDebug))

(event `CheckForRespawnableFloor`
  ;[1 1 1] Respawning from fall
  (bind _bvalidforrespawn (`self.IsHitSafeForRespawnableFloor` (`.HitResult` (break `FindFloorResult` (`CharacterMovementComponent.CurrentFloor` (`self.CharacterMovement`))))))
  (if _bvalidforrespawn
    (set `self.LastSafeFloorLocation` (`self.K2_GetActorLocation`))))

(event `self.ReceiveBeginPlay`
  ;[1 1 1] BeginPlay
  (`|ExecutionSequence`
    (:`then_0`
      (set `self.CurrentDepth` (.x (`self.K2_GetActorLocation`)))
      (add `self.OnReachedJumpApex` (`|CreateDelegate` :!event `ReachedJumpApex`))
      (set `self.LastSafeFloorLocation` (`self.K2_GetActorLocation`)))
    (:`then_1`
      (if (`self.bAutoRespawnBelowCertainZ`)
        (bind _returnvalue (`KismetSystemLibrary.K2_SetTimerDelegate` (`|CreateDelegate` :!event `CheckForKillZ`) 0.5 true))
        (set `self.CheckForKillZTimer` _returnvalue)))))

(event `EnhancedInput|/Game/EpicTemplates/PlatformerTemplate/Input/IA_Jump`
  (params (ActionValue :type Boolean) (ElapsedSeconds :type "Float (double-precision)") (TriggeredSeconds :type "Float (double-precision)") (InputAction :type "InputAction Object Reference" :default "/Game/EpicTemplates/PlatformerTemplate/Input/IA_Jump.IA_Jump"))
  ;[1 1 1] Input
  (:`Triggered`
    (if (not (`self.IsMoveInputIgnored`))
      (bind _output_get (set `self.JumpHeld` ActionValue))
      (if _output_get
        (if (not (`self.bLaunched`))
          (set `CharacterMovementComponent.bNotifyApex` true (`self.CharacterMovement`))
          (`self.Jump`))
        (else
          (`self.StopJumping`)
          (if (`NavMovementComponent.IsFalling` (`self.CharacterMovement`))
            (if (not (`self.bLaunched`))
              (set `CharacterMovementComponent.bNotifyApex` false (`self.CharacterMovement`))
              (`self.StartDrop`)
              (if (`KismetSystemLibrary.K2_IsTimerActiveHandle` (`self.ApexHoverTimer`))
                (`KismetSystemLibrary.K2_ClearAndInvalidateTimerHandle` (`self.ApexHoverTimer`))))))))))

(event `RespawnPlayerAtLastSafeLocation`
  (params (Damage :type "/Game/EpicTemplates/TemplateAgnostic/Blueprints/Structs/DamageStruct Structure (by ref)"))
  ;[1 1 1] Respawning from fall
  (`self.K2_SetActorLocation` (`self.LastSafeFloorLocation`))
  (`/Game/EpicTemplates/TemplateAgnostic/Blueprints/Interfaces/BPI_Damageable.ApplyDamage` (`self.HealthComponent`) Damage)
  (set `MovementComponent.Velocity` (0.0 0.0 0.0) (`self.CharacterMovement`)))

(event `HitReactFlicker`
  ;[1 1 1] Health Component
  (`SceneComponent.ToggleVisibility` (`self.Mesh`) true))

(event `UnlockInput`
  ;[1 1 1] Input
  (`self.EnableInput` (`self.CurrentPlayerCont`)))

(event `CheckForKillZ`
  ;[1 1 1] Respawning from fall
  (if (< (.z (`self.K2_GetActorLocation`)) (`self.AutoRespawnZThreshold`))
    (`self.RespawnPlayerAtLastSafeLocation` (struct))))

(event `self.HealthComponent.OnTookDamage`
  (params (Caller :type "/Game/EpicTemplates/TemplateAgnostic/Blueprints/Components/BP_HealthComponent Object Reference") (OldHealth :type "Float (double-precision)") (NewHealth :type "Float (double-precision)") (SpecialDamageName :type Name) (DamageStruct :type "/Game/EpicTemplates/TemplateAgnostic/Blueprints/Structs/DamageStruct Structure (by ref)"))
  ;[1 1 1] Health Component
  (`self.HandleTookDamage` DamageStruct NewHealth))

(event `EnhancedInput|/Game/EpicTemplates/WalkingSimTemplate/Input/IA_Cancel`
  (params (ActionValue :type Boolean) (ElapsedSeconds :type "Float (double-precision)") (TriggeredSeconds :type "Float (double-precision)") (InputAction :type "InputAction Object Reference" :default "/Game/EpicTemplates/WalkingSimTemplate/Input/IA_Cancel.IA_Cancel"))
  ;[1 1 1] Input
  ;;[1 1 1] Unused input
)

(event `EnhancedInput|/Game/EpicTemplates/PlatformerTemplate/Input/IA_VerticalMovement`
  (params (ActionValue :type "Float (double-precision)") (ElapsedSeconds :type "Float (double-precision)") (TriggeredSeconds :type "Float (double-precision)") (InputAction :type "InputAction Object Reference" :default "/Game/EpicTemplates/PlatformerTemplate/Input/IA_VerticalMovement.IA_VerticalMovement"))
  ;[1 1 1] Input
  ;;[1 1 1] Unused input
)

(event `EnhancedInput|/Game/EpicTemplates/PlatformerTemplate/Input/IA_Attack`
  (params (ActionValue :type Boolean) (ElapsedSeconds :type "Float (double-precision)") (TriggeredSeconds :type "Float (double-precision)") (InputAction :type "InputAction Object Reference" :default "/Game/EpicTemplates/PlatformerTemplate/Input/IA_Attack.IA_Attack"))
  ;[1 1 1] Input
  ;;[1 1 1] Unused input
)

(event `EndDamageReact`
  ;[1 1 1] Health Component
  (`/Game/EpicTemplates/TemplateAgnostic/Blueprints/Components/BP_HealthComponent.DisableInvincibility` (`self.HealthComponent`))
  (`KismetSystemLibrary.K2_ClearAndInvalidateTimerHandle` (`self.DamageReactFlickerTimer`))
  (`SceneComponent.SetVisibility` (`self.Mesh`) true true))

(event `self.ReceivePossessed`
  (params (NewController :type "Controller Object Reference"))
  ;[1 1 1] Possessed
  (`parent.ReceivePossessed` NewController)
  (bind _asplayer_controller (cast `PlayerController` NewController))
  (set `self.CurrentPlayerCont` _asplayer_controller)
  (`KismetSystemLibrary.DelayUntilNextTick`) ; One frame delay, because character isn't fully possessed until\nafter this funciton is over, and player controller's don't like mapping\ncotexts being added on the first frame they are alive
  (`|ExecutionSequence`
    (:`then_0`
      (`/Engine/EditorBlueprintResources/StandardMacros.DoOnce` false
        (:`Completed`
          (`EnhancedInputSubsystemInterface.AddMappingContext` (pcsubsystem `EnhancedInputLocalPlayerSubsystem` _asplayer_controller) "/Game/EpicTemplates/PlatformerTemplate/Input/IMC_Platformer.IMC_Platformer" 0 (struct)))))
    (:`then_1`
      (`/Game/EpicTemplates/TemplateAgnostic/Blueprints/EpicTemplatesObjectMacroLibrary.!!!IsNOTValid!!!` (`self.PlatformerUI`)
        (:`Is NOT Valid`
          (bind _returnvalue (`|CreateWidget` "/Game/EpicTemplates/PlatformerTemplate/UI/W_GameUI_Platformer.W_GameUI_Platformer_C" _asplayer_controller))
          (set `self.PlatformerUI` _returnvalue))))
    (:`then_2`
      (`UserWidget.AddToViewport` (`self.PlatformerUI`) 0))))

(event `self.HealthComponent.OnDied`
  (params (Caller :type "/Game/EpicTemplates/TemplateAgnostic/Blueprints/Components/BP_HealthComponent Object Reference") (KillingDamageSourceOwner :type "Actor Object Reference") (KillingDamageSource :type "Actor Object Reference") (KillingDamageLocation :type "Vector Structure") (KillingDamageDirection :type "Vector Structure") (HitBone :type Name) (SpecialDamageName :type Name))
  (bind _charactermovement (`self.CharacterMovement`))
  ;[1 1 1] Health Component
  (`self.DisableInput` (`self.CurrentPlayerCont`))
  (`SceneComponent.SetVisibility` (`self.Mesh`) false true)
  (`self.ClearAllTimers`)
  (`PrimitiveComponent.SetCollisionEnabled` (`self.CapsuleComponent`) "NoCollision")
  (set `CharacterMovementComponent.GravityScale` 0.0 _charactermovement)
  (set `MovementComponent.Velocity` (0.0 0.0 0.0) _charactermovement)
  (`ActorComponent.SetActive` (`self.CharacterMovement`) false false)
  (`/Game/EpicTemplates/TemplateAgnostic/Blueprints/EpicTemplatesObjectMacroLibrary.!!!IsNOTValid!!!` (`self.DeadPlayerPawn`)
    (:`Is NOT Valid`
      (bind _class (`|LoadAssetClass` (`self.DeadPlayerPawnClass`))
        (:`Completed`
          (bind _aspawn (castclass `Pawn` _class))
          (bind _returnvalue (`|SpawnActorFromClass` _aspawn (`self.GetTransform`) "AlwaysSpawn" "MultiplyWithRoot" (`self.GetController`) null))
          (set `self.DeadPlayerPawn` _returnvalue)
          (`self.PossessDeadPlayerPawn`))))
    (:`IsValid`
      (`self.PossessDeadPlayerPawn`))))

(event `ReachedJumpApex`
  ;[1 1 1] Jump Apex/Landed/Launched
  (set `CharacterMovementComponent.bNotifyApex` false (`self.CharacterMovement`))
  (if (not (`self.bLaunched`))
    (if (> (`self.ApexHoverTime`) 0.0)
      (set `CharacterMovementComponent.GravityScale` (`self.HoverGravityScale`) (`self.CharacterMovement`))
      (bind _returnvalue (`KismetSystemLibrary.K2_SetTimerDelegate` (delegate `StartDrop`) (`self.ApexHoverTime`)))
      (set `self.ApexHoverTimer` _returnvalue))
    (else
      (`self.StartDrop`))))

(event `self.K2_OnBecomeViewTarget`
  (params (PC :type "PlayerController Object Reference"))
  ;[1 1 1] OnBecomeViewTarget
  (`PlayerController.SetViewTargetWithBlend` PC (`self.GetPlatformerCameraActor`) 0.0 "VTBlend_Linear" 0.0 false))

(event `StartDrop`
  ;[1 1 1] Jump Apex/Landed/Launched
  (set `CharacterMovementComponent.GravityScale` (`self.DropGravityScale`) (`self.CharacterMovement`)))

(event `self.HealthComponent.OnRevived`
  (params (Caller :type "/Game/EpicTemplates/TemplateAgnostic/Blueprints/Components/BP_HealthComponent Object Reference") (ReviveSource :type "Actor Object Reference"))
  ;[1 1 1] Health Component
  (`self.K2_SetActorLocation` (`self.K2_GetActorLocation` ReviveSource) false true)
  (`SceneComponent.SetVisibility` (`self.Mesh`) true true)
  (`PrimitiveComponent.SetCollisionEnabled` (`self.CapsuleComponent`) "QueryAndPhysics")
  (set `CharacterMovementComponent.GravityScale` (`self.RegularGravityScale`) (`self.CharacterMovement`))
  (`Controller.Possess` (`self.CurrentPlayerCont`) self)
  (`self.EnableInput` (`self.CurrentPlayerCont`))
  (`ActorComponent.SetActive` (`self.CharacterMovement`) true true))

(event `PossessDeadPlayerPawn`
  ;[1 1 1] Health Component
  (message `/Game/EpicTemplates/PlatformerTemplate/Blueprints/Interfaces/BPI_RevivalSource.AddActorToRevive` (`self.DeadPlayerPawn`) self)
  (`Controller.Possess` (`self.CurrentPlayerCont`) (`self.DeadPlayerPawn`))
  (`PlayerController.SetViewTargetWithBlend` (`self.CurrentPlayerCont`) (`self.GetPlatformerCameraActor`) 0.0 "VTBlend_Linear" 0.0 false))

(event `self.OnLanded`
  (params (Hit :type "HitResult Structure (by ref)"))
  ;[1 1 1] Jump Apex/Landed/Launched
  (`self.HandleLanded` Hit))

(event `self.OnLaunched`
  (params (LaunchVelocity :type "Vector Structure") (bXYOverride :type Boolean) (bZOverride :type Boolean))
  ;[1 1 1] Jump Apex/Landed/Launched
  (set `CharacterMovementComponent.GravityScale` (`self.RegularGravityScale`) (`self.CharacterMovement`))
  (set `self.bLaunched` true)
  (set `CharacterMovementComponent.bNotifyApex` true (`self.CharacterMovement`))
  (`self.StopJumping`))

(event `self.CapsuleComponent.OnComponentHit`
  (params (HitComponent :type "PrimitiveComponent Object Reference") (OtherActor :type "Actor Object Reference") (OtherComp :type "PrimitiveComponent Object Reference") (NormalImpulse :type "Vector Structure") (Hit :type "HitResult Structure (by ref)"))
  ;[1 1 1] CapsuleHit
  (if (< (.z (`.Normal` (`GameplayStatics.BreakHitResult` Hit))) -0.707)
    (`self.HandleHitHead`)))

(event `self.K2_OnMovementModeChanged`
  (params (PrevMovementMode :type "EMovementMode Enum" :default "MOVE_None") (NewMovementMode :type "EMovementMode Enum" :default "MOVE_None") (PrevCustomMode :type Byte) (NewCustomMode :type Byte))
  ;[1 1 1] Jump Apex/Landed/Launched
  (if (and (`|EnumEquality` PrevMovementMode "MOVE_Walking") (`|EnumEquality` NewMovementMode "MOVE_Falling"))
    (`KismetSystemLibrary.K2_ClearAndInvalidateTimerHandle` (`self.CheckRespawnFloorTimer`))
    (elif (`|EnumEquality` NewMovementMode "MOVE_Walking")
      (`self.CheckForRespawnableFloor`)
      (bind _returnvalue (`KismetSystemLibrary.K2_SetTimerDelegate` (`|CreateDelegate` :!event `CheckForRespawnableFloor`) 0.5 true))
      (set `self.CheckRespawnFloorTimer` _returnvalue))))

(fn `Check For Input Duration Lock`
  (returns (bLockedForTime :type Boolean))
  (if (> (`self.DamageInputLockoutTime`) 0.0)
    (bind _returnvalue (`KismetSystemLibrary.K2_SetTimerDelegate` (`|CreateDelegate` :!event `UnlockInput`) (`self.DamageInputLockoutTime`)))
    (set `self.DamageInputLockoutTimer` _returnvalue)
    (return true)
    (else
      (return false))))

(fn `CheckForLockOnLand`
  (returns (LockingOnLand :type Boolean))
  (if (`NavMovementComponent.IsFalling` (`self.CharacterMovement`))
    (set `self.bUnlockInputOnLand` true)
    (return true)
    (else
      (return false))))

(fn `CheckForScreenEdgeInputBlock`
  (params (LRInputDir :type "Float (double-precision)"))
  (returns (CanInput :type Boolean))
  (locals (ScreenEdges :type "/Game/EpicTemplates/PlatformerTemplate/Blueprints/Structs/CameraScreenEdgeStruct Structure"))
  (if (`self.bBlockInputPastScreenEdge`)
    (bind _worldscreenedges (`/Game/EpicTemplates/PlatformerTemplate/Blueprints/Interfaces/BPI_Camera2D.GetWorldScreenEdges` (`self.GetPlatformerCameraInterface`)))
    (set `local.ScreenEdges` _worldscreenedges)
    (if (> (`local.LRInputDir`) 0.0)
      (return (< (.y (`self.K2_GetActorLocation`)) (- (`.Right_13_7EFAB1634420AE59C0AFED9C59F15558` (break `/Game/EpicTemplates/PlatformerTemplate/Blueprints/Structs/CameraScreenEdgeStruct` (`local.ScreenEdges`))) (`CapsuleComponent.GetScaledCapsuleRadius` (`self.CapsuleComponent`)))))
      (else
        (return (> (.y (`self.K2_GetActorLocation`)) (- (`.Left_12_CC421F0C4A6E7D92A89ED7AB4A00F83F` (break `/Game/EpicTemplates/PlatformerTemplate/Blueprints/Structs/CameraScreenEdgeStruct` (`local.ScreenEdges`))) (`CapsuleComponent.GetScaledCapsuleRadius` (`self.CapsuleComponent`)))))))
    (else
      (return true))))

(fn `ClearAllTimers`
  (`KismetSystemLibrary.K2_ClearAndInvalidateTimerHandle` (`self.DamageReactFlickerTimer`))
  (`KismetSystemLibrary.K2_ClearAndInvalidateTimerHandle` (`self.CheckRespawnFloorTimer`))
  (`KismetSystemLibrary.K2_ClearAndInvalidateTimerHandle` (`self.DamageInputLockoutTimer`))
  (`KismetSystemLibrary.K2_ClearAndInvalidateTimerHandle` (`self.CheckForKillZTimer`))
  (`KismetSystemLibrary.K2_ClearAndInvalidateTimerHandle` (`self.DamageReactTimer`))
  (`KismetSystemLibrary.K2_ClearAndInvalidateTimerHandle` (`self.ApexHoverTimer`)))

(fn `GetIsInDebug`
  (returns (bIsInDebug :type Boolean))
  (return (`self.In Is Debug`)))

(fn `GetPlatformerCameraActor`
  (returns (CameraActor :type "Actor Object Reference"))
  (`/Engine/EditorBlueprintResources/StandardMacros.IsValid` (`self.CachedPlatformerCamera`)
    (:`Is Valid`
      (return (`self.CachedPlatformerCamera`)))
    (:`Is Not Valid`
      (bind (_cameraactor _camerainterface) (`/Game/EpicTemplates/PlatformerTemplate/Blueprints/PlatformerFunctionLibrary.GetPlatformerCamera`))
      (bind _output_get (set `self.CachedPlatformerCamera` _cameraactor))
      (set `self.CachedPlatformerCameraInterface` _camerainterface)
      (return _output_get))))

(fn `GetPlatformerCameraInterface`
  (returns (CachedPlatformerCameraInterface :type "/Game/EpicTemplates/PlatformerTemplate/Blueprints/Interfaces/BPI_Camera2D Interface"))
  (if (`KismetSystemLibrary.IsValidInterface` (`self.CachedPlatformerCameraInterface`))
    (return (`self.CachedPlatformerCameraInterface`))
    (else
      (bind (_cameraactor _camerainterface) (`/Game/EpicTemplates/PlatformerTemplate/Blueprints/PlatformerFunctionLibrary.GetPlatformerCamera`))
      (set `self.CachedPlatformerCamera` _cameraactor)
      (bind _output_get (set `self.CachedPlatformerCameraInterface` _camerainterface))
      (return _output_get))))

(fn `HandleHitHead`
  (if (`NavMovementComponent.IsFalling` (`self.CharacterMovement`))
    (if (> (.z (`CharacterMovementComponent.GetLastUpdateVelocity` (`self.CharacterMovement`))) 0.0)
      (`KismetSystemLibrary.K2_ClearAndInvalidateTimerHandle` (`self.ApexHoverTimer`))
      (set `CharacterMovementComponent.bNotifyApex` false (`self.CharacterMovement`))
      (`self.StartDrop`)
      (set `MovementComponent.Velocity` (`KismetMathLibrary.MakeVector` 0.0 (.y (`MovementComponent.Velocity` (`self.CharacterMovement`)))) (`self.CharacterMovement`)))))

(fn `HandleLanded`
  (params (LandedHit :type "HitResult Structure (by ref)"))
  (bind (_bblockinghit _binitialoverlap _time _distance _location _impactpoint _normal _impactnormal _physmat _hitactor _hitcomponent _hitbonename) (`GameplayStatics.BreakHitResult` (`local.LandedHit`)))
  (`KismetSystemLibrary.K2_ClearAndInvalidateTimerHandle` (`self.ApexHoverTimer`))
  (set `CharacterMovementComponent.GravityScale` (`self.RegularGravityScale`) (`self.CharacterMovement`))
  (set `self.bLaunched` false)
  (`|ExecutionSequence`
    (:`then_0`
      (`KismetSystemLibrary.K2_ClearAndInvalidateTimerHandle` (`self.DamageInputLockoutTimer`))
      (if (`self.bUnlockInputOnLand`)
        (`self.UnlockInput`)
        (set `self.bUnlockInputOnLand` false)))
    (:`then_1`
      (if (> (.z (`.Normal` (`GameplayStatics.BreakHitResult` (`local.LandedHit`)))) 0.707)
        (bind _interfaceimplementingobject (`/Game/EpicTemplates/TemplateAgnostic/Blueprints/EpicTemplatesFunctionLibrary.SearchActorForInterface` (`.HitActor` (`GameplayStatics.BreakHitResult` (`local.LandedHit`))) "/Game/EpicTemplates/TemplateAgnostic/Blueprints/Interfaces/BPI_Damageable.BPI_Damageable_C"))
        (`/Engine/EditorBlueprintResources/StandardMacros.IsValid` _interfaceimplementingobject
          (:`Is Valid`
            (message `/Game/EpicTemplates/TemplateAgnostic/Blueprints/Interfaces/BPI_Damageable.ApplyDamage` _interfaceimplementingobject (make `/Game/EpicTemplates/TemplateAgnostic/Blueprints/Structs/DamageStruct` (`self.JumpDamage`) self (`self.GetController`) _impactpoint (0.0 0.0 -1.0) _hitbonename))
            (`self.LaunchCharacter` (`KismetMathLibrary.MakeVector` 0.0 0.0 (select `bool` (`self.JumpHeld`) :`false` (`self.HitEnemyLaunchVelocity`) :`true` (`self.HitEnemyLaunchVelocityJumpHeld`))) false true)))))))

(fn `HandleTookDamage`
  (params (DamageStruct :type "/Game/EpicTemplates/TemplateAgnostic/Blueprints/Structs/DamageStruct Structure (by ref)") (NewHealth :type "Float (double-precision)"))
  (bind (_x _y) (`KismetMathLibrary.BreakVector2D` (`KismetMathLibrary.Normal2D` (`KismetMathLibrary.MakeVector2D` (.y (`.DamageDirection_20_DE80E36A475894D4B74BC0909E89EF39` (break `/Game/EpicTemplates/TemplateAgnostic/Blueprints/Structs/DamageStruct` (`local.DamageStruct`)))) (+ (.z (`.DamageDirection_20_DE80E36A475894D4B74BC0909E89EF39` (break `/Game/EpicTemplates/TemplateAgnostic/Blueprints/Structs/DamageStruct` (`local.DamageStruct`)))) 1.0)))))
  (if (> (`.Damage_11_4BDBE22E4671030D7F6B5BBB0A6FB960` (break `/Game/EpicTemplates/TemplateAgnostic/Blueprints/Structs/DamageStruct` DamageStruct)) 0.0)
    (`/Game/EpicTemplates/TemplateAgnostic/Blueprints/Components/BP_HealthComponent.EnableInvincibility` (`self.HealthComponent`))
    (`|ExecutionSequence`
      (:`then_0`
        (bind _returnvalue (`KismetSystemLibrary.K2_SetTimerDelegate` (`|CreateDelegate` :!event `HitReactFlicker`) 0.05 true true))
        (set `self.DamageReactFlickerTimer` _returnvalue))
      (:`then_1`
        (bind _returnvalue_2 (`KismetSystemLibrary.K2_SetTimerDelegate` (`|CreateDelegate` :!event `EndDamageReact`) (`self.DamageInvincibilityTime`)))
        (set `self.DamageReactTimer` _returnvalue_2)
        (`self.LaunchCharacter` (* (`KismetMathLibrary.MakeVector` 0.0 _x _y) (`self.TakeDamageLaunchVelocity`)))
        (`/Engine/EditorBlueprintResources/StandardMacros.IsValid` (`self.CurrentPlayerCont`)
          (:`Is Valid`
            (`|ExecutionSequence`
              (:`then_0`
                (if (`|EnumInequality` (`self.DamageReactInputLogic`) "NewEnumerator0")
                  (`self.DisableInput` (`self.CurrentPlayerCont`))))
              (:`then_1`
                (switch `/Game/EpicTemplates/PlatformerTemplate/Blueprints/Enums/ETakeDamageInputLogic` (`self.DamageReactInputLogic`)
                  (:`NewEnumerator1`
                    (bind _blockedfortime (`self.Check For Input Duration Lock`))
                    (if (not _blockedfortime)
                      (`self.UnlockInput`)))
                  (:`NewEnumerator2`
                    (bind _lockingonland (`self.CheckForLockOnLand`))
                    (if (not _lockingonland)
                      (`self.UnlockInput`)))
                  (:`NewEnumerator3`
                    (bind _blockedfortime_2 (`self.Check For Input Duration Lock`))
                    (bind _lockingonland_2 (`self.CheckForLockOnLand`))
                    (if (and (not _blockedfortime_2) (not _lockingonland_2))
                      (`self.UnlockInput`))))))))))))

(fn `IsHitSafeForRespawnableFloor`
  (params (Hit :type "HitResult Structure (by ref)"))
  (returns (bValidForRespawn :type Boolean))
  (bind (_bblockinghit _binitialoverlap _time _distance _location _impactpoint _normal _impactnormal _physmat _hitactor _hitcomponent) (`GameplayStatics.BreakHitResult` Hit))
  (if (`CharacterMovementComponent.IsWalkable` (`self.CharacterMovement`) Hit)
    (if (> (.z _normal) 0.707)
      (if (`|EnumEquality` (`PrimitiveComponent.GetCollisionObjectType` _hitcomponent) "ECC_WorldStatic")
        (return true))
      (else
        (return false)))
    (else
      (return false))))

(fn `UpdateCurrentDepth`
  (params (NewDepth :type "Float (double-precision)"))
  (bind _output_get (set `self.CurrentDepth` NewDepth))
  (`MovementComponent.SetPlaneConstraintOrigin` (`self.CharacterMovement`) (`KismetMathLibrary.MakeVector` _output_get)))

(fn `UserConstructionScript`
  (`/Game/EpicTemplates/TemplateAgnostic/Blueprints/Components/BP_ThirdPersonInteractComponent.RegisterInteractOverlapComponent` (`self.ThirdPersonInteractComponent`) (`self.InteractSphere`)))