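; BP_Creature is a creature actor in the Walking Sim template, built from segmented head, body and tail parts with a Niagara-style trail effect.
; Events activate or deactivate the NSCreatureTrail effect on demand.
; A CreatureColour value selects a blue or grey material instance for every segment, applied in the construction script and updatable at runtime through UpdateCreatureColour.
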(event `Activate Creature Trail FX`
  (`ActorComponent.Activate` (`self.NS_CreatureTrail`) false))

(event `DeActivate Creature Trail FX`
  (`ActorComponent.Deactivate` (`self.NS_CreatureTrail`)))

(event `UpdateCreatureColour`
  (params (CreatureColour :type "/Game/EpicTemplates/WalkingSimTemplate/Gameplay/E_CreatureColour Enum" :default "NewEnumerator0"))
  (set `self.CreatureColour` CreatureColour)
  (`PrimitiveComponent.SetMaterial` (`self.Head_01`) 0 (select `/Game/EpicTemplates/WalkingSimTemplate/Gameplay/E_CreatureColour` (`self.CreatureColour`) :`NewEnumerator0` "/Game/EpicTemplates/WalkingSimTemplate/Materials/M_Creature_BlueInst.M_Creature_BlueInst" :`NewEnumerator1` "/Game/EpicTemplates/RailShooterTemplate/Materials/M_DefaultGeo_Inst01.M_DefaultGeo_Inst01" :!type "MaterialInterface Object Reference") :!label _label)
  (`PrimitiveComponent.SetMaterial` (`self.Head_02`) 0 (select `/Game/EpicTemplates/WalkingSimTemplate/Gameplay/E_CreatureColour` (`self.CreatureColour`) :`NewEnumerator0` "/Game/EpicTemplates/WalkingSimTemplate/Materials/M_Creature_BlueInst.M_Creature_BlueInst" :`NewEnumerator1` "/Game/EpicTemplates/RailShooterTemplate/Materials/M_DefaultGeo_Inst01.M_DefaultGeo_Inst01" :!type "MaterialInterface Object Reference"))
  (`PrimitiveComponent.SetMaterial` (`self.Head_03`) 0 (select `/Game/EpicTemplates/WalkingSimTemplate/Gameplay/E_CreatureColour` (`self.CreatureColour`) :`NewEnumerator0` "/Game/EpicTemplates/WalkingSimTemplate/Materials/M_Creature_BlueInst.M_Creature_BlueInst" :`NewEnumerator1` "/Game/EpicTemplates/RailShooterTemplate/Materials/M_DefaultGeo_Inst01.M_DefaultGeo_Inst01" :!type "MaterialInterface Object Reference"))
  (`PrimitiveComponent.SetMaterial` (`self.Head_04`) 0 (select `/Game/EpicTemplates/WalkingSimTemplate/Gameplay/E_CreatureColour` (`self.CreatureColour`) :`NewEnumerator0` "/Game/EpicTemplates/WalkingSimTemplate/Materials/M_Creature_BlueInst.M_Creature_BlueInst" :`NewEnumerator1` "/Game/EpicTemplates/RailShooterTemplate/Materials/M_DefaultGeo_Inst01.M_DefaultGeo_Inst01" :!type "MaterialInterface Object Reference"))
  (`PrimitiveComponent.SetMaterial` (`self.Body_01`) 0 (select `/Game/EpicTemplates/WalkingSimTemplate/Gameplay/E_CreatureColour` (`self.CreatureColour`) :`NewEnumerator0` "/Game/EpicTemplates/WalkingSimTemplate/Materials/M_Creature_BlueInst.M_Creature_BlueInst" :`NewEnumerator1` "/Game/EpicTemplates/RailShooterTemplate/Materials/M_DefaultGeo_Inst01.M_DefaultGeo_Inst01" :!type "MaterialInterface Object Reference"))
  (`PrimitiveComponent.SetMaterial` (`self.Body_02`) 0 (select `/Game/EpicTemplates/WalkingSimTemplate/Gameplay/E_CreatureColour` (`self.CreatureColour`) :`NewEnumerator0` "/Game/EpicTemplates/WalkingSimTemplate/Materials/M_Creature_BlueInst.M_Creature_BlueInst" :`NewEnumerator1` "/Game/EpicTemplates/RailShooterTemplate/Materials/M_DefaultGeo_Inst01.M_DefaultGeo_Inst01" :!type "MaterialInterface Object Reference"))
  (`PrimitiveComponent.SetMaterial` (`self.Body_03`) 0 (select `/Game/EpicTemplates/WalkingSimTemplate/Gameplay/E_CreatureColour` (`self.CreatureColour`) :`NewEnumerator0` "/Game/EpicTemplates/WalkingSimTemplate/Materials/M_Creature_BlueInst.M_Creature_BlueInst" :`NewEnumerator1` "/Game/EpicTemplates/RailShooterTemplate/Materials/M_DefaultGeo_Inst01.M_DefaultGeo_Inst01" :!type "MaterialInterface Object Reference"))
  (`PrimitiveComponent.SetMaterial` (`self.Body_04`) 0 (select `/Game/EpicTemplates/WalkingSimTemplate/Gameplay/E_CreatureColour` (`self.CreatureColour`) :`NewEnumerator0` "/Game/EpicTemplates/WalkingSimTemplate/Materials/M_Creature_BlueInst.M_Creature_BlueInst" :`NewEnumerator1` "/Game/EpicTemplates/RailShooterTemplate/Materials/M_DefaultGeo_Inst01.M_DefaultGeo_Inst01" :!type "MaterialInterface Object Reference"))
  (`PrimitiveComponent.SetMaterial` (`self.Tail_01`) 0 (select `/Game/EpicTemplates/WalkingSimTemplate/Gameplay/E_CreatureColour` (`self.CreatureColour`) :`NewEnumerator0` "/Game/EpicTemplates/WalkingSimTemplate/Materials/M_Creature_BlueInst.M_Creature_BlueInst" :`NewEnumerator1` "/Game/EpicTemplates/RailShooterTemplate/Materials/M_DefaultGeo_Inst01.M_DefaultGeo_Inst01" :!type "MaterialInterface Object Reference"))
  (`PrimitiveComponent.SetMaterial` (`self.Tail_02`) 0 (select `/Game/EpicTemplates/WalkingSimTemplate/Gameplay/E_CreatureColour` (`self.CreatureColour`) :`NewEnumerator0` "/Game/EpicTemplates/WalkingSimTemplate/Materials/M_Creature_BlueInst.M_Creature_BlueInst" :`NewEnumerator1` "/Game/EpicTemplates/RailShooterTemplate/Materials/M_DefaultGeo_Inst01.M_DefaultGeo_Inst01" :!type "MaterialInterface Object Reference"))
  (`PrimitiveComponent.SetMaterial` (`self.Tail_03`) 0 (select `/Game/EpicTemplates/WalkingSimTemplate/Gameplay/E_CreatureColour` (`self.CreatureColour`) :`NewEnumerator0` "/Game/EpicTemplates/WalkingSimTemplate/Materials/M_Creature_BlueInst.M_Creature_BlueInst" :`NewEnumerator1` "/Game/EpicTemplates/RailShooterTemplate/Materials/M_DefaultGeo_Inst01.M_DefaultGeo_Inst01" :!type "MaterialInterface Object Reference")))

(event `SetCreatureColour`
  (goto _label))

(fn `UserConstructionScript`
  (`self.SetCreatureColour`))