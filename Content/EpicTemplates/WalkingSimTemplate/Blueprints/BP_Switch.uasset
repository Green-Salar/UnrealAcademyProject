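; BP_Switch is an interactable toggle switch for the walking sim template that flips its state on interact and notifies other actors.
; Interaction comes through BP_SimpleInteractComponent, which receives its prompt text and locking level tag from the switch at construction.
; A state change recolors the light pad's dynamic material, messages soft-referenced listeners via BPI_SwitchListener and fires OnSwitchChanged.
; The construction script nullifies listener entries lacking that interface, printing a warning.
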(event `self.BP_SimpleInteractComponent.OnInteractStart`
  (params (InteractingController :type "Controller Object Reference"))
  (`self.UpdateIsOn` (not (`self.bSwitchOn`))))

(event `UpdateIsOn`
  (params (bSwitchOn :type Boolean))
  (if (!= bSwitchOn (`self.bSwitchOn`))
    (set `self.bSwitchOn` bSwitchOn)
    (`MaterialInstanceDynamic.SetVectorParameterValue` (`self.SwitchLightPadDynaMat`) (`self.ColorParameterName`) (select `bool` (`self.bSwitchOn`) :`false` (`self.LightPadColorOff`) :`true` (`self.LightPadColorOn`)))
    (`|ExecutionSequence`
      (:`then_0`
        (for _array_element (`self.SwitchListeners`)
          (if (`KismetSystemLibrary.IsValidSoftObjectReference` _array_element)
            (message `/Game/EpicTemplates/TemplateAgnostic/Blueprints/Interfaces/BPI_SwitchListener.SwitchToggled` (`|ConvertAsset` _array_element) self (`self.bSwitchOn`)))))
      (:`then_1`
        (`self.OnSwitchChanged` self (`self.bSwitchOn`))))))

(fn `UserConstructionScript`
  (bind _returnvalue (`PrimitiveComponent.CreateDynamicMaterialInstance` (`self.SwitchLightPad`) 0 "/Game/EpicTemplates/WalkingSimTemplate/Materials/M_FlatColor_Unlit.M_FlatColor_Unlit" "None"))
  (bind _output_get (set `self.SwitchLightPadDynaMat` _returnvalue))
  (`MaterialInstanceDynamic.SetVectorParameterValue` _output_get (`self.ColorParameterName`) (`self.LightPadColorOff`))
  (set `/Game/EpicTemplates/WalkingSimTemplate/Blueprints/Components/BP_SimpleInteractComponent.LockingLevelBoolTag` (`self.LockingLevelBoolTag`) (`self.BP_SimpleInteractComponent`))
  (set `/Game/EpicTemplates/WalkingSimTemplate/Blueprints/Components/BP_SimpleInteractComponent.InteractText` (`self.Interact Text`) (`self.BP_SimpleInteractComponent`))
  (for (_array_element _array_index) (`self.SwitchListeners`)
    (if (`KismetSystemLibrary.IsValidSoftObjectReference` _array_element)
      (if (not (`KismetSystemLibrary.DoesImplementInterface` (`|ConvertAsset` _array_element) "/Game/EpicTemplates/TemplateAgnostic/Blueprints/Interfaces/BPI_SwitchListener.BPI_SwitchListener_C"))
        (`KismetSystemLibrary.PrintString` (`KismetStringLibrary.Concat_StrStr` "Switch listener '" (`KismetSystemLibrary.Conv_SoftObjectReferenceToString` _array_element) "' doesn't implement the switch listener interface, nullifying entry"))
        (`KismetArrayLibrary.Array_Set` (`self.SwitchListeners`) _array_index)))))