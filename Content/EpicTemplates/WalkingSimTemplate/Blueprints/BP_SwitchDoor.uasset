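; BP_SwitchDoor is a walking-sim template door that slides between closed and open positions, toggled through SwitchToggled.
; UpdateDoorOpen acts on state changes, either snapping or playing/reversing TL_OpenDoor, whose alpha lerps DoorMesh's relative location along the DoorMovement offset.
; The construction script caches the start location and, like BeginPlay, snaps to StartOpen.
; OpenDoor passes false just like CloseDoor, so it closes the door as written.
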(event `self.ReceiveBeginPlay`
  (`self.UpdateDoorOpen` (`self.bStartOpen`) true))

(event `UpdateDoorOpen`
  (params (bDoorOpen :type Boolean) (bSnap :type Boolean))
  (if (!= bDoorOpen (`self.bDoorOpen`))
    (set `self.bDoorOpen` bDoorOpen)
    (if bSnap
      (bind (_direction _dooropenalpha) (`Timeline|TL_OpenDoor` :`NewTime` (select `bool` (`self.bDoorOpen`) :`true` 1.0 :!type "Float (single-precision)") :!via `SetNewTime` :!label _label)
        (:`Update`
          (`self.UpdateDoorOpenAlpha` _dooropenalpha)))
      (elif (`self.bDoorOpen`)
        (goto _label)
        (else
          (goto _label :!via `Reverse`))))))

(event `CloseDoor`
  (`self.UpdateDoorOpen` false))

(event `UpdateDoorOpenAlpha`
  (params (OpenAlpha :type "Float (double-precision)"))
  (`SceneComponent.K2_SetRelativeLocation` (`self.DoorMesh`) (`KismetMathLibrary.VLerp` (`self.DoorStartLoc`) (+ (`self.DoorStartLoc`) (`self.DoorMovement`)) OpenAlpha) false false))

(event `OpenDoor`
  (`self.UpdateDoorOpen` false))

(event `/Game/EpicTemplates/TemplateAgnostic/Blueprints/Interfaces/BPI_SwitchListener.SwitchToggled`
  (params (SwitchActor :type "Actor Object Reference") (bSwitchIsOn :type Boolean))
  (`self.UpdateDoorOpen` (not (`self.bDoorOpen`))))

(fn `UserConstructionScript`
  (set `self.DoorStartLoc` (`SceneComponent.RelativeLocation` (`self.DoorMesh`)))
  (`self.UpdateDoorOpen` (`self.bStartOpen`) true))