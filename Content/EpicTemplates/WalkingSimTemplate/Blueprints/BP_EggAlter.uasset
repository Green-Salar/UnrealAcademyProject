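; Egg altar for the walking sim template that takes an egg from the player and destroys it at the push of a switch.
; Interacting removes a BP_SmallCubePickup through the player's BPI_SimpleInventory and places it at the egg root.
; With an egg placed and a valid creature reference, the switch animates, fires OnSwitchPushed and shows forcefield meshes.
; A timeline lerps the egg to an end transform, then hides the forcefields and re-arms the switch.
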(event `self.EggInteract.OnInteractStart`
  (params (InteractingController :type "Controller Object Reference"))
  (bind (_returnvalue_location _returnvalue_rotation) (`KismetMathLibrary.BreakTransform` (`SceneComponent.K2_GetComponentToWorld` (`self.EggRoot`))))
  ;[0.8122 1 0.9392 0.3 30] Place Egg in Alter
  (bind _interfaceimplementingobject (`/Game/EpicTemplates/TemplateAgnostic/Blueprints/EpicTemplatesFunctionLibrary.SearchActorForInterface` (`GameplayStatics.GetPlayerPawn` 0) "/Game/EpicTemplates/WalkingSimTemplate/Blueprints/Interfaces/BPI_SimpleInventory.BPI_SimpleInventory_C"))
  (bind _asbpi_simple_inventory (cast `/Game/EpicTemplates/WalkingSimTemplate/Blueprints/Interfaces/BPI_SimpleInventory` _interfaceimplementingobject))
  (bind _iteminstance (`/Game/EpicTemplates/WalkingSimTemplate/Blueprints/Interfaces/BPI_SimpleInventory.RemoveAndPlaceItemByClass` _asbpi_simple_inventory "/Game/EpicTemplates/WalkingSimTemplate/Blueprints/Pickups/BP_SmallCubePickup.BP_SmallCubePickup_C" _returnvalue_location _returnvalue_rotation true true))
  (set `self.bEggPlaced` true)
  (bind _output_get (set `self.CurrentEggRef` _iteminstance))
  (`/Engine/EditorBlueprintResources/StandardMacros.IsValid` _output_get
    (:`Is Valid`
      (`self.K2_DetachFromActor` _output_get "KeepWorld" "KeepWorld" "KeepWorld"))))

(event `self.SwitchInteract.OnInteractStart`
  (params (InteractingController :type "Controller Object Reference"))
  ;[0.8122 1 0.9392 0.3 30] Destory Egg Switch
  (if (and (`self.bEggPlaced`) (`KismetSystemLibrary.IsValid` (`self.CurrentCreatureRef`)))
    (`/Engine/EditorBlueprintResources/StandardMacros.DoOnce` false :!label _label
      (:`Completed`
        (`|ExecutionSequence`
          (:`then_0`
            (bind (_direction _newtrack_0) (`Timeline|TL_SwitchPush` :!via `PlayFromStart`)
              (:`Update`
                (`SceneComponent.K2_SetRelativeLocation` (`self.SM_EggAltar_Button`) (`KismetMathLibrary.VLerp` (-21.870246 0.0 38.086207) (-21.070825 0.0 36.371843) _newtrack_0) false false))))
          (:`then_1`
            (`self.OnSwitchPushed`)
            (`self.SetActorHiddenInGame` (`self.ForcefieldMesh04`) false)
            (`self.SetActorHiddenInGame` (`self.ForcefieldMesh01`) false)
            (`self.SetActorHiddenInGame` (`self.ForcefieldMesh02`) false)
            (`self.SetActorHiddenInGame` (`self.ForcefieldMesh03`) false)
            (bind (_direction_2 _destroyegg) (`Timeline|TL_DissolveEgg` :!via `PlayFromStart`)
              (:`Update`
                (bind _currenteggref (`self.CurrentEggRef`)
                  (:`then`
                    (`self.K2_SetActorTransform` _currenteggref (`KismetMathLibrary.TLerp` (`SceneComponent.K2_GetComponentToWorld` (`self.EggRoot`)) (`SceneComponent.K2_GetComponentToWorld` (`self.EggEndTransform`)) _destroyegg) false false))
                  (:`else`)))
              (:`Finished`
                (`self.SetActorHiddenInGame` (`self.ForcefieldMesh01`) true)
                (`self.SetActorHiddenInGame` (`self.ForcefieldMesh02`) true)
                (`self.SetActorHiddenInGame` (`self.ForcefieldMesh03`) true)
                (`self.SetActorHiddenInGame` (`self.ForcefieldMesh04`) true)
                (set `self.bEggPlaced` false)
                (set `self.CurrentEggRef` null)
                (`self.ResetSwitch`)))))))))

(event `ResetSwitch`
  ;[0.8122 1 0.9392 0.3 30] Destory Egg Switch
  (goto _label :!via `Reset`))

(fn `UserConstructionScript`)