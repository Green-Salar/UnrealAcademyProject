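; Base static pickup for the walking sim template that the player can pick up, examine, rotate, put down or take.
; Interacting asks the BPI_PickupManipulator implementer on the player's pawn to examine it.
; Pickup interface events then advance its state, store the put-down transform, call notifications and disable mesh collision during transitions.
; While examined, horizontal and vertical input rotate it relative to the player's view.
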(event `/Game/EpicTemplates/WalkingSimTemplate/Blueprints/Interfaces/BPI_FirstPersonInteractable.InteractStart`
  (params (InteractingController :type "Controller Object Reference"))
  ;[1 1 1] Interact Interface
  (if (and (`|EnumEquality` (`self.CurrentPickupState`) "NewEnumerator0") (`self.bCanBePickedUp`))
    (bind _interfaceimplementingobject (`/Game/EpicTemplates/TemplateAgnostic/Blueprints/EpicTemplatesFunctionLibrary.SearchActorForInterface` (`Controller.K2_GetPawn` InteractingController) "/Game/EpicTemplates/WalkingSimTemplate/Blueprints/Interfaces/BPI_PickupManipulator.BPI_PickupManipulator_C"))
    (`/Engine/EditorBlueprintResources/StandardMacros.IsValid` _interfaceimplementingobject
      (:`Is Valid`
        (message `/Game/EpicTemplates/WalkingSimTemplate/Blueprints/Interfaces/BPI_PickupManipulator.ExamineNewPickup` _interfaceimplementingobject self)))))

(event `/Game/EpicTemplates/WalkingSimTemplate/Blueprints/Interfaces/BPI_FirstPersonInteractable.HorizontalInput`
  (params (InteractingController :type "Controller Object Reference") (Input :type "Float (double-precision)"))
  ;[1 1 1] Interact Interface
  (if (`|EnumEquality` (`self.CurrentPickupState`) "NewEnumerator2")
    (`self.Handle Rotate Pickup` InteractingController (* Input (`self.YawRate`) -1.0))))

(event `/Game/EpicTemplates/WalkingSimTemplate/Blueprints/Interfaces/BPI_FirstPersonInteractable.VerticalInput`
  (params (InteractingController :type "Controller Object Reference") (Input :type "Float (double-precision)"))
  ;[1 1 1] Interact Interface
  (if (`|EnumEquality` (`self.CurrentPickupState`) "NewEnumerator2")
    (`self.Handle Rotate Pickup` InteractingController 0.0 (* Input (`self.PitchRate`) -1.0))))

(event `/Game/EpicTemplates/WalkingSimTemplate/Blueprints/Interfaces/BPI_Pickup.UpdateCanBePickedUp`
  (params (InCanBePickedUp :type Boolean))
  ;[1 1 1] Pickup Interface
  (set `self.bCanBePickedUp` InCanBePickedUp))

(event `/Game/EpicTemplates/WalkingSimTemplate/Blueprints/Interfaces/BPI_Pickup.StartedPickUp`
  (params (Interactor :type "/Game/EpicTemplates/WalkingSimTemplate/Blueprints/Interfaces/BPI_PickupManipulator Interface"))
  ;[1 1 1] Pickup Interface
  (`PrimitiveComponent.SetCollisionEnabled` (`self.Mesh`) "NoCollision")
  (`|ExecutionSequence`
    (:`then_0`
      (if (`|EnumEquality` (`self.CurrentPickupState`) "NewEnumerator0")
        (set `self.PutDownTransform` (`self.GetTransform`))))
    (:`then_1`
      (set `self.CurrentPickupState` "NewEnumerator1")
      (`self.OnPickedUp` self))))

(event `/Game/EpicTemplates/WalkingSimTemplate/Blueprints/Interfaces/BPI_Pickup.ReachedPickupExaminePoint`
  (params (Interactor :type "/Game/EpicTemplates/WalkingSimTemplate/Blueprints/Interfaces/BPI_PickupManipulator Interface"))
  ;[1 1 1] Pickup Interface
  (`PrimitiveComponent.SetCollisionEnabled` (`self.Mesh`) "QueryOnly")
  (set `self.CurrentPickupState` "NewEnumerator2"))

(event `/Game/EpicTemplates/WalkingSimTemplate/Blueprints/Interfaces/BPI_Pickup.ReachedPutDownPoint`
  (params (Interactor :type "/Game/EpicTemplates/WalkingSimTemplate/Blueprints/Interfaces/BPI_PickupManipulator Interface"))
  ;[1 1 1] Pickup Interface
  (`PrimitiveComponent.SetCollisionEnabled` (`self.Mesh`) "QueryOnly")
  (set `self.CurrentPickupState` "NewEnumerator0"))

(event `/Game/EpicTemplates/WalkingSimTemplate/Blueprints/Interfaces/BPI_Pickup.StartedPutDown`
  (params (Interactor :type "/Game/EpicTemplates/WalkingSimTemplate/Blueprints/Interfaces/BPI_PickupManipulator Interface"))
  ;[1 1 1] Pickup Interface
  (`PrimitiveComponent.SetCollisionEnabled` (`self.Mesh`) "NoCollision")
  (set `self.CurrentPickupState` "NewEnumerator3")
  (`self.OnPutDown` self))

(event `/Game/EpicTemplates/WalkingSimTemplate/Blueprints/Interfaces/BPI_Pickup.UpdateCanBeTaken`
  (params (InCanBeTaken :type Boolean))
  ;[1 1 1] Pickup Interface
  (set `self.bCan be Taken` InCanBeTaken))

(event `/Game/EpicTemplates/WalkingSimTemplate/Blueprints/Interfaces/BPI_Pickup.Taken`
  ;[1 1 1] Pickup Interface
  (set `self.CurrentPickupState` "NewEnumerator0")
  (`self.OnTaken` self))

(event `/Game/EpicTemplates/WalkingSimTemplate/Blueprints/Interfaces/BPI_Pickup.UpdatePutDownTransform`
  (params (NewPutDownTransform :type "Transform Structure"))
  ;[1 1 1] Pickup Interface
  (set `self.PutDownTransform` NewPutDownTransform))

(fn `CanBeTaken`
  (returns (bCanBeTaken :type Boolean))
  (return (`self.bCan be Taken`)))

(fn `GetExamineViewDistance`
  (returns (ExamienViewDistance :type "Float (double-precision)"))
  (return (`self.ExaminePickupDistance`)))

(fn `GetInitialExamineRotation`
  (returns (ExamineRotation :type "Rotator Structure"))
  (return (`self.InitialExamineRotation`)))

(fn `GetInteractParentActor`
  (returns (ParentActor :type "Actor Object Reference"))
  (return self))

(fn `GetInteractText`
  (returns (InteractName :type Text))
  (return (`self.PickupName`)))

(fn `GetIsInteractLocked`
  (returns (bIsInteractLocked :type Boolean))
  (return false))

(fn `GetPutDownTransform`
  (returns (PutDownTransform :type "Transform Structure"))
  (return (`self.PutDownTransform`)))

(fn `Handle Rotate Pickup`
  (params (InteractingController :type "Controller Object Reference") (YawInput :type "Float (single-precision)") (PitchInput :type "Float (double-precision)"))
  (locals (PlayerViewRotTrans :type "Transform Structure"))
  (set `local.PlayerViewRotTrans` (`KismetMathLibrary.MakeTransform` (0.0 0.0 0.0) (`.Rotation` (`Controller.GetPlayerViewPoint` InteractingController))))
  (`self.K2_SetActorRotation` (`KismetMathLibrary.TransformRotation` (`local.PlayerViewRotTrans`) (`KismetMathLibrary.ComposeRotators` (`KismetMathLibrary.InverseTransformRotation` (`local.PlayerViewRotTrans`) (`self.K2_GetActorRotation`)) (`KismetMathLibrary.MakeRotator` 0.0 (`local.PitchInput`) (`local.YawInput`))))))

(fn `UserConstructionScript`)