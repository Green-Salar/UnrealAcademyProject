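; First-person player character for the walking sim template, handling movement, look and interaction input.
; Possession adds the walking sim Enhanced Input mapping context and unpossession removes it.
; Movement pauses while interacting or examining a pickup; look input goes to the current interactable, or is ignored during examination.
; Tick smooths actor yaw and camera pitch toward control rotation, while movement follows raw control yaw.
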(event `self.ReceivePossessed`
  (params (NewController :type "Controller Object Reference"))
  ;[1 1 1] Possessed/Unpossessed
  (bind _asplayer_controller (cast `PlayerController` NewController))
  (bind _output_get (set `self.OwningPlayerController` _asplayer_controller))
  (`KismetSystemLibrary.DelayUntilNextTick`)
  (`EnhancedInputSubsystemInterface.AddMappingContext` (pcsubsystem `EnhancedInputLocalPlayerSubsystem` _output_get) "/Game/EpicTemplates/WalkingSimTemplate/Input/IMC_WalkingSim.IMC_WalkingSim" 0 (struct)))

(event `self.ReceiveBeginPlay`
  ;[1 1 1] BeginPlay
  ;;[1 1 1] Align eye height with camera for the sake of GetActorEyesViewpoint calls
  (set `self.BaseEyeHeight` (.z (`SceneComponent.RelativeLocation` (`self.Camera`)))))

(event `self.ReceiveUnpossessed`
  (params (OldController :type "Controller Object Reference"))
  (bind _owningplayercontroller (`self.OwningPlayerController`))
  ;[1 1 1] Possessed/Unpossessed
  (`/Engine/EditorBlueprintResources/StandardMacros.IsValid` _owningplayercontroller
    (:`Is Valid`
      (`EnhancedInputSubsystemInterface.RemoveMappingContext` (pcsubsystem `EnhancedInputLocalPlayerSubsystem` _owningplayercontroller) "/Game/EpicTemplates/WalkingSimTemplate/Input/IMC_WalkingSim.IMC_WalkingSim" (struct))
      (set `self.OwningPlayerController` null))))

(event `self.ReceiveTick`
  (params (DeltaSeconds :type "Float (single-precision)"))
  ;[1 1 1] Tick
  (`self.InterpActorYawToControlYaw` DeltaSeconds)
  (`self.InterpCameraPitchToControlPitch` DeltaSeconds))

(event `EnhancedInput|/Game/EpicTemplates/WalkingSimTemplate/Input/IA_Read`
  (params (ActionValue :type Boolean) (ElapsedSeconds :type "Float (double-precision)") (TriggeredSeconds :type "Float (double-precision)") (InputAction :type "InputAction Object Reference" :default "/Game/EpicTemplates/WalkingSimTemplate/Input/IA_Read.IA_Read"))
  ;[1 1 1] Input
  ;;[1 1 1] Current does nothing
)

(event `EnhancedInput|/Game/EpicTemplates/WalkingSimTemplate/Input/IA_MoveForward`
  (params (ActionValue :type "Float (double-precision)") (ElapsedSeconds :type "Float (double-precision)") (TriggeredSeconds :type "Float (double-precision)") (InputAction :type "InputAction Object Reference" :default "/Game/EpicTemplates/WalkingSimTemplate/Input/IA_MoveForward.IA_MoveForward"))
  ;[1 1 1] Input
  (:`Triggered`
    (bind _bisinteracting (`/Game/EpicTemplates/WalkingSimTemplate/Blueprints/Interfaces/BPI_FirstPersonInteractor.IsInteracting` (`self.FirstPersonInteractComponent`)))
    (if (not _bisinteracting)
      (bind _bisexaminingpickup (`/Game/EpicTemplates/WalkingSimTemplate/Blueprints/Interfaces/BPI_PickupManipulator.IsExaminingPickup` (`self.PickupInteractComponent`)))
      (if (not _bisexaminingpickup)
        (`PawnMovementComponent.AddInputVector` (`self.CharacterMovement`) (* (`KismetMathLibrary.GetForwardVector` (`self.GetMovementRotation`)) ActionValue) false)))))

(event `EnhancedInput|/Game/EpicTemplates/WalkingSimTemplate/Input/IA_MoveRight`
  (params (ActionValue :type "Float (double-precision)") (ElapsedSeconds :type "Float (double-precision)") (TriggeredSeconds :type "Float (double-precision)") (InputAction :type "InputAction Object Reference" :default "/Game/EpicTemplates/WalkingSimTemplate/Input/IA_MoveRight.IA_MoveRight"))
  ;[1 1 1] Input
  (:`Triggered`
    (bind _bisinteracting (`/Game/EpicTemplates/WalkingSimTemplate/Blueprints/Interfaces/BPI_FirstPersonInteractor.IsInteracting` (`self.FirstPersonInteractComponent`)))
    (if (not _bisinteracting)
      (bind _bisexaminingpickup (`/Game/EpicTemplates/WalkingSimTemplate/Blueprints/Interfaces/BPI_PickupManipulator.IsExaminingPickup` (`self.PickupInteractComponent`)))
      (if (not _bisexaminingpickup)
        (`PawnMovementComponent.AddInputVector` (`self.CharacterMovement`) (* (`KismetMathLibrary.GetRightVector` (`self.GetMovementRotation`)) ActionValue) false)))))

(event `EnhancedInput|/Game/EpicTemplates/WalkingSimTemplate/Input/IA_Turn`
  (params (ActionValue :type "Float (double-precision)") (ElapsedSeconds :type "Float (double-precision)") (TriggeredSeconds :type "Float (double-precision)") (InputAction :type "InputAction Object Reference" :default "/Game/EpicTemplates/WalkingSimTemplate/Input/IA_Turn.IA_Turn"))
  ;[1 1 1] Input
  (:`Triggered`
    (bind (_currentinteractingobject _interactableinterface) (`/Game/EpicTemplates/WalkingSimTemplate/Blueprints/Interfaces/BPI_FirstPersonInteractor.GetCurrentInteractingObject` (`self.FirstPersonInteractComponent`)))
    (`/Engine/EditorBlueprintResources/StandardMacros.IsValid` _currentinteractingobject
      (:`Is Valid`
        (`/Game/EpicTemplates/WalkingSimTemplate/Blueprints/Interfaces/BPI_FirstPersonInteractable.HorizontalInput` _interactableinterface (`self.GetController`) ActionValue))
      (:`Is Not Valid`
        (bind _bisexaminingpickup (`/Game/EpicTemplates/WalkingSimTemplate/Blueprints/Interfaces/BPI_PickupManipulator.IsExaminingPickup` (`self.PickupInteractComponent`)))
        (if (not _bisexaminingpickup)
          (`PlayerController.AddYawInput` (`self.OwningPlayerController`) ActionValue))))))

(event `EnhancedInput|/Game/EpicTemplates/WalkingSimTemplate/Input/IA_LookUp`
  (params (ActionValue :type "Float (double-precision)") (ElapsedSeconds :type "Float (double-precision)") (TriggeredSeconds :type "Float (double-precision)") (InputAction :type "InputAction Object Reference" :default "/Game/EpicTemplates/WalkingSimTemplate/Input/IA_LookUp.IA_LookUp"))
  ;[1 1 1] Input
  (:`Triggered`
    (bind (_currentinteractingobject _interactableinterface) (`/Game/EpicTemplates/WalkingSimTemplate/Blueprints/Interfaces/BPI_FirstPersonInteractor.GetCurrentInteractingObject` (`self.FirstPersonInteractComponent`)))
    (`/Engine/EditorBlueprintResources/StandardMacros.IsValid` _currentinteractingobject
      (:`Is Valid`
        (`/Game/EpicTemplates/WalkingSimTemplate/Blueprints/Interfaces/BPI_FirstPersonInteractable.VerticalInput` _interactableinterface (`self.GetController`) ActionValue))
      (:`Is Not Valid`
        (bind _bisexaminingpickup (`/Game/EpicTemplates/WalkingSimTemplate/Blueprints/Interfaces/BPI_PickupManipulator.IsExaminingPickup` (`self.PickupInteractComponent`)))
        (if (not _bisexaminingpickup)
          (`PlayerController.AddPitchInput` (`self.OwningPlayerController`) (* ActionValue -1.0)))))))

(fn `GetMovementRotation`
  (returns (MovementRotation :type "Rotator Structure"))
  (return (`KismetMathLibrary.MakeRotator` 0.0 0.0 (.yaw (`self.GetControlRotation`)))))

(fn `InterpActorYawToControlYaw`
  (params (DeltaTime :type "Float (double-precision)"))
  (bind (_returnvalue_roll _returnvalue_pitch) (`KismetMathLibrary.BreakRotator` (`self.K2_GetActorRotation`)))
  (bind (_returnvalue_roll_2 _returnvalue_pitch_2 _returnvalue_yaw) (`KismetMathLibrary.BreakRotator` (`self.K2_GetActorRotation`)))
  (bind (_returnvalue_roll_3 _returnvalue_pitch_3 _returnvalue_yaw_2) (`KismetMathLibrary.BreakRotator` (`self.GetControlRotation`)))
  (bind (_returnvalue_roll_4 _returnvalue_pitch_4 _returnvalue_yaw_3) (`KismetMathLibrary.BreakRotator` (`KismetMathLibrary.RInterpTo` (`KismetMathLibrary.MakeRotator` 0.0 0.0 _returnvalue_yaw) (`KismetMathLibrary.MakeRotator` 0.0 0.0 _returnvalue_yaw_2) DeltaTime (`self.YawInterpSpeed`))))
  (`self.K2_SetActorRotation` (`KismetMathLibrary.MakeRotator` _returnvalue_roll _returnvalue_pitch _returnvalue_yaw_3)))

(fn `InterpCameraPitchToControlPitch`
  (params (DeltaTime :type "Float (double-precision)"))
  (bind (_relativerotation_roll _relativerotation_pitch _relativerotation_yaw) (`KismetMathLibrary.BreakRotator` (`SceneComponent.RelativeRotation` (`self.Camera`))))
  (`SceneComponent.K2_SetRelativeRotation` (`self.Camera`) (`KismetMathLibrary.MakeRotator` _relativerotation_roll (`KismetMathLibrary.FInterpTo` _relativerotation_pitch (.pitch (`KismetMathLibrary.InverseTransformRotation` (`SceneComponent.K2_GetComponentToWorld` (`self.CapsuleComponent`)) (`self.GetControlRotation`))) DeltaTime (`self.CameraPitchInterpSpeed`)) _relativerotation_yaw) false false))

(fn `UserConstructionScript`)