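; Player controller for the walking sim template that manages the game cursor and button prompts for examining pickups.
; It creates the cursor widget on BeginPlay and, on possess, binds to the pawn's BP_PickupInteractComponent examine events.
; Examining frees and centers the cursor and shows Put Down, plus Take if allowed; stopping hides both prompts.
; The GetCursorScreenPosition override reports screen center unless the cursor is free.
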(event `self.ReceiveBeginPlay`
  (`parent.ReceiveBeginPlay`)
  (bind _returnvalue (`|CreateWidget` "/Game/EpicTemplates/WalkingSimTemplate/UI/W_PlayerGameCursor_WalkingSim.W_PlayerGameCursor_WalkingSim_C"))
  (bind _output_get (set `self.GameCursor` _returnvalue))
  (`UserWidget.AddToViewport` _output_get 0))

(event `self.ReceivePossess`
  (params (PossessedPawn :type "Pawn Object Reference"))
  (`parent.ReceivePossess` PossessedPawn)
  (`self.TryBindToPawnPickupEvents` PossessedPawn))

(event `PawnStartedExaminingPickup`
  (params (Caller :type "/Game/EpicTemplates/WalkingSimTemplate/Blueprints/Components/BP_PickupInteractComponent Object Reference") (NewPickupActor :type "Actor Object Reference") (PickupInterface :type "/Game/EpicTemplates/WalkingSimTemplate/Blueprints/Interfaces/BPI_Pickup Interface"))
  (set `self.bCursorFree` true)
  (`self.SetCursorScreenPosition` (* (`WidgetLayoutLibrary.GetViewportSize`) 0.5))
  (`self.DisplayButtonPrompt` (`self.CancelPickupPromptID`) "/Game/EpicTemplates/WalkingSimTemplate/Input/IA_Cancel.IA_Cancel" "Put Down" "NewEnumerator1")
  (bind _bcanbetaken (`/Game/EpicTemplates/WalkingSimTemplate/Blueprints/Interfaces/BPI_Pickup.CanBeTaken` PickupInterface))
  (if _bcanbetaken
    (`self.DisplayButtonPrompt` (`self.TakePickupPromptID`) "/Game/EpicTemplates/WalkingSimTemplate/Input/IA_Take.IA_Take" "Take" "NewEnumerator1")))

(event `PawnStoppedExaminingPickup`
  (params (Caller :type "/Game/EpicTemplates/WalkingSimTemplate/Blueprints/Components/BP_PickupInteractComponent Object Reference") (PuttingDownPickupActor :type "Actor Object Reference") (PickupInterface :type "/Game/EpicTemplates/WalkingSimTemplate/Blueprints/Interfaces/BPI_Pickup Interface"))
  (set `self.bCursorFree` false)
  (`self.HideButtonPrompt` (`self.CancelPickupPromptID`))
  (`self.HideButtonPrompt` (`self.TakePickupPromptID`)))

(fn `CancelPickupPromptID`
  (returns (ReturnValue :type Name))
  (return "CancelPickup"))

(fn `GetCursorScreenPosition`
  (returns (ScreenPos :type "Vector2D Structure"))
  (if (`self.bCursorFree`)
    (bind _screenpos (`parent.GetCursorScreenPosition`))
    (return _screenpos)
    (else
      (return (* (`WidgetLayoutLibrary.GetViewportSize`) 0.5)))))

(fn `TakePickupPromptID`
  (returns (ReturnValue :type Name))
  (return "TakePickup"))

(fn `TryBindToPawnPickupEvents`
  (params (Pawn :type "Actor Object Reference"))
  (locals (PickupInteractorComponent :type "/Game/EpicTemplates/WalkingSimTemplate/Blueprints/Components/BP_PickupInteractComponent Object Reference"))
  (bind _output_get (set `local.PickupInteractorComponent` (`self.GetComponentByClass` Pawn "/Game/EpicTemplates/WalkingSimTemplate/Blueprints/Components/BP_PickupInteractComponent.BP_PickupInteractComponent_C")))
  (`/Engine/EditorBlueprintResources/StandardMacros.IsValid` _output_get
    (:`Is Valid`
      (set `self.CurrentBoundPickupComp` _output_get)
      (add `/Game/EpicTemplates/WalkingSimTemplate/Blueprints/Components/BP_PickupInteractComponent.OnStartedExaminingPickup` (`local.PickupInteractorComponent`) (`|CreateDelegate` :!event `PawnStartedExaminingPickup`))
      (add `/Game/EpicTemplates/WalkingSimTemplate/Blueprints/Components/BP_PickupInteractComponent.OnStoppedExaminingPickup` (`local.PickupInteractorComponent`) (`|CreateDelegate` :!event `PawnStoppedExaminingPickup`)))))

(fn `TryUnbindFromPawnPickupEvents`
  (params (Pawn :type "Actor Object Reference"))
  (locals (PickupInteractorComponent :type "/Game/EpicTemplates/WalkingSimTemplate/Blueprints/Components/BP_PickupInteractComponent Object Reference"))
  (bind _output_get (set `local.PickupInteractorComponent` (`self.GetComponentByClass` Pawn "/Game/EpicTemplates/WalkingSimTemplate/Blueprints/Components/BP_PickupInteractComponent.BP_PickupInteractComponent_C")))
  (`/Engine/EditorBlueprintResources/StandardMacros.IsValid` _output_get
    (:`Is Valid`
      (remove `/Game/EpicTemplates/WalkingSimTemplate/Blueprints/Components/BP_PickupInteractComponent.OnStartedExaminingPickup` (`local.PickupInteractorComponent`) (`|CreateDelegate` :!event `PawnStartedExaminingPickup`))
      (remove `/Game/EpicTemplates/WalkingSimTemplate/Blueprints/Components/BP_PickupInteractComponent.OnStoppedExaminingPickup` (`local.PickupInteractorComponent`) (`|CreateDelegate` :!event `PawnStoppedExaminingPickup`)))))

(fn `UserConstructionScript`
  (`parent.UserConstructionScript`))