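; Interactable collision component for the walking sim template that makes its owning actor a target for player interaction.
; It relays hover, interact start/end and horizontal/vertical input through event dispatchers, and exposes prompt text, owner and a collision toggle.
; It reports locked if manually locked or if gated by a gameplay tag.
; A valid tag starts it locked, then follows the inverse of that level bool via game mode updates.
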(event `self.ReceiveBeginPlay`
  (if (`BlueprintGameplayTagLibrary.IsGameplayTagValid` (`self.LockingLevelBoolTag`))
    (set `self.IsGameplayTagLocked` true)
    (bind _asbp_game_mode_template_base (cast `/Game/EpicTemplates/TemplateAgnostic/Blueprints/Core/BP_GameMode_TemplateBase` (`GameplayStatics.GetGameMode`)))
    (add `/Game/EpicTemplates/TemplateAgnostic/Blueprints/Core/BP_GameMode_TemplateBase.OnLevelBoolUpdated` _asbp_game_mode_template_base (delegate `LevelBoolUpdated`))))

(event `LevelBoolUpdated`
  (params (LevelBoolTag :type "GameplayTag Structure") (NewValue :type Boolean))
  (if (== (`self.LockingLevelBoolTag`) LevelBoolTag)
    (set `self.IsGameplayTagLocked` (not NewValue))))

(event `/Game/EpicTemplates/WalkingSimTemplate/Blueprints/Interfaces/BPI_FirstPersonInteractable.InteractStart`
  (params (InteractingController :type "Controller Object Reference"))
  (`self.OnInteractStart` InteractingController))

(event `/Game/EpicTemplates/WalkingSimTemplate/Blueprints/Interfaces/BPI_FirstPersonInteractable.UpdateInteractLocked`
  (params (bNewLocked :type Boolean))
  (set `self.IsInteractLocked` bNewLocked))

(event `/Game/EpicTemplates/WalkingSimTemplate/Blueprints/Interfaces/BPI_FirstPersonInteractable.InteractEnd`
  (params (InteractingController :type "Controller Object Reference"))
  (`self.OnInteractEnd` InteractingController))

(event `UpdateCollisionEnabled`
  (params (IsEnabled :type Boolean))
  (`self.SetCollisionEnabled` (select `bool` IsEnabled :`false` "NoCollision" :`true` "QueryOnly" :!type "ECollisionEnabled Enum")))

(event `/Game/EpicTemplates/WalkingSimTemplate/Blueprints/Interfaces/BPI_FirstPersonInteractable.UnHovered`
  (params (InteractingController :type "Controller Object Reference"))
  (`self.OnUnhovered` InteractingController))

(event `/Game/EpicTemplates/WalkingSimTemplate/Blueprints/Interfaces/BPI_FirstPersonInteractable.VerticalInput`
  (params (InteractingController :type "Controller Object Reference") (Input :type "Float (double-precision)"))
  (`self.OnVerticalInput` InteractingController Input))

(event `/Game/EpicTemplates/WalkingSimTemplate/Blueprints/Interfaces/BPI_FirstPersonInteractable.Hovered`
  (params (InteractingController :type "Controller Object Reference"))
  (`self.OnHovered` InteractingController))

(event `/Game/EpicTemplates/WalkingSimTemplate/Blueprints/Interfaces/BPI_FirstPersonInteractable.HorizontalInput`
  (params (InteractingController :type "Controller Object Reference") (Input :type "Float (double-precision)"))
  (`self.OnHorizontalInput` InteractingController Input))

(fn `GetInteractParentActor`
  (returns (ParentActor :type "Actor Object Reference"))
  (return (`self.GetOwner`)))

(fn `GetInteractText`
  (returns (InteractName :type Text))
  (return (`self.InteractText`)))

(fn `GetIsInteractLocked`
  (returns (bIsInteractLocked :type Boolean))
  (return (or (`self.IsInteractLocked`) (`self.IsGameplayTagLocked`))))