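; Walking-sim actor component that lets its owner examine BPI_Pickup actors, put them down, or take them into a BPI_SimpleInventory found on the owner.
; Examining moves the pickup in front of the eye view or an override transform component, using a BP_PickupInteractData object per movement.
; Replaced or cancelled pickups join a returning list, so several can move back simultaneously.
; Tick drives these movements and switches itself off once all finish.
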(event `EnhancedInput|/Game/EpicTemplates/WalkingSimTemplate/Input/IA_Cancel`
  (params (ActionValue :type Boolean) (ElapsedSeconds :type "Float (double-precision)") (TriggeredSeconds :type "Float (double-precision)") (InputAction :type "InputAction Object Reference" :default "/Game/EpicTemplates/WalkingSimTemplate/Input/IA_Cancel.IA_Cancel"))
  ;[1 1 1] Input
  (:`Triggered`
    (bind _bisexaminingpickup (`/Game/EpicTemplates/WalkingSimTemplate/Blueprints/Interfaces/BPI_PickupManipulator.IsExaminingPickup`))
    (if _bisexaminingpickup
      (`/Game/EpicTemplates/WalkingSimTemplate/Blueprints/Interfaces/BPI_PickupManipulator.PutDownCurrentExaminedPickup`))))

(event `self.ReceiveBeginPlay`
  ;[1 1 1] Begin Play
  (set `self.PickupMoveSpeed` (/ 1.0 (`self.PickupMoveTime`)))
  (bind (_interfaceimplementingobject _foundimplementingobject) (`/Game/EpicTemplates/TemplateAgnostic/Blueprints/EpicTemplatesFunctionLibrary.SearchActorForInterface` (`self.GetOwner`) "/Game/EpicTemplates/WalkingSimTemplate/Blueprints/Interfaces/BPI_SimpleInventory.BPI_SimpleInventory_C"))
  (if _foundimplementingobject
    (set `self.InventoryObject` _interfaceimplementingobject)))

(event `/Game/EpicTemplates/WalkingSimTemplate/Blueprints/Interfaces/BPI_PickupManipulator.ExamineNewPickup`
  (params (NewPickup :type "Actor Object Reference"))
  ;[1 1 1] BPI_PickupManipulator
  (`self.HandleExamineNewPickup` NewPickup))

(event `/Game/EpicTemplates/WalkingSimTemplate/Blueprints/Interfaces/BPI_PickupManipulator.PutDownCurrentExaminedPickup`
  ;[1 1 1] BPI_PickupManipulator
  (`self.HandlePutDownCurrentExaminedPickup`))

(event `EnhancedInput|/Game/EpicTemplates/WalkingSimTemplate/Input/IA_Take`
  (params (ActionValue :type Boolean) (ElapsedSeconds :type "Float (double-precision)") (TriggeredSeconds :type "Float (double-precision)") (InputAction :type "InputAction Object Reference" :default "/Game/EpicTemplates/WalkingSimTemplate/Input/IA_Take.IA_Take"))
  ;[1 1 1] Input
  (:`Triggered`
    (`/Game/EpicTemplates/WalkingSimTemplate/Blueprints/Interfaces/BPI_PickupManipulator.TryTakeCurrentPickup` (`self.InventoryObject`))))

(event `self.ReceiveTick`
  (params (DeltaSeconds :type "Float (single-precision)"))
  ;[1 1 1] Tick
  (`self.HandlePickupMovements` DeltaSeconds))

(event `AssignOverrideExamineTransformComponent`
  (params (ExamineTransformComponent :type "SceneComponent Object Reference"))
  ;[1 1 1] AssignOverrideExamineTransform
  (set `self.OverrideExamineTransformComponent` ExamineTransformComponent))

(fn `CheckForDisableTick`
  (if (and (not (`self.MidPickupMovement`)) (== (`KismetArrayLibrary.Array_Length` (`self.ReturningPickups`)) 0))
    (`self.SetComponentTickEnabled` false)))

(fn `GetCurrentExaminedPickup`
  (returns (CurrentExaminedPickup :type "Actor Object Reference") (ExaminingPickupInterface :type "/Game/EpicTemplates/WalkingSimTemplate/Blueprints/Interfaces/BPI_Pickup Interface"))
  (bind _currentexaminingpickupdata (`self.CurrentExaminingPickupData`))
  (`/Engine/EditorBlueprintResources/StandardMacros.IsValid` _currentexaminingpickupdata
    (:`Is Valid`
      (return (`/Game/EpicTemplates/WalkingSimTemplate/Blueprints/BP_PickupInteractData.Pickup` _currentexaminingpickupdata) (`/Game/EpicTemplates/WalkingSimTemplate/Blueprints/BP_PickupInteractData.PickupInterface` _currentexaminingpickupdata)))
    (:`Is Not Valid`
      (return null null))))

(fn `HandleExamineNewPickup`
  (params (NewPickup :type "Actor Object Reference"))
  (locals (CurrentPickupActor :type "Actor Object Reference") (ExamineTrans :type "Transform Structure"))
  (bind _overrideexaminetransformcomponent (`self.OverrideExamineTransformComponent`))
  (bind _newpickup (`local.NewPickup`))
  (bind _newpickup_2 (`local.NewPickup`))
  (bind (_outlocation _outrotation) (`Actor.GetActorEyesViewPoint` (`self.GetOwner`)))
  (`/Engine/EditorBlueprintResources/StandardMacros.IsValid` NewPickup
    (:`Is Valid`
      (if (`KismetSystemLibrary.DoesImplementInterface` (`local.NewPickup`) "/Game/EpicTemplates/WalkingSimTemplate/Blueprints/Interfaces/BPI_Pickup.BPI_Pickup_C")
        (bind _currentexaminedpickup (`self.GetCurrentExaminedPickup`))
        (bind _output_get (set `local.CurrentPickupActor` _currentexaminedpickup))
        (if (== _output_get (`local.NewPickup`))
          (return)
          (else
            (`self.HandlePutDownCurrentExaminedPickup`)
            (bind _returnvalue (`|GenericCreateObject` "/Game/EpicTemplates/WalkingSimTemplate/Blueprints/BP_PickupInteractData.BP_PickupInteractData_C"))
            (bind _output_get_2 (set `self.CurrentExaminingPickupData` _returnvalue))
            (`/Game/EpicTemplates/WalkingSimTemplate/Blueprints/BP_PickupInteractData.Setup` _output_get_2 (`local.NewPickup`))
            (`|ExecutionSequence`
              (:`then_0`
                (`/Engine/EditorBlueprintResources/StandardMacros.IsValid` _overrideexaminetransformcomponent
                  (:`Is Valid`
                    (set `local.ExamineTrans` (`SceneComponent.K2_GetComponentToWorld` _overrideexaminetransformcomponent)))
                  (:`Is Not Valid`
                    (set `local.ExamineTrans` (`KismetMathLibrary.MakeTransform` _outlocation _outrotation)))))
              (:`then_1`
                (bind _examienviewdistance (message `/Game/EpicTemplates/WalkingSimTemplate/Blueprints/Interfaces/BPI_Pickup.GetExamineViewDistance` _newpickup))
                (bind _examinerotation (message `/Game/EpicTemplates/WalkingSimTemplate/Blueprints/Interfaces/BPI_Pickup.GetInitialExamineRotation` _newpickup))
                (`/Game/EpicTemplates/WalkingSimTemplate/Blueprints/BP_PickupInteractData.StartNewMovement` (`self.CurrentExaminingPickupData`) (`KismetMathLibrary.ComposeTransforms` (`KismetMathLibrary.MakeTransform` (`KismetMathLibrary.MakeVector` _examienviewdistance) _examinerotation) (`local.ExamineTrans`)))
                (message `/Game/EpicTemplates/WalkingSimTemplate/Blueprints/Interfaces/BPI_Pickup.StartedPickUp` (`local.NewPickup`) self)
                (set `self.MidPickupMovement` true)
                (`self.SetComponentTickEnabled` true)
                (bind _asbpi_pickup (cast `/Game/EpicTemplates/WalkingSimTemplate/Blueprints/Interfaces/BPI_Pickup` _newpickup_2))
                (`self.OnStartedExaminingPickup` self _newpickup_2 _asbpi_pickup)))))
        (else
          (`KismetSystemLibrary.PrintString` (`KismetStringLibrary.Concat_StrStr` "BP_PickupInteractComponent::ExamineNewPickup - Pickup '" (`KismetSystemLibrary.GetDisplayName` (`local.NewPickup`)) "' doesn't implement the BPi_Pickup interface, so cannot be interacted with.")))))))

(fn `HandlePickupMovements`
  (params (DeltaSeconds :type "Float (single-precision)"))
  (locals (CheckForDisable :type Boolean) (TempReturningPickupData :type "/Game/EpicTemplates/WalkingSimTemplate/Blueprints/BP_PickupInteractData Object Reference") (TempReturningPickupIdx :type Integer))
  (bind _currentexaminingpickupdata (`self.CurrentExaminingPickupData`))
  (`|ExecutionSequence`
    (:`then_0`
      (if (`self.MidPickupMovement`)
        (`/Engine/EditorBlueprintResources/StandardMacros.IsValid` _currentexaminingpickupdata
          (:`Is Valid`
            (bind _bmovementfinished (`/Game/EpicTemplates/WalkingSimTemplate/Blueprints/BP_PickupInteractData.MoveToTargetTransform` _currentexaminingpickupdata (`self.PickupMoveSpeed`) (`local.DeltaSeconds`)))
            (if _bmovementfinished
              (set `self.MidPickupMovement` false)
              (message `/Game/EpicTemplates/WalkingSimTemplate/Blueprints/Interfaces/BPI_Pickup.ReachedPickupExaminePoint` (`/Game/EpicTemplates/WalkingSimTemplate/Blueprints/BP_PickupInteractData.Pickup` (`self.CurrentExaminingPickupData`)) self)
              (set `local.CheckForDisable` true))))))
    (:`then_1`
      (bind (_arrayindex _arrayelement) (`/Engine/EditorBlueprintResources/StandardMacros.ReverseForEachLoop` (`self.ReturningPickups`))
        (:`LoopBody`
          (set `local.TempReturningPickupIdx` _arrayindex)
          (bind _output_get (set `local.TempReturningPickupData` _arrayelement))
          (`/Engine/EditorBlueprintResources/StandardMacros.IsValid` _output_get
            (:`Is Valid`
              (bind _bmovementfinished_2 (`/Game/EpicTemplates/WalkingSimTemplate/Blueprints/BP_PickupInteractData.MoveToTargetTransform` (`local.TempReturningPickupData`) (`self.PickupMoveSpeed`) (`local.DeltaSeconds`)))
              (if _bmovementfinished_2
                (`KismetArrayLibrary.Array_Remove` (`self.ReturningPickups`) (`local.TempReturningPickupIdx`))
                (message `/Game/EpicTemplates/WalkingSimTemplate/Blueprints/Interfaces/BPI_Pickup.ReachedPutDownPoint` (`/Game/EpicTemplates/WalkingSimTemplate/Blueprints/BP_PickupInteractData.Pickup` (`local.TempReturningPickupData`)) self)
                (set `local.CheckForDisable` true)))
            (:`Is Not Valid`
              (`KismetArrayLibrary.Array_Remove` (`self.ReturningPickups`) (`local.TempReturningPickupIdx`)))))))
    (:`then_2`
      (if (`local.CheckForDisable`)
        (`self.CheckForDisableTick`)))))

(fn `HandlePutDownCurrentExaminedPickup`
  (locals (CurrentPickupActor :type "Actor Object Reference"))
  (bind _currentpickupactor (`local.CurrentPickupActor`))
  (bind _currentexaminedpickup (`self.GetCurrentExaminedPickup`))
  (bind _output_get (set `local.CurrentPickupActor` _currentexaminedpickup))
  (`/Engine/EditorBlueprintResources/StandardMacros.IsValid` _output_get
    (:`Is Valid`
      (`KismetArrayLibrary.Array_Add` (`self.ReturningPickups`) (`self.CurrentExaminingPickupData`))
      (bind _putdowntransform (message `/Game/EpicTemplates/WalkingSimTemplate/Blueprints/Interfaces/BPI_Pickup.GetPutDownTransform` (`local.CurrentPickupActor`)))
      (`/Game/EpicTemplates/WalkingSimTemplate/Blueprints/BP_PickupInteractData.StartNewMovement` (`self.CurrentExaminingPickupData`) _putdowntransform)
      (set `self.CurrentExaminingPickupData` null)
      (`self.SetComponentTickEnabled` true)
      (bind _asbpi_pickup (cast `/Game/EpicTemplates/WalkingSimTemplate/Blueprints/Interfaces/BPI_Pickup` _currentpickupactor))
      (`self.OnStoppedExaminingPickup` self _currentpickupactor _asbpi_pickup))))

(fn `IsExaminingPickup`
  (returns (bIsExaminingPickup :type Boolean))
  (bind _currentexaminingpickupdata (`self.CurrentExaminingPickupData`))
  (`/Engine/EditorBlueprintResources/StandardMacros.IsValid` _currentexaminingpickupdata
    (:`Is Valid`
      (return (`/Game/EpicTemplates/WalkingSimTemplate/Blueprints/BP_PickupInteractData.IsValidPickupData` _currentexaminingpickupdata)))
    (:`Is Not Valid`
      (return false))))

(fn `TryTakeCurrentPickup`
  (params (InventoryObject :type "Object Object Reference"))
  (returns (bDidTake :type Boolean))
  (locals (CurrentExaminingPickup :type "Actor Object Reference") (ExaminingPickupInterface :type "/Game/EpicTemplates/WalkingSimTemplate/Blueprints/Interfaces/BPI_Pickup Interface"))
  (if (not (`self.MidPickupMovement`))
    (bind (_currentexaminedpickup _examiningpickupinterface) (`self.GetCurrentExaminedPickup`))
    (bind _output_get (set `local.CurrentExaminingPickup` _currentexaminedpickup))
    (`/Engine/EditorBlueprintResources/StandardMacros.IsValid` _output_get
      (:`Is Valid`
        (set `local.ExaminingPickupInterface` _examiningpickupinterface)
        (bind _bcanbetaken (message `/Game/EpicTemplates/WalkingSimTemplate/Blueprints/Interfaces/BPI_Pickup.CanBeTaken` (`local.CurrentExaminingPickup`)))
        (if _bcanbetaken
          (if (`KismetSystemLibrary.DoesImplementInterface` (`local.InventoryObject`) "/Game/EpicTemplates/WalkingSimTemplate/Blueprints/Interfaces/BPI_SimpleInventory.BPI_SimpleInventory_C")
            (set `self.CurrentExaminingPickupData` null)
            (message `/Game/EpicTemplates/WalkingSimTemplate/Blueprints/Interfaces/BPI_SimpleInventory.AddItem` (`local.InventoryObject`) (`local.CurrentExaminingPickup`))
            (message `/Game/EpicTemplates/WalkingSimTemplate/Blueprints/Interfaces/BPI_Pickup.Taken` (`local.CurrentExaminingPickup`))
            (`self.OnStoppedExaminingPickup` self (`local.CurrentExaminingPickup`) (`local.ExaminingPickupInterface`))
            (return true)
            (else
              (return false)))
          (else
            (return false)))))))