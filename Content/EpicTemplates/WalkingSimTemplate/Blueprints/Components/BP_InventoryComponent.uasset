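; Inventory component for the Walking Sim template that stores picked-up item actors on its owner.
; AddItem hides the actor, disables its collision, attaches it to the owner and broadcasts an item-added event.
; Lookup and removal match items by class, including child classes; removal can keep, reveal or destroy the actor and broadcasts an item-removed event.
; RemoveAndPlaceItemByClass also detaches the item and teleports it to a given transform.
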(event `/Game/EpicTemplates/WalkingSimTemplate/Blueprints/Interfaces/BPI_SimpleInventory.AddItem`
  (params (ItemToAdd :type "Actor Object Reference"))
  (`KismetArrayLibrary.Array_Add` (`self.ContainedItems`) ItemToAdd)
  (`Actor.SetActorEnableCollision` ItemToAdd false)
  (`Actor.SetActorHiddenInGame` ItemToAdd true)
  (`Actor.K2_AttachToActor` ItemToAdd (`self.GetOwner`) "None" "SnapToTarget" "SnapToTarget" "SnapToTarget" false)
  (`self.OnItemAdded` self ItemToAdd))

(fn `DoesContainItemByClass`
  (params (ItemClass :type "Actor Class Reference"))
  (returns (ItemInstance :type "Actor Object Reference") (bContainsItem :type Boolean))
  (for _array_element (`self.ContainedItems`)
    (if (`KismetMathLibrary.ClassIsChildOf` (`GameplayStatics.GetObjectClass` _array_element) (`local.ItemClass`))
      (return _array_element true)))
  (return null false))

(fn `GetAllContainedItems`
  (returns (Items :type "Array of Actor Object Reference"))
  (return (`self.ContainedItems`)))

(fn `RemoveAndPlaceItemByClass`
  (params (ItemClass :type "Actor Class Reference") (PlaceLocation :type "Vector Structure (by ref)") (PlaceRotation :type "Rotator Structure (by ref)") (bUnhide :type Boolean) (bTurnOnCollision :type Boolean))
  (returns (ItemInstance :type "Actor Object Reference") (bItemFoundAndRemoved :type Boolean))
  (locals (ItemInst :type "Actor Object Reference"))
  (bind _iteminst (`local.ItemInst`))
  (bind (_iteminstance _bitemfoundandremoved) (`self.RemoveItemByClass` ItemClass))
  (if _bitemfoundandremoved
    (bind _output_get (set `local.ItemInst` _iteminstance))
    (`Actor.K2_DetachFromActor` _output_get "KeepWorld" "KeepWorld" "KeepWorld")
    (`Actor.K2_SetActorLocationAndRotation` (`local.ItemInst`) (`local.PlaceLocation`) (`local.PlaceRotation`) false true)
    (`|ExecutionSequence`
      (:`then_0`
        (if (`local.bUnhide`)
          (`Actor.SetActorHiddenInGame` _iteminst false)))
      (:`then_1`
        (if (`local.bTurnOnCollision`)
          (`Actor.SetActorEnableCollision` _iteminst true)))
      (:`then_2`
        (return (`local.ItemInst`) true)))
    (else
      (return null false))))

(fn `RemoveItemByClass`
  (params (ItemClass :type "Actor Class Reference") (RemoveBehaviour :type "/Game/EpicTemplates/WalkingSimTemplate/Blueprints/Enums/EIInventoryItemRemoveBehaviour Enum" :default "NewEnumerator0"))
  (returns (ItemInstance :type "Actor Object Reference") (bItemFoundAndRemoved :type Boolean))
  (locals (TempItem :type "Actor Object Reference"))
  (bind _tempitem (`local.TempItem`))
  (bind _tempitem_2 (`local.TempItem`))
  (for (_array_element _array_index) (`self.ContainedItems`)
    (set `local.TempItem` _array_element)
    (if (`KismetMathLibrary.ClassIsChildOf` (`GameplayStatics.GetObjectClass` _array_element) (`local.ItemClass`))
      (`KismetArrayLibrary.Array_Remove` (`self.ContainedItems`) _array_index)
      (`|ExecutionSequence`
        (:`then_0`
          (switch `/Game/EpicTemplates/WalkingSimTemplate/Blueprints/Enums/EIInventoryItemRemoveBehaviour` (`local.RemoveBehaviour`)
            (:`NewEnumerator1`
              (`Actor.SetActorEnableCollision` _tempitem true)
              (`Actor.SetActorHiddenInGame` _tempitem false))
            (:`NewEnumerator2`
              (`self.OnItemRemoved` self _tempitem_2)
              (`Actor.K2_DestroyActor` _tempitem_2)
              (return null true))))
        (:`then_1`
          (`self.OnItemRemoved` self (`local.TempItem`))
          (return (`local.TempItem`) true)))))
  (return null false))