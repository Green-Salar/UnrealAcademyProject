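; BP_PickupInteractData tracks a pickup actor during interaction in the walking sim template and moves it between transforms.
; Setup stores the actor and its BPI_Pickup interface, and a validity check tests both.
; StartNewMovement captures start and end transforms, then MoveToTargetTransform advances an alpha by speed and delta time per call.
; The actor is teleport-free, unswept and eased along that path, returning true on arrival.
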(fn `IsValidPickupData`
  (returns (IsValid :type Boolean))
  (return (and (`KismetSystemLibrary.IsValid` (`self.Pickup`)) (`KismetSystemLibrary.IsValidInterface` (`self.PickupInterface`)))))

(fn `MoveToTargetTransform`
  (params (Speed :type "Float (double-precision)") (deltaTime :type "Float (double-precision)"))
  (returns (bMovementFinished :type Boolean))
  (bind _output_get (set `self.MovementAlpha` (`KismetMathLibrary.FMin` (+ (`self.MovementAlpha`) (* Speed deltaTime)) 1.0)))
  (`Actor.K2_SetActorTransform` (`self.Pickup`) (`KismetMathLibrary.TLerp` (`self.MoveStartTrans`) (`self.MoveEndTrans`) (`|EaseFunction` (`self.MoveEaseFunction`) _output_get 0.0 1.0 (`self.MoveEaseExponent`))) false false)
  (return (>= (`self.MovementAlpha`) 1.0)))

(fn `Setup`
  (params (Pickup :type "Actor Object Reference"))
  (bind _output_get (set `self.Pickup` Pickup))
  (bind _asbpi_pickup (cast `/Game/EpicTemplates/WalkingSimTemplate/Blueprints/Interfaces/BPI_Pickup` _output_get))
  (set `self.PickupInterface` _asbpi_pickup))

(fn `StartNewMovement`
  (params (NewEndTrans :type "Transform Structure (by ref)"))
  (set `self.MoveEndTrans` NewEndTrans)
  (set `self.MoveStartTrans` (`Actor.GetTransform` (`self.Pickup`)))
  (set `self.MovementAlpha` 0.0))