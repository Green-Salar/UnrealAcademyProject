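; BP_SwitchLight is a switchable spotlight actor in the walking sim template.
; Its construction script applies exposed settings for intensity, color, cone angles, radius and starting on/off state to the SpotLight component.
; The SwitchToggled event flips the spotlight's visibility, turning it on or off each time it fires.
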(event `/Game/EpicTemplates/TemplateAgnostic/Blueprints/Interfaces/BPI_SwitchListener.SwitchToggled`
  (params (SwitchActor :type "Actor Object Reference") (bSwitchIsOn :type Boolean))
  (bind _spotlight (`self.SpotLight`))
  (`SceneComponent.SetVisibility` _spotlight (not (`SceneComponent.IsVisible` _spotlight)) false))

(fn `UserConstructionScript`
  (bind _spotlight (`self.SpotLight`))
  (`LightComponent.SetIntensity` _spotlight (`self.LightIntensity`))
  (`SceneComponent.SetVisibility` _spotlight (`self.StartOn`) false)
  (`SpotLightComponent.SetOuterConeAngle` _spotlight (`self.OuterConeAngle`))
  (`SpotLightComponent.SetInnerConeAngle` _spotlight (`self.InnerConeAngle`))
  (`LightComponent.SetLightColor` _spotlight (`self.LightColour`) true)
  (`LocalLightComponent.SetAttenuationRadius` _spotlight (`self.Radius`)))