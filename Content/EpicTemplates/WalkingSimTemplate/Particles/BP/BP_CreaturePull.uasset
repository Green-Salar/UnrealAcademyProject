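; Walking sim Blueprint that pulls a creature to one of three destination actors chosen by ID, with a Niagara pull effect.
; ActivateCreature moves this actor to the destination as the VFX origin, then a timeline lerps the creature's transform there.
; A 0.1-second looping timer, used instead of Tick, feeds the creature's body location to Niagara.
; On completion it stops the effect, hides the marker and, after three catches, plays the altar door-opening sequence.
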(event `ActivateCreature`
  (params (`Creature Ref` :type "/Game/EpicTemplates/WalkingSimTemplate/Gameplay/BP_Creature Object Reference") (CreatureID :type Integer))
  (bind _output (`|ConvertAsset` (select `int` (`self.CreatureID`) :`0` null :`1` (`self.CreaturePullTransform_01`) :`2` (`self.CreaturePullTransform_02`) :`3` (`self.CreaturePullTransform_03`))))
  (set `self.Creature Ref` `Creature Ref`)
  (set `self.CreatureID` CreatureID)
  (`/Engine/EditorBlueprintResources/StandardMacros.IsValid` _output
    (:`Is Valid`
      (set `self.EndTransform` (`self.GetTransform` _output))
      (`self.K2_SetActorLocation` (`self.K2_GetActorLocation` _output)) ; This moves the whole Blueprint to the location we're 'pulling' in as the VFX originate from this BP
      (`ActorComponent.Activate` (`self.NS_CreaturePullForce`) false)
      (bind _returnvalue (`KismetSystemLibrary.K2_SetTimerDelegate` (delegate `UpdateParticles`) 0.1 true)) ; Instead of 'Tick' we just update every .1 secs
      (set `self.Timer_UpdateVFX` _returnvalue)
      (bind _creature_ref (`self.Creature Ref`)
        (:`then`
          (set `self.StartTransform` (`self.GetTransform` _creature_ref))
          (bind (_direction _creature) (`Timeline|TL_CreaturePull` :!via `PlayFromStart`)
            (:`Update`
              (bind _creature_ref_2 (`self.Creature Ref`)
                (:`then`
                  (`self.K2_SetActorTransform` _creature_ref_2 (`KismetMathLibrary.TLerp` (`self.StartTransform`) (`self.EndTransform`) _creature) false false))
                (:`else`)))
            (:`Finished`
              (`self.DeactivateCreature`) ; Stops VFX
              (`self.SetActorHiddenInGame` (select `int` (`self.CreatureID`) :`0` null :`1` (`|ConvertAsset` (`self.CreaturePullTransform_01`)) :`2` (`|ConvertAsset` (`self.CreaturePullTransform_02`)) :`3` (`|ConvertAsset` (`self.CreaturePullTransform_03`)) :!type "Actor Object Reference") true) ; Hides root location as create is now there
              (bind _result (`/Engine/EditorBlueprintResources/StandardMacros.IncrementInt` (`self.TotalNumberOfCreaturesCaught`)) ; Count to 3
                (:`  `
                  (if (>= _result 3)
                    (`/Engine/EditorBlueprintResources/StandardMacros.DoOnce` false
                      (:`Completed`
                        (bind (_outactor _returnvalue_2) (`LevelSequencePlayer.CreateLevelSequencePlayer` (`|ConvertAsset` (`self.SEQ_OpenAlterDoor`)))) ; Open the door now that all the creatures are caught
                        (`MovieSceneSequencePlayer.Play` _returnvalue_2)))))))))
        (:`else`)))))

(event `UpdateParticles`
  ;[0.9833 0.5527 1 0.3] VFX Activated
  (bind _creature_ref (`self.Creature Ref`)
    (:`then`
      (`NiagaraComponent.SetVariableVec3` (`self.NS_CreaturePullForce`) "Creature Location" (`SceneComponent.K2_GetComponentLocation` (`/Game/EpicTemplates/WalkingSimTemplate/Gameplay/BP_Creature.Body_03` _creature_ref))))
    (:`else`)))

(event `DeactivateCreature`
  ;[0.9833 0.5527 1 0.3] VFX Activated
  (set `self.Creature Ref` null)
  (`KismetSystemLibrary.K2_PauseTimerHandle` (`self.Timer_UpdateVFX`))
  (`ActorComponent.Deactivate` (`self.NS_CreaturePullForce`)))

(fn `UserConstructionScript`
  (bind _creature_ref (`self.Creature Ref`)
    (:`then`
      (`NiagaraComponent.SetVariableVec3` (`self.NS_CreaturePullForce`) "Creature Location" (`SceneComponent.K2_GetComponentLocation` (`/Game/EpicTemplates/WalkingSimTemplate/Gameplay/BP_Creature.Body_03` _creature_ref))))
    (:`else`)))