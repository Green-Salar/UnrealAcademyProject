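; BP_Pavement is a construction-time smart mesh that builds a pavement strip sized by the Shaper vector.
; The construction script creates an instanced static mesh component and repeats the Pavement mesh along local Y at Width intervals to cover Shaper.Y.
; It then adds a static mesh component oriented by GroundRotation and scaled from Shaper's Y and negated Z, with a fixed Z scale.
; The event graph holds no active logic.
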(fn `UserConstructionScript`
  (locals (NewLocalVar :type "Vector Structure" :default (0.0 0.0 0.0)))
  (bind (_shaper_x _shaper_y) (`KismetMathLibrary.BreakVector` (`self.Shaper`)))
  (bind (_shaper_x_2 _shaper_y_2 _shaper_z) (`KismetMathLibrary.BreakVector` (`self.Shaper`)))
  (`|ExecutionSequence`
    (:`then_0`
      (bind _returnvalue (`AddComponent|NODE_AddInstancedStaticMeshComponent-0`))
      (bind _output_get (set `self.Static mesh compenent` _returnvalue))
      (`StaticMeshComponent.SetStaticMesh` _output_get "/Game/SmartMeshes/Pavement.Pavement"))
    (:`then_1`
      (for _index (range (`KismetMathLibrary.Round` (/ _shaper_y (`self.Width`))))
        (`InstancedStaticMeshComponent.AddInstance` (`self.Static mesh compenent`) (`KismetMathLibrary.MakeTransform` (`KismetMathLibrary.MakeVector` 0.0 (* _index (`self.Width`)))) false)))
    (:`then_2`
      (`AddComponent|NODE_AddStaticMeshComponent-0` :`RelativeTransform` (`KismetMathLibrary.MakeTransform` (`KismetMathLibrary.MakeVector` (`self.Relative Transform Location Y`)) (`self.GroundRotation`) (`KismetMathLibrary.MakeVector` (- 0.0 _shaper_z) _shaper_y_2 1000.0))))))