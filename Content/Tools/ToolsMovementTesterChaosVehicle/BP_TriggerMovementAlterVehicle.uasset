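; BP_TriggerMovementAlterVehicle is an actor in the Chaos vehicle movement tester tools that opens the vehicle menu widget for a nearby player.
; Shortly after BeginPlay, it makes a single distance check against the player pawn rather than using an overlap.
; If the pawn is within range, it creates W_VehicleMenuWidget, adds it to the viewport and shows the mouse cursor.
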(event `self.ReceiveBeginPlay`
  (`KismetSystemLibrary.Delay` 0.2)
  (if (< (`KismetMathLibrary.Vector_Distance` (`self.K2_GetActorLocation` (`GameplayStatics.GetPlayerPawn` 0)) (`self.K2_GetActorLocation`)) 2000.0)
    (bind _returnvalue (`|CreateWidget` "/Game/Tools/ToolsMovementTesterChaosVehicle/W_VehicleMenuWidget.W_VehicleMenuWidget_C"))
    (`UserWidget.AddToViewport` _returnvalue 0)
    (set `PlayerController.bShowMouseCursor` true (`GameplayStatics.GetPlayerController` 0))))

(fn `UserConstructionScript`)